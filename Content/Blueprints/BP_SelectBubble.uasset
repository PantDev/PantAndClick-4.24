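; BP_SelectBubble is a drifting, camera-facing bubble actor that also acts as its own spawner.
; The instance flagged TheOG hides its mesh and, on a looping RespawnTime timer, spawns copies at its construction-time transform, passing on VelocityConstant.
; Non-TheOG instances use a roughly 30 Hz timer instead of Tick to ease mesh rotation toward the player camera and step position by VelocityConstant.
; The Blueprint itself never destroys the spawned copies.
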(event EventBeginPlay
  (Transformation|SetWorldRotation (Variables|Default|GetStaticMesh) (Math|Rotator|FindLookatRotation (Transformation|GetActorLocation) (Camera|GetCameraLocation (Game|GetPlayerCameraManager 0))) false false)
  (if (Variables|Default|GetThe_OG)
    (Utilities|Time|SetTimerbyFunctionName self "Spawn" (Variables|Default|GetRespawnTime) true)
    (Rendering|SetVisibility (Variables|Default|GetStaticMesh) false false)
    (else
      (Utilities|Time|SetTimerbyFunctionName self "RotateTimer" 0.033333 true))))

(event Collision|EventActorBeginOverlap
  (params (OtherActor :type Actor%20Object%20Reference)))

(event EventTick
  (params (DeltaSeconds :type Float%20%28single-precision%29)))

(fn ConstructionScript
  (Variables|Default|SetStartTransform (Transformation|GetActorTransform)))

(fn RotateTimer
  (Transformation|SetWorldRotation (Variables|Default|GetStaticMesh) (Math|Interpolation|RInterpTo (Transformation|GetWorldRotation (Variables|Default|GetStaticMesh)) (Math|Rotator|FindLookatRotation (Transformation|GetActorLocation) (Camera|GetCameraLocation (Game|GetPlayerCameraManager 0))) (Utilities|Time|GetWorldDeltaSeconds) 2e+01) false false)
  (Transformation|SetActorLocation (+ (Variables|Default|GetVelocityConstant) (Transformation|GetActorLocation)) false false))

(fn Spawn
  (bind _returnvalue (Game|SpawnActorfromClass "BP_SelectBubble_C" (Variables|Default|GetStartTransform) "Undefined" 0 0))
  (Variables|BP_SelectBubble_C|SetVelocityConstant _returnvalue (Variables|Default|GetVelocityConstant)))