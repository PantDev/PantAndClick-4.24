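; BP_Icon is a floating desktop-style icon or folder that the player hovers, selects and double-clicks, with optional zipped and shortcut looks.
; Select bubbles trigger clicks, and a timed window detects double-clicks; an airborne player hitting a selected icon also double-clicks it and gets launched.
; Certain props are destroyed on overlap to fill it, and double-clicking a full icon spawns a ring of BP_File actors.
; Timelines animate bob and bounce, a timer faces the camera, and traces place the blob shadow.
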(event OnComponentBeginOverlap(HitSphere)
  (params (OverlappedComponent :type Primitive%20Component%20Object%20Reference) (OtherActor :type Actor%20Object%20Reference) (OtherComp :type Primitive%20Component%20Object%20Reference) (OtherBodyIndex :type Integer) (bFromSweep :type Boolean) (SweepResult :type Hit%20Result%20Structure%20%28by%20ref%29))
  (bind _returnvalue (Utilities|GetClass OtherActor))
  (bind _tl_bounceanim (Variables|Default|GetTL_BounceAnim))
  (Variables|Default|SetOverlappedActor OtherActor)
  (if (and (Math|Boolean|ORBoolean (== _returnvalue "/Game/Blueprints/BP_WoodenBlock.BP_WoodenBlock_C") (== _returnvalue "/Game/Blueprints/BP_Domino.BP_Domino_C") (== _returnvalue "/Game/Blueprints/BP_Mushroom.BP_Mushroom_C") (== _returnvalue "/Game/Blueprints/BP_ThumbTack.BP_ThumbTack_C") (== _returnvalue "/Game/Blueprints/BP_BasicObject.BP_BasicObject_C")) (not (Variables|Default|GetFull)))
    (bind _output_get (Variables|Default|SetHeldActor OtherActor))
    (Actor|DestroyActor _output_get)
    (Components|Timeline|SetNewTime _tl_bounceanim 0.35)
    (Audio|Components|Audio|Play _tl_bounceanim)
    (Variables|Default|SetFull true)
    (Rendering|SetVisibility (Variables|Default|GetFiller) true false)
    (else
      (if (== _returnvalue "/Game/Blueprints/BP_SelectBubble.BP_SelectBubble_C")
        (Default|Clicked self)
        (Utilities|Casting|CastToBP_ThirdPersonCharacter (Game|GetPlayerCharacter 0))
        (Rendering|SetVisibility (Variables|Default|GetIconSelectBubble) true false)
        (Actor|DestroyActor (Variables|Default|GetOverlappedActor))
        (elif (and (== _returnvalue "/Game/ThirdPersonBP/Blueprints/BP_ThirdPersonCharacter.BP_ThirdPersonCharacter_C") (Variables|Default|GetSelected))
          (bind _asbp_third_person_character (Utilities|Casting|CastToBP_ThirdPersonCharacter OtherActor))
          (if (Pawn|Components|CharacterMovement|IsWalking (Variables|/Script/Engine.Character|GetCharacterMovement _asbp_third_person_character))
            _
            (else
              (CallFunction|DoubleClick)
              (Default|BounceLaunch _asbp_third_person_character "0, 0,1400.000000")
              (Components|Animation|PlayAnimation (Variables|/Game/ThirdPersonBP/Blueprints/BP_ThirdPersonCharacter.BP_ThirdPersonCharacter_C|GetDenimMesh _asbp_third_person_character) "/Game/Meshes/Denim/NewFolder/Denim_Armature_Roll.Denim_Armature_Roll" true)
              (Components|Activation|Activate (Variables|/Game/ThirdPersonBP/Blueprints/BP_ThirdPersonCharacter.BP_ThirdPersonCharacter_C|GetParticleSystem4 _asbp_third_person_character) false)
              (Components|Timeline|PlayfromStart (Variables|/Game/ThirdPersonBP/Blueprints/BP_ThirdPersonCharacter.BP_ThirdPersonCharacter_C|GetJumpTL _asbp_third_person_character))
              (Rendering|Material|SetMaterial (Variables|Default|GetIconSelectBubble) 0 "/Game/Materials/Mat_Icon_Outline.Mat_Icon_Outline")
              (Rendering|SetVisibility (Variables|Default|GetIconSelectBubble) false false)
              (Variables|Default|SetSelected false)))))
      (if (Audio|Components|Audio|IsPlaying (Variables|Default|GetTL_BounceAnim))
        _
        (else
          (Components|Timeline|PlayfromStart _tl_bounceanim)))))
  (CallFunction|TakeDamage "0, 0, 0" "0, 0, 0"))

(event Custom|HoverDoOnce
  (Utilities|FlowControl|DoOnce false
    (:Completed
      (Components|Timeline|PlayfromStart (Variables|Default|GetTL_OutlinePop)))))

(event Custom|HoverDoOnceReset
  (Utilities|FlowControl|DoOnce false) ; enters at Reset
)

(event Custom|UpdateShadow
  (bind _returnvalue (Transformation|GetActorLocation))
  (bind (_x _y _z) (Math|Vector|BreakVector _returnvalue))
  (bind (_outhit _returnvalue_2) (Collision|LineTraceByChannel _returnvalue (Math|Vector|MakeVector _x _y (- _z 1e+04)) "TraceTypeQuery1" false (Utilities|Array|MakeArray (Components|GetOwner (Game|GetPlayerCharacter 0))) "None"))
  (if _returnvalue_2
    (Transformation|SetWorldLocationAndRotation (Variables|Default|GetBlobShadow) (Math|Vector|MakeVector (.X (Math|Vector|BreakVector (.Location (Collision|BreakHitResult _outhit)))) (.Y (Math|Vector|BreakVector (.Location (Collision|BreakHitResult _outhit)))) (+ (.Z (Math|Vector|BreakVector (.Location (Collision|BreakHitResult _outhit)))) 5.0)) (Math|Rotator|MakeRotfromZ (.ImpactNormal (Collision|BreakHitResult _outhit))) false false)
    (Utilities|FlowControl|Delay 0.1)
    (CallFunction|UpdateShadow)))

(event Custom|ParticleBurst
  (Audio|PlaySoundatLocation "/Game/Audio/SFX/Pop.Pop" (Transformation|GetActorLocation) "0, 0, 0" 0.5 (Math|Random|RandomFloatinRange 0.55 0.8) 0.0 "/Game/Audio/Attenuation/SA_Default.SA_Default" "/Game/Audio/Attenuation/SC_Default.SC_Default" 0)
  (Components|Activation|Activate (Variables|Default|GetP_BubblePop) false)
  (Utilities|FlowControl|Delay 0.2)
  (Components|Activation|Deactivate (Variables|Default|GetP_BubblePop)))

(event EventBeginPlay
  (bind _hover_tl (Variables|Default|GetHover_TL))
  (Utilities|FlowControl|Sequence
    (:then_0
      (bind _newtrack_0 (Timeline|Hover_TL PlayFromStart)
        (:Update
          (if (Variables|Default|GetSpinPlaying)
            (Variables|Default|SetTargetLoc (Math|Vector|MakeVector 0.0 0.0 (Math|Float|Lerp -12.0 12.0 _newtrack_0)))
            (else
              (Transformation|SetRelativeLocation (Variables|Default|GetIconMesh) (Math|Vector|MakeVector 0.0 0.0 (Math|Float|Lerp -12.0 12.0 _newtrack_0)) false false))))
        (:Finished
          (Components|Timeline|SetPlayRate _hover_tl (Math|Random|RandomFloatinRange 0.6 1.2))
          (Components|Timeline|PlayfromStart _hover_tl))))
    (:then_1
      (Utilities|Time|SetTimerbyFunctionName 0 "RotateTimer" 0.033333 true))))

(event EventTakeDamage
  (params (ForwardVector :type Vector :default "0, 0, 0") (Location :type Vector :default "0, 0, 0"))
  (if (not (Variables|Default|GetSpinPlaying))
    (Variables|Default|SetThreshold false)
    (Components|Timeline|SetPlayRate (Variables|Default|GetTL_BounceAnim) 0.875)))

(fn ConstructionScript
  (bind _returnvalue (Transformation|GetActorLocation))
  (bind _iconmesh (Variables|Default|GetIconMesh))
  (bind _shortcutmesh (Variables|Default|GetShortcutMesh))
  (bind _filler (Variables|Default|GetFiller))
  (bind (_x _y _z) (Math|Vector|BreakVector _returnvalue))
  (bind (_outhit _returnvalue_2) (Collision|LineTraceByChannel _returnvalue (Math|Vector|MakeVector _x _y (- _z 1e+04)) "TraceTypeQuery1" false 0 "None"))
  (if _returnvalue_2
    (Transformation|SetWorldLocationAndRotation (Variables|Default|GetBlobShadow) (Math|Vector|MakeVector (.X (Math|Vector|BreakVector (.Location (Collision|BreakHitResult _outhit)))) (.Y (Math|Vector|BreakVector (.Location (Collision|BreakHitResult _outhit)))) (+ (.Z (Math|Vector|BreakVector (.Location (Collision|BreakHitResult _outhit)))) 5.0)) (Math|Rotator|MakeRotfromZ (.ImpactNormal (Collision|BreakHitResult _outhit))) false false)
    (else
      (Rendering|SetVisibility (Variables|Default|GetBlobShadow) false false)))
  (if (Variables|Default|GetAlignToFloor)
    (CallFunction|FloorAlign))
  (Rendering|Components|TextRender|SetText (Variables|Default|GetIconText) (Variables|Default|GetName))
  (if (Variables|Default|GetZipped)
    (Components|StaticMesh|SetStaticMesh _iconmesh "/Game/Meshes/Folder_Zipped.Folder_Zipped")
    (Rendering|Material|SetMaterial _iconmesh 1 "/Game/StarterContent/Materials/M_Metal_Chrome.M_Metal_Chrome")
    (if (Variables|Default|GetShortcut) :!label _label
      (Rendering|SetVisibility _shortcutmesh true false)
      (else
        (Rendering|SetVisibility _shortcutmesh false false)))
    (else
      (Components|StaticMesh|SetStaticMesh (Variables|Default|GetIconMesh) (Variables|Default|GetStaticMesh))
      (Utilities|FlowControl|Sequence
        (:then_0
          (goto _label))
        (:then_1
          (if (Variables|Default|GetFull)
            (Rendering|SetVisibility _filler true false)
            (else
              (Rendering|SetVisibility _filler false false))))))))

(fn FloorAlign
  (bind _returnvalue (Transformation|GetActorLocation))
  (bind (_x _y _z) (Math|Vector|BreakVector _returnvalue))
  (Variables|Default|SetAlignToFloor false)
  (bind (_outhit _returnvalue_2) (Collision|LineTraceByChannel _returnvalue (Math|Vector|MakeVector _x _y (- _z 1e+04)) "TraceTypeQuery1" false 0 "None"))
  (if _returnvalue_2
    (Transformation|SetActorLocation (Math|Vector|MakeVector (.X (Math|Vector|BreakVector (.Location (Collision|BreakHitResult _outhit)))) (.Y (Math|Vector|BreakVector (.Location (Collision|BreakHitResult _outhit)))) (+ (.Z (Math|Vector|BreakVector (.Location (Collision|BreakHitResult _outhit)))) 1.5e+02)) false false)
    (CallFunction|UpdateShadow)))

(fn RotateTimer
  (bind _output_get (Variables|Default|SetTargetRot (Math|Interpolation|RInterpTo (Transformation|GetWorldRotation (Variables|Default|GetMainArm)) (Math|Rotator|FindLookatRotation (Transformation|GetActorLocation) (Camera|GetCameraLocation (Game|GetPlayerCameraManager 0))) (Utilities|Time|GetWorldDeltaSeconds) 1e+01)))
  (Transformation|SetWorldRotation (Variables|Default|GetMainArm) _output_get false false))

(fn DoubleClick
  (CallFunction|ParticleBurst)
  (Rendering|Material|SetMaterial (Variables|Default|GetIconSelectBubble) 0 "/Game/Materials/Mat_Icon_Outline.Mat_Icon_Outline")
  (Variables|Default|SetSelected false)
  (Components|Timeline|PlayfromStart (Variables|Default|GetTL_BounceAnim))
  (if (Variables|Default|GetFull)
    (Variables|Default|SetBursts (- (Variables|Default|GetBursts) 1))
    (while (not (== (Variables|Default|GetBurstQuantity) (Variables|Default|GetFileNumber)))
      (Transformation|SetRelativeRotation (Variables|Default|GetDistributionArm) (Math|Rotator|MakeRotator 0.0 0.0 (* (/ 3.6e+02 (Math|Conversions|ToFloat(Integer) (Variables|Default|GetBurstQuantity))) (Math|Conversions|ToFloat(Integer) (Variables|Default|GetFileNumber)))) false false)
      (Variables|Default|SetFileNumber (+ (Variables|Default|GetFileNumber) 1))
      (bind _returnvalue (Game|SpawnActorfromClass "/Game/Blueprints/BP_File.BP_File_C" (Math|Transform|MakeTransform (Transformation|GetWorldLocation (Variables|Default|GetDefaultSceneRoot))) "Undefined" 0 0))
      (Variables|/Game/Blueprints/BP_File.BP_File_C|SetSpawnDestination _returnvalue (Transformation|GetWorldLocation (Variables|Default|GetDistributionTarget)))
      (Components|Timeline|PlayfromStart (Variables|/Game/Blueprints/BP_File.BP_File_C|GetTL_SpawnFromFolder _returnvalue)))
    (Variables|Default|SetFileNumber 0)
    (if (<= (Variables|Default|GetBursts) 0)
      (Variables|Default|SetFull false)
      (Rendering|SetVisibility (Variables|Default|GetFiller) false false))))

(fn SelectIcon
  (bind _asbp_third_person_character (Utilities|Casting|CastToBP_ThirdPersonCharacter (Game|GetPlayerCharacter 0)))
  (Rendering|Material|SetMaterial (Variables|Default|GetIconSelectBubble) 0 "/Game/Materials/Mat_Icon_Outline_2.Mat_Icon_Outline_2")
  (Variables|Default|SetSelected true)
  (CallFunction|ParticleBurst)
  (if (== (Variables|/Game/ThirdPersonBP/Blueprints/BP_ThirdPersonCharacter.BP_ThirdPersonCharacter_C|GetSelectedIcon _asbp_third_person_character) self)
    _
    (else
      (Variables|BP_Icon_C|SetSelected (Variables|/Game/ThirdPersonBP/Blueprints/BP_ThirdPersonCharacter.BP_ThirdPersonCharacter_C|GetSelectedIcon _asbp_third_person_character) false)
      (Rendering|Material|SetMaterial (Variables|BP_Icon_C|GetIconSelectBubble (Variables|/Game/ThirdPersonBP/Blueprints/BP_ThirdPersonCharacter.BP_ThirdPersonCharacter_C|GetSelectedIcon _asbp_third_person_character)) 0 "/Game/Materials/Mat_Icon_Outline.Mat_Icon_Outline")
      (Rendering|SetVisibility (Variables|BP_Icon_C|GetIconSelectBubble (Variables|/Game/ThirdPersonBP/Blueprints/BP_ThirdPersonCharacter.BP_ThirdPersonCharacter_C|GetSelectedIcon _asbp_third_person_character)) false false)
      (Variables|/Game/ThirdPersonBP/Blueprints/BP_ThirdPersonCharacter.BP_ThirdPersonCharacter_C|SetSelectedIcon _asbp_third_person_character self)))
  (Components|Timeline|PlayfromStart (Variables|Default|GetTL_OutlinePop)))

(fn Attachto
  (params (ChildActor :type Actor%20Object%20Reference))
  (return 0))

(fn Clicked
  (if (Variables|Default|GetDoubleClickOpen)
    (CallFunction|DoubleClick)
    (else
      (Components|Timeline|PlayfromStart (Variables|Default|GetTL_DoubleClickWindow))
      (CallFunction|SelectIcon)
      (return false))))

(fn DisableCollision
  (return false))

(fn DoesParentHaveParent
  (return false))

(fn EnableCollision
  (return false))

(fn GetAttached
  (return 0))

(fn GetShrinkScale
  (return "0, 0, 0" "0, 0, 0"))

(fn GetSnapLoc
  (params (CursorLoc :type Vector :default "0, 0, 0"))
  (return "0, 0, 0" "0, 0, 0"))

(fn Grabbed
  (return 0))

(fn LetGo
  (params (ParentComponent :type Actor%20Component%20Object%20Reference) (ParentActor :type Actor%20Object%20Reference))
  (return false))

(fn OnHover
  (Rendering|SetVisibility (Variables|Default|GetIconSelectBubble) true false)
  (Components|Timeline|PlayfromStart (Variables|Default|GetTL_Hover))
  (return false))

(fn PassChildAlong
  (return 0 0))