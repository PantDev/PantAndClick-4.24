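; Scatter actor that carries a BP_DustMote from its own location toward a randomized offset point, then destroys itself.
; On BeginPlay it randomizes spring arm length and a height value; MoveAlongSpline later moves the mote toward the Arrow's location.
; A timeline drives separate XY and Z alphas to shape the path, with no spline sampling.
; The mote's sphere overlaps and camera lag are off until the move finishes.
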(event EventBeginPlay
  (Variables|Default|SetForwardRandom (Math|Random|RandomFloatinRange 1.2e+02 1.8e+02))
  (Variables|Default|SetHeightRandom (Math|Random|RandomFloatinRange 45.0 75.0))
  (Variables|/Script/Engine.SpringArmComponent|SetTargetArmLength (Variables|Default|GetSpringArm) (Variables|Default|GetForwardRandom)))

(event Collision|EventActorBeginOverlap
  (params (OtherActor :type Actor%20Object%20Reference)))

(event EventTick
  (params (DeltaSeconds :type Float%20%28single-precision%29)))

(event Custom|MoveAlongSpline
  (params (InputActor :type Actor%20Object%20Reference))
  (bind _output_get (Variables|Default|SetSplineFollowActor InputActor))
  (bind _asbp_dust_mote (Utilities|Casting|CastToBP_DustMote _output_get))
  (Variables|/Script/Engine.PrimitiveComponent|SetbGenerateOverlapEvents (Variables|/Game/Blueprints/BP_DustMote.BP_DustMote_C|GetSphere _asbp_dust_mote) false)
  (Variables|/Script/Engine.SpringArmComponent|SetbEnableCameraLag (Variables|/Game/Blueprints/BP_DustMote.BP_DustMote_C|GetSpringArm _asbp_dust_mote) false)
  (bind (_direction _xy_alpha _z_alpha) (Timeline|MoveAlong_TL PlayFromStart)
    (:Update
      (Transformation|SetActorLocation (Variables|Default|GetSplineFollowActor) (Math|Vector|MakeVector (.X (Math|Vector|BreakVector (Math|Vector|Lerp(Vector) (Transformation|GetActorLocation) (Transformation|GetWorldLocation (Variables|Default|GetArrow)) _xy_alpha))) (.Y (Math|Vector|BreakVector (Math|Vector|Lerp(Vector) (Transformation|GetActorLocation) (Transformation|GetWorldLocation (Variables|Default|GetArrow)) _xy_alpha))) (+ (.Z (Math|Vector|BreakVector (Transformation|GetActorLocation))) (Math|Float|Lerp 0.0 (Variables|Default|GetHeightRandom) _z_alpha))) false false))
    (:Finished
      (bind _asbp_dust_mote_2 (Utilities|Casting|CastToBP_DustMote (Variables|Default|GetSplineFollowActor)))
      (Variables|/Script/Engine.PrimitiveComponent|SetbGenerateOverlapEvents (Variables|/Game/Blueprints/BP_DustMote.BP_DustMote_C|GetSphere _asbp_dust_mote_2) true)
      (Variables|/Script/Engine.SpringArmComponent|SetbEnableCameraLag (Variables|/Game/Blueprints/BP_DustMote.BP_DustMote_C|GetSpringArm _asbp_dust_mote_2) true)
      (Actor|DestroyActor))))

(fn ConstructionScript)