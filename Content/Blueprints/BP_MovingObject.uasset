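; BP_MovingObject is an actor that moves along the spline of a referenced FollowRail.
; The construction script places it along the spline at its Offset fraction of the length.
; On BeginPlay, a timeline starts from half the Offset value, with TimeScale as play rate.
; The timeline's update maps its track value to spline distance and sets world location without sweeping.
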(event EventBeginPlay
  (bind _tl_movealongspline (Variables|Default|GetTL_MoveAlongSpline))
  (Components|Timeline|SetNewTime _tl_movealongspline (/ (Variables|Default|GetOffset) 2.0))
  (Components|Timeline|SetPlayRate _tl_movealongspline (Variables|Default|GetTimeScale))
  (Audio|Components|Audio|Play _tl_movealongspline))

(event Collision|EventActorBeginOverlap
  (params (OtherActor :type Actor%20Object%20Reference)))

(event EventTick
  (params (DeltaSeconds :type Float%20%28single-precision%29)))

(fn ConstructionScript
  (bind _followrail (Variables|Default|GetFollowRail))
  (bind _spline (Variables|/Game/Blueprints/BP_FollowRail.BP_FollowRail_C|GetSpline _followrail))
  (Transformation|SetActorLocation (Spline|GetLocationatDistanceAlongSpline _spline (Math|Float|Lerp 0.0 (Spline|GetSplineLength _spline) (Variables|Default|GetOffset)) "World") false false))