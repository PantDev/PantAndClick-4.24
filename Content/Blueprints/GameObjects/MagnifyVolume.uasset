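; MagnifyVolume is a pokeable volume that zooms the player into a close-up view from its linked CameraActor.
; When poked while the player is not busy, it activates ActivateArray targets, releases any previous magnify actor and blends to the camera with a zoom sound.
; It blocks movement, hands the active cursor to the camera's cursor, disables its own box collision and briefly flags the camera busy.
; The grab, click and hover functions are empty stubs.
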(event EventBeginPlay)

(event Collision|EventActorBeginOverlap
  (params (OtherActor :type Actor%20Object%20Reference)))

(event EventPokeEvent
  (bind _returnvalue (Game|GetPlayerController 0))
  (bind _cameraactor (Variables|Default|GetCameraActor))
  (bind _cameraactor_2 (Variables|Default|GetCameraActor))
  (bind _asbp_pant_controller (Utilities|Casting|CastToBP_PantController (Game|GetPlayerCharacter 0)))
  (if (not (Variables|/Game/PantControllerBP/Blueprints/BP_PantController.BP_PantController_C|GetIsBusy _asbp_pant_controller))
    (for _array_element (Variables|Default|GetActivateArray)
      (if (Utilities|DoesObjectImplementInterface _array_element "/Game/Blueprints/BPI/BPI_Activate.BPI_Activate_C")
        (Class|BPIActivate|Activate(Message) _array_element 0.0 true)))
    (bind _asbp_pant_controller_2 (Utilities|Casting|CastToBP_PantController (Game|GetPlayerCharacter 0))
      (:then
        (Class|PlayerController|SetMouseLocation _returnvalue (Math|Float|Truncate (.X (Math|Vector2D|BreakVector2D (.ScreenPosition (Class|GameplayStatics|ProjectWorldtoScreen _returnvalue (Transformation|GetWorldLocation (Variables|/Game/PantControllerBP/Blueprints/BP_PantController.BP_PantController_C|GetActiveCursorMesh _asbp_pant_controller_2)) true))))) (Math|Float|Truncate (.Y (Math|Vector2D|BreakVector2D (.ScreenPosition (Class|GameplayStatics|ProjectWorldtoScreen _returnvalue (Transformation|GetWorldLocation (Variables|/Game/PantControllerBP/Blueprints/BP_PantController.BP_PantController_C|GetActiveCursorMesh _asbp_pant_controller_2)) true))))))
        (Utilities|IsValid (Variables|/Game/PantControllerBP/Blueprints/BP_PantController.BP_PantController_C|GetMagnifyActor _asbp_pant_controller_2)
          (:Is%20Valid
            (Rendering|SetVisibility (Variables|/Game/Blueprints/GameObjects/MagnifyCamera.MagnifyCamera_C|GetCursor (Variables|/Game/PantControllerBP/Blueprints/BP_PantController.BP_PantController_C|GetMagnifyActor _asbp_pant_controller_2)) false false)
            (Collision|SetCollisionEnabled (Variables|MagnifyVolume_C|GetBox (Variables|/Game/Blueprints/GameObjects/MagnifyCamera.MagnifyCamera_C|GetMagVolume (Variables|/Game/PantControllerBP/Blueprints/BP_PantController.BP_PantController_C|GetMagnifyActor _asbp_pant_controller_2))) "QueryOnly")
            (Variables|/Game/PantControllerBP/Blueprints/BP_PantController.BP_PantController_C|SetMagnifyActor _asbp_pant_controller_2 0))
          (:Is%20Not%20Valid
            _)))
      (:CastFailed
        _))
    (Game|Player|SetViewTargetwithBlend (Game|GetPlayerController 0) _cameraactor 0.48 "VTBlend_Cubic" 5e+01 false)
    (if (Variables|/Game/PantControllerBP/Blueprints/BP_PantController.BP_PantController_C|GetIsBubbleOpen _asbp_pant_controller_2)
      _
      (else
        _))
    (Utilities|FlowControl|Sequence
      (:then_0
        (Variables|/Game/PantControllerBP/Blueprints/BP_PantController.BP_PantController_C|SetCamBusy _asbp_pant_controller_2 true)
        (Components|StaticMesh|SetStaticMesh (Variables|/Game/PantControllerBP/Blueprints/BP_PantController.BP_PantController_C|GetActiveCursorMesh _asbp_pant_controller_2) "/Game/Meshes/Cursor_Arrow_New.Cursor_Arrow_New")
        (Utilities|FlowControl|Delay 0.5)
        (Variables|/Game/PantControllerBP/Blueprints/BP_PantController.BP_PantController_C|SetCamBusy _asbp_pant_controller_2 false))
      (:then_1
        (Audio|PlaySoundatLocation "/Game/Audio/SFX/ZoomIn.ZoomIn" (Transformation|GetActorLocation) "0, 0, 0" 0.6 1.3 0.0 "/Game/Audio/Attenuation/SA_ShortRange.SA_ShortRange" "/Game/Audio/Attenuation/SC_Default.SC_Default" 0)
        (Variables|/Game/Blueprints/GameObjects/MagnifyCamera.MagnifyCamera_C|SetActive _cameraactor true)
        (bind _asbp_pant_controller_3 (Utilities|Casting|CastToBP_PantController (Game|GetPlayerCharacter 0)))
        (Variables|/Game/PantControllerBP/Blueprints/BP_PantController.BP_PantController_C|SetBlockMovement _asbp_pant_controller_3 true)
        (Rendering|SetVisibility (Variables|/Game/PantControllerBP/Blueprints/BP_PantController.BP_PantController_C|GetDenimMesh _asbp_pant_controller_3) false false)
        (Rendering|SetVisibility (Variables|/Game/Blueprints/GameObjects/MagnifyCamera.MagnifyCamera_C|GetCursor (Variables|Default|GetCameraActor)) true false)
        (Variables|/Game/PantControllerBP/Blueprints/BP_PantController.BP_PantController_C|SetMagnifyActor _asbp_pant_controller_3 _cameraactor_2)
        (Variables|/Game/PantControllerBP/Blueprints/BP_PantController.BP_PantController_C|SetActiveCursorMesh _asbp_pant_controller_3 (Variables|/Game/Blueprints/GameObjects/MagnifyCamera.MagnifyCamera_C|GetCursor _cameraactor_2))
        (Collision|SetCollisionEnabled (Variables|Default|GetBox) "NoCollision")
        (Components|StaticMesh|SetStaticMesh (Variables|/Game/PantControllerBP/Blueprints/BP_PantController.BP_PantController_C|GetActiveCursorMesh _asbp_pant_controller_3) "/Game/Meshes/Cursor_Arrow_New.Cursor_Arrow_New")))))

(fn ConstructionScript
  (Transformation|SetWorldScale3D (Variables|Default|GetStaticMesh) "0.600000,0.600000,0.600000"))

(fn Attachto
  (params (ChildActor :type Actor%20Object%20Reference))
  (return 0))

(fn CanGrab
  (return false))

(fn Clicked
  (return false))

(fn DisableCollision
  (return false))

(fn DoesParentHaveParent
  (return false))

(fn EnableCollision
  (return false))

(fn GetAttached
  (return 0))

(fn GetCustomCursor
  (return false 0))

(fn GetShrinkScale
  (return "0, 0, 0" "0, 0, 0"))

(fn GetSnapLoc
  (params (CursorLoc :type Vector :default "0, 0, 0"))
  (return "0, 0, 0" "0, 0, 0"))

(fn Grabbed
  (return 0))

(fn LetGo
  (params (ParentComponent :type Actor%20Component%20Object%20Reference) (ParentActor :type Actor%20Object%20Reference))
  (return false))

(fn OnHover
  (return false))

(fn PassChildAlong
  (return 0 0))