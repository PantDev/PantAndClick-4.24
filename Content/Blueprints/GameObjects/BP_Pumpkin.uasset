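; BP_Pumpkin is a clickable prop that toggles between a plain pumpkin and a jack-o'-lantern.
; Its Clicked function fires a custom event that plays a pitch-randomized sound and uses a FlipFlop to swap the static mesh.
; Each swap restarts a bounce timeline that drives the mesh's scale.
; The other interaction functions, covering grab, hover, attach and snap, are stubs with default returns.
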(event Custom|CustomClickEvent
  (bind _pumpkinmesh (Variables|Default|GetPumpkinMesh))
  (Audio|PlaySoundatLocation "/Game/Audio/SFX/ScreenSaverCube.ScreenSaverCube" (Transformation|GetActorLocation) "0, 0, 0" 0.6 (Math|Random|RandomFloatinRange 1.1 1.3) 0.28 "/Game/Audio/Attenuation/SA_ShortRange.SA_ShortRange" "/Game/Audio/Attenuation/SC_Default.SC_Default" 0)
  (Utilities|FlowControl|FlipFlop
    (:A
      (Components|StaticMesh|SetStaticMesh _pumpkinmesh "/Game/Meshes/Pumpkin_Jack.Pumpkin_Jack")
      (bind _newtrack_0 (Timeline|TL_Bounce PlayFromStart)
        (:Update
          (Transformation|SetRelativeScale3D (Variables|Default|GetPumpkinMesh) _newtrack_0))))
    (:B
      (Components|StaticMesh|SetStaticMesh _pumpkinmesh "/Game/Meshes/Pumpkin.Pumpkin")
      (Timeline|TL_Bounce PlayFromStart))))

(fn ConstructionScript)

(fn Attachto
  (params (ChildActor :type Actor%20Object%20Reference))
  (return 0))

(fn CanGrab
  (return false))

(fn Clicked
  (CallFunction|CustomClickEvent)
  (return false))

(fn DisableCollision
  (return false))

(fn DoesParentHaveParent
  (return false))

(fn EnableCollision
  (return false))

(fn GetAttached
  (return 0))

(fn GetCustomCursor
  (return false 0))

(fn GetShrinkScale
  (return "0, 0, 0" "0, 0, 0"))

(fn GetSnapLoc
  (params (CursorLoc :type Vector :default "0, 0, 0"))
  (return "0, 0, 0" "0, 0, 0"))

(fn Grabbed
  (return 0))

(fn LetGo
  (params (ParentComponent :type Actor%20Component%20Object%20Reference) (ParentActor :type Actor%20Object%20Reference))
  (return false))

(fn OnHover
  (return false))

(fn PassChildAlong
  (return 0 0))