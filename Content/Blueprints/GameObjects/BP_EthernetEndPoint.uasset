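; Ethernet cable endpoint that carries the player along a spline to its paired OtherEnd, acting as a two-way transit point.
; Poking or touching an uncapped end hides the player, switches to flying and chains timelines for entry, spline travel and exit, with camera, sound and effects.
; Capped ends only bounce when poked; arriving from the other side pops the cap.
; Uncapped state persists through SaveManager, keyed by level and actor name.
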(event OnComponentBeginOverlap(Box)
  (params (OverlappedComponent :type Primitive%20Component%20Object%20Reference) (OtherActor :type Actor%20Object%20Reference) (OtherComp :type Primitive%20Component%20Object%20Reference) (OtherBodyIndex :type Integer) (bFromSweep :type Boolean) (SweepResult :type Hit%20Result%20Structure%20%28by%20ref%29))
  (if (not (Variables|Default|GetIsCapped))
    (bind _asbp_pant_controller (Utilities|Casting|CastToBP_PantController OtherActor))
    (if (Rendering|IsVisible (Variables|/Game/PantControllerBP/Blueprints/BP_PantController.BP_PantController_C|GetDenimMesh _asbp_pant_controller))
      (CallFunction|PokeEvent))))

(event Custom|CapOff
  (bind _ethernetplug_cap (Variables|Default|GetEthernetPlug_Cap))
  (bind _ethernetplug_cap_2 (Variables|Default|GetEthernetPlug_Cap))
  (bind _returnvalue (Transformation|GetWorldTransform _ethernetplug_cap_2))
  (bind (_location _rotation) (Math|Transform|BreakTransform _returnvalue))
  (Default|SetCollected (Variables|Default|GetSaveManager) (Variables|Default|GetUID))
  (Variables|Default|SetRandRot (Math|Random|RandomFloatinRange -3e+01 3e+01))
  (Variables|Default|SetRandRot2 (Math|Random|RandomFloatinRange -3e+01 3e+01))
  (Components|Timeline|SetPlayRate (Variables|Default|GetTL_CapOff) 0.5)
  (Audio|PlaySoundatLocation "/Game/Audio/SFX/Pop.Pop" (Transformation|GetActorLocation) "0, 0, 0" 1.5 (Math|Random|RandomFloatinRange 0.6 0.9) 0.0 "/Game/Audio/Attenuation/SA_ShortRange.SA_ShortRange" 0 0)
  (bind (_direction _lengthalpha _rotalpha _scalealpha _updownalpha) (Timeline|TL_CapOff PlayFromStart)
    (:Update
      (Variables|/Script/Engine.SpringArmComponent|SetTargetArmLength (Variables|Default|GetSpringArm) (Math|Float|Lerp 0.0 5e+02 _lengthalpha))
      (Transformation|SetRelativeRotation _ethernetplug_cap (Math|Rotator|MakeRotator (Math|Float|Lerp 0.0 (Variables|Default|GetRandRot) _rotalpha) (Math|Float|Lerp 0.0 (Variables|Default|GetRandRot2) _rotalpha) 9e+01) false false)
      (Transformation|SetRelativeScale3D _ethernetplug_cap (Math|Vector|MakeVector _scalealpha _scalealpha _scalealpha))
      (Transformation|SetRelativeLocation (Variables|Default|GetEthernetPlug_Cap) (Math|Vector|MakeVector 0.0 0.0 (Math|Float|Lerp 0.0 5e+01 _updownalpha)) false false))
    (:Finished
      (Game|SpawnActorfromClass "/Game/Blueprints/FX/BP_KillPoof.BP_KillPoof_C" (Math|Transform|MakeTransform _location _rotation) "Undefined" 0 0))))

(event EventBeginPlay
  (Default|InitiateCollectible (Variables|Default|GetSaveManager) (Variables|Default|GetUID) (not (Variables|Default|GetIsCapped))))

(event Collision|EventActorBeginOverlap
  (params (OtherActor :type Actor%20Object%20Reference)))

(event EventTick
  (params (DeltaSeconds :type Float%20%28single-precision%29)))

(event EventPokeEvent
  (bind _returnvalue (Game|GetPlayerCharacter 0))
  (bind _returnvalue_2 (Transformation|GetActorLocation))
  (if (Variables|Default|GetIsCapped)
    (Components|Timeline|PlayfromStart (Variables|Default|GetTL_CapBounce))
    (Audio|PlaySoundatLocation "/Game/Audio/SFX/Bounce.Bounce" _returnvalue_2 "0, 0, 0" 0.4 1.3 0.15 "/Game/Audio/Attenuation/SA_ShortRange.SA_ShortRange" 0 0)
    (else
      (Audio|PlaySoundatLocation "/Game/Audio/SFX/FloppyLockDisp.FloppyLockDisp" _returnvalue_2 "0, 0, 0" 0.675 (Math|Random|RandomFloatinRange 0.8 1.25) 0.5 "/Game/Audio/Attenuation/SA_ShortRange.SA_ShortRange" 0 0)
      (Variables|Default|SetLastLoc (Transformation|GetActorLocation _returnvalue))
      (Variables|Default|SetTargetLoc (Transformation|GetWorldLocation (Variables|Default|GetBox)))
      (bind _asbp_pant_controller (Utilities|Casting|CastToBP_PantController _returnvalue))
      (Default|HideSecondary _asbp_pant_controller)
      (Rendering|SetVisibility (Variables|/Game/PantControllerBP/Blueprints/BP_PantController.BP_PantController_C|GetDenimMesh _asbp_pant_controller) false false)
      (Components|Activation|Deactivate (Variables|/Game/PantControllerBP/Blueprints/BP_PantController.BP_PantController_C|GetParticleSystem6 _asbp_pant_controller))
      (Pawn|Components|CharacterMovement|SetMovementMode (Variables|/Script/Engine.Character|GetCharacterMovement _asbp_pant_controller) "MOVE_Flying" 0)
      (Variables|/Script/Engine.MovementComponent|SetVelocity (Pawn|GetMovementComponent _asbp_pant_controller) "0, 0, 0")
      (Components|Activation|Activate (Variables|/Game/PantControllerBP/Blueprints/BP_PantController.BP_PantController_C|GetParticleSystem7 _asbp_pant_controller) false)
      (Components|Timeline|PlayfromStart (Variables|Default|GetTL_Start))
      (Game|SpawnActorfromClass "/Game/Blueprints/FX/BP_KillPoof1.BP_KillPoof1_C" (Math|Transform|MakeTransform (.Location (Math|Transform|BreakTransform (Transformation|GetActorTransform (Game|GetPlayerCharacter 0)))) "0, 0, 0" "1.500000,1.500000,1.500000") "Undefined" 0 0)
      (if (Variables|/Game/PantControllerBP/Blueprints/BP_PantController.BP_PantController_C|GetZoomedCam _asbp_pant_controller)
        (Variables|Default|SetArmLengthTarget 425.0)
        (else
          (Variables|Default|SetArmLengthTarget 6.5e+02))))))

(event EventInitBoolTrue
  (Rendering|SetVisibility (Variables|Default|GetEthernetPlug_Cap) false false)
  (Variables|Default|SetIsCapped false))

(fn ConstructionScript
  (bind _ethernetplug_cap (Variables|Default|GetEthernetPlug_Cap))
  (bind _bulge (Variables|Default|GetBulge))
  (CallFunction|CreateUID)
  (bind _returnvalue (Rendering|Material|CreateDynamicMaterialInstance (Variables|Default|GetStaticMesh) 5 "/Game/Materials/LightBulbGlass4.LightBulbGlass4" "None" :!class /Script/Engine.PrimitiveComponent))
  (bind _output_get (Variables|Default|SetGlassMat _returnvalue))
  (Rendering|Material|SetMaterial (Variables|Default|GetStaticMesh) 5 _output_get)
  (bind _returnvalue_2 (Rendering|Material|CreateDynamicMaterialInstance _bulge 5 "/Game/Meshes/Skeletal/Material_005.Material_005" "None" :!class /Script/Engine.PrimitiveComponent))
  (bind _output_get_2 (Variables|Default|SetBulgeMat _returnvalue_2))
  (Rendering|Material|SetMaterial _bulge 0 _output_get_2)
  (if (Variables|Default|GetIsCapped)
    (Rendering|SetVisibility _ethernetplug_cap true false)
    (else
      (Rendering|SetVisibility _ethernetplug_cap false false))))

(fn CreateUID
  (bind _returnvalue (Game|GetCurrentLevelName true))
  (Variables|Default|SetUID (Utilities|String|Append _returnvalue (Utilities|GetDisplayName self))))

(fn Attachto
  (params (ChildActor :type Actor%20Object%20Reference))
  (return 0))

(fn CanGrab
  (return false))

(fn Clicked
  (return false))

(fn DisableCollision
  (return false))

(fn DoesParentHaveParent
  (return false))

(fn EnableCollision
  (return false))

(fn GetAttached
  (return 0))

(fn GetCustomCursor
  (return false 0))

(fn GetObjectUID
  (return (Variables|Default|GetUID)))

(fn GetShrinkScale
  (return "0, 0, 0" "0, 0, 0"))

(fn GetSnapLoc
  (params (CursorLoc :type Vector :default "0, 0, 0"))
  (return "0, 0, 0" "0, 0, 0"))

(fn GetTrueFalse
  (return (not (Variables|Default|GetIsCapped))))

(fn Grabbed
  (return 0))

(fn LetGo
  (params (ParentComponent :type Actor%20Component%20Object%20Reference) (ParentActor :type Actor%20Object%20Reference))
  (return false))

(fn OnHover
  (return false))

(fn PassChildAlong
  (return 0 0))

(fn RightClickEvent
  (return (Variables|Default|GetClick%20Message) (Transformation|GetActorLocation)))