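; T-junction pipe valve that routes power between its front port and either the left or right port, according to a lever.
; Activate and Deactivate track powered ports, message neighboring targets and swap the glow material, with cross-resetting DoOnce gates blocking repeats.
; Poking plays a sound and timeline intended to swing the lever, blend shut-off morph targets, then flip direction and reroute power.
; Most other interaction functions are empty stubs.
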(event EventBeginPlay
  (bind _base_skeletal (Variables|Default|GetBase_Skeletal))
  (bind _base_skeletal_2 (Variables|Default|GetBase_Skeletal))
  (if (Variables|Default|GetFrontPowered)
    (Rendering|Material|SetMaterial _base_skeletal_2 2 "/Game/Materials/Glow_Mat.Glow_Mat")
    (switch Utilities|FlowControl|Switch|SwitchonValveDir_Enum (Variables|Default|GetDirection)
      (:NewEnumerator0
        (Class|BPISteamPowered|Activate(Message) (Variables|Default|GetLeftTarget) (Variables|Default|GetLeftDir)))
      (:NewEnumerator1
        (Class|BPISteamPowered|Activate(Message) (Variables|Default|GetRightTarget) (Variables|Default|GetRightDir))))
    (else
      (Rendering|Material|SetMaterial _base_skeletal_2 2 "/Game/Materials/Glow_MatDull.Glow_MatDull")))
  (switch Utilities|FlowControl|Switch|SwitchonValveDir_Enum (Variables|Default|GetDirection)
    (:NewEnumerator0
      (Components|SkeletalMesh|SetMorphTarget _base_skeletal "RightOff" 1.0 true))
    (:NewEnumerator1
      (Components|SkeletalMesh|SetMorphTarget _base_skeletal "LeftOff" 1.0 true))))

(event Collision|EventActorBeginOverlap
  (params (OtherActor :type Actor%20Object%20Reference)))

(event EventTick
  (params (DeltaSeconds :type Float%20%28single-precision%29)))

(event EventPokeEvent
  (bind _returnvalue (Transformation|GetActorLocation))
  (bind _returnvalue_2 (Math|Random|RandomFloatinRange 0.72 0.95))
  (bind _tl_morphs (Variables|Default|GetTL_Morphs))
  (if (not (Audio|Components|Audio|IsPlaying (Variables|Default|GetTL_Morphs)))
    (switch Utilities|FlowControl|Switch|SwitchonValveDir_Enum (Variables|Default|GetDirection)
      (:NewEnumerator0
        (Components|Timeline|ReversefromEnd _tl_morphs)
        (Audio|PlaySoundatLocation "/Game/Audio/SFX/KnobLeft.KnobLeft" _returnvalue "0, 0, 0" 0.18 _returnvalue_2 0.0 "/Game/Audio/Attenuation/SA_ShortRange.SA_ShortRange" 0 0))
      (:NewEnumerator1
        (Components|Timeline|PlayfromStart _tl_morphs)
        (Audio|PlaySoundatLocation "/Game/Audio/SFX/KnobRight.KnobRight" _returnvalue "0, 0, 0" 0.18 _returnvalue_2 0.0 0 0 0)))))

(event EventActivate
  (params (Direction :type SteamDir_Enum%20Enum :default "NewEnumerator0"))
  (bind _base_skeletal (Variables|Default|GetBase_Skeletal))
  (bind _base_skeletal_2 (Variables|Default|GetBase_Skeletal))
  (bind _base_skeletal_3 (Variables|Default|GetBase_Skeletal))
  (bind _base_skeletal_4 (Variables|Default|GetBase_Skeletal))
  (bind _fronttarget (Variables|Default|GetFrontTarget))
  (bind _frontdir (Variables|Default|GetFrontDir))
  (bind _base_skeletal_5 (Variables|Default|GetBase_Skeletal))
  (Utilities|FlowControl|Sequence
    (:then_0
      (Utilities|FlowControl|DoOnce false
        (:Completed
          (switch Utilities|FlowControl|Switch|SwitchonSteamDir_Enum Direction
            (:NewEnumerator0
              (Variables|Default|SetFrontPowered true)
              (Rendering|Material|SetMaterial (Variables|Default|GetBase_Skeletal) 2 "/Game/Materials/Glow_Mat.Glow_Mat")
              (switch Utilities|FlowControl|Switch|SwitchonValveDir_Enum (Variables|Default|GetDirection)
                (:NewEnumerator0
                  (Class|BPISteamPowered|Activate(Message) (Variables|Default|GetLeftTarget) (Variables|Default|GetLeftDir)))
                (:NewEnumerator1
                  (Class|BPISteamPowered|Activate(Message) (Variables|Default|GetRightTarget) (Variables|Default|GetRightDir))))
              (switch Utilities|FlowControl|Switch|SwitchonValveDir_Enum (Variables|Default|GetDirection)
                (:NewEnumerator0
                  (Components|SkeletalMesh|SetMorphTarget _base_skeletal_2 "RightOff" 1.0 true))
                (:NewEnumerator1
                  (Components|SkeletalMesh|SetMorphTarget _base_skeletal_2 "LeftOff" 1.0 true))))
            (:NewEnumerator1
              (Variables|Default|SetLeftPowered true)
              (switch Utilities|FlowControl|Switch|SwitchonValveDir_Enum (Variables|Default|GetDirection)
                (:NewEnumerator0
                  (Class|BPISteamPowered|Activate(Message) (Variables|Default|GetFrontTarget) (Variables|Default|GetFrontDir))
                  (Rendering|Material|SetMaterial _base_skeletal_3 2 "/Game/Materials/Glow_Mat.Glow_Mat")
                  (Components|SkeletalMesh|SetMorphTarget _base_skeletal_4 "RightOff" 1.0 true))
                (:NewEnumerator1
                  (Rendering|Material|SetMaterial _base_skeletal_3 2 "/Game/Materials/Glow_MatDull.Glow_MatDull")
                  (Components|SkeletalMesh|SetMorphTarget _base_skeletal_4 "LeftOff" 1.0 true))))
            (:NewEnumerator2
              (Variables|Default|SetRightPowered true)
              (switch Utilities|FlowControl|Switch|SwitchonValveDir_Enum (Variables|Default|GetDirection)
                (:NewEnumerator0
                  (Rendering|Material|SetMaterial _base_skeletal_5 2 "/Game/Materials/Glow_MatDull.Glow_MatDull")
                  (Components|SkeletalMesh|SetMorphTarget _base_skeletal "RightOff" 1.0 true))
                (:NewEnumerator1
                  (Class|BPISteamPowered|Activate(Message) (Variables|Default|GetFrontTarget) (Variables|Default|GetFrontDir))
                  (Rendering|Material|SetMaterial _base_skeletal_5 2 "/Game/Materials/Glow_Mat.Glow_Mat")
                  (Components|SkeletalMesh|SetMorphTarget _base_skeletal "LeftOff" 1.0 true))))))))
    (:then_1
      (Utilities|FlowControl|DoOnce false) ; enters at Reset
    )))

(event EventDeactivate
  (params (Direction :type SteamDir_Enum%20Enum :default "NewEnumerator0"))
  (bind _base_skeletal (Variables|Default|GetBase_Skeletal))
  (bind _base_skeletal_2 (Variables|Default|GetBase_Skeletal))
  (bind _base_skeletal_3 (Variables|Default|GetBase_Skeletal))
  (bind _base_skeletal_4 (Variables|Default|GetBase_Skeletal))
  (bind _fronttarget (Variables|Default|GetFrontTarget))
  (bind _frontdir (Variables|Default|GetFrontDir))
  (bind _base_skeletal_5 (Variables|Default|GetBase_Skeletal))
  (Utilities|FlowControl|Sequence
    (:then_0
      (Utilities|FlowControl|DoOnce false
        (:Completed
          (switch Utilities|FlowControl|Switch|SwitchonSteamDir_Enum Direction
            (:NewEnumerator0
              (Variables|Default|SetFrontPowered false)
              (Class|BPISteamPowered|Deactivate(Message) (Variables|Default|GetLeftTarget) Direction)
              (Class|BPISteamPowered|Deactivate(Message) (Variables|Default|GetRightTarget) Direction))
            (:NewEnumerator1
              (Variables|Default|SetLeftPowered false)
              (Class|BPISteamPowered|Deactivate(Message) _fronttarget _frontdir)
              (switch Utilities|FlowControl|Switch|SwitchonValveDir_Enum (Variables|Default|GetDirection)
                (:NewEnumerator0
                  _)))
            (:NewEnumerator2
              (Variables|Default|SetRightPowered false)
              (Class|BPISteamPowered|Deactivate(Message) _fronttarget _frontdir)
              (switch Utilities|FlowControl|Switch|SwitchonValveDir_Enum (Variables|Default|GetDirection)
                (:NewEnumerator1
                  _))))
          (Rendering|Material|SetMaterial (Variables|Default|GetBase_Skeletal) 2 "/Game/Materials/Glow_MatDull.Glow_MatDull"))))
    (:then_1
      (Utilities|FlowControl|DoOnce false) ; enters at Reset
    )))

(fn ConstructionScript
  (bind _levermesh (Variables|Default|GetLeverMesh))
  (switch Utilities|FlowControl|Switch|SwitchonValveDir_Enum (Variables|Default|GetDirection)
    (:NewEnumerator0
      (Transformation|SetRelativeRotation _levermesh "0,-30.000000, 0" false false))
    (:NewEnumerator1
      (Transformation|SetRelativeRotation _levermesh "0,30.000000, 0" false false))))

(fn Attachto
  (params (ChildActor :type Actor%20Object%20Reference))
  (return 0))

(fn CanGrab
  (return false))

(fn Clicked
  (return false))

(fn DisableCollision
  (return false))

(fn DoesParentHaveParent
  (return false))

(fn EnableCollision
  (return false))

(fn GetAttached
  (return 0))

(fn GetCustomCursor
  (return false 0))

(fn GetShrinkScale
  (return "0, 0, 0" "0, 0, 0"))

(fn GetSnapLoc
  (params (CursorLoc :type Vector :default "0, 0, 0"))
  (return "0, 0, 0" "0, 0, 0"))

(fn Grabbed
  (return 0))

(fn LetGo
  (params (ParentComponent :type Actor%20Component%20Object%20Reference) (ParentActor :type Actor%20Object%20Reference))
  (return false))

(fn OnHover
  (return false))

(fn PassChildAlong
  (return 0 0))

(fn RightClickEvent
  (return (Variables|Default|GetClick%20Message) (Transformation|GetActorLocation)))