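; BP_Cookie is a collectible cookie that is eaten in three pokes.
; Each PokeEvent plays a random bite sound and bounce timeline, steps CookieHealth down, and shows munch particles with a bitten mesh swap.
; The final bite hides the cookie, increments the shared Counter and spawns an "n/8" count effect; the eighth also spawns a named BP_Floppy that flies off.
; Grab, click and hover functions are default stubs.
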(event EventPokeEvent
  (bind _returnvalue (Transformation|GetActorLocation))
  (bind _p_cookiemunch1 (Variables|Default|GetP_CookieMunch1))
  (bind _p_cookiemunch2 (Variables|Default|GetP_CookieMunch2))
  (bind _p_cookiemunch3 (Variables|Default|GetP_CookieMunch3))
  (bind _counter (Variables|Default|GetCounter))
  (bind (_x _y _z) (Math|Vector|BreakVector _returnvalue))
  (Audio|PlaySoundatLocation (.OutItem (Utilities|Array|Random (Utilities|Array|MakeArray "/Game/Audio/SFX/Bite1.Bite1" "/Game/Audio/SFX/Bite2.Bite2"))) (Transformation|GetWorldLocation (Variables|Default|GetCookieMesh)) "0, 0, 0" 0.5 (Math|Random|RandomFloatinRange 0.88 1.12) 0.0 "/Game/Audio/Attenuation/SA_ShortRange.SA_ShortRange" "/Game/Audio/Attenuation/SC_Default.SC_Default" 0)
  (Components|Timeline|PlayfromStart (Variables|Default|GetTL_bounce))
  (switch int (Variables|Default|GetCookieHealth)
    (:1
      (Utilities|FlowControl|Sequence
        (:then_0
          (Components|Activation|Activate _p_cookiemunch3 false)
          (Utilities|FlowControl|Delay 0.5)
          (Components|Activation|Deactivate _p_cookiemunch3))
        (:then_1
          (Utilities|FlowControl|Delay 0.08)
          (Rendering|SetVisibility (Variables|Default|GetCookieMesh) false false)
          (Components|DestroyComponent (Variables|Default|GetBox))
          (bind _output_get (Variables|/Game/Blueprints/GameObjects/BP_CookieCounter.BP_CookieCounter_C|SetCookieCount _counter (+ (Variables|/Game/Blueprints/GameObjects/BP_CookieCounter.BP_CookieCounter_C|GetCookieCount _counter) 1)))
          (Variables|Default|SetCountNum _output_get)
          (bind _returnvalue_2 (Game|SpawnActorfromClass "/Game/Blueprints/GameObjects/BP_CookieCountFX.BP_CookieCountFX_C" (Math|Transform|MakeTransform (Transformation|GetActorLocation)) "Undefined" 0 0))
          (Rendering|Components|TextRender|SetText (Variables|/Game/Blueprints/GameObjects/BP_CookieCountFX.BP_CookieCountFX_C|GetTextRender _returnvalue_2) (Utilities|Text|ToText(String) (Utilities|String|Append (Utilities|String|ToString(Integer) (Variables|Default|GetCountNum)) "/8")))
          (if (== (Variables|Default|GetCountNum) 8)
            (Utilities|FlowControl|Delay 0.6)
            (bind _returnvalue_3 (Game|SpawnActorfromClass "/Game/Blueprints/GameObjects/BP_Floppy.BP_Floppy_C" (Math|Transform|MakeTransform (Math|Vector|MakeVector _x _y (+ _z 5e+01)) "0, 0, 0" "0.010000,0.010000,0.010000") "Undefined" 0 "" 0 0))
            (Default|SpawnEntity _returnvalue_3)
            (Variables|/Game/Blueprints/GameObjects/BP_Floppy.BP_Floppy_C|SetName _returnvalue_3 (Variables|/Game/Blueprints/GameObjects/BP_CookieCounter.BP_CookieCounter_C|GetFloppyName (Variables|Default|GetCounter)))
            (Default|FlytoEvent _returnvalue_3))
          (Variables|Default|SetCookieHealth (- (Variables|Default|GetCookieHealth) 1) :!label _label))))
    (:2
      (Components|StaticMesh|SetStaticMesh (Variables|Default|GetCookieMesh) "/Game/Meshes/CookieBite2.CookieBite2")
      (Utilities|FlowControl|Sequence
        (:then_0
          (Components|Activation|Activate _p_cookiemunch2 false)
          (Utilities|FlowControl|Delay 0.5)
          (Components|Activation|Deactivate _p_cookiemunch2))
        (:then_1
          (goto _label))))
    (:3
      (Components|StaticMesh|SetStaticMesh (Variables|Default|GetCookieMesh) "/Game/Meshes/CookieBite1.CookieBite1")
      (Utilities|FlowControl|Sequence
        (:then_0
          (Components|Activation|Activate _p_cookiemunch1 false)
          (Utilities|FlowControl|Delay 0.5)
          (Components|Activation|Deactivate _p_cookiemunch1))
        (:then_1
          (goto _label))))))

(fn ConstructionScript)

(fn Attachto
  (params (ChildActor :type Actor%20Object%20Reference))
  (return 0))

(fn CanGrab
  (return false))

(fn Clicked
  (return false))

(fn DisableCollision
  (return false))

(fn DoesParentHaveParent
  (return false))

(fn EnableCollision
  (return false))

(fn GetAttached
  (return 0))

(fn GetCustomCursor
  (return false 0))

(fn GetShrinkScale
  (return "0, 0, 0" "0, 0, 0"))

(fn GetSnapLoc
  (params (CursorLoc :type Vector :default "0, 0, 0"))
  (return "0, 0, 0" "0, 0, 0"))

(fn Grabbed
  (return 0))

(fn LetGo
  (params (ParentComponent :type Actor%20Component%20Object%20Reference) (ParentActor :type Actor%20Object%20Reference))
  (return false))

(fn OnHover
  (return false))

(fn PassChildAlong
  (return 0 0))

(fn RightClickEvent
  (return (Variables|Default|GetClick%20Message) (Transformation|GetActorLocation)))