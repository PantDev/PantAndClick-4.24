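; BP_TitleSign is the main menu title sign, whose stone spins when poked.
; PokeEvent restarts the TL_SignSpin timeline, whose alpha lerps the MenuTitleSignStone relative rotation through a full turn.
; The grab, click, hover, snap and attach functions are empty stubs returning default values, so the sign does nothing else.
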(event EventBeginPlay)

(event Collision|EventActorBeginOverlap
  (params (OtherActor :type Actor%20Object%20Reference)))

(event EventTick
  (params (DeltaSeconds :type Float%20%28single-precision%29)))

(event EventPokeEvent
  (bind _alpha (Timeline|TL_SignSpin PlayFromStart)
    (:Update
      (Transformation|SetRelativeRotation (Variables|Default|GetMenuTitleSignStone) (Math|Rotator|Lerp(Rotator) "0, 0, 0" "0,360.000000, 0" _alpha) false false))))

(fn ConstructionScript)

(fn Attachto
  (params (ChildActor :type Actor%20Object%20Reference))
  (return 0))

(fn CanGrab
  (return false))

(fn Clicked
  (return false))

(fn DisableCollision
  (return false))

(fn DoesParentHaveParent
  (return false))

(fn EnableCollision
  (return false))

(fn GetAttached
  (return 0))

(fn GetCustomCursor
  (return false 0))

(fn GetShrinkScale
  (return "0, 0, 0" "0, 0, 0"))

(fn GetSnapLoc
  (params (CursorLoc :type Vector :default "0, 0, 0"))
  (return "0, 0, 0" "0, 0, 0"))

(fn Grabbed
  (return 0))

(fn LetGo
  (params (ParentComponent :type Actor%20Component%20Object%20Reference) (ParentActor :type Actor%20Object%20Reference))
  (return false))

(fn OnHover
  (return false))

(fn PassChildAlong
  (return 0 0))