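; BP_HyperLink is a clickable swing point styled as a web hyperlink, with spinning brackets, a hover underline and yellow/purple link colors.
; Clicking it spawns a chain and puts the pants character into a swing, with timelines animating the brackets and moving an attach point along a spline.
; Tick pins the player to that point while easing the spline toward camera yaw.
; Letting go destroys the chain and launches the player vertically, scaled by swing alpha.
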(event EventBeginPlay
  (bind _tl_bracketidle (Variables|Default|GetTL_BracketIdle))
  (Components|Timeline|SetPlayRate _tl_bracketidle 0.82)
  (Components|Timeline|PlayfromStart _tl_bracketidle))

(event Collision|EventActorBeginOverlap
  (params (OtherActor :type Actor%20Object%20Reference)))

(event EventEndOverlap
  (bind _tl_underline (Variables|Default|GetTL_Underline))
  (Components|Timeline|SetNewTime _tl_underline 0.03)
  (Utilities|String|Reverse _tl_underline)
  (Variables|Default|SetIsHover false))

(event EventTick
  (params (DeltaSeconds :type Float%20%28single-precision%29))
  (bind _returnvalue (Game|GetPlayerCharacter 0))
  (bind _returnvalue_2 (Utilities|Time|GetWorldDeltaSeconds))
  (bind _spline (Variables|Default|GetSpline))
  (bind _returnvalue_3 (Pawn|GetControlRotation _returnvalue :!class /Script/Engine.Pawn))
  (bind _returnvalue_4 (Transformation|GetWorldRotation _spline))
  (bind _yaw (Math|Rotator|BreakRotator _returnvalue_3))
  (bind _returnvalue_5 (+ _yaw 1.8e+02))
  (bind _returnvalue_6 (Math|Rotator|MakeRotator 0.0 0.0 _returnvalue_5))
  (bind _returnvalue_7 (Math|Interpolation|RInterpTo _returnvalue_4 _returnvalue_6 _returnvalue_2 5.0))
  (bind (_roll _pitch _yaw_2) (Math|Rotator|BreakRotator _returnvalue_7))
  (if (Variables|Default|GetActive)
    (Transformation|SetActorLocation _returnvalue (Transformation|GetWorldLocation (Variables|Default|GetAttachLoc)) false false)
    (Transformation|SetActorRotation _returnvalue (Math|Rotator|MakeRotator _roll _pitch (- _yaw_2 1.8e+02)))
    (Transformation|SetWorldRotation _spline _returnvalue_7 false false)
    (bind _asbp_pant_controller (Utilities|Casting|CastToBP_PantController (Game|GetPlayerCharacter 0)))
    (Transformation|SetWorldLocation (Variables|Default|GetSphere) (Math|Vector|MakeVector (.X (Math|Vector|BreakVector (Transformation|GetWorldLocation (Variables|/Game/PantControllerBP/Blueprints/BP_PantController.BP_PantController_C|GetDenimMesh _asbp_pant_controller)))) (.Y (Math|Vector|BreakVector (Transformation|GetWorldLocation (Variables|/Game/PantControllerBP/Blueprints/BP_PantController.BP_PantController_C|GetDenimMesh _asbp_pant_controller)))) (+ (.Z (Math|Vector|BreakVector (Transformation|GetWorldLocation (Variables|/Game/PantControllerBP/Blueprints/BP_PantController.BP_PantController_C|GetDenimMesh _asbp_pant_controller)))) 5e+01)) false false)))

(fn ConstructionScript)

(fn Attachto
  (params (ChildActor :type Actor%20Object%20Reference))
  (return 0))

(fn CanGrab
  (return true))

(fn Clicked
  (Components|Timeline|ReversefromEnd (Variables|Default|GetTL_Underline))
  (Audio|PlaySoundatLocation "/Game/Audio/SFX/ChainLinked.ChainLinked" (Transformation|GetActorLocation) "0, 0, 0" 0.35 (Math|Random|RandomFloatinRange 0.75 1.0) 0.1 "/Game/Audio/Attenuation/SA_ShortRange.SA_ShortRange" 0 0)
  (Game|SpawnActorfromClass "/Game/Blueprints/FX/BP_PopParticle.BP_PopParticle_C" (Math|Transform|MakeTransform (Transformation|GetActorLocation (Game|GetPlayerCharacter 0))) "Undefined" 0 0)
  (Transformation|SetWorldRotation (Variables|Default|GetSpline) (Math|Rotator|MakeRotator 0.0 0.0 (.Yaw (Math|Rotator|BreakRotator (Math|Rotator|FindLookatRotation (Transformation|GetActorLocation) (Transformation|GetActorLocation (Game|GetPlayerCharacter 0)))))) false false)
  (bind _asbp_pant_controller (Utilities|Casting|CastToBP_PantController (Game|GetPlayerCharacter 0)))
  (Components|Activation|Deactivate (Variables|/Game/PantControllerBP/Blueprints/BP_PantController.BP_PantController_C|GetParticleSystem2 _asbp_pant_controller))
  (Variables|/Game/PantControllerBP/Blueprints/BP_PantController.BP_PantController_C|SetSwinging _asbp_pant_controller true)
  (Components|Animation|PlayAnimation (Variables|/Game/PantControllerBP/Blueprints/BP_PantController.BP_PantController_C|GetDenimMesh _asbp_pant_controller) "/Game/Meshes/PantMesh/Master/Denim_Armature_Roll.Denim_Armature_Roll" true)
  (Variables|Default|SetActive true)
  (Components|Timeline|PlayfromStart (Variables|Default|GetTL_LerpTo))
  (Rendering|SetVisibility (Variables|Default|GetSphere) true true)
  (Components|Timeline|PlayfromStart (Variables|Default|GetTL_Grabbed))
  (bind _returnvalue (Game|SpawnActorfromClass "/Game/Blueprints/GameObjects/BP_LinkChain.BP_LinkChain_C" (Math|Transform|MakeTransform (Transformation|GetActorLocation)) "Undefined" 0 0))
  (Variables|Default|SetChain _returnvalue)
  (Rendering|Material|SetMaterial (Variables|Default|GetBracket1) 0 "/Game/Materials/HyperLink_Yellow_Mat.HyperLink_Yellow_Mat")
  (Rendering|Material|SetMaterial (Variables|Default|GetUnderlineMesh) 1 "/Game/Materials/HyperLink_Yellow_Mat.HyperLink_Yellow_Mat")
  (return false))

(fn DisableCollision
  (return false))

(fn DoesParentHaveParent
  (return false))

(fn EnableCollision
  (return false))

(fn GetAttached
  (return 0))

(fn GetShrinkScale
  (return "0, 0, 0" "0, 0, 0"))

(fn GetSnapLoc
  (params (CursorLoc :type Vector :default "0, 0, 0"))
  (return "0, 0, 0" "0, 0, 0"))

(fn Grabbed
  (return 0))

(fn LetGo
  (params (ParentComponent :type Actor%20Component%20Object%20Reference) (ParentActor :type Actor%20Object%20Reference))
  (Audio|PlaySoundatLocation "/Game/Audio/SFX/ClickMusicSFX/Click4.Click4" (Transformation|GetActorLocation (Game|GetPlayerCharacter 0)) "0, 0, 0" 0.22 (Math|Random|RandomFloatinRange 1.3 1.45) 0.1 "/Game/Audio/Attenuation/SA_ShortRange.SA_ShortRange" 0 0)
  (Game|SpawnActorfromClass "/Game/Blueprints/FX/BP_PopParticle.BP_PopParticle_C" (Math|Transform|MakeTransform (Transformation|GetActorLocation (Game|GetPlayerCharacter 0))) "Undefined" 0 0)
  (Rendering|SetVisibility (Variables|Default|GetSphere) false true)
  (bind _asbp_pant_controller (Utilities|Casting|CastToBP_PantController (Game|GetPlayerCharacter 0)))
  (Components|Activation|Deactivate (Variables|/Game/PantControllerBP/Blueprints/BP_PantController.BP_PantController_C|GetParticleSystem2 _asbp_pant_controller))
  (Variables|/Game/PantControllerBP/Blueprints/BP_PantController.BP_PantController_C|SetDoubleJumpUsed _asbp_pant_controller false)
  (Variables|/Game/PantControllerBP/Blueprints/BP_PantController.BP_PantController_C|SetIsDiving _asbp_pant_controller false)
  (Audio|Components|Audio|Stop (Variables|Default|GetTL_Swing))
  (Transformation|SetWorldLocation (Variables|Default|GetAttachLoc) (Transformation|GetWorldLocation (Variables|Default|GetAttachLoc1)) false false)
  (Variables|/Game/PantControllerBP/Blueprints/BP_PantController.BP_PantController_C|SetSwinging _asbp_pant_controller false)
  (Variables|Default|SetActive false)
  (Character|LaunchCharacter _asbp_pant_controller (Math|Vector|Lerp(Vector) "0, 0,-150.000000" "0, 0,2800.000000" (Variables|Default|GetSwingAlpha)) false true)
  (Actor|DestroyActor (Variables|Default|GetChain))
  (Rendering|Material|SetMaterial (Variables|Default|GetBracket1) 0 "/Game/Materials/HyperLink_Purple_Mat.HyperLink_Purple_Mat")
  (Rendering|Material|SetMaterial (Variables|Default|GetUnderlineMesh) 1 "/Game/Materials/HyperLink_Purple_Mat.HyperLink_Purple_Mat")
  (Audio|Components|Audio|AdjustVolume (Variables|Default|GetAudio) 0.2 0.0 "Linear" :!class /Script/Engine.AudioComponent)
  (Variables|Default|SetInterp%20Speed 1e+01)
  (return false))

(fn OnHover
  (if (not (Variables|Default|GetIsHover))
    (Variables|Default|SetIsHover true)
    (Rendering|SetVisibility (Variables|Default|GetUnderlineMesh) true false)
    (Components|Timeline|PlayfromStart (Variables|Default|GetTL_Underline))
    (return false)))

(fn PassChildAlong
  (return 0 0))