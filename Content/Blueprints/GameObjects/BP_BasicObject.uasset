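; BP_BasicObject is a grabbable, placeable object with a configurable mesh, offsets and optional physics.
; Clicked stops physics and re-centers the actor on its mesh; LetGo restores physics and plays a random-pitch pop with a timeline scale pulse.
; BeginPlay attaches mushrooms from GetAttached to the mesh, AddOffsetZ yaws it, and cursor hover destroys the actor.
; Most other interaction functions are stubs, and the overlap-shrink logic is unconnected.
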(event Custom|LetGoEvent
  (Audio|PlaySoundatLocation "/Game/Audio/SFX/Pop.Pop" (Transformation|GetActorLocation) "0, 0, 0" 1.0 (Math|Random|RandomFloatinRange 0.7 1.1) 0.0 "/Game/Audio/Attenuation/SA_Default.SA_Default" "/Game/Audio/Attenuation/SC_Default.SC_Default" 0)
  (Variables|Default|SetScaleDest (Transformation|GetWorldScale (Variables|Default|GetStaticMesh)))
  (bind _alpha (Timeline|SpawnAnim PlayFromStart)
    (:Update
      (Transformation|SetWorldScale3D (Variables|Default|GetStaticMesh) (Math|Vector|Lerp(Vector) (Variables|Default|GetScaleDest) (Math|Vector|MakeVector (* (.X (Math|Vector|BreakVector (Variables|Default|GetScaleDest))) 1.2) (* (.Y (Math|Vector|BreakVector (Variables|Default|GetScaleDest))) 1.2) (* (.Z (Math|Vector|BreakVector (Variables|Default|GetScaleDest))) 1.2)) _alpha)))))

(event Custom|BreakCheckLoop
  (bind _staticmesh (Variables|Default|GetStaticMesh))
  (Utilities|Array|ForEachLoopwithBreak (stale _outactors)) ; enters at Break
)

(event EventBeginPlay
  (bind _attachedactors (CallFunction|GetAttached))
  (for _array_element _attachedactors
    (bind _asbp_mushroom (Utilities|Casting|CastToBP_Mushroom _array_element))
    (Transformation|AttachComponentToComponent (Variables|/Game/Blueprints/GameObjects/BP_Mushroom.BP_Mushroom_C|GetStaticMesh _asbp_mushroom) (Variables|Default|GetStaticMesh) "None" "KeepWorld" "KeepWorld" "KeepWorld" true)))

(event EventAddOffsetZ
  (params (Offset_Z :type Float%20%28single-precision%29))
  (Transformation|AddRelativeRotation (Variables|Default|GetStaticMesh) (Math|Rotator|MakeRotator 0.0 0.0 Offset_Z) false false))

(event MouseInput|EventActorBeginCursorOver
  (Actor|DestroyActor))

(fn ConstructionScript
  (Components|StaticMesh|SetStaticMesh (Variables|Default|GetStaticMesh) (Variables|Default|GetMesh))
  (Rendering|Material|SetMaterial (Variables|Default|GetStaticMesh) 0 0)
  (Transformation|SetRelativeLocationAndRotation (Variables|Default|GetStaticMesh) (Variables|Default|GetLocationOffset) (Variables|Default|GetRotationOffset) false false)
  (Variables|Default|SetOriginalScale (Transformation|GetActorScale3D)))

(fn Attachto
  (params (ChildActor :type Actor%20Object%20Reference))
  (return (Utilities|Array|MakeArray 0)))

(fn Clicked
  (Physics|SetSimulatePhysics (Variables|Default|GetStaticMesh) false)
  (Transformation|SetActorLocation (Transformation|GetWorldLocation (Variables|Default|GetStaticMesh)) false true)
  (Transformation|SetRelativeLocation (Variables|Default|GetStaticMesh) "0, 0, 0" false true)
  (return false))

(fn DisableCollision
  (return false))

(fn DoesParentHaveParent
  (return false))

(fn EnableCollision
  (return false))

(fn GetAttached
  (return (Utilities|Array|MakeArray 0)))

(fn GetShrinkScale
  (return (Variables|Default|GetShrinkScale) (Variables|Default|GetOriginalScale)))

(fn GetSnapLoc
  (params (CursorLoc :type Vector :default "0, 0, 0"))
  (return "0, 0, 0" "0, 0, 0"))

(fn Grabbed
  (return 0))

(fn LetGo
  (params (ParentComponent :type Actor%20Component%20Object%20Reference) (ParentActor :type Actor%20Object%20Reference))
  (CallFunction|LetGoEvent)
  (Physics|SetSimulatePhysics (Variables|Default|GetStaticMesh) (Variables|Default|GetActivatePhysics))
  (return false))

(fn OnHover
  (return false))

(fn PassChildAlong
  (return 0 0))