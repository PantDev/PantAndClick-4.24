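; BP_FloppyCage is a floppy cage game object that can play a short pop-and-vanish effect.
; PopEvent fires the PFloppyPop effect and enlarges StaticMesh2, then after a very brief delay hides the mesh and deactivates the effect.
; Its cursor, grab, snap and attach functions are empty stubs returning defaults, so it cannot be grabbed and has no custom cursor.
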(event Custom|PopEvent
  (bind _p_floppypop (Variables|Default|GetP_FloppyPop))
  (bind _staticmesh2 (Variables|Default|GetStaticMesh2))
  (Components|Activation|Activate _p_floppypop false)
  (Transformation|SetRelativeScale3D _staticmesh2 "1.300000,1.300000,1.300000")
  (Utilities|FlowControl|Delay 0.02)
  (Rendering|SetVisibility _staticmesh2 false false)
  (Components|Activation|Deactivate _p_floppypop))

(event EventBeginPlay)

(event Collision|EventActorBeginOverlap
  (params (OtherActor :type Actor%20Object%20Reference)))

(event EventTick
  (params (DeltaSeconds :type Float%20%28single-precision%29)))

(fn ConstructionScript)

(fn GetCustomCursor
  (return false 0))

(fn CanGrab
  (return false))

(fn PassChildAlong
  (return 0 0))

(fn DoesParentHaveParent
  (return false))

(fn GetShrinkScale
  (return "0, 0, 0" "0, 0, 0"))

(fn GetSnapLoc
  (params (CursorLoc :type Vector :default "0, 0, 0"))
  (return "0, 0, 0" "0, 0, 0"))

(fn GetAttached
  (return 0))

(fn EnableCollision
  (return false))

(fn DisableCollision
  (return false))

(fn Attachto
  (params (ChildActor :type Actor%20Object%20Reference))
  (return 0))

(fn Grabbed
  (return 0))

(fn OnHover
  (return false))

(fn LetGo
  (params (ParentComponent :type Actor%20Component%20Object%20Reference) (ParentActor :type Actor%20Object%20Reference))
  (return false))

(fn Clicked
  (return false))