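; BP_Pencil is a pencil game object that can bob up and down in place when Hovering is set.
; Its construction script applies Color through a dynamic material instance and caches the start location.
; On BeginPlay, a timeline scaled by HoverDuration ping-pongs, teleporting the actor vertically across HoverDistance, shifted down by Zoffset.
; A stepped-on timeline that would animate Zoffset is present but never triggered.
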(event EventBeginPlay
  (bind _startloc (Variables|Default|GetStartLoc))
  (bind _tl_hover (Variables|Default|GetTL_Hover))
  (bind (_x _y _z) (Math|Vector|BreakVector _startloc))
  (bind (_x_2 _y_2 _z_2) (Math|Vector|BreakVector _startloc))
  (if (Variables|Default|GetHovering)
    (Components|Timeline|SetPlayRate (Variables|Default|GetTL_Hover) (/ 1.0 (Variables|Default|GetHoverDuration)))
    (bind (_direction _alpha) (Timeline|TL_Hover PlayFromStart)
      (:Update
        (Transformation|SetActorLocation (Math|Vector|Lerp(Vector) (Math|Vector|MakeVector _x _y (- _z (Variables|Default|GetZoffset))) (Math|Vector|MakeVector _x_2 _y_2 (- (+ _z_2 (Variables|Default|GetHoverDistance)) (Variables|Default|GetZoffset))) _alpha) false true))
      (:Finished
        (switch Utilities|FlowControl|Switch|SwitchonETimelineDirection _direction
          (:Forward
            (Components|Timeline|ReversefromEnd _tl_hover))
          (:Backward
            (Components|Timeline|PlayfromStart _tl_hover)))))))

(fn ConstructionScript
  (bind _returnvalue (Rendering|Material|CreateDynamicMaterialInstance (Variables|Default|GetPencilMesh) 0 "/Game/Materials/Pencil_Mat.Pencil_Mat" "None" :!class /Script/Engine.PrimitiveComponent))
  (bind _output_get (Variables|Default|SetMaterialInstance _returnvalue))
  (Rendering|Material|SetVectorParameterValue _output_get "Color" (Variables|Default|GetColor) :!class /Script/Engine.MaterialInstanceDynamic)
  (Variables|Default|SetStartLoc (Transformation|GetActorLocation)))