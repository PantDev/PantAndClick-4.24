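; BP_Drum is a snare drum launch pad that returns a velocity along its mesh-to-arrow direction, scaled by Velocity.Z.
; GetLaunchVelocity, also triggered by PokeEvent, plays a pitch-randomized snare sound, pulses dust and restarts two timelines.
; The timelines drive morph-target deformation, a squash-and-stretch bounce, and a randomly rotated, expanding impact plane using a dynamic material.
; Its grab, click, hover, attach and snap functions are empty stubs.
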(event Custom|Dust
  (Components|Activation|Activate (Variables|Default|GetParticleSystem) false)
  (Utilities|FlowControl|Delay 0.01)
  (Components|Activation|Deactivate (Variables|Default|GetParticleSystem)))

(event EventBeginPlay)

(event Collision|EventActorBeginOverlap
  (params (OtherActor :type Actor%20Object%20Reference)))

(event EventTick
  (params (DeltaSeconds :type Float%20%28single-precision%29)))

(event EventPokeEvent
  (CallFunction|GetLaunchVelocity))

(fn ConstructionScript
  (bind _returnvalue (Rendering|Material|CreateDynamicMaterialInstance (Variables|Default|GetPlane) 0 "/Game/Meshes/DAW/Drums/DrumImpact_Mat.DrumImpact_Mat" "None" :!class /Script/Engine.PrimitiveComponent))
  (bind _output_get (Variables|Default|SetImpactMat _returnvalue))
  (Rendering|Material|SetMaterial (Variables|Default|GetPlane) 0 _output_get))

(fn Attachto
  (params (ChildActor :type Actor%20Object%20Reference))
  (return 0))

(fn CanGrab
  (return false))

(fn Clicked
  (return false))

(fn DisableCollision
  (return false))

(fn DoesParentHaveParent
  (return false))

(fn EnableCollision
  (return false))

(fn GetAttached
  (return 0))

(fn GetCustomCursor
  (return false 0))

(fn GetLaunchVelocity
  (Audio|PlaySoundatLocation "/Game/Audio/DAW/SFX/Snare.Snare" (Transformation|GetActorLocation) "0, 0, 0" 1.0 (Math|Random|RandomFloatinRange 0.5 0.85) 0.0 "/Game/Audio/Attenuation/SA_ShortRange.SA_ShortRange" "/Game/Audio/Attenuation/SC_Default.SC_Default" 0)
  (Components|Timeline|PlayfromStart (Variables|Default|GetTL_ImpactAnim))
  (Transformation|SetRelativeRotation (Variables|Default|GetPlane) (Math|Rotator|MakeRotator 0.0 0.0 (Math|Random|RandomFloatinRange 0.0 3.6e+02)) false false)
  (CallFunction|Dust)
  (return (* (Math|Vector|GetUnitDirection(Vector) (Transformation|GetWorldLocation (Variables|Default|GetStaticMesh)) (Transformation|GetWorldLocation (Variables|Default|GetArrow))) (.Z (Math|Vector|BreakVector (Variables|Default|GetVelocity))))))

(fn GetShrinkScale
  (return "0, 0, 0" "0, 0, 0"))

(fn GetSnapLoc
  (params (CursorLoc :type Vector :default "0, 0, 0"))
  (return "0, 0, 0" "0, 0, 0"))

(fn Grabbed
  (return 0))

(fn LetGo
  (params (ParentComponent :type Actor%20Component%20Object%20Reference) (ParentActor :type Actor%20Object%20Reference))
  (return false))

(fn OnHover
  (return false))

(fn PassChildAlong
  (return 0 0))