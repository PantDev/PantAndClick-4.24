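; BP_Crayon is a crayon prop that gives each placed instance a random color and yaw.
; The Construction Script creates dynamic material instances for the crayon and wrapper slots, then calls RandomizeColor and spins the mesh around Z.
; RandomizeColor picks one random RGB color, setting a darkened version on the crayon and a brightened one on the wrapper.
; The event graph has no active logic.
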(event EventBeginPlay)

(event Collision|EventActorBeginOverlap
  (params (OtherActor :type Actor%20Object%20Reference)))

(event EventTick
  (params (DeltaSeconds :type Float%20%28single-precision%29)))

(fn ConstructionScript
  (bind _staticmesh (Variables|Default|GetStaticMesh))
  (bind _staticmesh_2 (Variables|Default|GetStaticMesh))
  (bind _returnvalue (Rendering|Material|CreateDynamicMaterialInstance _staticmesh 0 "/Game/Materials/Crayon_Mat.Crayon_Mat" "None" :!class /Script/Engine.PrimitiveComponent))
  (Variables|Default|SetCrayonMat _returnvalue)
  (bind _returnvalue_2 (Rendering|Material|CreateDynamicMaterialInstance _staticmesh 1 "/Game/Materials/CrayonWrap_Mat.CrayonWrap_Mat" "None" :!class /Script/Engine.PrimitiveComponent))
  (Variables|Default|SetCrayonWrapMat _returnvalue_2)
  (Rendering|Material|SetMaterial _staticmesh_2 0 (Variables|Default|GetCrayonMat))
  (Rendering|Material|SetMaterial _staticmesh_2 1 (Variables|Default|GetCrayonWrapMat))
  (CallFunction|RandomizeColor)
  (Transformation|SetRelativeRotation (Variables|Default|GetStaticMesh) (Math|Rotator|MakeRotator 0.0 0.0 (Math|Random|RandomFloatinRange 0.0 3.6e+02)) false false))

(fn RandomizeColor
  (LocalVariables|SetTempColor (Math|Color|MakeColor (Math|Random|RandomFloatinRange 0.0 1.0) (Math|Random|RandomFloatinRange 0.0 1.0) (Math|Random|RandomFloatinRange 0.0 1.0)))
  (Rendering|Material|SetVectorParameterValue (Variables|Default|GetCrayonMat) "Color" (Math|Color|MakeColor (/ (.R (Math|Color|BreakColor (LocalVariables|GetTempColor))) 3.0) (/ (.G (Math|Color|BreakColor (LocalVariables|GetTempColor))) 3.0) (/ (.B (Math|Color|BreakColor (LocalVariables|GetTempColor))) 3.0) (.A (Math|Color|BreakColor (LocalVariables|GetTempColor)))) :!class /Script/Engine.MaterialInstanceDynamic)
  (Rendering|Material|SetVectorParameterValue (Variables|Default|GetCrayonWrapMat) "Color" (Math|Color|MakeColor (* (.R (Math|Color|BreakColor (LocalVariables|GetTempColor))) 2.0) (* (.G (Math|Color|BreakColor (LocalVariables|GetTempColor))) 2.0) (* (.B (Math|Color|BreakColor (LocalVariables|GetTempColor))) 2.0) (.A (Math|Color|BreakColor (LocalVariables|GetTempColor)))) :!class /Script/Engine.MaterialInstanceDynamic))