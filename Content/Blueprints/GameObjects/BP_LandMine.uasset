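; Land mine game object that explodes when its sphere is overlapped, then reappears and kills the overlapping actor if it is a BP_PantController.
; The overlap hides the mesh, fires particles and scales up the explosion through a timeline, with the kill delayed until it finishes.
; PokeEvent plays a spin sound and a pulse timeline meant to speed up rotation and redden the dynamic material.
; Grab, click, hover and attach functions are inert stubs.
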(event OnComponentBeginOverlap(Sphere)
  (params (OverlappedComponent :type Primitive%20Component%20Object%20Reference) (OtherActor :type Actor%20Object%20Reference) (OtherComp :type Primitive%20Component%20Object%20Reference) (OtherBodyIndex :type Integer) (bFromSweep :type Boolean) (SweepResult :type Hit%20Result%20Structure%20%28by%20ref%29))
  (Components|Activation|Activate (Variables|Default|GetP_splosion) false)
  (Rendering|SetVisibility (Variables|Default|GetMineMesh) false false)
  (bind _newtrack_0 (Timeline|TL_Splosion PlayFromStart)
    (:Update
      (Transformation|SetRelativeScale3D (Variables|Default|GetSplosion) (Math|Vector|Lerp(Vector) "0.800000,0.800000,0.800000" "1.400000,1.400000,1.400000" _newtrack_0)))
    (:Finished
      (Components|Activation|Deactivate (Variables|Default|GetP_splosion))
      (Rendering|SetVisibility (Variables|Default|GetMineMesh) true false)
      (bind _asbp_pant_controller (Utilities|Casting|CastToBP_PantController OtherActor))
      (Default|Kill _asbp_pant_controller "NewEnumerator0"))))

(event EventBeginPlay)

(event Collision|EventActorBeginOverlap
  (params (OtherActor :type Actor%20Object%20Reference)))

(event EventTick
  (params (DeltaSeconds :type Float%20%28single-precision%29)))

(event EventPokeEvent
  (Components|Timeline|PlayfromStart (Variables|Default|GetTL_Pulse))
  (Audio|PlaySoundatLocation "/Game/Audio/SFX/Minespin.Minespin" (Transformation|GetActorLocation) "0, 0, 0" 0.3 (Math|Random|RandomFloatinRange 0.9 1.1) 0.0 "/Game/Audio/Attenuation/SA_ShortRange.SA_ShortRange" 0 0))

(fn ConstructionScript
  (bind _returnvalue (Rendering|Material|CreateDynamicMaterialInstance (Variables|Default|GetMineMesh) 0 "/Game/Meshes/Material2.Material2" "None" :!class /Script/Engine.PrimitiveComponent))
  (Variables|Default|SetNewVar_0 _returnvalue))

(fn Attachto
  (params (ChildActor :type Actor%20Object%20Reference))
  (return 0))

(fn CanGrab
  (return false))

(fn Clicked
  (return false))

(fn DisableCollision
  (return false))

(fn DoesParentHaveParent
  (return false))

(fn EnableCollision
  (return false))

(fn GetAttached
  (return 0))

(fn GetCustomCursor
  (return false 0))

(fn GetShrinkScale
  (return "0, 0, 0" "0, 0, 0"))

(fn GetSnapLoc
  (params (CursorLoc :type Vector :default "0, 0, 0"))
  (return "0, 0, 0" "0, 0, 0"))

(fn Grabbed
  (return 0))

(fn LetGo
  (params (ParentComponent :type Actor%20Component%20Object%20Reference) (ParentActor :type Actor%20Object%20Reference))
  (return false))

(fn OnHover
  (return false))

(fn PassChildAlong
  (return 0 0))