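; BP_PaperStack is a paper stack game object that disappears in a poof when damaged.
; Its TakeDamage event activates the Poof component, hides the static mesh, disables its collision and plays a quiet, pitched-up randomized sound at its location.
; After a short delay, the actor destroys itself.
; The node that orients Poof along the incoming ForwardVector is disconnected, so that input is unused.
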(event EventBeginPlay)

(event Collision|EventActorBeginOverlap
  (params (OtherActor :type Actor%20Object%20Reference)))

(event EventTick
  (params (DeltaSeconds :type Float%20%28single-precision%29)))

(event EventTakeDamage
  (params (ForwardVector :type Vector :default "0, 0, 0") (Location :type Vector :default "0, 0, 0"))
  (bind _staticmesh (Variables|Default|GetStaticMesh))
  (Components|Activation|Activate (Variables|Default|GetPoof) false)
  (Collision|SetCollisionEnabled _staticmesh "NoCollision")
  (Rendering|SetVisibility _staticmesh false false)
  (Audio|PlaySoundatLocation "/Game/Audio/SFX/Random_58.Random_58" (Transformation|GetActorLocation) "0, 0, 0" 0.1 1.45 0.08 "/Game/Audio/Attenuation/SA_Default.SA_Default" "/Game/Audio/Attenuation/SC_Default.SC_Default" 0)
  (Utilities|FlowControl|Delay 1.0)
  (Actor|DestroyActor))

(fn ConstructionScript)