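; BP_ZipperClasp_Use is a zipper clasp game object that spins and keeps facing the player.
; Each Tick rotates the clasp mesh locally at a frame-rate independent speed, then turns the whole actor to look at the player pawn.
; Its Collect event only casts the player to BP_PantController, with no pickup logic after it.
; Leftover bob timeline and movement-stop nodes are disconnected.
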(event EventBeginPlay)

(event Collision|EventActorBeginOverlap
  (params (OtherActor :type Actor%20Object%20Reference)))

(event EventTick
  (params (DeltaSeconds :type Float%20%28single-precision%29))
  (Transformation|AddLocalRotation (Variables|Default|GetZipper_Clasp_Mesh) (* "0.000000,180.000000,0.000000" DeltaSeconds) false false)
  (Transformation|SetActorRotation (Math|Rotator|FindLookatRotation (Transformation|GetActorLocation) (Transformation|GetActorLocation (Game|Player|GetPlayerPawn 0)))))

(event EventCollect
  (params (PlayerCharacter :type BP%20Pant%20Controller%20Object%20Reference))
  (Utilities|Casting|CastToBP_PantController PlayerCharacter))

(fn ConstructionScript)