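; A desktop-style folder icon actor that shows flavor dialogue when right-clicked, with zipped and empty variants.
; The construction script tints the skeletal folder through dynamic material instances, using a slightly darker shade on one slot, and also colors the label text and, when zipped, the icon mesh.
; BeginPlay replaces the click message based on the Zipped and Full flags, with empty taking priority.
; RightClickEvent returns that message and the actor's location as a focus point.
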(event EventBeginPlay
  (|CallParentFunction)
  (if (Variables|Default|GetZipped)
    (Variables|Default|SetClickMessage (Utilities|Array|MakeArray "A zipped folder!" "I know you're eager to unzip, 
but keep your belt on, Pant." "We need to find a zipper clasp 
if we want to get it open.")))
  (if (not (Variables|Default|GetFull))
    (Variables|Default|SetClickMessage (Utilities|Array|MakeArray "An empty folder!" "If it had anything in it 
before, it doesn't now!"))))

(event Collision|EventActorBeginOverlap
  (params (OtherActor :type Actor%20Object%20Reference)))

(event EventTick
  (params (DeltaSeconds :type Float%20%28single-precision%29)))

(event EventTakeDamage
  (params (ForwardVector :type Vector :default "0, 0, 0") (Location :type Vector :default "0, 0, 0")))

(fn ConstructionScript
  (bind _color (Variables|Default|GetColor))
  (bind (_r _g _b _a) (Math|Color|BreakColor _color))
  (|CallParentFunction)
  (bind _returnvalue (Rendering|Material|CreateDynamicMaterialInstance (Variables|Default|GetFolderSkeletal) 0 "/Game/Materials/Material_002.Material_002" "None" :!class /Script/Engine.PrimitiveComponent))
  (Rendering|Material|SetVectorParameterValue _returnvalue "Color" _color :!class /Script/Engine.MaterialInstanceDynamic)
  (bind _returnvalue_2 (Rendering|Material|CreateDynamicMaterialInstance (Variables|Default|GetFolderSkeletal) 2 "/Game/Materials/Material_002.Material_002" "None" :!class /Script/Engine.PrimitiveComponent))
  (Rendering|Material|SetVectorParameterValue _returnvalue_2 "Color" (Math|Color|MakeColor (- _r 0.09) (- _g 0.09) (- _b 0.09) _a) :!class /Script/Engine.MaterialInstanceDynamic)
  (if (Variables|Default|GetZipped)
    (bind _returnvalue_3 (Rendering|Material|CreateDynamicMaterialInstance (Variables|Default|GetIconMesh) 0 "/Game/Materials/Material_002.Material_002" "None" :!class /Script/Engine.PrimitiveComponent))
    (Rendering|Material|SetVectorParameterValue _returnvalue_3 "Color" (Variables|Default|GetColor) :!class /Script/Engine.MaterialInstanceDynamic))
  (Rendering|Components|TextRender|SetTextRenderColor (Variables|Default|GetIconText) (Variables|Default|GetTextColor)))

(fn RightClickEvent
  (return (Variables|Default|GetClickMessage) (Transformation|GetActorLocation)))