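; Recycle bin prop that bobs in the air and smoothly turns to face the player camera.
; A timeline drives the vertical hover and replays at a new random speed each cycle, while Tick interpolates the rotation.
; The construction script shows or hides the full-bin component from the Full flag.
; AlignToFloor acts as a one-shot placement toggle, tracing down to position the actor just above the surface below.
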(event EventBeginPlay
  (bind _hover_tl (Variables|Default|GetHover_TL))
  (bind _newtrack_0 (Timeline|Hover_TL PlayFromStart)
    (:Update
      (Transformation|SetRelativeLocation (Variables|Default|GetFolder_Full) (Math|Vector|MakeVector 0.0 0.0 (Math|Float|Lerp -12.0 12.0 _newtrack_0)) false false))
    (:Finished
      (Components|Timeline|SetPlayRate _hover_tl (Math|Random|RandomFloatinRange 0.6 1.2))
      (Components|Timeline|PlayfromStart _hover_tl))))

(event Collision|EventActorBeginOverlap
  (params (OtherActor :type Actor%20Object%20Reference)))

(event EventTick
  (params (DeltaSeconds :type Float%20%28single-precision%29))
  (Transformation|SetWorldRotation (Variables|Default|GetFolder_Full) (Math|Interpolation|RInterpTo (Transformation|GetWorldRotation (Variables|Default|GetFolder_Full)) (Math|Rotator|FindLookatRotation (Transformation|GetActorLocation) (Camera|GetCameraLocation (Game|GetPlayerCameraManager 0))) DeltaSeconds 15.0) false false))

(fn ConstructionScript
  (bind _folder_full1 (Variables|Default|GetFolder_Full1))
  (if (Variables|Default|GetAlignToFloor)
    (CallFunction|FloorAlign))
  (if (Variables|Default|GetFull)
    (Rendering|SetVisibility _folder_full1 true true)
    (else
      (Rendering|SetVisibility _folder_full1 false true))))

(fn FloorAlign
  (bind _returnvalue (Transformation|GetActorLocation))
  (bind (_x _y _z) (Math|Vector|BreakVector _returnvalue))
  (Variables|Default|SetAlignToFloor false)
  (bind (_outhit _returnvalue_2) (Collision|LineTraceByChannel _returnvalue (Math|Vector|MakeVector _x _y (- _z 1e+04)) "TraceTypeQuery1" false 0 "None"))
  (if _returnvalue_2
    (Transformation|SetActorLocation (Math|Vector|MakeVector (.X (Math|Vector|BreakVector (.Location (Collision|BreakHitResult _outhit)))) (.Y (Math|Vector|BreakVector (.Location (Collision|BreakHitResult _outhit)))) (+ (.Z (Math|Vector|BreakVector (.Location (Collision|BreakHitResult _outhit)))) 1e+02)) false false))
  (return (Math|Vector|MakeVector (.X (Math|Vector|BreakVector (.Location (Collision|BreakHitResult _outhit)))) (.Y (Math|Vector|BreakVector (.Location (Collision|BreakHitResult _outhit)))) (+ (.Z (Math|Vector|BreakVector (.Location (Collision|BreakHitResult _outhit)))) 1e+02)) _returnvalue_2))