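; BP_LikeButton is a social-media icon button actor (like, heart, repost, X, smile, random or alternate) poked by the player capsule overlapping it or by OnLand.
; Construction and BeginPlay set its icon, color and burst particle through templates and dynamic materials.
; A debounced PokeEvent either flip-flops it on and off with timelines, particles and sound, or in Cycling mode advances the icon.
; CycleIcon signals an optional Activator whether the icon matches CorrectIcon.
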(event OnComponentBeginOverlap(Box2)
  (params (OverlappedComponent :type Primitive%20Component%20Object%20Reference) (OtherActor :type Actor%20Object%20Reference) (OtherComp :type Primitive%20Component%20Object%20Reference) (OtherBodyIndex :type Integer) (bFromSweep :type Boolean) (SweepResult :type Hit%20Result%20Structure%20%28by%20ref%29))
  (bind _asbp_pant_controller (Utilities|Casting|CastToBP_PantController OtherActor))
  (if (== OtherComp (Variables|/Script/Engine.Character|GetCapsuleComponent _asbp_pant_controller))
    (CallFunction|PokeEvent)))

(event EventBeginPlay
  (bind _likebutton_skeletal (Variables|Default|GetLikeButton_Skeletal))
  (Components|Timeline|SetPlayRate (Variables|Default|GetTL_LikeSquash) 2.0)
  (bind _returnvalue (Rendering|Material|CreateDynamicMaterialInstance (Variables|Default|GetLikeButton_Skeletal) 0 "/Game/Materials/LikeButton_Thumbs_Mat1.LikeButton_Thumbs_Mat1" "None" :!class /Script/Engine.PrimitiveComponent))
  (Variables|Default|SetButtonMat _returnvalue)
  (Rendering|Material|SetMaterial (Variables|Default|GetLikeButton_Skeletal) 0 (Variables|Default|GetButtonMat))
  (if (Variables|Default|GetUseAlt)
    (Rendering|Material|SetTextureParameterValue (Variables|Default|GetButtonMat) "Texture" (Variables|Default|GetAlt))
    (Rendering|Material|SetTextureParameterValue (Variables|Default|GetButtonMat) "NormalTex" (Variables|Default|GetAlt_N))
    (else
      (switch Utilities|FlowControl|Switch|SwitchonLikeButtonIcon_Enum (Variables|Default|GetIconType)
        (:NewEnumerator0
          (Rendering|Material|SetTextureParameterValue (Variables|Default|GetButtonMat) "Texture" "/Game/Materials/Textures/LikeButton_Thumbs.LikeButton_Thumbs" :!label _label)
          (Rendering|Material|SetTextureParameterValue (Variables|Default|GetButtonMat) "NormalTex" "/Game/Materials/Textures/IconButton_ThumbsUp_N.IconButton_ThumbsUp_N"))
        (:NewEnumerator1
          (Rendering|Material|SetTextureParameterValue (Variables|Default|GetButtonMat) "Texture" "/Game/Materials/Textures/IconButton_Heart.IconButton_Heart" :!label _label_2)
          (Rendering|Material|SetTextureParameterValue (Variables|Default|GetButtonMat) "NormalTex" "/Game/Materials/Textures/IconButton_Heart_N.IconButton_Heart_N"))
        (:NewEnumerator2
          (Rendering|Material|SetTextureParameterValue (Variables|Default|GetButtonMat) "Texture" "/Game/Materials/Textures/IconButton_Share.IconButton_Share" :!label _label_3)
          (Rendering|Material|SetTextureParameterValue (Variables|Default|GetButtonMat) "NormalTex" "/Game/Materials/Textures/IconButton_Share_N.IconButton_Share_N"))
        (:NewEnumerator4
          (Rendering|Material|SetTextureParameterValue (Variables|Default|GetButtonMat) "Texture" "/Game/Materials/Textures/IconButton_X.IconButton_X" :!label _label_4)
          (Rendering|Material|SetTextureParameterValue (Variables|Default|GetButtonMat) "NormalTex" "/Game/Materials/Textures/IconButton_X_N.IconButton_X_N"))
        (:NewEnumerator5
          (Rendering|Material|SetTextureParameterValue (Variables|Default|GetButtonMat) "Texture" "/Game/Materials/Textures/IconButton_Smile.IconButton_Smile" :!label _label_5)
          (Rendering|Material|SetTextureParameterValue (Variables|Default|GetButtonMat) "NormalTex" "/Game/Materials/Textures/IconButton_Smile_N.IconButton_Smile_N"))
        (:NewEnumerator6
          (switch int (Math|Random|RandomIntegerinRange 0 4)
            (:0
              (goto _label))
            (:1
              (goto _label_2))
            (:2
              (goto _label_3))
            (:3
              (goto _label_4))
            (:4
              (goto _label_5)))))))
  (Components|Timeline|PlayfromStart (Variables|Default|GetTimeline_0))
  (Rendering|Material|SetMaterial _likebutton_skeletal 1 "/Game/Materials/PopupBorder_Mat_Inst1.PopupBorder_Mat_Inst1")
  (Rendering|Material|SetMaterial _likebutton_skeletal 2 "/Game/Materials/PopupBorder_Mat_Inst2.PopupBorder_Mat_Inst2")
  (Audio|PlaySoundatLocation "/Game/Audio/SFX/LikeButtonOff.LikeButtonOff" (Transformation|GetActorLocation) "0, 0, 0" 0.22 (Math|Random|RandomFloatinRange 0.95 1.35) 0.0 "/Game/Audio/Attenuation/SA_ShortRange.SA_ShortRange" 0 0)
  (CallFunction|PokeEvent))

(event EventPokeEvent
  (bind _likebutton_skeletal (Variables|Default|GetLikeButton_Skeletal))
  (bind _likebutton_skeletal_2 (Variables|Default|GetLikeButton_Skeletal))
  (Utilities|FlowControl|Sequence
    (:then_0
      (Utilities|FlowControl|DoOnce false :!label _label
        (:Completed
          (if (Audio|Components|Audio|IsPlaying (Variables|Default|GetTL_LikeSquash))
            (if (> (Components|Timeline|GetPlaybackPosition (Variables|Default|GetTL_LikeSquash)) 0.2)
              (Audio|Components|Audio|Stop (Variables|Default|GetTimeline_0) :!label _label_2)
              (Utilities|IsValid (Variables|Default|GetButtonMat)
                (:Is%20Valid
                  (if (Variables|Default|GetCycling)
                    (CallFunction|CycleIcon)
                    (Components|Timeline|PlayfromStart (Variables|Default|GetTL_LikeSquash))
                    (Components|Activation|Activate (Variables|Default|GetP_LikeBurst) false :!label _label_3)
                    (Audio|PlaySoundatLocation "/Game/Audio/SFX/LikeButtonOn.LikeButtonOn" (Transformation|GetActorLocation) "0, 0, 0" 0.15 (Math|Random|RandomFloatinRange 0.95 1.35) 0.0 "/Game/Audio/Attenuation/SA_ShortRange.SA_ShortRange" 0 0)
                    (else
                      (Utilities|FlowControl|FlipFlop :!label _label_4
                        (:A
                          (Components|Timeline|PlayfromStart (Variables|Default|GetTL_LikeSquash))
                          (bind _returnvalue (Rendering|Material|CreateDynamicMaterialInstance _likebutton_skeletal_2 1 "/Game/Materials/PopupBorder_Mat_Inst3.PopupBorder_Mat_Inst3" "None" :!class /Script/Engine.PrimitiveComponent))
                          (Rendering|Material|SetVectorParameterValue _returnvalue "Color" (Math|Conversions|ToLinearColor(Color) (Variables|Default|GetColor)) :!class /Script/Engine.MaterialInstanceDynamic)
                          (Rendering|Material|SetMaterial _likebutton_skeletal_2 1 _returnvalue)
                          (bind _returnvalue_2 (Rendering|Material|CreateDynamicMaterialInstance (Variables|Default|GetLikeButton_Skeletal) 2 "/Game/Materials/PopupBorder_Mat_Inst3.PopupBorder_Mat_Inst3" "None" :!class /Script/Engine.PrimitiveComponent))
                          (Rendering|Material|SetVectorParameterValue _returnvalue_2 "Color" (Math|Conversions|ToLinearColor(Color) (Variables|Default|GetColor)) :!class /Script/Engine.MaterialInstanceDynamic)
                          (Rendering|Material|SetScalarParameterValue _returnvalue_2 "Mult" 5.0 :!class /Script/Engine.MaterialInstanceDynamic)
                          (Rendering|Material|SetMaterial (Variables|Default|GetLikeButton_Skeletal) 2 _returnvalue_2)
                          (goto _label_3))
                        (:B
                          (Components|Timeline|PlayfromStart (Variables|Default|GetTimeline_0))
                          (Rendering|Material|SetMaterial _likebutton_skeletal 1 "/Game/Materials/PopupBorder_Mat_Inst1.PopupBorder_Mat_Inst1")
                          (Rendering|Material|SetMaterial _likebutton_skeletal 2 "/Game/Materials/PopupBorder_Mat_Inst2.PopupBorder_Mat_Inst2")
                          (Audio|PlaySoundatLocation "/Game/Audio/SFX/LikeButtonOff.LikeButtonOff" (Transformation|GetActorLocation) "0, 0, 0" 0.22 (Math|Random|RandomFloatinRange 0.95 1.35) 0.0 "/Game/Audio/Attenuation/SA_ShortRange.SA_ShortRange" 0 0)
                          (CallFunction|PokeEvent))))))
                (:Is%20Not%20Valid
                  (bind _returnvalue_3 (Rendering|Material|CreateDynamicMaterialInstance (Variables|Default|GetLikeButton_Skeletal) 0 "/Game/Materials/LikeButton_Thumbs_Mat1.LikeButton_Thumbs_Mat1" "None" :!class /Script/Engine.PrimitiveComponent))
                  (bind _output_get (Variables|Default|SetButtonMat _returnvalue_3))
                  (Rendering|Material|SetMaterial (Variables|Default|GetLikeButton_Skeletal) 0 _output_get)
                  (Rendering|Material|SetTextureParameterValue (Variables|Default|GetButtonMat) "Texture" (Variables|Default|GetIcon))
                  (goto _label_4))))
            (else
              (goto _label_2))))))
    (:then_1
      (Utilities|FlowControl|Delay 0.12)
      (goto _label Reset))))

(event EventOnLand
  (CallFunction|PokeEvent))

(fn ConstructionScript
  (bind _likebutton_skeletal (Variables|Default|GetLikeButton_Skeletal))
  (bind _likebutton_skeletal_2 (Variables|Default|GetLikeButton_Skeletal))
  (bind _likebutton_skeletal_3 (Variables|Default|GetLikeButton_Skeletal))
  (bind _likebutton_skeletal_4 (Variables|Default|GetLikeButton_Skeletal))
  (bind _likebutton_skeletal_5 (Variables|Default|GetLikeButton_Skeletal))
  (bind _likebutton_skeletal_6 (Variables|Default|GetLikeButton_Skeletal))
  (if (Variables|Default|GetUseAlt)
    (Effects|Components|ParticleSystem|SetTemplate (Variables|Default|GetP_LikeBurst) (Variables|Default|GetAltParticle))
    (bind _returnvalue (Rendering|Material|CreateDynamicMaterialInstance _likebutton_skeletal_6 0 (Variables|Default|GetAltMat) "None" :!class /Script/Engine.PrimitiveComponent))
    (Rendering|Material|SetTextureParameterValue _returnvalue "Texture" (Variables|Default|GetAlt))
    (Rendering|Material|SetTextureParameterValue _returnvalue "NormalTex" (Variables|Default|GetAlt_N))
    (bind _returnvalue_2 (Rendering|Material|CreateDynamicMaterialInstance _likebutton_skeletal_6 2 "/Game/Materials/PopupBorder_Mat_Inst3.PopupBorder_Mat_Inst3" "None" :!class /Script/Engine.PrimitiveComponent))
    (Rendering|Material|SetVectorParameterValue _returnvalue_2 "Color" (Variables|Default|GetAltColor) :!class /Script/Engine.MaterialInstanceDynamic)
    (Variables|Default|SetColor (Math|Conversions|ToColor(LinearColor) (Variables|Default|GetAltColor)))
    (else
      (switch Utilities|FlowControl|Switch|SwitchonLikeButtonIcon_Enum (Variables|Default|GetIconType)
        (:NewEnumerator0
          (Effects|Components|ParticleSystem|SetTemplate (Variables|Default|GetP_LikeBurst) "/Game/Effects/Particles/P_LikeBurst.P_LikeBurst" :!label _label)
          (bind _returnvalue_3 (Rendering|Material|CreateDynamicMaterialInstance _likebutton_skeletal_3 0 "/Game/Materials/Textures/LikeButton_Thumbs_Mat.LikeButton_Thumbs_Mat" "None" :!class /Script/Engine.PrimitiveComponent))
          (Rendering|Material|SetTextureParameterValue _returnvalue_3 "Texture" "/Game/Materials/Textures/LikeButton_Thumbs.LikeButton_Thumbs")
          (Rendering|Material|SetTextureParameterValue _returnvalue_3 "NormalTex" "/Game/Materials/Textures/IconButton_ThumbsUp_N.IconButton_ThumbsUp_N")
          (bind _returnvalue_4 (Rendering|Material|CreateDynamicMaterialInstance _likebutton_skeletal_3 2 "/Game/Materials/PopupBorder_Mat_Inst3.PopupBorder_Mat_Inst3" "None" :!class /Script/Engine.PrimitiveComponent))
          (Rendering|Material|SetVectorParameterValue _returnvalue_4 "Color" "(R=0.000000,G=0.080220,B=1.000000,A=1.000000)" :!class /Script/Engine.MaterialInstanceDynamic)
          (Variables|Default|SetColor (Math|Color|MakeColor 255 80 0 255)))
        (:NewEnumerator1
          (Effects|Components|ParticleSystem|SetTemplate (Variables|Default|GetP_LikeBurst) "/Game/Effects/Particles/P_HeartBurst.P_HeartBurst" :!label _label_2)
          (bind _returnvalue_5 (Rendering|Material|CreateDynamicMaterialInstance _likebutton_skeletal_2 0 "/Game/Materials/Textures/LikeButton_Thumbs_Mat.LikeButton_Thumbs_Mat" "None" :!class /Script/Engine.PrimitiveComponent))
          (Rendering|Material|SetTextureParameterValue _returnvalue_5 "Texture" "/Game/Materials/Textures/IconButton_Heart.IconButton_Heart")
          (Rendering|Material|SetTextureParameterValue _returnvalue_5 "NormalTex" "/Game/Materials/Textures/IconButton_Heart_N.IconButton_Heart_N")
          (bind _returnvalue_6 (Rendering|Material|CreateDynamicMaterialInstance _likebutton_skeletal_2 2 "/Game/Materials/PopupBorder_Mat_Inst3.PopupBorder_Mat_Inst3" "None" :!class /Script/Engine.PrimitiveComponent))
          (Rendering|Material|SetVectorParameterValue _returnvalue_6 "Color" "(R=1.000000,G=0.000000,B=0.398660,A=1.000000)" :!class /Script/Engine.MaterialInstanceDynamic)
          (Variables|Default|SetColor (Math|Color|MakeColor 170 0 255 255)))
        (:NewEnumerator2
          (Effects|Components|ParticleSystem|SetTemplate (Variables|Default|GetP_LikeBurst) "/Game/Effects/Particles/P_ShareBurst.P_ShareBurst" :!label _label_3)
          (bind _returnvalue_7 (Rendering|Material|CreateDynamicMaterialInstance _likebutton_skeletal_4 0 "/Game/Materials/Textures/LikeButton_Thumbs_Mat.LikeButton_Thumbs_Mat" "None" :!class /Script/Engine.PrimitiveComponent))
          (Rendering|Material|SetTextureParameterValue _returnvalue_7 "Texture" "/Game/Materials/Textures/IconButton_Share.IconButton_Share")
          (Rendering|Material|SetTextureParameterValue _returnvalue_7 "NormalTex" "/Game/Materials/Textures/IconButton_Share_N.IconButton_Share_N")
          (bind _returnvalue_8 (Rendering|Material|CreateDynamicMaterialInstance _likebutton_skeletal_4 2 "/Game/Materials/PopupBorder_Mat_Inst3.PopupBorder_Mat_Inst3" "None" :!class /Script/Engine.PrimitiveComponent))
          (Rendering|Material|SetVectorParameterValue _returnvalue_8 "Color" "(R=0.002125,G=0.775822,B=0.000000,A=1.000000)" :!class /Script/Engine.MaterialInstanceDynamic)
          (Variables|Default|SetColor (Math|Color|MakeColor 0 228 7 255)))
        (:NewEnumerator4
          (Effects|Components|ParticleSystem|SetTemplate (Variables|Default|GetP_LikeBurst) "/Game/Effects/Particles/P_XBurst.P_XBurst" :!label _label_4)
          (bind _returnvalue_9 (Rendering|Material|CreateDynamicMaterialInstance _likebutton_skeletal_5 0 "/Game/Materials/Textures/LikeButton_Thumbs_Mat.LikeButton_Thumbs_Mat" "None" :!class /Script/Engine.PrimitiveComponent))
          (Rendering|Material|SetTextureParameterValue _returnvalue_9 "Texture" "/Game/Materials/Textures/IconButton_X.IconButton_X")
          (Rendering|Material|SetTextureParameterValue _returnvalue_9 "NormalTex" "/Game/Materials/Textures/IconButton_X_N.IconButton_X_N")
          (bind _returnvalue_10 (Rendering|Material|CreateDynamicMaterialInstance _likebutton_skeletal_5 2 "/Game/Materials/PopupBorder_Mat_Inst3.PopupBorder_Mat_Inst3" "None" :!class /Script/Engine.PrimitiveComponent))
          (Rendering|Material|SetVectorParameterValue _returnvalue_10 "Color" "(R=1.000000,G=0.000000,B=0.012815,A=1.000000)" :!class /Script/Engine.MaterialInstanceDynamic)
          (Variables|Default|SetColor (Math|Color|MakeColor 29 0 255 255)))
        (:NewEnumerator5
          (Effects|Components|ParticleSystem|SetTemplate (Variables|Default|GetP_LikeBurst) "/Game/Effects/Particles/P_SmileBurst.P_SmileBurst" :!label _label_5)
          (bind _returnvalue_11 (Rendering|Material|CreateDynamicMaterialInstance _likebutton_skeletal 0 "/Game/Materials/Textures/LikeButton_Thumbs_Mat.LikeButton_Thumbs_Mat" "None" :!class /Script/Engine.PrimitiveComponent))
          (Rendering|Material|SetTextureParameterValue _returnvalue_11 "Texture" "/Game/Materials/Textures/IconButton_Smile.IconButton_Smile")
          (Rendering|Material|SetTextureParameterValue _returnvalue_11 "NormalTex" "/Game/Materials/Textures/IconButton_Smile_N.IconButton_Smile_N")
          (bind _returnvalue_12 (Rendering|Material|CreateDynamicMaterialInstance _likebutton_skeletal 2 "/Game/Materials/PopupBorder_Mat_Inst3.PopupBorder_Mat_Inst3" "None" :!class /Script/Engine.PrimitiveComponent))
          (Rendering|Material|SetVectorParameterValue _returnvalue_12 "Color" "(R=1.000000,G=0.916800,B=0.000000,A=1.000000)" :!class /Script/Engine.MaterialInstanceDynamic)
          (Variables|Default|SetColor (Math|Color|MakeColor 0 246 255 255)))
        (:NewEnumerator6
          (switch int (Math|Random|RandomIntegerinRange 0 4)
            (:0
              (Variables|Default|SetIconType "NewEnumerator0")
              (goto _label))
            (:1
              (Variables|Default|SetIconType "NewEnumerator1")
              (goto _label_2))
            (:2
              (Variables|Default|SetIconType "NewEnumerator2")
              (goto _label_3))
            (:3
              (Variables|Default|SetIconType "NewEnumerator4")
              (goto _label_4))
            (:4
              (Variables|Default|SetIconType "NewEnumerator5")
              (goto _label_5))))))))

(fn CycleIcon
  (bind _likebutton_skeletal (Variables|Default|GetLikeButton_Skeletal))
  (bind _likebutton_skeletal_2 (Variables|Default|GetLikeButton_Skeletal))
  (bind _activator (Variables|Default|GetActivator))
  (bind _likebutton_skeletal_3 (Variables|Default|GetLikeButton_Skeletal))
  (bind _likebutton_skeletal_4 (Variables|Default|GetLikeButton_Skeletal))
  (bind _likebutton_skeletal_5 (Variables|Default|GetLikeButton_Skeletal))
  (switch Utilities|FlowControl|Switch|SwitchonLikeButtonIcon_Enum (Variables|Default|GetIconType)
    (:NewEnumerator0
      (Variables|Default|SetIconType "NewEnumerator1")
      (Effects|Components|ParticleSystem|SetTemplate (Variables|Default|GetP_LikeBurst) "/Game/Effects/Particles/P_HeartBurst.P_HeartBurst")
      (bind _returnvalue (Rendering|Material|CreateDynamicMaterialInstance _likebutton_skeletal_2 0 "/Game/Materials/Textures/LikeButton_Thumbs_Mat.LikeButton_Thumbs_Mat" "None" :!class /Script/Engine.PrimitiveComponent))
      (Rendering|Material|SetTextureParameterValue _returnvalue "Texture" "/Game/Materials/Textures/IconButton_Heart.IconButton_Heart")
      (Rendering|Material|SetTextureParameterValue _returnvalue "NormalTex" "/Game/Materials/Textures/IconButton_Heart_N.IconButton_Heart_N")
      (bind _returnvalue_2 (Rendering|Material|CreateDynamicMaterialInstance _likebutton_skeletal_2 2 "/Game/Materials/PopupBorder_Mat_Inst3.PopupBorder_Mat_Inst3" "None" :!class /Script/Engine.PrimitiveComponent))
      (Rendering|Material|SetVectorParameterValue _returnvalue_2 "Color" "(R=1.000000,G=0.000000,B=0.398660,A=1.000000)" :!class /Script/Engine.MaterialInstanceDynamic)
      (Variables|Default|SetColor (Math|Color|MakeColor 170 0 255 255)))
    (:NewEnumerator1
      (Variables|Default|SetIconType "NewEnumerator2")
      (Effects|Components|ParticleSystem|SetTemplate (Variables|Default|GetP_LikeBurst) "/Game/Effects/Particles/P_ShareBurst.P_ShareBurst")
      (bind _returnvalue_3 (Rendering|Material|CreateDynamicMaterialInstance _likebutton_skeletal_3 0 "/Game/Materials/Textures/LikeButton_Thumbs_Mat.LikeButton_Thumbs_Mat" "None" :!class /Script/Engine.PrimitiveComponent))
      (Rendering|Material|SetTextureParameterValue _returnvalue_3 "Texture" "/Game/Materials/Textures/IconButton_Share.IconButton_Share")
      (Rendering|Material|SetTextureParameterValue _returnvalue_3 "NormalTex" "/Game/Materials/Textures/IconButton_Share_N.IconButton_Share_N")
      (bind _returnvalue_4 (Rendering|Material|CreateDynamicMaterialInstance _likebutton_skeletal_3 2 "/Game/Materials/PopupBorder_Mat_Inst3.PopupBorder_Mat_Inst3" "None" :!class /Script/Engine.PrimitiveComponent))
      (Rendering|Material|SetVectorParameterValue _returnvalue_4 "Color" "(R=0.002125,G=0.775822,B=0.000000,A=1.000000)" :!class /Script/Engine.MaterialInstanceDynamic)
      (Variables|Default|SetColor (Math|Color|MakeColor 0 228 7 255)))
    (:NewEnumerator2
      (Variables|Default|SetIconType "NewEnumerator4")
      (Effects|Components|ParticleSystem|SetTemplate (Variables|Default|GetP_LikeBurst) "/Game/Effects/Particles/P_XBurst.P_XBurst")
      (bind _returnvalue_5 (Rendering|Material|CreateDynamicMaterialInstance _likebutton_skeletal_4 0 "/Game/Materials/Textures/LikeButton_Thumbs_Mat.LikeButton_Thumbs_Mat" "None" :!class /Script/Engine.PrimitiveComponent))
      (Rendering|Material|SetTextureParameterValue _returnvalue_5 "Texture" "/Game/Materials/Textures/IconButton_X.IconButton_X")
      (Rendering|Material|SetTextureParameterValue _returnvalue_5 "NormalTex" "/Game/Materials/Textures/IconButton_X_N.IconButton_X_N")
      (bind _returnvalue_6 (Rendering|Material|CreateDynamicMaterialInstance _likebutton_skeletal_4 2 "/Game/Materials/PopupBorder_Mat_Inst3.PopupBorder_Mat_Inst3" "None" :!class /Script/Engine.PrimitiveComponent))
      (Rendering|Material|SetVectorParameterValue _returnvalue_6 "Color" "(R=1.000000,G=0.000000,B=0.012815,A=1.000000)" :!class /Script/Engine.MaterialInstanceDynamic)
      (Variables|Default|SetColor (Math|Color|MakeColor 29 0 255 255)))
    (:NewEnumerator4
      (Variables|Default|SetIconType "NewEnumerator5")
      (Effects|Components|ParticleSystem|SetTemplate (Variables|Default|GetP_LikeBurst) "/Game/Effects/Particles/P_SmileBurst.P_SmileBurst")
      (bind _returnvalue_7 (Rendering|Material|CreateDynamicMaterialInstance _likebutton_skeletal 0 "/Game/Materials/Textures/LikeButton_Thumbs_Mat.LikeButton_Thumbs_Mat" "None" :!class /Script/Engine.PrimitiveComponent))
      (Rendering|Material|SetTextureParameterValue _returnvalue_7 "Texture" "/Game/Materials/Textures/IconButton_Smile.IconButton_Smile")
      (Rendering|Material|SetTextureParameterValue _returnvalue_7 "NormalTex" "/Game/Materials/Textures/IconButton_Smile_N.IconButton_Smile_N")
      (bind _returnvalue_8 (Rendering|Material|CreateDynamicMaterialInstance _likebutton_skeletal 2 "/Game/Materials/PopupBorder_Mat_Inst3.PopupBorder_Mat_Inst3" "None" :!class /Script/Engine.PrimitiveComponent))
      (Rendering|Material|SetVectorParameterValue _returnvalue_8 "Color" "(R=1.000000,G=0.916800,B=0.000000,A=1.000000)" :!class /Script/Engine.MaterialInstanceDynamic)
      (Variables|Default|SetColor (Math|Color|MakeColor 0 246 255 255)))
    (:NewEnumerator5
      (Variables|Default|SetIconType "NewEnumerator0")
      (Effects|Components|ParticleSystem|SetTemplate (Variables|Default|GetP_LikeBurst) "/Game/Effects/Particles/P_LikeBurst.P_LikeBurst")
      (bind _returnvalue_9 (Rendering|Material|CreateDynamicMaterialInstance _likebutton_skeletal_5 0 "/Game/Materials/Textures/LikeButton_Thumbs_Mat.LikeButton_Thumbs_Mat" "None" :!class /Script/Engine.PrimitiveComponent))
      (Rendering|Material|SetTextureParameterValue _returnvalue_9 "Texture" "/Game/Materials/Textures/LikeButton_Thumbs.LikeButton_Thumbs")
      (Rendering|Material|SetTextureParameterValue _returnvalue_9 "NormalTex" "/Game/Materials/Textures/IconButton_ThumbsUp_N.IconButton_ThumbsUp_N")
      (bind _returnvalue_10 (Rendering|Material|CreateDynamicMaterialInstance _likebutton_skeletal_5 2 "/Game/Materials/PopupBorder_Mat_Inst3.PopupBorder_Mat_Inst3" "None" :!class /Script/Engine.PrimitiveComponent))
      (Rendering|Material|SetVectorParameterValue _returnvalue_10 "Color" "(R=0.000000,G=0.080220,B=1.000000,A=1.000000)" :!class /Script/Engine.MaterialInstanceDynamic)
      (Variables|Default|SetColor (Math|Color|MakeColor 255 80 0 255))))
  (Utilities|IsValid _activator
    (:Is%20Valid
      (if (== (Variables|Default|GetCorrectIcon) (Variables|Default|GetIconType))
        (Default|Activate _activator 0.0 true)
        (Variables|Default|SetDoonceBool false)
        (elif (not (Variables|Default|GetDoonceBool))
          (Variables|Default|SetDoonceBool true)
          (Default|Activate _activator 0.0 false))))))

(fn Attachto
  (params (ChildActor :type Actor%20Object%20Reference))
  (return 0))

(fn CanGrab
  (return false))

(fn Clicked
  (return false))

(fn DisableCollision
  (return false))

(fn DoesParentHaveParent
  (return false))

(fn EnableCollision
  (return false))

(fn GetAttached
  (return 0))

(fn GetCustomCursor
  (return false 0))

(fn GetShrinkScale
  (return "0, 0, 0" "0, 0, 0"))

(fn GetSnapLoc
  (params (CursorLoc :type Vector :default "0, 0, 0"))
  (return "0, 0, 0" "0, 0, 0"))

(fn Grabbed
  (return 0))

(fn LetGo
  (params (ParentComponent :type Actor%20Component%20Object%20Reference) (ParentActor :type Actor%20Object%20Reference))
  (return false))

(fn OnHover
  (return false))

(fn PassChildAlong
  (return 0 0))

(fn RightClickEvent
  (return (Variables|Default|GetClick%20Message) (Transformation|GetActorLocation)))