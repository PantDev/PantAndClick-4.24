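; BP_TinyDuck is a pokeable collectible duck that reports its discovery to a Totem actor.
; Every PokeEvent plays a randomly pitched quack and a scale timeline, pitched lower once found.
; The first poke also disables player input, bursts particles, swaps the material and calls the Totem's message.
; Number-text animation logic is partly disconnected, and the grab and click interface functions are empty stubs.
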(event EventBeginPlay
  (bind _box (Variables|Default|GetBox))
  (if (Variables|Default|GetIsSolid)
    (Collision|SetCollisionEnabled _box "QueryAndPhysics")
    (else
      (Collision|SetCollisionEnabled _box "NoCollision"))))

(event Collision|EventActorBeginOverlap
  (params (OtherActor :type Actor%20Object%20Reference)))

(event EventTick
  (params (DeltaSeconds :type Float%20%28single-precision%29)))

(event EventPokeEvent
  (if (Variables|Default|GetGotten)
    (Variables|Default|SetRandoPitch (Math|Random|RandomFloatinRange 0.8 1.1))
    (else
      (Variables|Default|SetRandoPitch (Math|Random|RandomFloatinRange 1.2 1.45))
      (Input|DisableInput (Game|GetPlayerCharacter 0) (Game|GetPlayerController 0))))
  (Utilities|FlowControl|Sequence
    (:then_0
      (Utilities|FlowControl|Delay 0.02)
      (Audio|PlaySoundatLocation "/Game/Audio/SFX/Duck.Duck" (Transformation|GetActorLocation) "0, 0, 0" 0.825 (Variables|Default|GetRandoPitch) 0.0 "/Game/Audio/Attenuation/SA_ShortRange.SA_ShortRange" "/Game/Audio/Attenuation/SC_Default.SC_Default" 0)
      (bind _newtrack_0 (Timeline|Timeline_0 PlayFromStart)
        (:Update
          (Transformation|SetRelativeScale3D (Variables|Default|GetStaticMesh) (* _newtrack_0 0.125)))))
    (:then_1
      (Utilities|FlowControl|DoOnce false
        (:Completed
          (Variables|Default|SetGotten true)
          (Utilities|FlowControl|Sequence
            (:then_0
              (Components|Activation|Activate (Variables|Default|GetParticleSystem) false))
            (:then_1
              (Utilities|FlowControl|Delay 0.128)
              (Components|Activation|Deactivate (Variables|Default|GetParticleSystem))
              (Rendering|Components|TextRender|SetText (Variables|Default|GetNumberText) (Utilities|Text|ToText(Integer) (+ (Variables|/Game/Blueprints/GameObjects/BP_DuckTotem.BP_DuckTotem_C|GetFoundDucks (Variables|Default|GetTotem)) 1)))
              (Class|BPIActivate|Activate(Message) (Variables|Default|GetTotem) 0.0 false)
              (Audio|PlaySoundatLocation "/Game/Audio/SFX/LikeButtonOn.LikeButtonOn" (Transformation|GetActorLocation) "0, 0, 0" 0.08 1.4 0.1 "/Game/Audio/Attenuation/SA_ShortRange.SA_ShortRange" 0 0)
              (Components|Timeline|SetPlayRate (Variables|Default|GetTL_NumberAnim) 1.5)
              (Rendering|SetVisibility (Variables|Default|GetNumberText) false false)
              (Components|Timeline|PlayfromStart (Variables|Default|GetTL_NumberAnim))
              (Rendering|Material|SetMaterial (Variables|Default|GetStaticMesh) (Variables|Default|GetElement%20Index) (Variables|Default|GetSwitchToMat)))))))))

(fn ConstructionScript)

(fn Attachto
  (params (ChildActor :type Actor%20Object%20Reference))
  (return 0))

(fn CanGrab
  (return false))

(fn Clicked
  (return false))

(fn DisableCollision
  (return false))

(fn DoesParentHaveParent
  (return false))

(fn EnableCollision
  (return false))

(fn GetAttached
  (return 0))

(fn GetCustomCursor
  (return false 0))

(fn GetShrinkScale
  (return "0, 0, 0" "0, 0, 0"))

(fn GetSnapLoc
  (params (CursorLoc :type Vector :default "0, 0, 0"))
  (return "0, 0, 0" "0, 0, 0"))

(fn Grabbed
  (return 0))

(fn LetGo
  (params (ParentComponent :type Actor%20Component%20Object%20Reference) (ParentActor :type Actor%20Object%20Reference))
  (return false))

(fn OnHover
  (return false))

(fn PassChildAlong
  (return 0 0))

(fn RightClickEvent
  (return (Variables|Default|GetClick%20Message) (Transformation|GetActorLocation)))