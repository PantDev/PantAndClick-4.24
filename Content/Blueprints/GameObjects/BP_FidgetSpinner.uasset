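; BP_FidgetSpinner is a pokeable fidget spinner toy.
; Each poke plays a random click, runs a scale bounce timeline and adds a speed boost that grows as it spins faster.
; Tick rotates the spinner, decays and clamps its speed, and, with Hover on, eases the base to a height proportional to speed.
; Grab, click and attach interface functions are mostly empty stubs.
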(event EventTick
  (params (DeltaSeconds :type Float%20%28single-precision%29))
  (if (> (Variables|Default|GetSpeed) 0.0)
    (Transformation|AddLocalRotation (Variables|Default|GetSpinner) (Math|Rotator|MakeRotator 0.0 0.0 (* DeltaSeconds (Variables|Default|GetSpeed))) false false))
  (Variables|Default|SetSpeed (Math|Float|Clamp(Float) (- (Variables|Default|GetSpeed) (* (Variables|Default|GetDecRate) DeltaSeconds)) 0.0 1e+03))
  (if (Variables|Default|GetHover)
    (Transformation|SetRelativeLocation (Variables|Default|GetBase) (Math|Interpolation|VInterpTo (.Location (Math|Transform|BreakTransform (Transformation|GetRelativeTransform (Variables|Default|GetBase)))) (Math|Vector|MakeVector 0.0 0.0 (Math|Float|Lerp 0.0 (Variables|Default|GetHoverHeight) (/ (Math|Float|Clamp(Float) (- (Variables|Default|GetSpeed) (* (Variables|Default|GetDecRate) DeltaSeconds)) 0.0 1e+03) 1e+03))) (Utilities|Time|GetWorldDeltaSeconds) 2.0) false false)))

(event EventPokeEvent
  (Audio|PlaySoundatLocation (Utilities|Select :Index (Math|Random|RandomIntegerinRange 0 2) :Option%200 "/Game/Audio/SFX/ClickMusicSFX/Click1.Click1" :Option%201 "/Game/Audio/SFX/ClickMusicSFX/Click2.Click2" :Option%202 "/Game/Audio/SFX/ClickMusicSFX/Click3.Click3") (Transformation|GetActorLocation) "0, 0, 0" 0.6 1.0 0.25 "/Game/Audio/Attenuation/SA_ShortRange.SA_ShortRange" "/Game/Audio/Attenuation/SC_Default.SC_Default" 0)
  (Variables|Default|SetSpeed (Math|Float|Clamp(Float) (+ (Variables|Default|GetSpeed) (Math|Float|Lerp 1e+02 2.3e+02 (/ (Variables|Default|GetSpeed) 1.4e+03))) 25.0 1.4e+03))
  (bind _newtrack_0 (Timeline|TL_BounceAnim PlayFromStart)
    (:Update
      (Transformation|SetRelativeScale3D (Variables|Default|GetBase) (Math|Vector|MakeVector (+ (.X (Math|Vector|BreakVector _newtrack_0)) 3.0) (+ (.Y (Math|Vector|BreakVector _newtrack_0)) 3.0) (+ (.Z (Math|Vector|BreakVector _newtrack_0)) 3.0))))))

(fn ConstructionScript)

(fn Attachto
  (params (ChildActor :type Actor%20Object%20Reference))
  (return 0))

(fn CanGrab
  (return false))

(fn Clicked
  (return false))

(fn DisableCollision
  (return false))

(fn DoesParentHaveParent
  (return false))

(fn EnableCollision
  (return false))

(fn GetAttached
  (return 0))

(fn GetCustomCursor
  (return false 0))

(fn GetShrinkScale
  (return "0, 0, 0" "0, 0, 0"))

(fn GetSnapLoc
  (params (CursorLoc :type Vector :default "0, 0, 0"))
  (return "0, 0, 0" "0, 0, 0"))

(fn Grabbed
  (return 0))

(fn LetGo
  (params (ParentComponent :type Actor%20Component%20Object%20Reference) (ParentActor :type Actor%20Object%20Reference))
  (return false))

(fn OnHover
  (return false))

(fn PassChildAlong
  (return 0 0))

(fn RightClickEvent
  (return (Variables|Default|GetClick%20Message) (Transformation|GetActorLocation)))