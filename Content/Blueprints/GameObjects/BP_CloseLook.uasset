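; BP_CloseLook is a pokeable object that opens a close-look overlay showing its own text and texture.
; PokeEvent hides its mesh and the cursor, hides and pauses BP_PantController's speech bubble, plays a sound, then fills and animates CloseLookWidget.
; The Active flag and Activate event toggle the sphere's collision, and construction applies the mesh material.
; Other interaction functions are empty stubs, and nothing here closes the view.
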(event EventPokeEvent
  (bind _asbp_pant_controller (Utilities|Casting|CastToBP_PantController (Game|GetPlayerCharacter 0)))
  (if (Widget|IsVisible (Variables|/Game/PantControllerBP/Blueprints/BP_PantController.BP_PantController_C|GetSpeechBubbleWidget _asbp_pant_controller))
    (Widget|SetVisibility (Variables|/Game/PantControllerBP/Blueprints/BP_PantController.BP_PantController_C|GetSpeechBubbleWidget _asbp_pant_controller) "Hidden")
    (Variables|Default|SetWasPlayingSpeech true)
    (else
      (Variables|Default|SetWasPlayingSpeech false)))
  (Components|Timeline|SetPlayRate (Variables|/Game/PantControllerBP/Blueprints/BP_PantController.BP_PantController_C|GetTL_SpeechBubbleStay _asbp_pant_controller) 0.0)
  (Audio|PlaySoundatLocation (Variables|Default|GetSFX) (Transformation|GetActorLocation) "0, 0, 0" 1.0 0.5 0.01 "/Game/Audio/Attenuation/SA_ShortRange.SA_ShortRange" "/Game/Audio/Attenuation/SC_Default.SC_Default" 0)
  (Rendering|SetVisibility (Variables|/Game/PantControllerBP/Blueprints/BP_PantController.BP_PantController_C|GetActiveCursorMesh _asbp_pant_controller) false false)
  (Widget|SetVisibility (Variables|/Game/PantControllerBP/Blueprints/BP_PantController.BP_PantController_C|GetCloseLookWidget _asbp_pant_controller) "Visible")
  (Rendering|SetVisibility (Variables|Default|GetStaticMesh) false false)
  (bind _asbp_pant_controller_2 (Utilities|Casting|CastToBP_PantController (Game|GetPlayerCharacter 0)))
  (Rendering|Components|TextRender|SetText (Variables|/Game/UserInterface/CloseLook_Widget.CloseLook_Widget_C|GetTextBlock_0 (Variables|/Game/PantControllerBP/Blueprints/BP_PantController.BP_PantController_C|GetCloseLookWidget _asbp_pant_controller_2)) (Variables|Default|GetDisplay%20text))
  (Appearance|SetBrushfromTexture (Variables|/Game/UserInterface/CloseLook_Widget.CloseLook_Widget_C|GetImage_107 (Variables|/Game/PantControllerBP/Blueprints/BP_PantController.BP_PantController_C|GetCloseLookWidget _asbp_pant_controller_2)) (Variables|Default|GetTexture) false)
  (UserInterface|Animation|PlayAnimation (Variables|/Game/PantControllerBP/Blueprints/BP_PantController.BP_PantController_C|GetCloseLookWidget _asbp_pant_controller_2) (Variables|/Game/UserInterface/CloseLook_Widget.CloseLook_Widget_C|GetBlurOnAnim (Variables|/Game/PantControllerBP/Blueprints/BP_PantController.BP_PantController_C|GetCloseLookWidget _asbp_pant_controller_2)) 0.0 1 "Forward" 1.0 false)
  (UserInterface|Animation|PlayAnimation (Variables|/Game/PantControllerBP/Blueprints/BP_PantController.BP_PantController_C|GetCloseLookWidget _asbp_pant_controller_2) (Variables|/Game/UserInterface/CloseLook_Widget.CloseLook_Widget_C|GetBounceAnim (Variables|/Game/PantControllerBP/Blueprints/BP_PantController.BP_PantController_C|GetCloseLookWidget _asbp_pant_controller_2)) 0.0 1 "Forward" 1.5 false))

(event EventActivate
  (params (Delay :type Float%20%28single-precision%29) (Bool :type Boolean))
  (bind _sphere (Variables|Default|GetSphere))
  (if Bool
    (Collision|SetCollisionEnabled _sphere "QueryAndPhysics")
    (else
      (Collision|SetCollisionEnabled _sphere "NoCollision"))))

(event EventBeginPlay
  (bind _sphere (Variables|Default|GetSphere))
  (if (Variables|Default|GetActive)
    (Collision|SetCollisionEnabled _sphere "QueryOnly")
    (else
      (Collision|SetCollisionEnabled _sphere "NoCollision"))))

(fn ConstructionScript
  (Rendering|Material|SetMaterial (Variables|Default|GetStaticMesh) 0 (Variables|Default|GetMaterial)))

(fn Attachto
  (params (ChildActor :type Actor%20Object%20Reference))
  (return 0))

(fn CanGrab
  (return false))

(fn Clicked
  (return false))

(fn DisableCollision
  (return false))

(fn DoesParentHaveParent
  (return false))

(fn EnableCollision
  (return false))

(fn GetAttached
  (return 0))

(fn GetCustomCursor
  (return false 0))

(fn GetShrinkScale
  (return "0, 0, 0" "0, 0, 0"))

(fn GetSnapLoc
  (params (CursorLoc :type Vector :default "0, 0, 0"))
  (return "0, 0, 0" "0, 0, 0"))

(fn Grabbed
  (return 0))

(fn IsBusy
  (return false))

(fn LetGo
  (params (ParentComponent :type Actor%20Component%20Object%20Reference) (ParentActor :type Actor%20Object%20Reference))
  (return false))

(fn OnHover
  (return false))

(fn PassChildAlong
  (return 0 0))