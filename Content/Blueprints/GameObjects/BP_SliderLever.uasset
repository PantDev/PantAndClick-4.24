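; Grabbable slider lever on a spline that turns up to two rotator actors and switches a sign actor's icon.
; While held or sliding, Tick converts the closest spline distance to an alpha driving rotations and the segment-based, offset icon.
; On release, it finds the nearest evenly spaced segment point and starts a slide-to-nearest timeline, or plays a stop sound if already there.
; A looping timer started on click fades slide audio with movement.
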(event EventBeginPlay
  (bind _signactor (Variables|Default|GetSignActor))
  (Utilities|IsValid _signactor
    (:Is%20Valid
      (Default|SetMat _signactor (Variables|Default|GetStartIcon))
      (Default|CustomStart _signactor (Variables|Default|GetValue)))))

(event Collision|EventActorBeginOverlap
  (params (OtherActor :type Actor%20Object%20Reference)))

(event EventTick
  (params (DeltaSeconds :type Float%20%28single-precision%29))
  (bind _rotatoractor2 (Variables|Default|GetRotatorActor2))
  (bind _splineactor (Variables|Default|GetSplineActor))
  (bind _spline (Variables|/Game/Blueprints/GameObjects/BP_PathSpline.BP_PathSpline_C|GetSpline _splineactor))
  (if (and (or (Variables|Default|GetHeld) (Audio|Components|Audio|IsPlaying (Variables|Default|GetTL_SlideToNearest))) (Utilities|IsValid (Variables|Default|GetRotatorActor)))
    (bind _distance (CallFunction|FindDistanceAlongSplineClosesttoWorldLocation (Transformation|GetActorLocation) _spline))
    (bind _output_get (Variables|Default|SetCurrentAlpha (/ _distance (Spline|GetSplineLength _spline))))
    (Transformation|SetRelativeRotation (Variables|/Game/Blueprints/GameObjects/BP_SliderRotator.BP_SliderRotator_C|GetStaticMesh (Variables|Default|GetRotatorActor)) (Math|Rotator|Lerp(Rotator) "0, 0, 0" "0,360.000000, 0" _output_get) false false)
    (Default|SetMat (Variables|Default|GetSignActor) (Utilities|Select :Index (Math|Integer|%(Integer) (+ (Math|Float|Round (* (Variables|Default|GetCurrentAlpha) (Math|Conversions|ToFloat(Integer) (Variables|Default|GetSegments)))) (Variables|Default|GetOffset)) (Variables|Default|GetSegments)) :Option%200 "NewEnumerator0" :Option%201 "NewEnumerator1" :Option%202 "NewEnumerator2" :Option%203 "NewEnumerator4"))
    (if (Utilities|IsValid _rotatoractor2)
      (Transformation|SetRelativeRotation (Variables|/Game/Blueprints/GameObjects/BP_SliderRotator.BP_SliderRotator_C|GetStaticMesh _rotatoractor2) (Math|Rotator|Lerp(Rotator) "0, 0, 0" "0,4320.000000, 0" _output_get) false false))))

(event EventGetLetGo
  (bind _splineactor (Variables|Default|GetSplineActor))
  (bind _spline (Variables|/Game/Blueprints/GameObjects/BP_PathSpline.BP_PathSpline_C|GetSpline _splineactor))
  (if (> (Variables|Default|GetSegments) 0)
    (Variables|Default|SetStartSlideLoc (Transformation|GetActorLocation))
    (for _index (range 0 (Variables|Default|GetSegments))
      (if (== _index 0)
        (Variables|Default|SetEndSlideLoc (Spline|GetLocationatDistanceAlongSpline _spline 0.0 "World"))
        (elif (< (Math|Float|Absolute(Float) (Math|Vector|VectorLength (- (Spline|GetLocationatDistanceAlongSpline _spline (* (Math|Conversions|ToFloat(Integer) _index) (/ (Spline|GetSplineLength _spline) (Math|Conversions|ToFloat(Integer) (Variables|Default|GetSegments)))) "World") (Transformation|GetActorLocation)))) (Math|Float|Absolute(Float) (Math|Vector|VectorLength (- (Transformation|GetActorLocation) (Variables|Default|GetEndSlideLoc)))))
          (Variables|Default|SetEndSlideLoc (Spline|GetLocationatDistanceAlongSpline _spline (* (Math|Conversions|ToFloat(Integer) _index) (/ (Spline|GetSplineLength _spline) (Math|Conversions|ToFloat(Integer) (Variables|Default|GetSegments)))) "World")))))
    (if (> (Math|Vector|VectorLength (- (Variables|Default|GetStartSlideLoc) (Variables|Default|GetEndSlideLoc))) 0.0)
      (Components|Timeline|PlayfromStart (Variables|Default|GetTL_SlideToNearest))
      (else
        (Audio|PlaySoundatLocation "/Game/Audio/SFX/SliderStop1.SliderStop1" (Transformation|GetActorLocation) "0, 0, 0" 0.6 (Math|Random|RandomFloatinRange 1.1 1.15) 0.0 "/Game/Audio/Attenuation/SA_Default.SA_Default" "/Game/Audio/Attenuation/SC_Default.SC_Default" 0)))))

(fn ConstructionScript
  (bind _self self)
  (bind _rotatoractor (Variables|Default|GetRotatorActor))
  (bind _rotatoractor2 (Variables|Default|GetRotatorActor2))
  (Variables|Default|SetOriginalScale (Transformation|GetActorScale3D))
  (Utilities|IsValid _rotatoractor
    (:Is%20Valid
      (Variables|/Game/Blueprints/GameObjects/BP_SliderRotator.BP_SliderRotator_C|SetSliderActor _rotatoractor _self))
    (:Is%20Not%20Valid
      _))
  (Utilities|IsValid _rotatoractor2
    (:Is%20Valid
      (Variables|/Game/Blueprints/GameObjects/BP_SliderRotator.BP_SliderRotator_C|SetSliderActor _rotatoractor2 _self))))

(fn SoundTick
  (if (> (Math|Vector|VectorLength (- (Variables|Default|GetLastLoc) (Transformation|GetActorLocation))) 0.0)
    (if (Audio|Components|Audio|IsPlaying (Variables|Default|GetTL_SlideToNearest))
      (Components|Activation|Activate (Variables|Default|GetSliderFX1) false)
      (Components|Activation|Deactivate (Variables|Default|GetSliderFX))
      (else
        (Audio|Components|Audio|AdjustVolume (Variables|Default|GetSliderFX) 0.225 1.0 "SCurve" :!class /Script/Engine.AudioComponent)))
    (else
      (Audio|Components|Audio|AdjustVolume (Variables|Default|GetSliderFX) 0.1 0.0 "SCurve" :!class /Script/Engine.AudioComponent)
      (Components|Activation|Deactivate (Variables|Default|GetSliderFX1))))
  (Variables|Default|SetLastLoc (Transformation|GetActorLocation)))

(fn FindDistanceAlongSplineClosesttoWorldLocation
  (params (Location :type Vector) (Spline :type Spline%20Component%20Object%20Reference))
  (bind _returnvalue (Class|SplineComponent|FindInputKeyClosesttoWorldLocation Spline Location))
  (bind _returnvalue_2 (Math|Float|Truncate _returnvalue))
  (bind _returnvalue_3 (Spline|GetDistanceAlongSplineatSplinePoint Spline _returnvalue_2))
  (return (+ _returnvalue_3 (* (- (Spline|GetDistanceAlongSplineatSplinePoint Spline (Math|Float|Truncate (+ _returnvalue 1.0))) _returnvalue_3) (- _returnvalue (Math|Conversions|ToFloat(Integer) _returnvalue_2))))))

(fn Attachto
  (params (ChildActor :type Actor%20Object%20Reference))
  (return (Utilities|Array|MakeArray 0)))

(fn CanGrab
  (return true))

(fn Clicked
  (Variables|Default|SetHeld true)
  (Audio|Components|Audio|Stop (Variables|Default|GetTL_SlideToNearest))
  (Utilities|Time|SetTimerbyFunctionName 0 "SoundTick" 0.035556 true)
  (Components|Activation|Activate (Variables|Default|GetSliderFX) false)
  (return false))

(fn DisableCollision
  (return false))

(fn DoesParentHaveParent
  (return false))

(fn EnableCollision
  (return false))

(fn GetAttached
  (return (Utilities|Array|MakeArray 0)))

(fn GetBreakDistance
  (return (Variables|Default|GetBreak%20Distance)))

(fn GetCustomCursor
  (return false 0))

(fn GetPathSpline
  (return (Variables|Default|GetSplineActor)))

(fn GetShrinkScale
  (return (Variables|Default|GetShrinkScale) (Variables|Default|GetOriginalScale)))

(fn GetSnapLoc
  (params (CursorLoc :type Vector :default "0, 0, 0"))
  (return "0, 0, 0" "0, 0, 0"))

(fn Grabbed
  (return 0))

(fn LetGo
  (params (ParentComponent :type Actor%20Component%20Object%20Reference) (ParentActor :type Actor%20Object%20Reference))
  (Variables|Default|SetHeld false)
  (return false))

(fn OnHover
  (return false))

(fn PassChildAlong
  (return 0 0))