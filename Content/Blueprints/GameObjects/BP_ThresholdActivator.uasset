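; BP_ThresholdActivator is a counter gate that opens a linked button's gate when activations reach a target threshold.
; One second after BeginPlay, the count is set to Offset.
; Activate(true) increments the count and sets GateOpen on ButtonToUngate only upon stepping exactly onto TargetThreshold.
; Activate(false) decrements the count, clamped between zero and the threshold, and always closes the gate; IsBusy always returns false.
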(event EventBeginPlay
  (Utilities|FlowControl|Delay 1.0)
  (Variables|Default|SetCurrentValue (Variables|Default|GetOffset)))

(event Collision|EventActorBeginOverlap
  (params (OtherActor :type Actor%20Object%20Reference)))

(event EventActivate
  (params (Delay :type Float%20%28single-precision%29) (Bool :type Boolean))
  (bind _targetthreshold (Variables|Default|GetTargetThreshold))
  (bind _buttontoungate (Variables|Default|GetButtonToUngate))
  (bind _buttontoungate_2 (Variables|Default|GetButtonToUngate))
  (if Bool
    (if (== (Variables|Default|GetCurrentValue) (- _targetthreshold 1.0))
      (Variables|Default|SetCurrentValue (Variables|Default|GetTargetThreshold))
      (Utilities|IsValid _buttontoungate_2
        (:Is%20Valid
          (Variables|/Game/Blueprints/GameObjects/BP_ButtonSwitch.BP_ButtonSwitch_C|SetGateOpen _buttontoungate_2 true)))
      (else
        (Variables|Default|SetCurrentValue (+ (Variables|Default|GetCurrentValue) 1.0))))
    (else
      (Variables|Default|SetCurrentValue (Math|Float|Clamp(Float) (- (Variables|Default|GetCurrentValue) 1.0) 0.0 _targetthreshold))
      (Utilities|IsValid _buttontoungate
        (:Is%20Valid
          (Variables|/Game/Blueprints/GameObjects/BP_ButtonSwitch.BP_ButtonSwitch_C|SetGateOpen _buttontoungate false))))))

(fn ConstructionScript)

(fn IsBusy
  (return false))