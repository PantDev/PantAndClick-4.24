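; BP_MazeWalls is a maze wall actor that grows vertically when activated.
; Activate plays the TL_SquishWall timeline from the start, lerping the root component's world Z scale from 0 to 1.
; IsBusy always returns false, so it never reports busy during the animation.
; A delayed forward/reverse loop on the timeline is left unconnected, so the wall does not lower itself again.
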(event EventBeginPlay)

(event Collision|EventActorBeginOverlap
  (params (OtherActor :type Actor%20Object%20Reference)))

(event EventTick
  (params (DeltaSeconds :type Float%20%28single-precision%29)))

(event EventActivate
  (params (Delay :type Float%20%28single-precision%29) (Bool :type Boolean))
  (bind (_direction _alpha) (Timeline|TL_SquishWall PlayFromStart)
    (:Update
      (Transformation|SetWorldScale3D (Variables|Default|GetDefaultSceneRoot) (Math|Vector|MakeVector 1.0 1.0 (Math|Float|Lerp 0.0 1.0 _alpha))))))

(fn ConstructionScript)

(fn IsBusy
  (return false))