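; Helper actor that animates one indexed sticky on the book's skeletal mesh by driving its "S" and "L" morph targets, whose names are built from the index.
; Forward plays a transition timeline from a given position with a glitch sound, then hands off to a loop timeline; reverse stops the loop and plays the transition backward.
; A newly-collected event presets the "L" morph, then animates it with sound after an index-staggered delay.
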(event Custom|EventDriverForward
  (params (NewPosition :type Float%20%28single-precision%29))
  (bind _bookbp (Variables|Default|GetBookBP))
  (bind _bookbp_2 (Variables|Default|GetBookBP))
  (bind _int (Variables|Default|GetInt))
  (bind _int_2 (Variables|Default|GetInt))
  (bind _returnvalue (Utilities|String|ToString(Integer) _int))
  (bind _returnvalue_2 (Utilities|String|ToString(Integer) _int_2))
  (bind _bookskeletalmesh (Variables|/Game/Blueprints/GameObjects/BP_Book.BP_Book_C|GetBookSkeletalMesh _bookbp))
  (bind _bookskeletalmesh_2 (Variables|/Game/Blueprints/GameObjects/BP_Book.BP_Book_C|GetBookSkeletalMesh _bookbp_2))
  (Variables|Default|SetTags self (Utilities|Array|MakeArray (Utilities|String|StringToName (Utilities|String|ToString(Integer) (Variables|Default|GetInt)))))
  (Components|Timeline|SetPlaybackPosition (Variables|Default|GetTL_DriverAnim) NewPosition false true)
  (Audio|PlaySoundatLocation "/Game/Audio/SFX/GlitchHiccup.GlitchHiccup" (Transformation|GetActorLocation) "0, 0, 0" 0.6 (Math|Random|RandomFloatinRange 1.1 1.6) 0.025 "/Game/Audio/Attenuation/SA_ShortRange.SA_ShortRange" "/Game/Audio/Attenuation/SC_Default.SC_Default" 0)
  (Audio|Components|Audio|Stop (Variables|Default|GetTL_DriverLoop))
  (bind (_direction _alpha _alpha2) (Timeline|TL_DriverAnim Play)
    (:Update
      (Components|SkeletalMesh|SetMorphTarget _bookskeletalmesh_2 (Utilities|String|StringToName (Utilities|String|Append "S" _returnvalue_2)) _alpha true)
      (Components|SkeletalMesh|SetMorphTarget _bookskeletalmesh_2 (Utilities|String|StringToName (Utilities|String|Append "L" _returnvalue_2)) _alpha2 true))
    (:Finished
      (switch Utilities|FlowControl|Switch|SwitchonETimelineDirection _direction
        (:Forward
          (bind (_direction_2 _alpha_2 _alpha2_2) (Timeline|TL_DriverLoop PlayFromStart)
            (:Update
              (Components|SkeletalMesh|SetMorphTarget _bookskeletalmesh (Utilities|String|StringToName (Utilities|String|Append "S" _returnvalue)) _alpha_2 true)
              (Components|SkeletalMesh|SetMorphTarget _bookskeletalmesh (Utilities|String|StringToName (Utilities|String|Append "L" _returnvalue)) _alpha2_2 true))))))))

(event Custom|EventDriverReverse
  (bind _bookbp (Variables|Default|GetBookBP))
  (bind _bookbp_2 (Variables|Default|GetBookBP))
  (bind _int (Variables|Default|GetInt))
  (bind _int_2 (Variables|Default|GetInt))
  (bind _returnvalue (Utilities|String|ToString(Integer) _int))
  (bind _returnvalue_2 (Utilities|String|ToString(Integer) _int_2))
  (bind _bookskeletalmesh (Variables|/Game/Blueprints/GameObjects/BP_Book.BP_Book_C|GetBookSkeletalMesh _bookbp))
  (bind _bookskeletalmesh_2 (Variables|/Game/Blueprints/GameObjects/BP_Book.BP_Book_C|GetBookSkeletalMesh _bookbp_2))
  (Audio|Components|Audio|Stop (Variables|Default|GetTL_DriverLoop))
  (bind (_direction _alpha _alpha2) (Timeline|TL_DriverAnim Reverse)
    (:Update
      (Components|SkeletalMesh|SetMorphTarget _bookskeletalmesh_2 (Utilities|String|StringToName (Utilities|String|Append "S" _returnvalue_2)) _alpha true)
      (Components|SkeletalMesh|SetMorphTarget _bookskeletalmesh_2 (Utilities|String|StringToName (Utilities|String|Append "L" _returnvalue_2)) _alpha2 true))
    (:Finished
      (switch Utilities|FlowControl|Switch|SwitchonETimelineDirection _direction
        (:Forward
          (bind (_direction_2 _alpha_2 _alpha2_2) (Timeline|TL_DriverLoop PlayFromStart)
            (:Update
              (Components|SkeletalMesh|SetMorphTarget _bookskeletalmesh (Utilities|String|StringToName (Utilities|String|Append "S" _returnvalue)) _alpha_2 true)
              (Components|SkeletalMesh|SetMorphTarget _bookskeletalmesh (Utilities|String|StringToName (Utilities|String|Append "L" _returnvalue)) _alpha2_2 true))))))))

(event Custom|EventNewlyCollected
  (params (DelayInt :type Integer))
  (Variables|Default|SetTags self (Utilities|Array|MakeArray (Utilities|String|StringToName (Utilities|String|ToString(Integer) (Variables|Default|GetInt)))))
  (Components|SkeletalMesh|SetMorphTarget (Variables|/Game/Blueprints/GameObjects/BP_Book.BP_Book_C|GetBookSkeletalMesh (Variables|Default|GetBookBP)) (Utilities|String|StringToName (Utilities|String|Append "L" (Utilities|String|ToString(Integer) (Variables|Default|GetInt)))) -0.03 true)
  (Utilities|FlowControl|Delay (+ 0.5 (* (Math|Conversions|ToFloat(Integer) DelayInt) 0.08)))
  (bind _alpha (Timeline|TL_NewlyCollected PlayFromStart)
    (:Update
      (Components|SkeletalMesh|SetMorphTarget (Variables|/Game/Blueprints/GameObjects/BP_Book.BP_Book_C|GetBookSkeletalMesh (Variables|Default|GetBookBP)) (Utilities|String|StringToName (Utilities|String|Append "L" (Utilities|String|ToString(Integer) (Variables|Default|GetInt)))) _alpha true))
    (:SFX
      (Audio|PlaySoundatLocation "/Game/Audio/SFX/Random_58.Random_58" (Transformation|GetActorLocation) "0, 0, 0" 0.15 (Math|Random|RandomFloatinRange 1.4 2.0) 0.17 "/Game/Audio/Attenuation/SA_ShortRange.SA_ShortRange" "/Game/Audio/Attenuation/SC_Default.SC_Default" 0))))

(fn ConstructionScript)