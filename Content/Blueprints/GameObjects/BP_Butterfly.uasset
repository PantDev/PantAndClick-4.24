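; BP_Butterfly is an ambient butterfly that flies away when BP_PantController overlaps it.
; It starts its animation at a random position, and on overlap disables its sphere collision and picks a random distant point above it.
; A timeline lerps it from the transform cached in the construction script toward that point, turning it and speeding up its animation, then destroys it.
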(event EventBeginPlay
  (Components|Animation|SetPosition (Variables|Default|GetButterflyAnim1) (Math|Random|RandomFloat) true))

(event Collision|EventActorBeginOverlap
  (params (OtherActor :type Actor%20Object%20Reference))
  (bind _originloc (Variables|Default|GetOriginLoc))
  (if (== (Utilities|GetClass OtherActor) "/Game/PantControllerBP/Blueprints/BP_PantController.BP_PantController_C")
    (Collision|SetCollisionEnabled (Variables|Default|GetSphere) "NoCollision")
    (Variables|Default|SetFlyLoc (+ (Transformation|GetWorldLocation (Variables|Default|GetDefaultSceneRoot)) (Math|Vector|MakeVector (Math|Random|RandomFloatinRange -1e+04 1e+04) (Math|Random|RandomFloatinRange -1e+04 1e+04) (Math|Random|RandomFloatinRange 2e+03 8e+03))))
    (Components|Timeline|SetPlayRate (Variables|Default|GetTL_Fly) 1.0)
    (bind (_direction _flyalpha _rotalpha) (Timeline|TL_Fly PlayFromStart)
      (:Update
        (Transformation|SetActorRotation (Math|Rotator|Lerp(Rotator) (Variables|Default|GetOriginRot) (Math|Rotator|FindLookatRotation _originloc (Variables|Default|GetFlyLoc)) _rotalpha true))
        (Transformation|SetActorLocation (Math|Vector|Lerp(Vector) _originloc (Variables|Default|GetFlyLoc) _flyalpha) false false)
        (Components|Timeline|SetPlayRate (Variables|Default|GetButterflyAnim1) (Math|Float|Lerp 1.0 2.5 _rotalpha)))
      (:Finished
        (Actor|DestroyActor)))))

(event EventTick
  (params (DeltaSeconds :type Float%20%28single-precision%29)))

(fn ConstructionScript
  (Variables|Default|SetOriginLoc (Transformation|GetActorLocation))
  (Variables|Default|SetOriginRot (Transformation|GetActorRotation)))