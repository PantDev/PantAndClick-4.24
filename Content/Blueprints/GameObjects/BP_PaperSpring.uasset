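; BP_PaperSpring is a paper spring bounce pad that supplies a launch velocity aimed at its Arrow component, scaled by Velocity.Z.
; Requesting that velocity, poking or letting go triggers a bounce: particles, random-pitch sound and a timeline-driven mesh scale.
; The construction script optionally snaps it to the ground once, picks static or skeletal mesh and tints the static mesh.
; Most interaction functions are stubs, so it cannot be grabbed.
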(event Custom|Event_AnimBounce
  (bind _particlesystem (Variables|Default|GetParticleSystem))
  (Audio|Components|Audio|Stop (Variables|Default|GetTL_Bounce))
  (Components|Activation|Deactivate _particlesystem)
  (Components|Activation|Activate _particlesystem false)
  (Audio|PlaySoundatLocation "/Game/Audio/SFX/Bounce.Bounce" (Transformation|GetActorLocation) "0, 0, 0" 1.0 (Math|Random|RandomFloatinRange 0.8 1.2) 0.0 "/Game/Audio/Attenuation/SA_Default.SA_Default" "/Game/Audio/Attenuation/SC_Default.SC_Default" 0)
  (bind _meshscale3d (Timeline|TL_Bounce PlayFromStart)
    (:Update
      (Transformation|SetRelativeScale3D (Variables|Default|GetSkeletalMesh) _meshscale3d))
    (:Finished
      (Components|Activation|Deactivate (Variables|Default|GetParticleSystem)))))

(event Custom|LetGoEvent
  (Components|Activation|Activate (Variables|Default|GetParticleSystem) false)
  (Audio|PlaySoundatLocation "/Game/Audio/SFX/Bounce.Bounce" (Transformation|GetActorLocation) "0, 0, 0" 1.0 (Math|Random|RandomFloatinRange 0.8 1.2) 0.0 "/Game/Audio/Attenuation/SA_Default.SA_Default" "/Game/Audio/Attenuation/SC_Default.SC_Default" 0)
  (bind _meshscale3d (Timeline|TL_Bounce PlayFromStart)
    (:Update
      (Transformation|SetRelativeScale3D (Variables|Default|GetSkeletalMesh) _meshscale3d))
    (:Finished
      (Components|Activation|Deactivate (Variables|Default|GetParticleSystem)))))

(event EventPokeEvent
  (CallFunction|EventAnimBounce))

(event EventTick
  (params (DeltaSeconds :type Float%20%28single-precision%29)))

(fn ConstructionScript
  (bind _returnvalue (Transformation|GetActorLocation))
  (bind _staticmesh (Variables|Default|GetStaticMesh))
  (bind (_x _y _z) (Math|Vector|BreakVector _returnvalue))
  (Variables|Default|SetOriginalScale (Transformation|GetActorScale3D))
  (if (Variables|Default|GetPlantOnGround)
    (Variables|Default|SetPlantOnGround false)
    (bind _outhit (Collision|LineTraceByChannel _returnvalue (Math|Vector|MakeVector _x _y (- _z 1e+04)) "TraceTypeQuery1" false 0 "None"))
    (Transformation|SetActorLocation (.Location (Collision|BreakHitResult _outhit)) false false))
  (Transformation|SetActorScale3D (Variables|Default|GetMeshScale))
  (Components|StaticMesh|SetStaticMesh _staticmesh (Variables|Default|GetStatic))
  (Class|SkinnedMeshComponent|SetSkeletalMesh (Variables|Default|GetSkeletalMesh) (Variables|Default|GetSkeletal) true)
  (Rendering|Material|SetMaterial _staticmesh 0 0)
  (Rendering|Material|SetMaterial _staticmesh 1 0)
  (Rendering|Material|SetMaterial _staticmesh 2 0)
  (Rendering|Material|SetMaterial _staticmesh 3 0)
  (bind _returnvalue_2 (Rendering|Material|CreateDynamicMaterialInstance "/Game/Materials/PaperSpring_Mat.PaperSpring_Mat" "None" "None" :!class /Script/Engine.KismetMaterialLibrary))
  (bind _output_get (Variables|Default|SetMaterialInstance _returnvalue_2))
  (Rendering|Material|SetMaterial (Variables|Default|GetStaticMesh) 0 _output_get)
  (Rendering|Material|SetVectorParameterValue (Variables|Default|GetMaterialInstance) "Color" (Variables|Default|GetColor) :!class /Script/Engine.MaterialInstanceDynamic)
  (if (Variables|Default|GetUseSkeletal)
    (Rendering|SetVisibility (Variables|Default|GetSkeletalMesh) true false)
    (Rendering|SetVisibility (Variables|Default|GetStaticMesh) false false)
    (else
      (Rendering|SetVisibility (Variables|Default|GetStaticMesh) true false)
      (Rendering|SetVisibility (Variables|Default|GetSkeletalMesh) false false))))

(fn Attachto
  (params (ChildActor :type Actor%20Object%20Reference))
  (return (Utilities|Array|MakeArray 0)))

(fn CanGrab
  (return false))

(fn Clicked
  (return false))

(fn DisableCollision
  (return false))

(fn DoesParentHaveParent
  (return false))

(fn EnableCollision
  (return false))

(fn GetAttached
  (return (Utilities|Array|MakeArray 0)))

(fn GetCustomCursor
  (return false 0))

(fn GetLaunchVelocity
  (CallFunction|EventAnimBounce)
  (return (* (Math|Vector|GetUnitDirection(Vector) (Transformation|GetActorLocation) (Transformation|GetWorldLocation (Variables|Default|GetArrow))) (.Z (Math|Vector|BreakVector (Variables|Default|GetVelocity))))))

(fn GetShrinkScale
  (return (Variables|Default|GetShrinkScale) (Variables|Default|GetOriginalScale)))

(fn GetSnapLoc
  (params (CursorLoc :type Vector :default "0, 0, 0"))
  (return "0, 0, 0" "0, 0, 0"))

(fn Grabbed
  (return 0))

(fn LetGo
  (params (ParentComponent :type Actor%20Component%20Object%20Reference) (ParentActor :type Actor%20Object%20Reference))
  (CallFunction|LetGoEvent)
  (return false))

(fn OnHover
  (return false))

(fn PassChildAlong
  (return 0 0))