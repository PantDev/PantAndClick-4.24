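; Pokeable lever disguised as part of a chess set, which swings its arm and plays sounds.
; PokeEvent restarts a timeline that rotates ArmMesh and fires pitch-randomized sounds from event tracks, ignoring pokes early in playback.
; The first poke also sets ClickMessage to lines revealing the lever, which RightClickEvent returns with a focus location.
; The other interaction functions, such as grab and hover, are inert stubs.
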(event EventPokeEvent
  (bind _returnvalue (Transformation|GetActorLocation))
  (bind _returnvalue_2 (Math|Random|RandomFloatinRange 0.6 0.8))
  (bind _tl_leveranim (Variables|Default|GetTL_LeverAnim))
  (Utilities|FlowControl|Sequence
    (:then_0
      (Utilities|FlowControl|DoOnce false
        (:Completed
          (Variables|Default|SetClick%20Message (Utilities|Array|MakeArray "A lever!" "A cleverly disguised one too, 
if you ignore the hinge." "I don't think a standard 
chess set includes this.")))))
    (:then_1
      (if (Audio|Components|Audio|IsPlaying _tl_leveranim)
        (if (> (Components|Timeline|GetPlaybackPosition _tl_leveranim) 1.1)
          (Components|Timeline|SetPlayRate (Variables|Default|GetTL_LeverAnim) 1.0 :!label _label)
          (Audio|PlaySoundatLocation "/Game/Audio/SFX/CloseSpeech.CloseSpeech" (Transformation|GetActorLocation) "0, 0, 0" 0.4 (Math|Random|RandomFloatinRange 0.4 0.65) 0.18 "/Game/Audio/Attenuation/SA_ShortRange.SA_ShortRange" "/Game/Audio/Attenuation/SC_Default.SC_Default" 0)
          (bind _armrot (Timeline|TL_LeverAnim PlayFromStart)
            (:Update
              (Transformation|SetRelativeRotation (Variables|Default|GetArmMesh) (Math|Rotator|Lerp(Rotator) "0, 0, 0" "-90.000000, 0, 0" _armrot true) false false))
            (:NewTrack_1
              (Audio|PlaySoundatLocation "/Game/Audio/SFX/OpenSpeech.OpenSpeech" _returnvalue "0, 0, 0" 0.12 _returnvalue_2 0.08 "/Game/Audio/Attenuation/SA_ShortRange.SA_ShortRange" "/Game/Audio/Attenuation/SC_Default.SC_Default" 0)
              (Audio|PlaySoundatLocation "/Game/Audio/SFX/SliderStop1.SliderStop1" _returnvalue "0, 0, 0" 0.8 _returnvalue_2 0.0 "/Game/Audio/Attenuation/SA_Default.SA_Default" "/Game/Audio/Attenuation/SC_Default.SC_Default" 0))
            (:NewTrack_2
              (Audio|PlaySoundatLocation "/Game/Audio/SFX/SliderStop1.SliderStop1" "0, 0, 0" "0, 0, 0" 0.8 (Math|Random|RandomFloatinRange 0.8 1.2) 0.0 "/Game/Audio/Attenuation/SA_Default.SA_Default" "/Game/Audio/Attenuation/SC_Default.SC_Default" 0))
            (:NewTrack_3
              (Audio|PlaySoundatLocation "/Game/Audio/SFX/OpenSpeech.OpenSpeech" _returnvalue "0, 0, 0" 0.12 (Math|Random|RandomFloatinRange 0.95 1.05) 0.12 "/Game/Audio/Attenuation/SA_ShortRange.SA_ShortRange" "/Game/Audio/Attenuation/SC_Default.SC_Default" 0))))
        (else
          (goto _label))))))

(fn ConstructionScript)

(fn Attachto
  (params (ChildActor :type Actor%20Object%20Reference))
  (return 0))

(fn CanGrab
  (return false))

(fn Clicked
  (return false))

(fn DisableCollision
  (return false))

(fn DoesParentHaveParent
  (return false))

(fn EnableCollision
  (return false))

(fn GetAttached
  (return 0))

(fn GetCustomCursor
  (return false 0))

(fn GetShrinkScale
  (return "0, 0, 0" "0, 0, 0"))

(fn GetSnapLoc
  (params (CursorLoc :type Vector :default "0, 0, 0"))
  (return "0, 0, 0" "0, 0, 0"))

(fn Grabbed
  (return 0))

(fn LetGo
  (params (ParentComponent :type Actor%20Component%20Object%20Reference) (ParentActor :type Actor%20Object%20Reference))
  (return false))

(fn OnHover
  (return false))

(fn PassChildAlong
  (return 0 0))

(fn RightClickEvent
  (return (Variables|Default|GetClick%20Message) (Transformation|GetWorldLocation (Variables|Default|GetScene))))