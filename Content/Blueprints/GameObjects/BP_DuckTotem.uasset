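; Duck collection totem that counts activations up to eight, lighting a glowing marker for each with a scale-in and sound.
; Activate also freezes the player and blends to the totem camera, restoring control except after the eighth duck, which launches the Floppy.
; A one-shot reveal shows the spinning TinyDuck on first activation or player approach.
; Tick scales hologram audio volume by player distance and pitch by player speed.
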(event Custom|StartActivationEvent
  (bind _tl_onanim (Variables|Default|GetTL_OnAnim))
  (Utilities|FlowControl|DoOnce false
    (:Completed
      (Rendering|SetVisibility (Variables|Default|GetTinyDuck) true true)
      (Components|Timeline|SetPlayRate _tl_onanim 0.78)
      (Components|Timeline|PlayfromStart _tl_onanim)
      (Audio|PlaySoundatLocation "/Game/Audio/SFX/CheckPoint.CheckPoint" (Transformation|GetActorLocation) "0, 0, 0" 0.6 1.2 0.228 "/Game/Audio/Attenuation/SA_ShortRange.SA_ShortRange" 0 0))))

(event EventBeginPlay
  (bind _returnvalue (Rendering|Material|CreateDynamicMaterialInstance "/Game/Materials/Glow_Mat.Glow_Mat" "None" "None" :!class /Script/Engine.KismetMaterialLibrary))
  (Variables|Default|SetDynMat _returnvalue))

(event EventTick
  (params (DeltaSeconds :type Float%20%28single-precision%29))
  (bind _returnvalue (Game|GetPlayerCharacter 0))
  (bind _tl_onanim (Variables|Default|GetTL_OnAnim))
  (bind _hologlitch (Variables|Default|GetHoloGlitch))
  (Audio|Components|Audio|SetVolumeMultiplier _hologlitch (Math|Float|Lerp 0.0 2.0 (- 1.0 (/ (Math|Float|Clamp(Float) (Math|Vector|VectorLength (- (Transformation|GetWorldLocation _hologlitch) (Transformation|GetActorLocation _returnvalue))) 0.0 325.0) 325.0))) :!class /Script/Engine.AudioComponent)
  (Audio|Components|Audio|SetPitchMultiplier _hologlitch (Math|Float|Lerp 1.0 1.5 (/ (Math|Float|Clamp(Float) (Math|Vector|VectorLength (Transformation|GetVelocity _returnvalue)) 0.0 7.5e+02) 7.5e+02)))
  (Transformation|AddLocalRotation (Variables|Default|GetTinyDuck) (Math|Rotator|MakeRotator 0.0 0.0 (* DeltaSeconds 5e+01)) false false)
  (if (< (Math|Vector|VectorLength (- (Transformation|GetActorLocation (Game|GetPlayerCharacter 0)) (Transformation|GetActorLocation))) 6.5e+02)
    (Utilities|FlowControl|DoOnce false
      (:Completed
        (Rendering|SetVisibility (Variables|Default|GetTinyDuck) true true)
        (Components|Timeline|SetPlayRate _tl_onanim 0.78)
        (Components|Timeline|PlayfromStart _tl_onanim)
        (Audio|PlaySoundatLocation "/Game/Audio/SFX/CheckPoint.CheckPoint" (Transformation|GetActorLocation) "0, 0, 0" 0.6 1.2 0.228 "/Game/Audio/Attenuation/SA_ShortRange.SA_ShortRange" 0 0)))))

(event EventActivate
  (params (Delay :type Float%20%28single-precision%29) (Bool :type Boolean))
  (bind _returnvalue (Game|GetPlayerCharacter 0))
  (bind _returnvalue_2 (Game|GetPlayerCharacter 0))
  (bind _marker3 (Variables|Default|GetMarker3))
  (bind _marker4 (Variables|Default|GetMarker4))
  (bind _marker5 (Variables|Default|GetMarker5))
  (bind _marker6 (Variables|Default|GetMarker6))
  (bind _marker7 (Variables|Default|GetMarker7))
  (bind _marker8 (Variables|Default|GetMarker8))
  (bind _marker1 (Variables|Default|GetMarker1))
  (bind _dynmat (Variables|Default|GetDynMat))
  (bind _marker2 (Variables|Default|GetMarker2))
  (Utilities|FlowControl|Delay 0.5)
  (if (not (== (Variables|Default|GetFoundDucks) 8))
    (Utilities|FlowControl|Sequence
      (:then_0
        (Utilities|FlowControl|Delay 0.5)
        (if (== (Variables|Default|GetFoundDucks) 0)
          (CallFunction|StartActivationEvent)
          (Utilities|FlowControl|Delay 1.0))
        (Variables|Default|SetFoundDucks (+ (Variables|Default|GetFoundDucks) 1))
        (switch int (Variables|Default|GetFoundDucks)
          (:1
            (Rendering|Material|SetMaterial _marker1 1 _dynmat)
            (Rendering|Material|SetMaterial _marker1 0 _dynmat)
            (Variables|Default|SetMarker _marker1))
          (:2
            (Rendering|Material|SetMaterial _marker2 1 _dynmat)
            (Rendering|Material|SetMaterial _marker2 0 _dynmat)
            (Variables|Default|SetMarker _marker2))
          (:3
            (Rendering|Material|SetMaterial _marker3 1 _dynmat)
            (Rendering|Material|SetMaterial _marker3 0 _dynmat)
            (Variables|Default|SetMarker _marker3))
          (:4
            (Rendering|Material|SetMaterial _marker4 1 _dynmat)
            (Rendering|Material|SetMaterial _marker4 0 _dynmat)
            (Variables|Default|SetMarker _marker4))
          (:5
            (Rendering|Material|SetMaterial _marker5 1 _dynmat)
            (Rendering|Material|SetMaterial _marker5 0 _dynmat)
            (Variables|Default|SetMarker _marker5))
          (:6
            (Rendering|Material|SetMaterial _marker6 1 _dynmat)
            (Rendering|Material|SetMaterial _marker6 0 _dynmat)
            (Variables|Default|SetMarker _marker6))
          (:7
            (Rendering|Material|SetMaterial _marker7 1 _dynmat)
            (Rendering|Material|SetMaterial _marker7 0 _dynmat)
            (Variables|Default|SetMarker _marker7))
          (:8
            (Rendering|Material|SetMaterial _marker8 1 _dynmat)
            (Rendering|Material|SetMaterial _marker8 0 _dynmat)
            (Default|FlytoEvent (Variables|Default|GetFloppy))
            (Variables|Default|SetMarker _marker8)))
        (Components|Timeline|PlayfromStart (Variables|Default|GetTL_MarkerAnim))
        (Audio|PlaySoundatLocation "/Game/Audio/SFX/DuckGet.DuckGet" (Transformation|GetActorLocation) "0, 0, 0" 0.4 (Math|Random|RandomFloatinRange 0.95 1.05) 0.1 "/Game/Audio/Attenuation/SA_ShortRange.SA_ShortRange" 0 0))
      (:then_1
        (bind _asbp_pant_controller (Utilities|Casting|CastToBP_PantController (Game|GetPlayerCharacter 0))
          (:then
            (Utilities|IsValid (Variables|/Game/PantControllerBP/Blueprints/BP_PantController.BP_PantController_C|GetMagnifyActor _asbp_pant_controller)
              (:Is%20Valid
                (Variables|Default|SetMagnify%20Actor (Variables|/Game/PantControllerBP/Blueprints/BP_PantController.BP_PantController_C|GetMagnifyActor _asbp_pant_controller))
                (Default|SilentBackArrow _asbp_pant_controller))
              (:Is%20Not%20Valid
                _)))
          (:CastFailed
            _))
        (Variables|/Script/Engine.Actor|SetCustomTimeDilation _returnvalue_2 0.0)
        (Input|DisableInput _returnvalue_2 0)
        (Game|Player|SetViewTargetwithBlend (Game|GetPlayerController 0) (Variables|Default|GetCamera) 0.0 "VTBlend_EaseInOut" 2.5 false)
        (if (== (Variables|Default|GetFoundDucks) 0)
          (Utilities|FlowControl|Delay 2.8)
          (else
            (Utilities|FlowControl|Delay 1.5)))
        (if (not (== (Variables|Default|GetFoundDucks) 8))
          (Game|Player|SetViewTargetwithBlend (Game|GetPlayerController 0) (Game|GetPlayerCharacter 0) 0.0 "VTBlend_Linear" 2.5 false)
          (Utilities|FlowControl|Delay 0.5)
          (Variables|/Script/Engine.Actor|SetCustomTimeDilation _returnvalue 1.0)
          (Input|EnableInput _returnvalue (Game|GetPlayerController 0))
          (Utilities|IsValid (Variables|Default|GetMagnify%20Actor)
            (:Is%20Valid
              (Default|PokeEvent (Variables|/Game/Blueprints/GameObjects/MagnifyCamera.MagnifyCamera_C|GetMagVolume (Variables|Default|GetMagnify%20Actor)))
              (Variables|Default|SetMagnify%20Actor 0))))))))

(fn ConstructionScript)

(fn IsBusy
  (return false))