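; BP_ComboLock_Wheel is a single rotating digit wheel for a combination lock, holding a digit from 0 to 9.
; Activate picks DigitUp or DigitDown, whose timelines rotate the wheel one 36-degree step while fading and pitch-shifting the rotation sound, with Busy blocking overlapping turns.
; On finish it snaps the rotation, wraps CurrentDigit and calls UpdateNumbers on NumManager.
; The construction script pre-rotates the wheel to any non-zero starting digit.
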(event Custom|DigitUp
  (if (not (Variables|Default|GetBusy))
    (Audio|Components|Audio|AdjustVolume (Variables|Default|GetRotateSFX) 0.1 2.0 "SCurve" :!class /Script/Engine.AudioComponent)
    (bind _alpha (Timeline|TL_DigitUp PlayFromStart)
      (:Update
        (Utilities|FlowControl|Sequence
          (:then_0
            (Utilities|FlowControl|DoOnce false :!label _label
              (:Completed
                (Variables|Default|SetStartRot (Variables|/Script/Engine.SceneComponent|GetRelativeRotation (Variables|Default|GetLockWheel))))))
          (:then_1
            (Variables|Default|SetBusy true)
            (Transformation|SetRelativeRotation (Variables|Default|GetLockWheel) (Math|Rotator|Lerp(Rotator) (Variables|Default|GetStartRot) (Math|Rotator|MakeRotator (- (.Roll (Math|Rotator|BreakRotator (Variables|Default|GetStartRot))) 36.0) (.Pitch (Math|Rotator|BreakRotator (Variables|Default|GetStartRot))) (.Yaw (Math|Rotator|BreakRotator (Variables|Default|GetStartRot)))) _alpha true) false false)
            (Audio|Components|Audio|SetPitchMultiplier (Variables|Default|GetRotateSFX) (Math|Float|Lerp 1.0 0.63 _alpha)))))
      (:Finished
        (Utilities|FlowControl|Sequence
          (:then_0
            (goto _label Reset))
          (:then_1
            (Variables|Default|SetBusy false)
            (Transformation|SetRelativeRotation (Variables|Default|GetLockWheel) (Math|Rotator|MakeRotator (- (.Roll (Math|Rotator|BreakRotator (Variables|Default|GetStartRot))) 36.0) (.Pitch (Math|Rotator|BreakRotator (Variables|Default|GetStartRot))) (.Yaw (Math|Rotator|BreakRotator (Variables|Default|GetStartRot)))) false false)
            (if (== (Variables|Default|GetCurrentDigit) 9)
              (Variables|Default|SetCurrentDigit 0)
              (else
                (Math|Integer|IncrementInt (Variables|Default|GetCurrentDigit)
                  (:%20%20
                    _))))
            (Audio|Components|Audio|AdjustVolume (Variables|Default|GetRotateSFX) 0.1 0.0 "SCurve" :!class /Script/Engine.AudioComponent)
            (Components|Activation|Deactivate (Variables|Default|GetRotateSFX))
            (Default|UpdateNumbers (Variables|Default|GetNumManager))))))))

(event Custom|DigitDown
  (if (not (Variables|Default|GetBusy))
    (Audio|Components|Audio|AdjustVolume (Variables|Default|GetRotateSFX) 0.1 2.0 "SCurve" :!class /Script/Engine.AudioComponent)
    (bind _alpha (Timeline|TL_DigitDown PlayFromStart)
      (:Update
        (Utilities|FlowControl|Sequence
          (:then_0
            (Utilities|FlowControl|DoOnce false :!label _label
              (:Completed
                (Variables|Default|SetStartRot (Variables|/Script/Engine.SceneComponent|GetRelativeRotation (Variables|Default|GetLockWheel))))))
          (:then_1
            (Variables|Default|SetBusy true)
            (Transformation|SetRelativeRotation (Variables|Default|GetLockWheel) (Math|Rotator|Lerp(Rotator) (Variables|Default|GetStartRot) (Math|Rotator|MakeRotator (+ (.Roll (Math|Rotator|BreakRotator (Variables|Default|GetStartRot))) 36.0) (.Pitch (Math|Rotator|BreakRotator (Variables|Default|GetStartRot))) (.Yaw (Math|Rotator|BreakRotator (Variables|Default|GetStartRot)))) _alpha true) false false)
            (Audio|Components|Audio|SetPitchMultiplier (Variables|Default|GetRotateSFX) (Math|Float|Lerp 1.0 0.63 _alpha)))))
      (:Finished
        (Utilities|FlowControl|Sequence
          (:then_0
            (goto _label Reset))
          (:then_1
            (Variables|Default|SetBusy false)
            (Transformation|SetRelativeRotation (Variables|Default|GetLockWheel) (Math|Rotator|MakeRotator (+ (.Roll (Math|Rotator|BreakRotator (Variables|Default|GetStartRot))) 36.0) (.Pitch (Math|Rotator|BreakRotator (Variables|Default|GetStartRot))) (.Yaw (Math|Rotator|BreakRotator (Variables|Default|GetStartRot)))) false false)
            (if (== (Variables|Default|GetCurrentDigit) 0)
              (Variables|Default|SetCurrentDigit 9)
              (else
                (Math|Integer|DecrementInt (Variables|Default|GetCurrentDigit)
                  (:%20%20
                    _))))
            (Audio|Components|Audio|AdjustVolume (Variables|Default|GetRotateSFX) 0.1 0.0 "SCurve" :!class /Script/Engine.AudioComponent)
            (Components|Activation|Deactivate (Variables|Default|GetRotateSFX))
            (Default|UpdateNumbers (Variables|Default|GetNumManager))))))))

(event EventActivate
  (params (Delay :type Float%20%28single-precision%29) (Bool :type Boolean))
  (if (not (Variables|Default|GetBusy))
    (Components|Activation|Activate (Variables|Default|GetRotateSFX) false)
    (if Bool
      (CallFunction|DigitUp)
      (else
        (CallFunction|DigitDown)))))

(fn ConstructionScript
  (if (not (== (Variables|Default|GetCurrentDigit) 0))
    (Transformation|SetRelativeRotation (Variables|Default|GetLockWheel) (Math|Rotator|MakeRotator (- 1.8e+02 (Math|Conversions|ToFloat(Integer) (* (Variables|Default|GetCurrentDigit) 36))) 0.0 0.0) false false)))

(fn GetDigit
  (return (Variables|Default|GetCurrentDigit)))

(fn IsBusy
  (return (Variables|Default|GetBusy)))