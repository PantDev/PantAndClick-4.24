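; Sliding-tile puzzle master that builds, shuffles and tracks a grid of BP_SlideTile actors.
; SpawnTile recursively steps the master across the GridSize layout, spawning tiles with the first left empty, then calls Done.
; Each Done call enables collision on the empty slot's neighbours and, while ShuffleCount remains, pokes a random one other than LastTile at high timeline speed.
; Once shuffling ends, Done brightens tiles in their original position and dims the rest.
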(event Custom|SpawnTile
  (bind _returnvalue (Transformation|GetActorRotation))
  (bind _returnvalue_2 (Transformation|GetActorScale3D))
  (bind _returnvalue_3 (Transformation|GetActorLocation))
  (bind _intcurrent (Variables|Default|GetIntCurrent))
  (bind _gridsize (Variables|Default|GetGridSize))
  (bind _returnvalue_4 (Math|Transform|MakeTransform _returnvalue_3 _returnvalue _returnvalue_2))
  (bind (_x _y) (Math|Vector2D|BreakVector2D _gridsize))
  (if (== (Variables|Default|GetIntCurrent) 1)
    (bind _returnvalue_5 (Game|SpawnActorfromClass "/Game/Blueprints/GameObjects/SlidePuzzle/BP_SlideTile.BP_SlideTile_C" _returnvalue_4 "AlwaysSpawn" 0 0))
    (bind _output_get (Variables|Default|SetEmptyTile _returnvalue_5))
    (Utilities|Array|Add (Variables|Default|GetTileArray) _output_get)
    (Variables|/Game/Blueprints/GameObjects/SlidePuzzle/BP_SlideTile.BP_SlideTile_C|SetEmpty _output_get true)
    (Rendering|Material|SetMaterial (Variables|/Game/Blueprints/GameObjects/SlidePuzzle/BP_SlideTile.BP_SlideTile_C|GetPlane _output_get) 0 "/Game/Materials/NullMat.NullMat")
    (Collision|SetCollisionEnabled (Variables|/Game/Blueprints/GameObjects/SlidePuzzle/BP_SlideTile.BP_SlideTile_C|GetPlane _output_get) "NoCollision")
    (Variables|/Game/Blueprints/GameObjects/SlidePuzzle/BP_SlideTile.BP_SlideTile_C|SetMaster _returnvalue_5 self)
    (Variables|/Game/Blueprints/GameObjects/SlidePuzzle/BP_SlideTile.BP_SlideTile_C|SetTileOrigin _returnvalue_5 (Variables|Default|GetIntCurrent))
    (Variables|/Game/Blueprints/GameObjects/SlidePuzzle/BP_SlideTile.BP_SlideTile_C|SetTileNumber _returnvalue_5 1)
    (CallFunction|Increment :!label _label)
    (Utilities|FlowControl|Delay 0.01)
    (CallFunction|SpawnTile)
    (elif (== (+ (* _x _y) 1.0) (Math|Conversions|ToFloat(Integer) (Variables|Default|GetIntCurrent)))
      (CallFunction|Done)
      (else
        (if (== (Math|Integer|%(Integer) (- (Variables|Default|GetIntCurrent) 1) (Math|Float|Truncate (.X (Math|Vector2D|BreakVector2D (Variables|Default|GetGridSize))))) 0)
          (Transformation|SetActorLocation (Transformation|GetWorldLocation (Variables|Default|GetDown)) false false)
          (else
            (Transformation|SetActorLocation (Transformation|GetWorldLocation (Variables|Default|GetRight)) false false)))
        (bind _returnvalue_6 (Game|SpawnActorfromClass "/Game/Blueprints/GameObjects/SlidePuzzle/BP_SlideTile.BP_SlideTile_C" _returnvalue_4 "AlwaysSpawn" 0 0))
        (Utilities|Array|Add (Variables|Default|GetTileArray) _returnvalue_6)
        (Collision|SetCollisionEnabled (Variables|/Game/Blueprints/GameObjects/SlidePuzzle/BP_SlideTile.BP_SlideTile_C|GetPlane _returnvalue_6) "NoCollision")
        (Variables|/Game/Blueprints/GameObjects/SlidePuzzle/BP_SlideTile.BP_SlideTile_C|SetMaster _returnvalue_6 self)
        (Variables|/Game/Blueprints/GameObjects/SlidePuzzle/BP_SlideTile.BP_SlideTile_C|SetTileOrigin _returnvalue_6 (Variables|Default|GetIntCurrent))
        (Default|Start _returnvalue_6)
        (Variables|/Game/Blueprints/GameObjects/SlidePuzzle/BP_SlideTile.BP_SlideTile_C|SetTileOrigin _returnvalue_6 _intcurrent)
        (Variables|/Game/Blueprints/GameObjects/SlidePuzzle/BP_SlideTile.BP_SlideTile_C|SetTileNumber _returnvalue_6 _intcurrent)
        (bind _output_get_2 (Variables|/Game/Blueprints/GameObjects/SlidePuzzle/BP_SlideTile.BP_SlideTile_C|SetTilePosition _returnvalue_6 (Math|Vector2D|MakeVector2D (Math|Conversions|ToFloat(Integer) (Variables|Default|GetXCurrent)) (Math|Conversions|ToFloat(Integer) (Variables|Default|GetYCurrent)))))
        (Variables|/Game/Blueprints/GameObjects/SlidePuzzle/BP_SlideTile.BP_SlideTile_C|SetOriginPos _returnvalue_6 _output_get_2)
        (goto _label)))))

(event Custom|Done
  (bind _downvar (Variables|Default|GetDownVar))
  (bind _upvar (Variables|Default|GetUpVar))
  (bind _leftvar (Variables|Default|GetLeftVar))
  (bind _rightvar (Variables|Default|GetRightVar))
  (CallFunction|ActivateSurroundingTiles)
  (if (> (Variables|Default|GetShuffleCount) 0)
    (Variables|Default|SetShuffleCount (- (Variables|Default|GetShuffleCount) 1))
    (bind _output_get (Variables|Default|Setmovedir (Math|Random|RandomIntegerinRange 0 3)))
    (switch int _output_get
      (:0
        (Utilities|IsValid _upvar :!label _label
          (:Is%20Valid
            (if (== _upvar (Variables|Default|GetLastTile))
              (Utilities|IsValid _downvar :!label _label_2
                (:Is%20Valid
                  (if (== _downvar (Variables|Default|GetLastTile))
                    (Utilities|IsValid _leftvar :!label _label_3
                      (:Is%20Valid
                        (if (== _leftvar (Variables|Default|GetLastTile))
                          (Utilities|IsValid _rightvar :!label _label_4
                            (:Is%20Valid
                              (if (== _rightvar (Variables|Default|GetLastTile))
                                (goto _label)
                                (else
                                  (Default|PokeEvent _rightvar)
                                  (Components|Timeline|SetPlayRate (Variables|/Game/Blueprints/GameObjects/SlidePuzzle/BP_SlideTile.BP_SlideTile_C|GetTL_SwapTiles _rightvar) 5e+01))))
                            (:Is%20Not%20Valid
                              (goto _label)))
                          (else
                            (Default|PokeEvent _leftvar)
                            (Components|Timeline|SetPlayRate (Variables|/Game/Blueprints/GameObjects/SlidePuzzle/BP_SlideTile.BP_SlideTile_C|GetTL_SwapTiles _leftvar) 5e+01))))
                      (:Is%20Not%20Valid
                        (goto _label_4)))
                    (else
                      (Default|PokeEvent _downvar)
                      (Components|Timeline|SetPlayRate (Variables|/Game/Blueprints/GameObjects/SlidePuzzle/BP_SlideTile.BP_SlideTile_C|GetTL_SwapTiles _downvar) 5e+01))))
                (:Is%20Not%20Valid
                  (goto _label_3)))
              (else
                (Default|PokeEvent _upvar)
                (Components|Timeline|SetPlayRate (Variables|/Game/Blueprints/GameObjects/SlidePuzzle/BP_SlideTile.BP_SlideTile_C|GetTL_SwapTiles _upvar) 5e+01))))
          (:Is%20Not%20Valid
            (goto _label_2))))
      (:1
        (goto _label_2))
      (:2
        (goto _label_3))
      (:3
        (goto _label_4)))
    (else
      (for _array_element (Variables|Default|GetTileArray)
        (if (Math|Vector|Equal(Vector) (Variables|/Game/Blueprints/GameObjects/SlidePuzzle/BP_SlideTile.BP_SlideTile_C|GetTilePosition _array_element) (Variables|/Game/Blueprints/GameObjects/SlidePuzzle/BP_SlideTile.BP_SlideTile_C|GetOriginPos _array_element) 0.0001)
          (Utilities|IsValid (Variables|/Game/Blueprints/GameObjects/SlidePuzzle/BP_SlideTile.BP_SlideTile_C|GetDynamicMat _array_element)
            (:Is%20Valid
              (Rendering|Material|SetScalarParameterValue (Variables|/Game/Blueprints/GameObjects/SlidePuzzle/BP_SlideTile.BP_SlideTile_C|GetDynamicMat _array_element) "Mult" 0.35 :!class /Script/Engine.MaterialInstanceDynamic)))
          (else
            (Utilities|IsValid (Variables|/Game/Blueprints/GameObjects/SlidePuzzle/BP_SlideTile.BP_SlideTile_C|GetDynamicMat _array_element)
              (:Is%20Valid
                (Rendering|Material|SetScalarParameterValue (Variables|/Game/Blueprints/GameObjects/SlidePuzzle/BP_SlideTile.BP_SlideTile_C|GetDynamicMat _array_element) "Mult" 0.05 :!class /Script/Engine.MaterialInstanceDynamic)))))))))

(event EventBeginPlay
  (CallFunction|SpawnTile))

(fn ConstructionScript
  (bind _down (Variables|Default|GetDown))
  (bind _gridsize (Variables|Default|GetGridSize))
  (bind (_x _y) (Math|Vector2D|BreakVector2D _gridsize))
  (bind _relativelocation (Variables|/Script/Engine.SceneComponent|GetRelativeLocation _down))
  (bind (_x_2 _y_2 _z) (Math|Vector|BreakVector _relativelocation))
  (Transformation|SetRelativeLocation (Variables|Default|GetDown) (Math|Vector|MakeVector _x_2 (+ _y_2 (* (- _x (/ _x _y)) (* 1e+02 (/ _y _y)))) _z) false false)
  (Transformation|SetActorScale3D (Math|Vector|MakeVector (/ 3.0 _x) (/ 3.0 _y) 1.0)))

(fn Increment
  (if (== (Math|Integer|%(Integer) (Variables|Default|GetIntCurrent) (Math|Float|Truncate (.X (Math|Vector2D|BreakVector2D (Variables|Default|GetGridSize))))) 0)
    (Variables|Default|SetXCurrent (- (Variables|Default|GetXCurrent) (Math|Float|Truncate (- (.X (Math|Vector2D|BreakVector2D (Variables|Default|GetGridSize))) 1.0))))
    (Variables|Default|SetYCurrent (+ (Variables|Default|GetYCurrent) 1))
    (else
      (Variables|Default|SetXCurrent (+ (Variables|Default|GetXCurrent) 1))))
  (bind _result (Math|Integer|IncrementInt (Variables|Default|GetIntCurrent))
    (:%20%20
      (bind _output_get (Variables|Default|SetIntCurrent _result))
      (return _output_get (Variables|Default|GetXCurrent) (Variables|Default|GetYCurrent)))))

(fn ActivateSurroundingTiles
  (bind _emptytile (Variables|Default|GetEmptyTile))
  (bind _emptytile_2 (Variables|Default|GetEmptyTile))
  (bind _emptytile_3 (Variables|Default|GetEmptyTile))
  (bind _emptytile_4 (Variables|Default|GetEmptyTile))
  (bind _tileposition (Variables|/Game/Blueprints/GameObjects/SlidePuzzle/BP_SlideTile.BP_SlideTile_C|GetTilePosition _emptytile))
  (bind _tileposition_2 (Variables|/Game/Blueprints/GameObjects/SlidePuzzle/BP_SlideTile.BP_SlideTile_C|GetTilePosition _emptytile_2))
  (bind _tileposition_3 (Variables|/Game/Blueprints/GameObjects/SlidePuzzle/BP_SlideTile.BP_SlideTile_C|GetTilePosition _emptytile_3))
  (bind _tileposition_4 (Variables|/Game/Blueprints/GameObjects/SlidePuzzle/BP_SlideTile.BP_SlideTile_C|GetTilePosition _emptytile_4))
  (bind (_x _y) (Math|Vector2D|BreakVector2D _tileposition))
  (bind (_x_2 _y_2) (Math|Vector2D|BreakVector2D _tileposition_2))
  (bind (_x_3 _y_3) (Math|Vector2D|BreakVector2D _tileposition_3))
  (bind (_x_4 _y_4) (Math|Vector2D|BreakVector2D _tileposition_4))
  (Variables|Default|SetDownVar 0)
  (Variables|Default|SetUpVar 0)
  (Variables|Default|SetLeftVar 0)
  (Variables|Default|SetRight 0)
  (for _array_element (Variables|Default|GetTileArray)
    (if (Math|Vector|Equal(Vector) (Variables|/Game/Blueprints/GameObjects/SlidePuzzle/BP_SlideTile.BP_SlideTile_C|GetTilePosition _array_element) (Math|Vector2D|MakeVector2D (+ _x_4 1.0) _y_4) 0.0001)
      (Collision|SetCollisionEnabled (Variables|/Game/Blueprints/GameObjects/SlidePuzzle/BP_SlideTile.BP_SlideTile_C|GetPlane _array_element) "QueryAndPhysics")
      (Variables|Default|SetUpVar _array_element)))
  (for _array_element_2 (Variables|Default|GetTileArray)
    (if (Math|Vector|Equal(Vector) (Variables|/Game/Blueprints/GameObjects/SlidePuzzle/BP_SlideTile.BP_SlideTile_C|GetTilePosition _array_element_2) (Math|Vector2D|MakeVector2D (- _x_3 1.0) _y_3) 0.0001)
      (Collision|SetCollisionEnabled (Variables|/Game/Blueprints/GameObjects/SlidePuzzle/BP_SlideTile.BP_SlideTile_C|GetPlane _array_element_2) "QueryAndPhysics")
      (Variables|Default|SetDownVar _array_element_2)))
  (for _array_element_3 (Variables|Default|GetTileArray)
    (if (Math|Vector|Equal(Vector) (Variables|/Game/Blueprints/GameObjects/SlidePuzzle/BP_SlideTile.BP_SlideTile_C|GetTilePosition _array_element_3) (Math|Vector2D|MakeVector2D _x_2 (+ _y_2 1.0)) 0.0001)
      (Collision|SetCollisionEnabled (Variables|/Game/Blueprints/GameObjects/SlidePuzzle/BP_SlideTile.BP_SlideTile_C|GetPlane _array_element_3) "QueryAndPhysics")
      (Variables|Default|SetLeftVar _array_element_3)))
  (for _array_element_4 (Variables|Default|GetTileArray)
    (if (Math|Vector|Equal(Vector) (Variables|/Game/Blueprints/GameObjects/SlidePuzzle/BP_SlideTile.BP_SlideTile_C|GetTilePosition _array_element_4) (Math|Vector2D|MakeVector2D _x (- _y 1.0)) 0.0001)
      (Collision|SetCollisionEnabled (Variables|/Game/Blueprints/GameObjects/SlidePuzzle/BP_SlideTile.BP_SlideTile_C|GetPlane _array_element_4) "QueryAndPhysics")
      (Variables|Default|SetRightVar _array_element_4))))

(fn MoveRandomTile)