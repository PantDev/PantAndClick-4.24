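; A single tile in a sliding picture puzzle, showing its slice of the Master's texture through a dynamic material offset by grid position.
; Poking it plays a swap timeline with the Master's empty tile, exchanges grid positions and disables collision on all tiles.
; FastSwapFunc swaps instantly, then has the Master activate surrounding tiles.
; ActiveCheck raises the material multiplier and clicks when the tile is at its original position.
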(event Custom|Start
  (bind _tileposition (Variables|Default|GetTilePosition))
  (bind _master (Variables|Default|GetMaster))
  (bind _plane (Variables|Default|GetPlane))
  (bind (_x _y) (Math|Vector2D|BreakVector2D _tileposition))
  (bind _gridsize (Variables|/Game/Blueprints/GameObjects/SlidePuzzle/BP_SlideMaster.BP_SlideMaster_C|GetGridSize _master))
  (bind (_x_2 _y_2) (Math|Vector2D|BreakVector2D _gridsize))
  (Utilities|FlowControl|Delay 0.01)
  (Rendering|Components|TextRender|SetText (Variables|Default|GetTextRender) (Utilities|Text|ToText(String) (Variables|Default|GetTilePosition)))
  (if (not (== (Variables|Default|GetTileOrigin) 1))
    (bind _returnvalue (Rendering|Material|CreateDynamicMaterialInstance _plane 0 "/Game/Blueprints/GameObjects/SlidePuzzle/SlideTile_Mat.SlideTile_Mat" "None" :!class /Script/Engine.PrimitiveComponent))
    (bind _output_get (Variables|Default|SetDynamicMat _returnvalue))
    (Rendering|Material|SetMaterial _plane 0 _output_get)
    (Rendering|Material|SetScalarParameterValue (Variables|Default|GetDynamicMat) "OffsetX" (- _x 1.0) :!class /Script/Engine.MaterialInstanceDynamic)
    (Rendering|Material|SetScalarParameterValue (Variables|Default|GetDynamicMat) "OffsetY" (- _y 1.0) :!class /Script/Engine.MaterialInstanceDynamic)
    (Rendering|Material|SetTextureParameterValue (Variables|Default|GetDynamicMat) "Texture" (Variables|/Game/Blueprints/GameObjects/SlidePuzzle/BP_SlideMaster.BP_SlideMaster_C|GetTexture _master))
    (Rendering|Material|SetScalarParameterValue (Variables|Default|GetDynamicMat) "SizeX" _x_2 :!class /Script/Engine.MaterialInstanceDynamic)
    (Rendering|Material|SetScalarParameterValue (Variables|Default|GetDynamicMat) "SizeY" _y_2 :!class /Script/Engine.MaterialInstanceDynamic)))

(event Collision|EventActorBeginOverlap
  (params (OtherActor :type Actor%20Object%20Reference)))

(event EventTick
  (params (DeltaSeconds :type Float%20%28single-precision%29)))

(event EventPokeEvent
  (bind _master (Variables|Default|GetMaster))
  (bind _emptytile (Variables|/Game/Blueprints/GameObjects/SlidePuzzle/BP_SlideMaster.BP_SlideMaster_C|GetEmptyTile _master))
  (Audio|PlaySoundatLocation "/Game/Audio/SFX/Switch1.Switch1" (Transformation|GetActorLocation) "0, 0, 0" 0.65 (Math|Random|RandomFloatinRange 1.2 1.4) 0.0 "/Game/Audio/Attenuation/SA_ShortRange.SA_ShortRange" 0 0)
  (Variables|Default|SetSelfOrigin (Transformation|GetActorLocation))
  (Variables|Default|SetEmptyOrigin (Transformation|GetActorLocation (Variables|/Game/Blueprints/GameObjects/SlidePuzzle/BP_SlideMaster.BP_SlideMaster_C|GetEmptyTile (Variables|Default|GetMaster))))
  (Components|Timeline|PlayfromStart (Variables|Default|GetTL_SwapTiles))
  (for _array_element (Variables|/Game/Blueprints/GameObjects/SlidePuzzle/BP_SlideMaster.BP_SlideMaster_C|GetTileArray (Variables|Default|GetMaster))
    (Collision|SetCollisionEnabled (Variables|BP_SlideTile_C|GetPlane _array_element) "NoCollision"))
  (Variables|Default|SetTempPos (Variables|Default|GetTilePosition))
  (Variables|Default|SetTilePosition (Variables|BP_SlideTile_C|GetTilePosition _emptytile))
  (Variables|BP_SlideTile_C|SetTilePosition _emptytile (Variables|Default|GetTempPos)))

(fn ConstructionScript)

(fn FastSwapFunc
  (bind _master (Variables|Default|GetMaster))
  (bind _emptytile (Variables|/Game/Blueprints/GameObjects/SlidePuzzle/BP_SlideMaster.BP_SlideMaster_C|GetEmptyTile _master))
  (Variables|Default|SetSelfOrigin (Transformation|GetActorLocation))
  (Variables|Default|SetEmptyOrigin (Transformation|GetActorLocation (Variables|/Game/Blueprints/GameObjects/SlidePuzzle/BP_SlideMaster.BP_SlideMaster_C|GetEmptyTile (Variables|Default|GetMaster))))
  (Transformation|SetActorLocation (Variables|Default|GetEmptyOrigin) false false)
  (Transformation|SetActorLocation (Variables|/Game/Blueprints/GameObjects/SlidePuzzle/BP_SlideMaster.BP_SlideMaster_C|GetEmptyTile (Variables|Default|GetMaster)) (Variables|Default|GetSelfOrigin) false false)
  (Variables|Default|SetTempPos (Variables|Default|GetTilePosition))
  (Variables|Default|SetTilePosition (Variables|BP_SlideTile_C|GetTilePosition _emptytile))
  (Variables|BP_SlideTile_C|SetTilePosition _emptytile (Variables|Default|GetTempPos))
  (Default|ActivateSurroundingTiles _master))

(fn ActiveCheck
  (if (Math|Vector|Equal(Vector) (Variables|Default|GetTilePosition) (Variables|Default|GetOriginPos) 0.0001)
    (Rendering|Material|SetScalarParameterValue (Variables|Default|GetDynamicMat) "Mult" 0.35 :!class /Script/Engine.MaterialInstanceDynamic)
    (Audio|PlaySoundatLocation "/Game/Audio/SFX/ClickMusicSFX/Click6.Click6" (Transformation|GetActorLocation) "0, 0, 0" 0.2 (Math|Random|RandomFloatinRange 1.3 1.52) 0.0 "/Game/Audio/Attenuation/SA_ShortRange.SA_ShortRange" 0 0)
    (else
      (Rendering|Material|SetScalarParameterValue (Variables|Default|GetDynamicMat) "Mult" 0.05 :!class /Script/Engine.MaterialInstanceDynamic))))

(fn Attachto
  (params (ChildActor :type Actor%20Object%20Reference))
  (return 0))

(fn CanGrab
  (return false))

(fn Clicked
  (return false))

(fn DisableCollision
  (return false))

(fn DoesParentHaveParent
  (return false))

(fn EnableCollision
  (return false))

(fn GetAttached
  (return 0))

(fn GetShrinkScale
  (return "0, 0, 0" "0, 0, 0"))

(fn GetSnapLoc
  (params (CursorLoc :type Vector :default "0, 0, 0"))
  (return "0, 0, 0" "0, 0, 0"))

(fn Grabbed
  (return 0))

(fn LetGo
  (params (ParentComponent :type Actor%20Component%20Object%20Reference) (ParentActor :type Actor%20Object%20Reference))
  (return false))

(fn OnHover
  (return false))

(fn PassChildAlong
  (return 0 0))