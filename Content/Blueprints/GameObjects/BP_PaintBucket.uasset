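; BP_PaintBucket is a configurable paint bucket prop, upright or tipped, with optional lid states and a spilled puddle.
; The construction script toggles mesh variants from flags and sets a spring arm from lid length and yaw values.
; It tints bucket, fill and puddle through dynamic materials and enables puddle collision when spilled, though the lid-on branch skips this setup.
; RightClickEvent returns a click message and a focus point above the actor.
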(event EventBeginPlay)

(event Collision|EventActorBeginOverlap
  (params (OtherActor :type Actor%20Object%20Reference)))

(event EventTick
  (params (DeltaSeconds :type Float%20%28single-precision%29)))

(fn ConstructionScript
  (bind _puddle1 (Variables|Default|GetPuddle1))
  (bind _puddle1_2 (Variables|Default|GetPuddle1))
  (Variables|/Script/Engine.SpringArmComponent|SetTargetArmLength (Variables|Default|GetSpringArm) (Variables|Default|GetLidSpringLength))
  (Transformation|SetRelativeRotation (Variables|Default|GetSpringArm) (Math|Rotator|MakeRotator 0.0 0.0 (Variables|Default|GetLidSpringRot)) false false)
  (if (Variables|Default|GetUpright)
    (Rendering|SetVisibility (Variables|Default|GetBucketTipped) false false)
    (if (Variables|Default|GetNoLid)
      (Rendering|SetVisibility (Variables|Default|GetBucketUprightLidOff) false false)
      (bind _returnvalue (Rendering|Material|CreateDynamicMaterialInstance "/Game/Materials/Bucket.Bucket" "None" "None" :!class /Script/Engine.KismetMaterialLibrary :!label _label))
      (bind _output_get (Variables|Default|SetDynMatBucket _returnvalue))
      (Rendering|Material|SetMaterial (Variables|Default|GetBucketUpright) 0 _output_get)
      (Rendering|Material|SetMaterial (Variables|Default|GetBucketTipped) 0 _output_get)
      (Rendering|SetVisibility (Variables|Default|GetPuddle1) (Variables|Default|GetSpilled) false)
      (Rendering|Material|SetVectorParameterValue (Variables|Default|GetDynMatBucket) "Color" (Variables|Default|GetColor) :!class /Script/Engine.MaterialInstanceDynamic)
      (bind _returnvalue_2 (Rendering|Material|CreateDynamicMaterialInstance "/Game/Materials/PaintFill_Mat.PaintFill_Mat" "None" "None" :!class /Script/Engine.KismetMaterialLibrary))
      (bind _output_get_2 (Variables|Default|SetDynMatFill _returnvalue_2))
      (Rendering|Material|SetMaterial (Variables|Default|GetBucketUpright) 1 _output_get_2)
      (Rendering|Material|SetVectorParameterValue (Variables|Default|GetDynMatFill) "Color" (Variables|Default|GetColor) :!class /Script/Engine.MaterialInstanceDynamic)
      (bind _returnvalue_3 (Rendering|Material|CreateDynamicMaterialInstance "/Game/Materials/PaintSpill_Mat.PaintSpill_Mat" "None" "None" :!class /Script/Engine.KismetMaterialLibrary))
      (bind _output_get_3 (Variables|Default|SetDynMatSpill _returnvalue_3))
      (Rendering|Material|SetMaterial (Variables|Default|GetPuddle1) 0 _output_get_3)
      (Rendering|Material|SetVectorParameterValue (Variables|Default|GetDynMatSpill) "Color" (Variables|Default|GetColor) :!class /Script/Engine.MaterialInstanceDynamic)
      (if (Variables|Default|GetSpilled)
        (Collision|SetCollisionEnabled _puddle1 "QueryAndPhysics")
        (Collision|SetCollisionResponsetoAllChannels _puddle1 "ECR_Block")
        (else
          (Collision|SetCollisionEnabled _puddle1_2 "NoCollision")
          (Collision|SetCollisionResponsetoAllChannels _puddle1_2 "ECR_Ignore")))
      (elif (Variables|Default|GetSideLid)
        (Rendering|SetVisibility (Variables|Default|GetBucketUprightLidOn) false false)
        (goto _label)
        (else
          (Rendering|SetVisibility (Variables|Default|GetBucketUprightLidOff) false false)
          (if (Variables|Default|GetLidOn)
            (Rendering|SetVisibility (Variables|Default|GetBucketUprightLidOn) true false)
            (Rendering|SetVisibility (Variables|Default|GetBucketUprightLidPopped) false false)
            (else
              (Rendering|SetVisibility (Variables|Default|GetBucketUprightLidPopped) true false)
              (Rendering|SetVisibility (Variables|Default|GetBucketUprightLidOn) false false)
              (goto _label))))))
    (else
      (Rendering|SetVisibility (Variables|Default|GetBucketUprightLidOff) false false)
      (goto _label))))

(fn RightClickEvent
  (bind _returnvalue (Transformation|GetActorLocation))
  (bind (_x _y _z) (Math|Vector|BreakVector _returnvalue))
  (return (Variables|Default|GetClick%20Message) (Math|Vector|MakeVector _x _y (+ _z 35.0))))