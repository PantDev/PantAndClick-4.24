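; BP_NumberManager is a combination check that triggers a target actor when a set of digit actors forms the target number.
; UpdateNumbers reads each actor in DigitActorArray in order and builds FinalNumber by string concatenation, converted back to an integer.
; Activate compares FinalNumber with TargetNumber and, on a match, sends ActivateMessage to ActivateTarget if it implements BPI_Activate.
; IsBusy always returns false.
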(event Custom|UpdateNumbers
  (Variables|Default|SetFinalNumber 0)
  (bind (_array_element _array_index) (Utilities|Array|ForEachLoopwithBreak (Variables|Default|GetDigitActorArray))
    (:LoopBody
      (if (== _array_index 0)
        (bind _digitint (Class|BPIDigit|GetDigit(Message) _array_element))
        (Variables|Default|SetFinalNumber _digitint)
        (else
          (bind _digitint_2 (Class|BPIDigit|GetDigit(Message) _array_element))
          (Variables|Default|SetFinalNumber (Math|Conversions|ToInteger(Byte) (Utilities|String|Append (Utilities|String|ToString(Integer) (Variables|Default|GetFinalNumber)) (Utilities|String|ToString(Integer) _digitint_2)))))))))

(event EventActivate
  (params (Delay :type Float%20%28single-precision%29) (Bool :type Boolean))
  (bind _activatetarget (Variables|Default|GetActivateTarget))
  (if (== (Variables|Default|GetTargetNumber) (Variables|Default|GetFinalNumber))
    (if (Utilities|DoesObjectImplementInterface _activatetarget "/Game/Blueprints/BPI/BPI_Activate.BPI_Activate_C")
      (Class|BPIActivate|Activate(Message) _activatetarget 0.0 false))))

(fn ConstructionScript)

(fn IsBusy
  (return false))