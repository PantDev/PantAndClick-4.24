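; A pokeable filing cabinet prop whose two drawers toggle open and shut with pitch-randomized sounds.
; The construction script randomizes each drawer's extension and the bottom drawer's slight tilt, re-rolled on each poke-open.
; A timeline lerps spring arm lengths to slide the drawers and straightens the bottom one, while each poke also triggers a bounce timeline.
; Grab, attach and snap functions are stubs; right-click returns a message and focus location.
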(event EventProxEnd
  (Utilities|String|Reverse (Variables|Default|GetDrawerShut_TL)))

(event EventProxStart)

(event EventPokeEvent
  (bind _returnvalue (Transformation|GetActorLocation))
  (bind _tl_bounce (Variables|Default|GetTL_Bounce))
  (Audio|Components|Audio|Stop (Variables|Default|GetDrawerShut_TL))
  (if (Audio|Components|Audio|IsPlaying _tl_bounce)
    (Utilities|String|Reverse _tl_bounce)
    (else
      (Components|Timeline|PlayfromStart _tl_bounce)))
  (if (Variables|Default|GetIsClosed)
    (Variables|Default|SetIsClosed false)
    (Variables|Default|SetTopStartLength (Math|Random|RandomFloatinRange 15.0 45.0))
    (Variables|Default|SetBottomStartLength (Math|Random|RandomFloatinRange 15.0 45.0))
    (Variables|Default|SetBottomStartRot (Math|Rotator|MakeRotator (Math|Random|RandomFloatinRange 0.0 1.0) (Math|Random|RandomFloatinRange -2.0 2.0) (+ (Math|Random|RandomFloatinRange -2.0 2.0) 9e+01)))
    (Audio|PlaySoundatLocation "/Game/Audio/SFX/ButtonPress1.ButtonPress1" _returnvalue "0, 0, 0" 0.55 (Math|Random|RandomFloatinRange 0.7 1.0) 0.0 "/Game/Audio/Attenuation/SA_ShortRange.SA_ShortRange" 0 0)
    (bind (_direction _newtrack_0 _newtrack_1) (Timeline|DrawerShut_TL Reverse)
      (:Update
        (Variables|/Script/Engine.SpringArmComponent|SetTargetArmLength (Variables|Default|GetBottomSpring) (Math|Float|Lerp (Variables|Default|GetBottomStartLength) 0.0 _newtrack_1))
        (Variables|/Script/Engine.SpringArmComponent|SetTargetArmLength (Variables|Default|GetTopSpring) (Math|Float|Lerp (Variables|Default|GetTopStartLength) 0.0 _newtrack_0))
        (Transformation|SetRelativeRotation (Variables|Default|GetBottomDrawer) (Math|Rotator|Lerp(Rotator) (Variables|Default|GetBottomStartRot) "0,90.000000, 0" _newtrack_0 true) false false)))
    (else
      (Variables|Default|SetIsClosed true)
      (Audio|PlaySoundatLocation "/Game/Audio/SFX/ButtonPress1.ButtonPress1" "0, 0, 0" "0, 0, 0" 0.25 (Math|Random|RandomFloatinRange 0.6 0.9) 0.02 "/Game/Audio/Attenuation/SA_ShortRange.SA_ShortRange" 0 0)
      (Audio|PlaySoundatLocation "/Game/Audio/SFX/Switch1.Switch1" _returnvalue "0, 0, 0" 0.4 (Math|Random|RandomFloatinRange 0.4 0.6) 0.0 "/Game/Audio/Attenuation/SA_ShortRange.SA_ShortRange" 0 0)
      (Timeline|DrawerShut_TL Play))))

(fn ConstructionScript
  (bind _output_get (Variables|Default|SetTopStartLength (Math|Random|RandomFloatinRange 15.0 45.0)))
  (Variables|/Script/Engine.SpringArmComponent|SetTargetArmLength (Variables|Default|GetTopSpring) _output_get)
  (bind _output_get_2 (Variables|Default|SetBottomStartLength (Math|Random|RandomFloatinRange 15.0 45.0)))
  (Variables|/Script/Engine.SpringArmComponent|SetTargetArmLength (Variables|Default|GetBottomSpring) _output_get_2)
  (bind _output_get_3 (Variables|Default|SetBottomStartRot (Math|Rotator|MakeRotator (Math|Random|RandomFloatinRange 0.0 1.0) (Math|Random|RandomFloatinRange -2.0 2.0) (+ (Math|Random|RandomFloatinRange -2.0 2.0) 9e+01))))
  (Transformation|SetRelativeRotation (Variables|Default|GetBottomDrawer) _output_get_3 false false))

(fn Attachto
  (params (ChildActor :type Actor%20Object%20Reference))
  (return 0))

(fn CanGrab
  (return false))

(fn Clicked
  (return false))

(fn DisableCollision
  (return false))

(fn DoesParentHaveParent
  (return false))

(fn EnableCollision
  (return false))

(fn GetAttached
  (return 0))

(fn GetCustomCursor
  (return false 0))

(fn GetShrinkScale
  (return "0, 0, 0" "0, 0, 0"))

(fn GetSnapLoc
  (params (CursorLoc :type Vector :default "0, 0, 0"))
  (return "0, 0, 0" "0, 0, 0"))

(fn Grabbed
  (return 0))

(fn LetGo
  (params (ParentComponent :type Actor%20Component%20Object%20Reference) (ParentActor :type Actor%20Object%20Reference))
  (return false))

(fn OnHover
  (return false))

(fn PassChildAlong
  (return 0 0))

(fn RightClickEvent
  (return (Variables|Default|GetClick%20Message) (Transformation|GetWorldLocation (Variables|Default|GetBox1))))