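; BP_FollowClasp is a clasp object whose mesh eases into a pose relative to its SpringArm when play begins.
; The TL_Length timeline extends the arm from zero to full length while blending the mesh from its starting world rotation to the arm's rotation, offset by right angles in roll and yaw.
; Key spin and bob timelines, which would replay at randomized rates, are present but never started.
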(event EventBeginPlay
  (bind _springarm (Variables|Default|GetSpringArm))
  (bind _returnvalue (Transformation|GetWorldRotation _springarm))
  (bind (_roll _pitch _yaw) (Math|Rotator|BreakRotator _returnvalue))
  (Variables|Default|SetStartRot (Transformation|GetWorldRotation (Variables|Default|GetMesh)))
  (bind _newtrack_0 (Timeline|TL_Length PlayFromStart)
    (:Update
      (Variables|/Script/Engine.SpringArmComponent|SetTargetArmLength (Variables|Default|GetSpringArm) (Math|Float|Lerp 0.0 165.0 _newtrack_0))
      (Transformation|SetWorldRotation (Variables|Default|GetMesh) (Math|Rotator|Lerp(Rotator) (Variables|Default|GetStartRot) (Math|Rotator|MakeRotator (- _roll 9e+01) _pitch (+ _yaw 9e+01)) _newtrack_0 true) false false))))

(fn ConstructionScript)