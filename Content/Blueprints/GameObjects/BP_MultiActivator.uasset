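; BP_MultiActivator is an actor that triggers a group of activatable objects from a single Activate event, all or none.
; It first polls every BPI_Activate implementer in ActivateArray with IsBusyMessage.
; If any reports busy it clears the Busy flag and activates nothing; otherwise it sends each ActivateMessage with no delay.
; Its own IsBusy function always returns false.
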(event EventBeginPlay)

(event Collision|EventActorBeginOverlap
  (params (OtherActor :type Actor%20Object%20Reference)))

(event EventTick
  (params (DeltaSeconds :type Float%20%28single-precision%29)))

(event EventActivate
  (params (Delay :type Float%20%28single-precision%29) (Bool :type Boolean))
  (for _array_element (Variables|Default|GetActivateArray)
    (if (Utilities|DoesObjectImplementInterface _array_element "/Game/Blueprints/BPI/BPI_Activate.BPI_Activate_C")
      (bind _busy (Class|BPIActivate|IsBusy(Message) _array_element))
      (if _busy
        (Variables|Default|SetBusy true))))
  (if (Variables|Default|GetBusy)
    (Variables|Default|SetBusy false)
    (else
      (for _array_element_2 (Variables|Default|GetActivateArray)
        (if (Utilities|DoesObjectImplementInterface _array_element_2 "/Game/Blueprints/BPI/BPI_Activate.BPI_Activate_C")
          (Class|BPIActivate|Activate(Message) _array_element_2 0.0 false))))))

(fn ConstructionScript)

(fn IsBusy
  (return false))