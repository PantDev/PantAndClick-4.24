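; BP_BGMesh is an actor that animates distortion on a skeletal mesh, apparently as background scenery.
; On BeginPlay a timeline drives the "Var1" morph target between zero and a randomized strength.
; Each time the timeline finishes, it replays with a new random strength and play rate, both from lower ranges than the first pass, giving continuous, irregular deformation.
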(event EventBeginPlay
  (Variables|Default|SetDistortTarget (Math|Random|RandomFloatinRange 0.2 0.4))
  (Components|Timeline|SetPlayRate (Variables|Default|GetTL_Distort1) (Math|Random|RandomFloatinRange 0.08 0.2))
  (bind _alpha (Timeline|TL_Distort1 PlayFromStart)
    (:Update
      (Components|SkeletalMesh|SetMorphTarget (Variables|Default|GetSkeletalMesh) "Var1" (Math|Float|Lerp 0.0 (Variables|Default|GetDistortTarget) _alpha) true))
    (:Finished
      (Variables|Default|SetDistortTarget (Math|Random|RandomFloatinRange 0.15 0.2))
      (Components|Timeline|SetPlayRate (Variables|Default|GetTL_Distort1) (Math|Random|RandomFloatinRange 0.02 0.12))
      (Components|Timeline|PlayfromStart (Variables|Default|GetTL_Distort1)))))

(event Collision|EventActorBeginOverlap
  (params (OtherActor :type Actor%20Object%20Reference)))

(event EventTick
  (params (DeltaSeconds :type Float%20%28single-precision%29)))

(fn ConstructionScript)