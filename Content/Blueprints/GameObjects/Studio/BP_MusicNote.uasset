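; BP_MusicNote is a note actor that places itself at a pitch height, apparently on a musical staff.
; NoteSpawn maps 25 semitone indices to stepped Z offsets, showing extra meshes for what look like accidentals and ledger lines.
; Notes from index 12 upward rotate mesh and spring arm 180 degrees.
; A timeline slides the note in along Y, with a track that enables spring arm lag once.
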(event Custom|NoteSpawn
  (params (NoteInt :type Integer))
  (bind _returnvalue (Transformation|GetActorLocation))
  (bind _returnvalue_2 (Transformation|GetActorLocation))
  (bind _returnvalue_3 (Transformation|GetActorLocation))
  (bind _returnvalue_4 (Transformation|GetActorLocation))
  (bind _returnvalue_5 (Transformation|GetActorLocation))
  (bind _returnvalue_6 (Transformation|GetActorLocation))
  (bind _returnvalue_7 (Transformation|GetActorLocation))
  (bind _returnvalue_8 (Transformation|GetActorLocation))
  (bind _returnvalue_9 (Transformation|GetActorLocation))
  (bind _returnvalue_10 (Transformation|GetActorLocation))
  (bind _returnvalue_11 (Transformation|GetActorLocation))
  (bind _returnvalue_12 (Transformation|GetActorLocation))
  (bind _returnvalue_13 (Transformation|GetActorLocation))
  (bind _returnvalue_14 (Transformation|GetActorLocation))
  (bind _springarm (Variables|Default|GetSpringArm))
  (bind (_x _y _z) (Math|Vector|BreakVector _returnvalue))
  (bind (_x_2 _y_2 _z_2) (Math|Vector|BreakVector _returnvalue_3))
  (bind (_x_3 _y_3 _z_3) (Math|Vector|BreakVector _returnvalue_4))
  (bind (_x_4 _y_4 _z_4) (Math|Vector|BreakVector _returnvalue_5))
  (bind (_x_5 _y_5 _z_5) (Math|Vector|BreakVector _returnvalue_2))
  (bind (_x_6 _y_6 _z_6) (Math|Vector|BreakVector _returnvalue_6))
  (bind (_x_7 _y_7 _z_7) (Math|Vector|BreakVector _returnvalue_7))
  (bind (_x_8 _y_8 _z_8) (Math|Vector|BreakVector _returnvalue_8))
  (bind (_x_9 _y_9 _z_9) (Math|Vector|BreakVector _returnvalue_9))
  (bind (_x_10 _y_10 _z_10) (Math|Vector|BreakVector _returnvalue_10))
  (bind (_x_11 _y_11 _z_11) (Math|Vector|BreakVector _returnvalue_11))
  (bind (_x_12 _y_12 _z_12) (Math|Vector|BreakVector _returnvalue_12))
  (bind (_x_13 _y_13 _z_13) (Math|Vector|BreakVector _returnvalue_13))
  (bind (_x_14 _y_14 _z_14) (Math|Vector|BreakVector _returnvalue_14))
  (switch int NoteInt
    (:1
      (Rendering|SetVisibility (Variables|Default|GetStaticMesh2) true true :!label _label)
      (Transformation|SetWorldLocation (Variables|Default|GetStaticMesh) (Transformation|GetActorLocation) false false))
    (:2
      (Rendering|SetVisibility (Variables|Default|GetStaticMesh1) true true)
      (goto _label))
    (:3
      (Transformation|SetWorldLocation (Variables|Default|GetStaticMesh) (Math|Vector|MakeVector _x _y (+ _z 2e+01)) false false :!label _label_2))
    (:4
      (Rendering|SetVisibility (Variables|Default|GetStaticMesh1) true true)
      (goto _label_2))
    (:5
      (Transformation|SetWorldLocation (Variables|Default|GetStaticMesh) (Math|Vector|MakeVector _x_2 _y_2 (+ _z_2 4e+01)) false false))
    (:6
      (Transformation|SetWorldLocation (Variables|Default|GetStaticMesh) (Math|Vector|MakeVector _x_3 _y_3 (+ _z_3 6e+01)) false false :!label _label_3))
    (:7
      (Rendering|SetVisibility (Variables|Default|GetStaticMesh1) true true)
      (goto _label_3))
    (:8
      (Transformation|SetWorldLocation (Variables|Default|GetStaticMesh) (Math|Vector|MakeVector _x_4 _y_4 (+ _z_4 8e+01)) false false :!label _label_4))
    (:9
      (Rendering|SetVisibility (Variables|Default|GetStaticMesh1) true true)
      (goto _label_4))
    (:10
      (Transformation|SetWorldLocation (Variables|Default|GetStaticMesh) (Math|Vector|MakeVector _x_6 _y_6 (+ _z_6 1e+02)) false false :!label _label_5))
    (:11
      (Rendering|SetVisibility (Variables|Default|GetStaticMesh1) true true)
      (goto _label_5))
    (:12
      (Transformation|SetWorldLocation (Variables|Default|GetStaticMesh) (Math|Vector|MakeVector _x_7 _y_7 (+ _z_7 1.2e+02)) false false))
    (:13
      (Transformation|SetWorldLocation (Variables|Default|GetStaticMesh) (Math|Vector|MakeVector _x_8 _y_8 (+ _z_8 1.4e+02)) false false :!label _label_6))
    (:14
      (Rendering|SetVisibility (Variables|Default|GetStaticMesh1) true true)
      (goto _label_6))
    (:15
      (Transformation|SetWorldLocation (Variables|Default|GetStaticMesh) (Math|Vector|MakeVector _x_9 _y_9 (+ _z_9 1.6e+02)) false false :!label _label_7))
    (:16
      (Rendering|SetVisibility (Variables|Default|GetStaticMesh1) true true)
      (goto _label_7))
    (:17
      (Transformation|SetWorldLocation (Variables|Default|GetStaticMesh) (Math|Vector|MakeVector _x_10 _y_10 (+ _z_10 1.8e+02)) false false))
    (:18
      (Transformation|SetWorldLocation (Variables|Default|GetStaticMesh) (Math|Vector|MakeVector _x_11 _y_11 (+ _z_11 2e+02)) false false :!label _label_8))
    (:19
      (Rendering|SetVisibility (Variables|Default|GetStaticMesh1) true true)
      (goto _label_8))
    (:20
      (Transformation|SetWorldLocation (Variables|Default|GetStaticMesh) (Math|Vector|MakeVector _x_12 _y_12 (+ _z_12 2.2e+02)) false false :!label _label_9))
    (:21
      (Rendering|SetVisibility (Variables|Default|GetStaticMesh1) true true)
      (goto _label_9))
    (:22
      (Rendering|SetVisibility (Variables|Default|GetStaticMesh2) true true :!label _label_10)
      (Transformation|SetWorldLocation (Variables|Default|GetStaticMesh) (Math|Vector|MakeVector _x_13 _y_13 (+ _z_13 2.4e+02)) false false))
    (:23
      (Rendering|SetVisibility (Variables|Default|GetStaticMesh1) true true)
      (goto _label_10))
    (:24
      (Rendering|SetVisibility (Variables|Default|GetStaticMesh3) true true)
      (Transformation|SetWorldLocation (Variables|Default|GetStaticMesh) (Math|Vector|MakeVector _x_14 _y_14 (+ _z_14 2.6e+02)) false false))
    (:25
      (Rendering|SetVisibility (Variables|Default|GetStaticMesh2) true true)
      (Transformation|SetWorldLocation (Variables|Default|GetStaticMesh) (Math|Vector|MakeVector _x_5 _y_5 (+ _z_5 2.8e+02)) false false)))
  (Rendering|SetVisibility (Variables|Default|GetStaticMesh) true false)
  (Variables|Default|SetDestLoc (Transformation|GetWorldLocation (Variables|Default|GetStaticMesh)))
  (Math|Integer|CompareInt NoteInt 12
    (:>
      (Transformation|AddLocalRotation (Variables|Default|GetStaticMesh) "180.000000,0.000000, 0" false false :!label _label_11))
    (:==
      (goto _label_11))
    (:<
      _))
  (Components|Timeline|SetPlayRate (Variables|Default|GetTL_Spawn) 1.5)
  (bind _alpha (Timeline|TL_Spawn PlayFromStart)
    (:Update
      (Transformation|SetWorldLocation (Variables|Default|GetStaticMesh) (Math|Vector|Lerp(Vector) (Math|Vector|MakeVector (.X (Math|Vector|BreakVector (Variables|Default|GetDestLoc))) (+ (.Y (Math|Vector|BreakVector (Variables|Default|GetDestLoc))) 3.5e+02) (.Z (Math|Vector|BreakVector (Variables|Default|GetDestLoc)))) (Variables|Default|GetDestLoc) _alpha) false false))
    (:NewTrack_0
      (Utilities|FlowControl|DoOnce false
        (:Completed
          (Variables|/Script/Engine.SpringArmComponent|SetbEnableCameraRotationLag _springarm true)
          (Variables|/Script/Engine.SpringArmComponent|SetbEnableCameraLag _springarm true))))))

(fn ConstructionScript)