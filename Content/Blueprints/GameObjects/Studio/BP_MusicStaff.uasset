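; Music staff for the studio MIDI puzzle, which starts dark and displays up to eight spawned notes, clearing when full or deactivated.
; Activate fades its neon material and linked lights via a timeline, and CheckInput compares the entered notes to the solution.
; On a match it disables player input and recursively replays the melody through spawned key actuators, vibrating speakers and sound waves at note-scaled rates.
; It then sends out the floppy disk, starts a looping sequence and locks the puzzle.
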(event Custom|StaffSpawn
  (params (NoteInt :type Integer))
  (bind _notearray (Variables|Default|GetNoteArray))
  (bind _notearray_2 (Variables|Default|GetNoteArray))
  (if (not (Variables|Default|GetPuzzleComplete))
    (if (Variables|Default|GetActivated)
      (if (> (Variables|Default|GetIndex) 7)
        (for _array_element _notearray_2
          (Actor|DestroyActor _array_element))
        (Utilities|Array|Clear _notearray_2)
        (Variables|Default|SetIndex 0))
      (bind _returnvalue (Game|SpawnActorfromClass "/Game/Blueprints/GameObjects/Studio/BP_MusicNote.BP_MusicNote_C" (Math|Transform|MakeTransform (Transformation|GetWorldLocation (Utilities|Select :Index (Variables|Default|GetIndex) :Option%200 (Variables|Default|GetSpawn1) :Option%201 (Variables|Default|GetSpawn2) :Option%202 (Variables|Default|GetSpawn3) :Option%203 (Variables|Default|GetSpawn4) :Option%204 (Variables|Default|GetSpawn5) :Option%205 (Variables|Default|GetSpawn6) :Option%206 (Variables|Default|GetSpawn7) :Option%207 (Variables|Default|GetSpawn8))) (Transformation|GetActorRotation)) "Undefined" 0 0))
      (Default|NoteSpawn _returnvalue NoteInt)
      (Utilities|Array|Add (Variables|Default|GetNoteArray) _returnvalue)
      (Variables|Default|SetIndex (+ (Variables|Default|GetIndex) 1))
      (else
        (for _array_element_2 _notearray
          (Actor|DestroyActor _array_element_2))
        (Utilities|Array|Clear _notearray)
        (Variables|Default|SetIndex 0)))))

(event Custom|CheckInput
  (bind _returnvalue (Transformation|GetActorLocation))
  (if (not (Variables|Default|GetPuzzleComplete))
    (if (Utilities|Array|Identical (Variables|Default|GetSolutionArray) (Variables|Default|GetInputArray))
      (bind _asbp_pant_controller (Utilities|Casting|CastToBP_PantController (Game|GetPlayerCharacter 0))
        (:then
          (Utilities|IsValid (Variables|/Game/PantControllerBP/Blueprints/BP_PantController.BP_PantController_C|GetMagnifyActor _asbp_pant_controller)
            (:Is%20Valid
              (Variables|Default|SetMagnify%20Actor (Variables|/Game/PantControllerBP/Blueprints/BP_PantController.BP_PantController_C|GetMagnifyActor _asbp_pant_controller))
              (Default|SilentBackArrow _asbp_pant_controller))
            (:Is%20Not%20Valid
              _)))
        (:CastFailed
          _))
      (Input|DisableInput (Game|GetPlayerCharacter 0) 0)
      (Utilities|FlowControl|Delay 1.0)
      (CallFunction|RepeatNote)
      (else
        (Audio|PlaySoundatLocation "/Game/Audio/SFX/KnobRight.KnobRight" _returnvalue "0, 0, 0" 0.8 0.65 0.55 "/Game/Audio/Attenuation/SA_ShortRange.SA_ShortRange" "/Game/Audio/Attenuation/SC_Default.SC_Default" 0)
        (Audio|PlaySoundatLocation "/Game/Audio/SFX/BoxSpin.BoxSpin" _returnvalue "0, 0, 0" 0.4 0.65 0.2 "/Game/Audio/Attenuation/SA_ShortRange.SA_ShortRange" "/Game/Audio/Attenuation/SC_Default.SC_Default" 0)))))

(event Custom|RepeatNote
  (bind _midicontroller (Variables|Default|GetMidiController))
  (bind _solutionarray (Variables|Default|GetSolutionArray))
  (bind _currentelement (Variables|Default|GetCurrentElement))
  (bind _currentelement_2 (Variables|Default|GetCurrentElement))
  (bind _output (Utilities|Array|Get(acopy) _solutionarray _currentelement_2))
  (bind _returnvalue (Utilities|String|ToString(Byte) _output))
  (bind _returnvalue_2 (Math|Conversions|ToFloat(Integer) _returnvalue))
  (bind _returnvalue_3 (/ _returnvalue_2 25.0))
  (bind _returnvalue_4 (Math|Float|Lerp 0.78 1.12 _returnvalue_3))
  (bind _returnvalue_5 (Game|SpawnActorfromClass "/Game/Blueprints/GameObjects/Studio/BP_KeyActuator.BP_KeyActuator_C" (Math|Transform|MakeTransform (Transformation|GetActorLocation)) "Undefined" 0 0))
  (Variables|/Game/Blueprints/GameObjects/Studio/BP_KeyActuator.BP_KeyActuator_C|SetMidiParent _returnvalue_5 (Variables|Default|GetMidiController))
  (Default|KeyPress _returnvalue_5 (Utilities|String|StringToName (Utilities|String|Append "Key" _returnvalue)))
  (Utilities|FlowControl|Sequence
    (:then_0
      (Utilities|FlowControl|Delay 0.5)
      (Math|Integer|IncrementInt _currentelement
        (:%20%20
          (if (< _currentelement 8)
            (CallFunction|RepeatNote)
            (else
              (Default|FlytoEvent (Variables|Default|GetFloppyDisk))
              (Class|MovieSceneSequencePlayer|PlayLooping (Variables|/Script/LevelSequence.LevelSequenceActor|GetSequencePlayer (Variables|Default|GetThumpSequence)) -1)
              (Audio|PlaySound2D (Variables|Default|GetAudio%20Cue) 1.0 1.0 0.0 0 0)
              (Variables|Default|SetPuzzleComplete true))))))
    (:then_1
      (bind _array_element (Utilities|Array|ForEachLoopwithBreak (Variables|/Game/Blueprints/GameObjects/Studio/BP_MidiController.BP_MidiController_C|GetSoundWaves _midicontroller))
        (:LoopBody
          (Components|Timeline|SetPlayRate (Variables|/Game/Blueprints/GameObjects/Studio/BP_SoundWave.BP_SoundWave_C|GetTL_Vibrate1 _array_element) _returnvalue_4)
          (Components|Timeline|PlayfromStart (Variables|/Game/Blueprints/GameObjects/Studio/BP_SoundWave.BP_SoundWave_C|GetTL_Vibrate1 _array_element)))))
    (:then_2
      (bind _array_element_2 (Utilities|Array|ForEachLoopwithBreak (Variables|/Game/Blueprints/GameObjects/Studio/BP_MidiController.BP_MidiController_C|GetSpeakers _midicontroller))
        (:LoopBody
          (Components|Timeline|SetPlayRate (Variables|/Game/Blueprints/GameObjects/Studio/BP_SpeakerBlock.BP_SpeakerBlock_C|GetTL_Vibrate1 _array_element_2) _returnvalue_4)
          (Components|Timeline|PlayfromStart (Variables|/Game/Blueprints/GameObjects/Studio/BP_SpeakerBlock.BP_SpeakerBlock_C|GetTL_Vibrate1 _array_element_2)))))))

(event EventActivate
  (params (Delay :type Float%20%28single-precision%29) (Bool :type Boolean))
  (bind _dynamicmat (Variables|Default|GetDynamicMat))
  (if (not Bool)
    (Variables|Default|SetActivated true)
    (bind _alpha (Timeline|TL_LightOn Play)
      (:Update
        (Rendering|Material|SetScalarParameterValue _dynamicmat "Freq" (Math|Float|Lerp 0.0 24.0 _alpha) :!class /Script/Engine.MaterialInstanceDynamic)
        (Rendering|Material|SetVectorParameterValue _dynamicmat "BaseColor" (Math|Color|Lerp(LinearColor) "(R=0.000000,G=0.000000,B=0.000000,A=1.000000)" (Math|Color|MakeColor 0.458333 0.861574 1.0) _alpha) :!class /Script/Engine.MaterialInstanceDynamic)
        (Rendering|Material|SetScalarParameterValue _dynamicmat "MinClamp" (Math|Float|Lerp 0.0 0.6 _alpha) :!class /Script/Engine.MaterialInstanceDynamic)
        (Rendering|Material|SetScalarParameterValue _dynamicmat "MaxClamp" (Math|Float|Lerp 0.0 1.0 _alpha) :!class /Script/Engine.MaterialInstanceDynamic)
        (for _array_element (Variables|Default|GetLights)
          (Rendering|Components|Light|SetIntensity (Variables|/Script/Engine.PointLight|GetPointLightComponent _array_element) (Math|Float|Lerp 0.0 2.5 _alpha)))))
    (else
      (Variables|Default|SetActivated false)
      (CallFunction|StaffSpawn)
      (Timeline|TL_LightOn Reverse))))

(event EventBeginPlay
  (bind _staffmesh (Variables|Default|GetStaffMesh))
  (bind _returnvalue (Rendering|Material|CreateDynamicMaterialInstance "/Game/Materials/Glow_Neon.Glow_Neon" "None" "None" :!class /Script/Engine.KismetMaterialLibrary))
  (Variables|Default|SetDynamicMat _returnvalue)
  (Rendering|Material|SetMaterial _staffmesh 0 (Variables|Default|GetDynamicMat))
  (Rendering|Material|SetMaterial _staffmesh 2 (Variables|Default|GetDynamicMat))
  (Rendering|Material|SetVectorParameterValue :self (Variables|Default|GetDynamicMat) :ParameterName "BaseColor" :!class /Script/Engine.MaterialInstanceDynamic)
  (CallFunction|Activate 0.0 true))

(fn ConstructionScript)

(fn IsBusy
  (return false))