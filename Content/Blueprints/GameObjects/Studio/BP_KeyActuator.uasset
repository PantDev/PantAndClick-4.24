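; BP_KeyActuator is a short-lived actor that plays one key press on a studio MIDI keyboard, its MidiParent.
; KeyPress runs a timeline that drives the morph target named after the key, then destroys the actor.
; A timeline event parses the key number from that name to pick one of 25 sounds, played at the parent's first two speakers while its Staff is activated.
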(event Custom|KeyPress
  (params (KeyName :type Name))
  (bind _midiparent (Variables|Default|GetMidiParent))
  (Variables|Default|SetName KeyName)
  (bind _newtrack_0 (Timeline|TL_KeyAnim PlayFromStart)
    (:Update
      (Components|SkeletalMesh|SetMorphTarget (Variables|/Game/Blueprints/GameObjects/Studio/BP_MidiController.BP_MidiController_C|GetSkeletalMesh _midiparent) (Variables|Default|GetName) _newtrack_0 true))
    (:Finished
      (Actor|DestroyActor))
    (:NewTrack_1
      (bind (_array_element _array_index) (Utilities|Array|ForEachLoopwithBreak (Variables|/Game/Blueprints/GameObjects/Studio/BP_MidiController.BP_MidiController_C|GetSpeakers _midiparent))
        (:LoopBody
          (if (< _array_index 2)
            (if (Variables|/Game/Blueprints/GameObjects/Studio/BP_MusicStaff.BP_MusicStaff_C|GetActivated (Variables|/Game/Blueprints/GameObjects/Studio/BP_MidiController.BP_MidiController_C|GetStaff (Variables|Default|GetMidiParent)))
              (Audio|PlaySoundatLocation (Utilities|Select :Index (Math|Float|Truncate (- (Math|Conversions|ToFloat(Integer) (Utilities|String|Replace (Utilities|String|ToString(Name) (Variables|Default|GetName)) "Key")) 1.0)) :Option%200 "/Game/Audio/SFX/Midi/Key1.Key1" :Option%201 "/Game/Audio/SFX/Midi/Key2.Key2" :Option%202 "/Game/Audio/SFX/Midi/Key3.Key3" :Option%203 "/Game/Audio/SFX/Midi/Key4.Key4" :Option%204 "/Game/Audio/SFX/Midi/Key5.Key5" :Option%205 "/Game/Audio/SFX/Midi/Key6.Key6" :Option%206 "/Game/Audio/SFX/Midi/Key7.Key7" :Option%207 "/Game/Audio/SFX/Midi/Key8.Key8" :Option%208 "/Game/Audio/SFX/Midi/Key9.Key9" :Option%209 "/Game/Audio/SFX/Midi/Key10.Key10" :Option%2010 "/Game/Audio/SFX/Midi/Key11.Key11" :Option%2011 "/Game/Audio/SFX/Midi/Key12.Key12" :Option%2012 "/Game/Audio/SFX/Midi/Key13.Key13" :Option%2013 "/Game/Audio/SFX/Midi/Key14.Key14" :Option%2014 "/Game/Audio/SFX/Midi/Key15.Key15" :Option%2015 "/Game/Audio/SFX/Midi/Key16.Key16" :Option%2016 "/Game/Audio/SFX/Midi/Key17.Key17" :Option%2017 "/Game/Audio/SFX/Midi/Key18.Key18" :Option%2018 "/Game/Audio/SFX/Midi/Key19.Key19" :Option%2019 "/Game/Audio/SFX/Midi/Key20.Key20" :Option%2020 "/Game/Audio/SFX/Midi/Key21.Key21" :Option%2021 "/Game/Audio/SFX/Midi/Key22.Key22" :Option%2022 "/Game/Audio/SFX/Midi/Key23.Key23" :Option%2023 "/Game/Audio/SFX/Midi/Key24.Key24" :Option%2024 "/Game/Audio/SFX/Midi/Key25.Key25") (Transformation|GetActorLocation _array_element) "0, 0, 0" 0.4 1.0 0.0 "/Game/Audio/Attenuation/SA_ShortRange.SA_ShortRange" "/Game/Audio/Concurrency/AC_Files.AC_Files" 0))))))))

(fn ConstructionScript)