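; BP_MidiController is a studio MIDI keyboard that turns the player's key pokes into an eight-note input puzzle on a Staff.
; PokeEvent parses the key number from the poked component's name, spawns and records the note on Staff, and spawns a BP_KeyActuator to press the key.
; An activated Staff vibrates speakers and sound waves at key-scaled rates and checks input on the eighth note.
; Player capsule overlap with Pad1 animates its glow and morph target.
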(event OnComponentBeginOverlap(Pad1)
  (params (OverlappedComponent :type Primitive%20Component%20Object%20Reference) (OtherActor :type Actor%20Object%20Reference) (OtherComp :type Primitive%20Component%20Object%20Reference) (OtherBodyIndex :type Integer) (bFromSweep :type Boolean) (SweepResult :type Hit%20Result%20Structure%20%28by%20ref%29))
  (bind _asbp_pant_controller (Utilities|Casting|CastToBP_PantController OtherActor))
  (if (== (Variables|/Script/Engine.Character|GetCapsuleComponent _asbp_pant_controller) OtherComp)
    (bind _returnvalue (Rendering|Material|CreateDynamicMaterialInstance (Variables|Default|GetSkeletalMesh) 1 "/Game/Blueprints/GameObjects/Studio/Mesh/Mat_MidiPadGlow.Mat_MidiPadGlow" "None" :!class /Script/Engine.PrimitiveComponent))
    (bind _output_get (Variables|Default|SetPad1Mat _returnvalue))
    (Rendering|Material|SetMaterial (Variables|Default|GetSkeletalMesh) 1 _output_get)
    (bind _alpha (Timeline|TL_Pad1 PlayFromStart)
      (:Update
        (Rendering|Material|SetScalarParameterValue (Variables|Default|GetPad1Mat) "GlowMult" (Math|Float|Lerp 0.0 1e+01 _alpha) :!class /Script/Engine.MaterialInstanceDynamic)
        (Components|SkeletalMesh|SetMorphTarget (Variables|Default|GetSkeletalMesh) "Pad1" _alpha true)))))

(event EventPokeEvent
  (bind _staff (Variables|Default|GetStaff))
  (bind _index (Variables|/Game/Blueprints/GameObjects/Studio/BP_MusicStaff.BP_MusicStaff_C|GetIndex _staff))
  (bind _inputarray (Variables|/Game/Blueprints/GameObjects/Studio/BP_MusicStaff.BP_MusicStaff_C|GetInputArray _staff))
  (bind _returnvalue (- _index 1))
  (bind _asbp_pant_controller (Utilities|Casting|CastToBP_PantController (Game|GetPlayerCharacter 0)))
  (bind _output_get (Variables|Default|SetLastKey (Math|Conversions|ToInteger(Byte) (Utilities|String|Replace (Utilities|String|ToString(Name) (Utilities|String|StringToName (Utilities|String|ToString(Object) (Variables|/Game/PantControllerBP/Blueprints/BP_PantController.BP_PantController_C|GetPokeComponent _asbp_pant_controller)))) "Key"))))
  (Default|StaffSpawn _staff _output_get)
  (if (== _returnvalue 0)
    (for (_ _array_index) _inputarray
      (Utilities|Array|SetArrayElem _inputarray _array_index 0)))
  (Utilities|Array|SetArrayElem _inputarray _returnvalue (Math|Conversions|ToByte(Integer) _output_get))
  (bind _returnvalue_2 (Game|SpawnActorfromClass "/Game/Blueprints/GameObjects/Studio/BP_KeyActuator.BP_KeyActuator_C" (Math|Transform|MakeTransform (Transformation|GetActorLocation)) "Undefined" 0 0))
  (Variables|/Game/Blueprints/GameObjects/Studio/BP_KeyActuator.BP_KeyActuator_C|SetMidiParent _returnvalue_2 self)
  (bind _asbp_pant_controller_2 (Utilities|Casting|CastToBP_PantController (Game|GetPlayerCharacter 0)))
  (Default|KeyPress _returnvalue_2 (Utilities|String|StringToName (Utilities|String|ToString(Object) (Variables|/Game/PantControllerBP/Blueprints/BP_PantController.BP_PantController_C|GetPokeComponent _asbp_pant_controller_2))))
  (if (Variables|/Game/Blueprints/GameObjects/Studio/BP_MusicStaff.BP_MusicStaff_C|GetActivated (Variables|Default|GetStaff))
    (bind _array_element (Utilities|Array|ForEachLoopwithBreak (Variables|Default|GetSpeakers))
      (:LoopBody
        (Components|Timeline|SetPlayRate (Variables|/Game/Blueprints/GameObjects/Studio/BP_SpeakerBlock.BP_SpeakerBlock_C|GetTL_Vibrate1 _array_element) (Math|Float|Lerp 0.78 1.12 (/ (Math|Conversions|ToFloat(Integer) (Utilities|String|Replace (Utilities|String|ToString(Name) (Utilities|String|StringToName (Utilities|String|ToString(Object) (Variables|/Game/PantControllerBP/Blueprints/BP_PantController.BP_PantController_C|GetPokeComponent _asbp_pant_controller_2)))) "Key")) 25.0)))
        (Components|Timeline|PlayfromStart (Variables|/Game/Blueprints/GameObjects/Studio/BP_SpeakerBlock.BP_SpeakerBlock_C|GetTL_Vibrate1 _array_element)))
      (:Completed
        (bind _array_element_2 (Utilities|Array|ForEachLoopwithBreak (Variables|Default|GetSoundWaves))
          (:LoopBody
            (Components|Timeline|SetPlayRate (Variables|/Game/Blueprints/GameObjects/Studio/BP_SoundWave.BP_SoundWave_C|GetTL_Vibrate1 _array_element_2) (Math|Float|Lerp 0.78 1.12 (/ (Math|Conversions|ToFloat(Integer) (Utilities|String|Replace (Utilities|String|ToString(Name) (Utilities|String|StringToName (Utilities|String|ToString(Object) (Variables|/Game/PantControllerBP/Blueprints/BP_PantController.BP_PantController_C|GetPokeComponent _asbp_pant_controller_2)))) "Key")) 25.0)))
            (Components|Timeline|PlayfromStart (Variables|/Game/Blueprints/GameObjects/Studio/BP_SoundWave.BP_SoundWave_C|GetTL_Vibrate1 _array_element_2)))
          (:Completed
            (if (== (Variables|/Game/Blueprints/GameObjects/Studio/BP_MusicStaff.BP_MusicStaff_C|GetIndex (Variables|Default|GetStaff)) 8)
              (Default|CheckInput (Variables|Default|GetStaff)))))))))

(fn ConstructionScript)

(fn Attachto
  (params (ChildActor :type Actor%20Object%20Reference))
  (return 0))

(fn CanGrab
  (return false))

(fn Clicked
  (return false))

(fn DisableCollision
  (return false))

(fn DoesParentHaveParent
  (return false))

(fn EnableCollision
  (return false))

(fn GetAttached
  (return 0))

(fn GetCustomCursor
  (return false 0))

(fn GetShrinkScale
  (return "0, 0, 0" "0, 0, 0"))

(fn GetSnapLoc
  (params (CursorLoc :type Vector :default "0, 0, 0"))
  (return "0, 0, 0" "0, 0, 0"))

(fn Grabbed
  (return 0))

(fn LetGo
  (params (ParentComponent :type Actor%20Component%20Object%20Reference) (ParentActor :type Actor%20Object%20Reference))
  (return false))

(fn OnHover
  (return false))

(fn PassChildAlong
  (return 0 0))