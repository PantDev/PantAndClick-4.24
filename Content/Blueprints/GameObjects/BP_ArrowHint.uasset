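; BP_ArrowHint is an arrow hint actor that shrinks out of sight when a BP_PantController capsule enters its sphere and reappears when it leaves.
; Sphere overlaps play the TL_Scale timeline forward or in reverse to lerp mesh scale, hiding the mesh after shrinking.
; A TL_SpawnHover timeline drives height and scale, yielding scale control while the ScalingDown flag is set.
; The construction script applies Radius to the trigger sphere.
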(event OnComponentBeginOverlap(Sphere)
  (params (OverlappedComponent :type Primitive%20Component%20Object%20Reference) (OtherActor :type Actor%20Object%20Reference) (OtherComp :type Primitive%20Component%20Object%20Reference) (OtherBodyIndex :type Integer) (bFromSweep :type Boolean) (SweepResult :type Hit%20Result%20Structure%20%28by%20ref%29))
  (if (== (Utilities|GetClass OtherActor) "/Game/PantControllerBP/Blueprints/BP_PantController.BP_PantController_C")
    (bind _asbp_pant_controller (Utilities|Casting|CastToBP_PantController OtherActor))
    (if (== OtherComp (Variables|/Game/PantControllerBP/Blueprints/BP_PantController.BP_PantController_C|GetCapsule _asbp_pant_controller))
      (Variables|Default|SetScalingDown true)
      (Components|Timeline|PlayfromStart (Variables|Default|GetTL_Scale)))))

(event OnComponentEndOverlap(Sphere)
  (params (OverlappedComponent :type Primitive%20Component%20Object%20Reference) (OtherActor :type Actor%20Object%20Reference) (OtherComp :type Primitive%20Component%20Object%20Reference) (OtherBodyIndex :type Integer))
  (if (== (Utilities|GetClass OtherActor) "/Game/PantControllerBP/Blueprints/BP_PantController.BP_PantController_C")
    (bind _asbp_pant_controller (Utilities|Casting|CastToBP_PantController OtherActor))
    (if (== OtherComp (Variables|/Game/PantControllerBP/Blueprints/BP_PantController.BP_PantController_C|GetCapsule _asbp_pant_controller))
      (Variables|Default|SetScalingDown true)
      (Components|Timeline|ReversefromEnd (Variables|Default|GetTL_Scale))
      (Rendering|SetVisibility (Variables|Default|GetStaticMesh) true false))))

(fn ConstructionScript
  (Components|Sphere|SetSphereRadius (Variables|Default|GetSphere) (Variables|Default|GetRadius) true))