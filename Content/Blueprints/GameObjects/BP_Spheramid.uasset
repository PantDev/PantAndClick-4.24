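; BP_Spheramid is an actor with a skeletal mesh and rotating movement, holding distortion and bobbing animation logic that is currently disconnected.
; BeginPlay and the construction script are empty, so neither timeline chain runs.
; The distortion chain would, after a delay, drive three morph targets and a fast yaw spin from one timeline, then stop rotation.
; The bobbing chain would move the mesh vertically, replaying at random speeds.
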(event EventBeginPlay)

(fn ConstructionScript)