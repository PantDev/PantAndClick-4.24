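; Ceiling fan prop that spins its blades and toggles between spinning up and down when poked.
; A poke plays the switch movement timeline with a pitch-varied click, then flip-flops the rotator timeline between reverse and forward.
; That timeline ramps the yaw rate applied on Tick, disabling Tick once fully stopped.
; Collision and shadows are configurable; grab and attach interface functions are empty stubs.
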(event EventBeginPlay
  (bind _box (Variables|Default|GetBox))
  (Components|Timeline|SetNewTime (Variables|Default|GetTL_Rotator) 2.0)
  (if (Variables|Default|GetNoClick)
    (Collision|SetCollisionEnabled _box "NoCollision")
    (else
      (Collision|SetCollisionEnabled _box "QueryAndPhysics"))))

(event Collision|EventActorBeginOverlap
  (params (OtherActor :type Actor%20Object%20Reference)))

(event EventPokeEvent
  (bind _tl_rotator (Variables|Default|GetTL_Rotator))
  (if (not (Audio|Components|Audio|IsPlaying (Variables|Default|GetTL_UseSwitch)))
    (Components|Timeline|PlayfromStart (Variables|Default|GetTL_UseSwitch))
    (Audio|SpawnSoundatLocation "/Game/Audio/SFX/Switch1.Switch1" (Transformation|GetActorLocation) "0, 0, 0" 1.0 (Math|Random|RandomFloatinRange 0.85 1.05) 0.0 "/Game/Audio/Attenuation/SA_ShortRange.SA_ShortRange" "/Game/Audio/Attenuation/SC_Default.SC_Default")
    (Utilities|FlowControl|FlipFlop
      (:A
        (Utilities|String|Reverse _tl_rotator))
      (:B
        (Audio|Components|Audio|Play _tl_rotator)))))

(event EventTick
  (params (DeltaSeconds :type Float%20%28single-precision%29))
  (Transformation|AddLocalRotation (Variables|Default|GetBlades) (* (Math|Rotator|MakeRotator 0.0 0.0 (Variables|Default|GetRotRate)) DeltaSeconds) false false))

(fn ConstructionScript
  (Rendering|SetCastShadow (Variables|Default|GetBase) (Variables|Default|GetCastShadow)))

(fn Attachto
  (params (ChildActor :type Actor%20Object%20Reference))
  (return 0))

(fn CanGrab
  (return false))

(fn Clicked
  (return false))

(fn DisableCollision
  (return false))

(fn DoesParentHaveParent
  (return false))

(fn EnableCollision
  (return false))

(fn GetAttached
  (return 0))

(fn GetCustomCursor
  (return false 0))

(fn GetShrinkScale
  (return "0, 0, 0" "0, 0, 0"))

(fn GetSnapLoc
  (params (CursorLoc :type Vector :default "0, 0, 0"))
  (return "0, 0, 0" "0, 0, 0"))

(fn Grabbed
  (return 0))

(fn LetGo
  (params (ParentComponent :type Actor%20Component%20Object%20Reference) (ParentActor :type Actor%20Object%20Reference))
  (return false))

(fn OnHover
  (return false))

(fn PassChildAlong
  (return 0 0))