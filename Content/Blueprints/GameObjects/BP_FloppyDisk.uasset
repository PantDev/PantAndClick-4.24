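; Collectible floppy disk pickup that bobs in place and, when collected, notifies BP_PantController to update the floppy UI and count.
; A 30 Hz looping timer traces downward to keep a Blob marker aligned to the ground below.
; Collect disables collision, then chained timelines raise, spin up and rescale the disk before sound, particles and destruction.
; Construction applies scale and a tinted dynamic material; the random color-shift logic is disconnected.
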(event Custom|CollectEvent
  (Audio|Components|Audio|Stop (Variables|Default|GetBobbingAnimTL))
  (Collision|SetCollisionEnabled (Variables|Default|GetSphere) "NoCollision")
  (Components|Timeline|PlayfromStart (Variables|Default|GetCollectTL))
  (Utilities|FlowControl|Delay 0.6)
  (Components|Timeline|PlayfromStart (Variables|Default|GetPostCollectTL))
  (bind _asbp_pant_controller (Utilities|Casting|CastToBP_PantController (Variables|Default|GetPlayerCharacter)))
  (Default|FloppyWait _asbp_pant_controller)
  (if (Variables|/Game/PantControllerBP/Blueprints/BP_PantController.BP_PantController_C|GetFloppyHidden _asbp_pant_controller)
    (Default|Show/HideFilePanel _asbp_pant_controller true)
    (UserInterface|Animation|PlayAnimation (Variables|/Game/PantControllerBP/Blueprints/BP_PantController.BP_PantController_C|GetFloppyDiskWidget _asbp_pant_controller) (Variables|/Game/UserInterface/FloppyTotal_Widget.FloppyTotal_Widget_C|GetCollectPop (Variables|/Game/PantControllerBP/Blueprints/BP_PantController.BP_PantController_C|GetFloppyDiskWidget _asbp_pant_controller)) 0.0 1 "Forward" 1.0 false)
    (Math|Integer|IncrementInt (Variables|/Game/PantControllerBP/Blueprints/BP_PantController.BP_PantController_C|GetFloppyCount _asbp_pant_controller))))

(event Custom|ColorShiftEvent)

(event EventBeginPlay
  (Components|Timeline|PlayfromStart (Variables|Default|GetBobbingAnimTL))
  (Utilities|Time|SetTimerbyFunctionName 0 "TickFunc" 0.033333 true)
  (CallFunction|ColorShiftEvent))

(event EventCollect
  (params (PlayerCharacter :type BP%20Pant%20Controller%20Object%20Reference))
  (Variables|Default|SetPlayerCharacter PlayerCharacter)
  (CallFunction|CollectEvent))

(fn ConstructionScript
  (bind _returnvalue (Transformation|GetActorLocation))
  (bind (_x _y _z) (Math|Vector|BreakVector _returnvalue))
  (Transformation|SetActorScale3D (Variables|Default|GetScale))
  (bind _returnvalue_2 (Rendering|Material|CreateDynamicMaterialInstance (Variables|Default|GetStaticMesh) 0 0 "None" :!class /Script/Engine.PrimitiveComponent))
  (bind _output_get (Variables|Default|SetDynamicMat _returnvalue_2))
  (Rendering|Material|SetMaterial (Variables|Default|GetStaticMesh) 0 _output_get)
  (Rendering|Material|SetVectorParameterValue (Variables|Default|GetDynamicMat) "Color" (Variables|Default|GetColor) :!class /Script/Engine.MaterialInstanceDynamic)
  (bind (_outhit _returnvalue_3) (Collision|LineTraceByChannel _returnvalue (Math|Vector|MakeVector _x _y (- _z 1e+04)) "TraceTypeQuery1" false 0 "None"))
  (if _returnvalue_3
    (Transformation|SetWorldLocationAndRotation (Variables|Default|GetBlob) (.Location (Collision|BreakHitResult _outhit)) (Math|Rotator|MakeRotfromZ (.ImpactNormal (Collision|BreakHitResult _outhit))) false false)))

(fn TickFunc
  (bind _returnvalue (Transformation|GetActorLocation))
  (bind (_x _y _z) (Math|Vector|BreakVector _returnvalue))
  (bind (_outhit _returnvalue_2) (Collision|LineTraceByChannel _returnvalue (Math|Vector|MakeVector _x _y (- _z 1e+04)) "TraceTypeQuery1" false (Utilities|Array|MakeArray (Game|GetPlayerCharacter 0)) "None"))
  (if _returnvalue_2
    (Transformation|SetWorldLocationAndRotation (Variables|Default|GetBlob) (Math|Vector|MakeVector (.X (Math|Vector|BreakVector (.Location (Collision|BreakHitResult _outhit)))) (.Y (Math|Vector|BreakVector (.Location (Collision|BreakHitResult _outhit)))) (+ (.Z (Math|Vector|BreakVector (.Location (Collision|BreakHitResult _outhit)))) 5.0)) (Math|Rotator|MakeRotfromZ (.ImpactNormal (Collision|BreakHitResult _outhit))) false false)
    (Rendering|SetVisibility (Variables|Default|GetBlob) true false)
    (else
      (Rendering|SetVisibility (Variables|Default|GetBlob) false false))))