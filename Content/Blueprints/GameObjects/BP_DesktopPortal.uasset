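; Computer monitor portal that takes the player to another level, optionally locked behind a floppy count.
; Poking it plays a letterboxed unlock sequence or denied feedback; once unlocked, pokes power it on or cycle its screen image.
; An outer sphere shows the lock popup and powers down on exit; the inner sphere saves progress, sweeps the camera and async-loads Level0.
; Timelines drive morph-target ripples, light beams and dynamic-material screen effects.
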(event OnComponentBeginOverlap(Sphere)
  (params (OverlappedComponent :type Primitive%20Component%20Object%20Reference) (OtherActor :type Actor%20Object%20Reference) (OtherComp :type Primitive%20Component%20Object%20Reference) (OtherBodyIndex :type Integer) (bFromSweep :type Boolean) (SweepResult :type Hit%20Result%20Structure%20%28by%20ref%29))
  (bind _returnvalue (Game|GetPlayerController 0))
  (bind _tl_cameraanim (Variables|Default|GetTL_CameraAnim))
  (if (Variables|Default|GetPoweredOn)
    (bind _asbp_pant_controller (Utilities|Casting|CastToBP_PantController OtherActor))
    (if (not (Variables|/Game/PantControllerBP/Blueprints/BP_PantController.BP_PantController_C|GetIsIntro _asbp_pant_controller))
      (Utilities|IsValid _asbp_pant_controller
        (:Is%20Valid
          (Utilities|FlowControl|DoOnce false
            (:Completed
              (Rendering|SetVisibility (Variables|/Game/PantControllerBP/Blueprints/BP_PantController.BP_PantController_C|GetDenimMesh _asbp_pant_controller) false true)
              (Components|Timeline|PlayfromStart (Variables|Default|GetTL_PokeRipple))
              (Input|DisableInput _asbp_pant_controller _returnvalue)
              (AI|Navigation|StopMovement _returnvalue)
              (bind _asbp_pant_controller_2 (Utilities|Casting|CastToBP_PantController (Game|GetPlayerCharacter 0)))
              (Variables|/Script/Engine.MovementComponent|SetVelocity (Variables|/Script/Engine.Character|GetCharacterMovement _asbp_pant_controller_2) "0, 0, 0")
              (Pawn|Components|CharacterMovement|SetMovementMode (Variables|/Script/Engine.Character|GetCharacterMovement _asbp_pant_controller_2) "MOVE_Flying" 0)
              (Audio|PlaySoundatLocation "/Game/Audio/SFX/ScreenSaverCube.ScreenSaverCube" (Transformation|GetActorLocation) "0, 0, 0" 0.6 1.35 0.1 "/Game/Audio/Attenuation/SA_ShortRange.SA_ShortRange" "/Game/Audio/Attenuation/SC_Default.SC_Default" 0)
              (Game|Player|SetViewTargetwithBlend (Game|GetPlayerController 0) self 1.0 "VTBlend_EaseInOut" 2.0 false)
              (Audio|PlaySoundatLocation "/Game/Audio/SFX/MonitorEnter.MonitorEnter" (Transformation|GetActorLocation) "0, 0, 0" 0.36 1.0 0.0 "/Game/Audio/Attenuation/SA_Default.SA_Default" "/Game/Audio/Attenuation/SC_Default.SC_Default" 0)
              (Components|Timeline|SetPlayRate _tl_cameraanim 0.75)
              (Components|Timeline|PlayfromStart _tl_cameraanim)
              (bind _asbp_pant_controller_3 (Utilities|Casting|CastToBP_PantController (Game|GetPlayerCharacter 0)))
              (Variables|/Game/Data/SaveGame/SGO_SaveGame.SGO_SaveGame_C|SetFileCount (Variables|/Game/Data/SaveGame/BP_SaveManager.BP_SaveManager_C|GetSGO%20SaveGame (Variables|/Game/PantControllerBP/Blueprints/BP_PantController.BP_PantController_C|GetSaveManager _asbp_pant_controller_3)) (Variables|/Game/PantControllerBP/Blueprints/BP_PantController.BP_PantController_C|GetFileCount _asbp_pant_controller_3))
              (Variables|/Game/Data/SaveGame/SGO_SaveGame.SGO_SaveGame_C|SetFloppyCount (Variables|/Game/Data/SaveGame/BP_SaveManager.BP_SaveManager_C|GetSGO%20SaveGame (Variables|/Game/PantControllerBP/Blueprints/BP_PantController.BP_PantController_C|GetSaveManager _asbp_pant_controller_3)) (Variables|/Game/PantControllerBP/Blueprints/BP_PantController.BP_PantController_C|GetFloppyTotal _asbp_pant_controller_3))
              (SaveGame|SaveGametoSlot (Variables|/Game/Data/SaveGame/BP_SaveManager.BP_SaveManager_C|GetSGO%20SaveGame (Variables|/Game/PantControllerBP/Blueprints/BP_PantController.BP_PantController_C|GetSaveManager _asbp_pant_controller_3)) (Variables|/Game/Data/SaveGame/BP_SaveManager.BP_SaveManager_C|GetSaveName (Variables|/Game/PantControllerBP/Blueprints/BP_PantController.BP_PantController_C|GetSaveManager _asbp_pant_controller_3))))))))))

(event OnComponentBeginOverlap(Sphere1)
  (params (OverlappedComponent :type Primitive%20Component%20Object%20Reference) (OtherActor :type Actor%20Object%20Reference) (OtherComp :type Primitive%20Component%20Object%20Reference) (OtherBodyIndex :type Integer) (bFromSweep :type Boolean) (SweepResult :type Hit%20Result%20Structure%20%28by%20ref%29))
  (bind _tl_lockpopup (Variables|Default|GetTL_LockPopup))
  (bind _asbp_pant_controller (Utilities|Casting|CastToBP_PantController OtherActor))
  (if (not (Variables|/Game/PantControllerBP/Blueprints/BP_PantController.BP_PantController_C|GetIsIntro _asbp_pant_controller))
    (if (and (== OtherComp (Variables|/Game/PantControllerBP/Blueprints/BP_PantController.BP_PantController_C|GetCapsule _asbp_pant_controller)) (Variables|Default|GetLocked))
      (Audio|PlaySoundatLocation "/Game/Audio/SFX/FloppyLockDisp.FloppyLockDisp" (Transformation|GetActorLocation) "0, 0, 0" 0.2 1.12 0.0 "/Game/Audio/Attenuation/SA_ShortRange.SA_ShortRange" 0 0)
      (Audio|Components|Audio|Stop (Variables|Default|GetTL_LockHover))
      (Rendering|SetVisibility (Variables|Default|GetTextRender1) true false)
      (Components|Timeline|SetPlayRate _tl_lockpopup 0.7)
      (Components|Timeline|PlayfromStart _tl_lockpopup))))

(event OnComponentEndOverlap(Sphere1)
  (params (OverlappedComponent :type Primitive%20Component%20Object%20Reference) (OtherActor :type Actor%20Object%20Reference) (OtherComp :type Primitive%20Component%20Object%20Reference) (OtherBodyIndex :type Integer))
  (bind _tl_lightscale (Variables|Default|GetTL_LightScale))
  (bind _asbp_pant_controller (Utilities|Casting|CastToBP_PantController OtherActor))
  (if (not (Variables|/Game/PantControllerBP/Blueprints/BP_PantController.BP_PantController_C|GetIsIntro _asbp_pant_controller))
    (if (and (== OtherComp (Variables|/Game/PantControllerBP/Blueprints/BP_PantController.BP_PantController_C|GetCapsule _asbp_pant_controller)) (Variables|Default|GetPoweredOn))
      (Audio|PlaySoundatLocation "/Game/Audio/SFX/FloppyLockDisp.FloppyLockDisp" (Transformation|GetActorLocation) "0, 0, 0" 0.2 0.6 0.3 "/Game/Audio/Attenuation/SA_ShortRange.SA_ShortRange" 0 0)
      (Components|Timeline|SetPlayRate _tl_lightscale 1.0)
      (Components|Timeline|ReversefromEnd _tl_lightscale)
      (Variables|Default|SetPoweredOn false)
      (elif (and (== OtherComp (Variables|/Game/PantControllerBP/Blueprints/BP_PantController.BP_PantController_C|GetCapsule _asbp_pant_controller)) (Variables|Default|GetLocked))
        (Components|Timeline|SetPlayRate (Variables|Default|GetTL_LockPopup) 1.0)
        (Components|Timeline|ReversefromEnd (Variables|Default|GetTL_LockPopup))))))

(event Custom|RemoteEnter
  (bind _tl_cameraanim (Variables|Default|GetTL_CameraAnim))
  (Audio|PlaySoundatLocation "/Game/Audio/SFX/ScreenSaverCube.ScreenSaverCube" (Transformation|GetActorLocation) "0, 0, 0" 0.6 1.35 0.1 "/Game/Audio/Attenuation/SA_ShortRange.SA_ShortRange" "/Game/Audio/Attenuation/SC_Default.SC_Default" 0)
  (Game|Player|SetViewTargetwithBlend (Game|GetPlayerController 0) self 1.0 "VTBlend_EaseInOut" 2.0 false)
  (Audio|PlaySoundatLocation "/Game/Audio/SFX/MonitorEnter.MonitorEnter" (Transformation|GetActorLocation) "0, 0, 0" 0.36 1.0 0.0 "/Game/Audio/Attenuation/SA_Default.SA_Default" "/Game/Audio/Attenuation/SC_Default.SC_Default" 0)
  (Components|Timeline|SetPlayRate _tl_cameraanim 0.75)
  (Components|Timeline|PlayfromStart _tl_cameraanim)
  (bind _asbp_pant_controller (Utilities|Casting|CastToBP_PantController (Game|GetPlayerCharacter 0)))
  (Variables|/Game/Data/SaveGame/SGO_SaveGame.SGO_SaveGame_C|SetFileCount (Variables|/Game/Data/SaveGame/BP_SaveManager.BP_SaveManager_C|GetSGO%20SaveGame (Variables|/Game/PantControllerBP/Blueprints/BP_PantController.BP_PantController_C|GetSaveManager _asbp_pant_controller)) (Variables|/Game/PantControllerBP/Blueprints/BP_PantController.BP_PantController_C|GetFileCount _asbp_pant_controller))
  (Variables|/Game/Data/SaveGame/SGO_SaveGame.SGO_SaveGame_C|SetFloppyCount (Variables|/Game/Data/SaveGame/BP_SaveManager.BP_SaveManager_C|GetSGO%20SaveGame (Variables|/Game/PantControllerBP/Blueprints/BP_PantController.BP_PantController_C|GetSaveManager _asbp_pant_controller)) (Variables|/Game/PantControllerBP/Blueprints/BP_PantController.BP_PantController_C|GetFloppyTotal _asbp_pant_controller))
  (SaveGame|SaveGametoSlot (Variables|/Game/Data/SaveGame/BP_SaveManager.BP_SaveManager_C|GetSGO%20SaveGame (Variables|/Game/PantControllerBP/Blueprints/BP_PantController.BP_PantController_C|GetSaveManager _asbp_pant_controller)) (Variables|/Game/Data/SaveGame/BP_SaveManager.BP_SaveManager_C|GetSaveName (Variables|/Game/PantControllerBP/Blueprints/BP_PantController.BP_PantController_C|GetSaveManager _asbp_pant_controller))))

(event Custom|SpawnPlayerEvent
  (bind _returnvalue (Game|GetPlayerController 0))
  (bind _spawncam (Variables|Default|GetSpawnCam))
  (bind _flybycam (Variables|Default|GetFlyByCam))
  (Utilities|IsValid _flybycam
    (:Is%20Valid
      (Game|Player|SetViewTargetwithBlend (Game|GetPlayerController 0) _flybycam 0.0 "VTBlend_Linear" 0.0 false)
      (Utilities|FlowControl|Delay 3.3)
      (bind _asbp_pant_controller (Utilities|Casting|CastToBP_PantController (Game|GetPlayerCharacter 0)))
      (Variables|/Game/PantControllerBP/Blueprints/BP_PantController.BP_PantController_C|SetForceLoad _asbp_pant_controller true)
      (Utilities|FlowControl|Delay 1.7)
      (Game|Player|SetViewTargetwithBlend _returnvalue _spawncam 2.0 "VTBlend_EaseInOut" 1e+01 false))
    (:Is%20Not%20Valid
      (Game|Player|SetViewTargetwithBlend _returnvalue _spawncam 0.01 "VTBlend_EaseInOut" 1e+03 false)))
  (Rendering|SetVisibility (Variables|Default|GetMyComputer_LightBeams) true false)
  (bind _returnvalue_2 (Rendering|Material|CreateDynamicMaterialInstance (Variables|Default|GetSkeletalMesh) 0 "/Game/UserInterface/Images/ComputerMonitor_Mat.ComputerMonitor_Mat" "None" :!class /Script/Engine.PrimitiveComponent))
  (bind _output_get (Variables|Default|SetMat _returnvalue_2))
  (Rendering|Material|SetTextureParameterValue _output_get "Texture" (Variables|Default|GetDisplayTexture))
  (Components|Timeline|SetPlayRate (Variables|Default|GetTL_LightScale) 0.3)
  (Variables|Default|SetPoweredOn true))

(event Custom|RemoteDisable
  (bind _tl_lightscale (Variables|Default|GetTL_LightScale))
  (Audio|PlaySoundatLocation "/Game/Audio/SFX/FloppyLockDisp.FloppyLockDisp" (Transformation|GetActorLocation) "0, 0, 0" 0.2 0.6 0.3 "/Game/Audio/Attenuation/SA_ShortRange.SA_ShortRange" 0 0)
  (Components|Timeline|SetPlayRate _tl_lightscale 1.0)
  (Components|Timeline|ReversefromEnd _tl_lightscale)
  (Variables|Default|SetPoweredOn false))

(event EventBeginPlay
  (bind _returnvalue (UserInterface|CreateWidget "/Game/UserInterface/HourglassTransition_Widget.HourglassTransition_Widget_C"))
  (Variables|Default|SetNewVar_0 _returnvalue))

(event EventPokeEvent
  (bind _returnvalue (Transformation|GetActorLocation))
  (bind _returnvalue_2 (Transformation|GetActorLocation))
  (bind _returnvalue_3 (Transformation|GetActorLocation))
  (bind _tl_pokeripple (Variables|Default|GetTL_PokeRipple))
  (bind _tl_lightscale (Variables|Default|GetTL_LightScale))
  (if (Variables|Default|GetLocked)
    (bind _asbp_pant_controller (Utilities|Casting|CastToBP_PantController (Game|GetPlayerCharacter 0)))
    (if (>= (Variables|/Game/PantControllerBP/Blueprints/BP_PantController.BP_PantController_C|GetFloppyTotal _asbp_pant_controller) (Variables|Default|GetLockNum))
      (Utilities|FlowControl|Sequence
        (:then_0
          (Input|DisableInput (Game|GetPlayerCharacter 0) (Game|GetPlayerController 0))
          (Class|UserWidget|StopAllAnimations (Variables|/Game/PantControllerBP/Blueprints/BP_PantController.BP_PantController_C|GetFloppyCounter _asbp_pant_controller))
          (UserInterface|Animation|PlayAnimation (Variables|/Game/PantControllerBP/Blueprints/BP_PantController.BP_PantController_C|GetFloppyCounter _asbp_pant_controller) (Variables|/Game/UserInterface/FloppyCounterNew_Widget.FloppyCounterNew_Widget_C|GetUnlock (Variables|/Game/PantControllerBP/Blueprints/BP_PantController.BP_PantController_C|GetFloppyCounter _asbp_pant_controller)) 0.0 1 "Forward" 1.0 false)
          (Timeline|TL_UnlockEvents PlayFromStart
            (:Finished
              (Variables|Default|SetLocked false)
              (bind _asbp_pant_controller_2 (Utilities|Casting|CastToBP_PantController (Game|GetPlayerCharacter 0)))
              (Audio|PlaySoundatLocation "/Game/Audio/SFX/EthernetMoving1.EthernetMoving1" _returnvalue "0, 0, 0" 0.8 1.5 1.55 "/Game/Audio/Attenuation/SA_ShortRange.SA_ShortRange" "/Game/Audio/Attenuation/SC_Default.SC_Default" 0 :!label _label)
              (Audio|PlaySoundatLocation "/Game/Audio/SFX/ScreenSaverCube.ScreenSaverCube" _returnvalue "0, 0, 0" 0.6 1.35 0.1 "/Game/Audio/Attenuation/SA_ShortRange.SA_ShortRange" "/Game/Audio/Attenuation/SC_Default.SC_Default" 0)
              (bind _returnvalue_4 (Rendering|Material|CreateDynamicMaterialInstance (Variables|Default|GetSkeletalMesh) 0 "/Game/UserInterface/Images/ComputerMonitor_Mat.ComputerMonitor_Mat" "None" :!class /Script/Engine.PrimitiveComponent))
              (bind _output_get (Variables|Default|SetMat _returnvalue_4))
              (Rendering|Material|SetTextureParameterValue _output_get "Texture" (Variables|Default|GetDisplayTexture))
              (Components|Timeline|SetPlayRate _tl_lightscale 0.3)
              (Components|Timeline|PlayfromStart _tl_lightscale)
              (Rendering|SetVisibility (Variables|Default|GetMyComputer_LightBeams) true false)
              (Variables|Default|SetPoweredOn true)
              (Rendering|Material|SetScalarParameterValue (Variables|Default|GetMat) "ImageIndex" (Math|Conversions|ToFloat(Integer) (Variables|Default|GetDisplayedImage)) :!class /Script/Engine.MaterialInstanceDynamic)
              (bind _asbp_pant_controller_3 (Utilities|Casting|CastToBP_PantController (Game|GetPlayerCharacter 0)))
              (Default|HideSecondary _asbp_pant_controller_3))
            (:Event1
              (Components|Timeline|ReversefromEnd (Variables|Default|GetTL_LockPopup))
              (Audio|PlaySoundatLocation "/Game/Audio/SFX/DuckGet.DuckGet" _returnvalue_3 "0, 0, 0" 1.0 1.0 0.2 "/Game/Audio/Attenuation/SA_ShortRange.SA_ShortRange" 0 0))
            (:Event2
              (Audio|PlaySoundatLocation "/Game/Audio/SFX/ActivateJingle2.ActivateJingle2" _returnvalue_3 "0, 0, 0" 1.0 1.0 0.1 "/Game/Audio/Attenuation/SA_ShortRange.SA_ShortRange" 0 0))))
        (:then_1
          (Utilities|FlowControl|Delay 0.2)
          (bind _returnvalue_5 (UserInterface|CreateWidget "/Game/UserInterface/Letterbox_Widget.Letterbox_Widget_C" (Game|GetPlayerController 0)))
          (bind _output_get_2 (Variables|Default|SetLetterbox _returnvalue_5))
          (UserInterface|Viewport|AddtoViewport _output_get_2 0)
          (UserInterface|Animation|PlayAnimation (Variables|Default|GetLetterbox) (Variables|/Game/UserInterface/Letterbox_Widget.Letterbox_Widget_C|GetFadeIn (Variables|Default|GetLetterbox)) 0.0 1 "Forward" 0.5 false)
          (bind _asbp_pant_controller_4 (Utilities|Casting|CastToBP_PantController (Game|GetPlayerCharacter 0)))
          (Widget|SetVisibility (Variables|/Game/PantControllerBP/Blueprints/BP_PantController.BP_PantController_C|GetFileCounterWidget _asbp_pant_controller_4) "Hidden")
          (Audio|Components|Audio|Stop (Variables|/Game/PantControllerBP/Blueprints/BP_PantController.BP_PantController_C|GetTL_SpeechBubbleStay _asbp_pant_controller_4))
          (if (Variables|/Game/PantControllerBP/Blueprints/BP_PantController.BP_PantController_C|GetIsBubbleOpen _asbp_pant_controller_4)
            (Default|CloseSpeechBubble _asbp_pant_controller_4)
            (Widget|SetVisibility (Variables|/Game/PantControllerBP/Blueprints/BP_PantController.BP_PantController_C|GetSpeechBubbleWidget _asbp_pant_controller_4) "Hidden")))
        (:then_2
          (Utilities|FlowControl|Delay 4.0)
          (UserInterface|Animation|PlayAnimation (Variables|Default|GetLetterbox) (Variables|/Game/UserInterface/Letterbox_Widget.Letterbox_Widget_C|GetFadeIn (Variables|Default|GetLetterbox)) 0.0 1 "Reverse" 1.0 false)
          (Utilities|FlowControl|Delay 0.2)
          (bind _asbp_pant_controller_5 (Utilities|Casting|CastToBP_PantController (Game|GetPlayerCharacter 0)))
          (Widget|RemovefromParent (Variables|/Game/PantControllerBP/Blueprints/BP_PantController.BP_PantController_C|GetFloppyCounter _asbp_pant_controller_5))
          (Widget|SetVisibility (Variables|/Game/PantControllerBP/Blueprints/BP_PantController.BP_PantController_C|GetFloppyLineupWidget _asbp_pant_controller_5) "Visible")
          (Widget|RemovefromParent (Variables|Default|GetLetterbox))
          (bind _returnvalue_6 (UserInterface|CreateWidget "/Game/UserInterface/FloppyCounterNew_Widget.FloppyCounterNew_Widget_C" (Game|GetPlayerController 0)))
          (bind _output_get_3 (Variables|/Game/PantControllerBP/Blueprints/BP_PantController.BP_PantController_C|SetFloppyCounter _asbp_pant_controller_5 _returnvalue_6))
          (UserInterface|Viewport|AddtoViewport _output_get_3 0)
          (Input|EnableInput (Game|GetPlayerCharacter 0) (Game|GetPlayerController 0))))
      (else
        (Audio|PlaySoundatLocation "/Game/Audio/SFX/PopupSFX/SFX_PopupClose.SFX_PopupClose" (Transformation|GetActorLocation) "0, 0, 0" 0.085 0.6 0.15 "/Game/Audio/Attenuation/SA_ShortRange.SA_ShortRange" 0 0)
        (bind _alpha (Timeline|TL_Denied PlayFromStart)
          (:Update
            (Transformation|SetRelativeScale3D (Variables|Default|GetSpringArm1) (Math|Vector|Lerp(Vector) "1.000000,1.000000,1.000000" "1.200000,1.200000,1.200000" _alpha))))))
    (elif (Variables|Default|GetPoweredOn)
      (if (Audio|Components|Audio|IsPlaying _tl_pokeripple)
        (Audio|Components|Audio|Stop _tl_pokeripple))
      (Components|Timeline|SetPlayRate _tl_pokeripple 0.8)
      (Components|Timeline|PlayfromStart _tl_pokeripple)
      (Audio|PlaySoundatLocation "/Game/Audio/SFX/ScreenSaverCube.ScreenSaverCube" _returnvalue_2 "0, 0, 0" 0.8 1.35 0.1 "/Game/Audio/Attenuation/SA_ShortRange.SA_ShortRange" "/Game/Audio/Attenuation/SC_Default.SC_Default" 0)
      (if (== (Variables|Default|GetDisplayedImage) 3)
        (Variables|Default|SetDisplayedImage 0)
        (else
          (Variables|Default|SetDisplayedImage (+ (Variables|Default|GetDisplayedImage) 1))))
      (Audio|PlaySoundatLocation "/Game/Audio/SFX/EthernetMoving1.EthernetMoving1" _returnvalue_2 "0, 0, 0" 0.8 (Math|Random|RandomFloatinRange 0.8 1.2) 1.7 "/Game/Audio/Attenuation/SA_ShortRange.SA_ShortRange" "/Game/Audio/Attenuation/SC_Default.SC_Default" 0)
      (Rendering|Material|SetScalarParameterValue (Variables|Default|GetMat) "ImageIndex" (Math|Conversions|ToFloat(Integer) (Variables|Default|GetDisplayedImage)) :!class /Script/Engine.MaterialInstanceDynamic)
      (else
        (goto _label)))))

(fn ConstructionScript
  (Rendering|Components|TextRender|SetText (Variables|Default|GetTextRender1) (Utilities|Text|ToText(Integer) (Variables|Default|GetLockNum))))

(fn Attachto
  (params (ChildActor :type Actor%20Object%20Reference))
  (return 0))

(fn CanGrab
  (return false))

(fn Clicked
  (return false))

(fn DisableCollision
  (return false))

(fn DoesParentHaveParent
  (return false))

(fn EnableCollision
  (return false))

(fn GetAttached
  (return 0))

(fn GetCustomCursor
  (return false 0))

(fn GetShrinkScale
  (return "0, 0, 0" "0, 0, 0"))

(fn GetSnapLoc
  (params (CursorLoc :type Vector :default "0, 0, 0"))
  (return "0, 0, 0" "0, 0, 0"))

(fn Grabbed
  (return 0))

(fn IsBusy
  (return false))

(fn LetGo
  (params (ParentComponent :type Actor%20Component%20Object%20Reference) (ParentActor :type Actor%20Object%20Reference))
  (return false))

(fn OnHover
  (return false))

(fn PassChildAlong
  (return 0 0))

(fn RightClickEvent
  (return (Variables|Default|GetClick%20Message) (Transformation|GetWorldLocation (Variables|Default|GetSphere))))