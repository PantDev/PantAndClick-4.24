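; Target group actor that runs one wave of a chained target challenge, activating its Targets together and handing off to NextGroup.
; Timelines act as delays: one scaled by HoldTime keeps targets up, then their spawn animations reverse and a second precedes the next group.
; The first group also shows the target count widget on the player and dismisses the current NPC's dialogue.
; Later groups poke their MagVol and wait a camera delay before activating targets.
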(event EventBeginPlay)

(event Collision|EventActorBeginOverlap
  (params (OtherActor :type Actor%20Object%20Reference)))

(event EventTick
  (params (DeltaSeconds :type Float%20%28single-precision%29)))

(event EventActivate
  (params (Delay :type Float%20%28single-precision%29) (Bool :type Boolean))
  (if (Variables|Default|GetFirstGroup)
    (Utilities|FlowControl|Sequence
      (:then_0
        (bind _array_element (Utilities|Array|ForEachLoopwithBreak (Variables|Default|GetTargets) :!label _label)
          (:LoopBody
            (Default|Activate _array_element 0.0 false))
          (:Completed
            (Components|Timeline|SetPlayRate (Variables|Default|GetTL_Delay) (/ 1.0 (Variables|Default|GetHoldTime)))
            (Timeline|TL_Delay PlayFromStart
              (:Finished
                (bind _array_element_2 (Utilities|Array|ForEachLoopwithBreak (Variables|Default|GetTargets))
                  (:LoopBody
                    (bind _asbp_target (Utilities|Casting|CastToBP_Target _array_element_2))
                    (Components|Timeline|ReversefromEnd (Variables|/Game/Blueprints/GameObjects/BP_Target.BP_Target_C|GetTL_SpawnAnim _asbp_target)))
                  (:Completed
                    (Timeline|TL_Delay2 PlayFromStart
                      (:Finished
                        (Default|Activate (Variables|Default|GetNextGroup) 0.0 false))))))))))
      (:then_1
        (bind _returnvalue (UserInterface|CreateWidget "/Game/UserInterface/TargetCount_Widget.TargetCount_Widget_C" (Game|GetPlayerController 0)))
        (bind _asbp_pant_controller (Utilities|Casting|CastToBP_PantController (Game|GetPlayerCharacter 0)))
        (bind _output_get (Variables|/Game/PantControllerBP/Blueprints/BP_PantController.BP_PantController_C|SetTargetCountWidget _asbp_pant_controller _returnvalue))
        (UserInterface|Viewport|AddtoViewport _output_get 0)
        (UserInterface|Animation|PlayAnimation (Variables|/Game/PantControllerBP/Blueprints/BP_PantController.BP_PantController_C|GetTargetCountWidget _asbp_pant_controller) (Variables|/Game/UserInterface/TargetCount_Widget.TargetCount_Widget_C|GetStartAnim (Variables|/Game/PantControllerBP/Blueprints/BP_PantController.BP_PantController_C|GetTargetCountWidget _asbp_pant_controller)) 0.0 1 "Forward" 1.0 false)
        (Class|UserWidget|PlayAnimationReverse (Variables|/Game/Blueprints/GameObjects/BP_GregTest.BP_GregTest_C|GetDialogueBoxWidget (Variables|/Game/PantControllerBP/Blueprints/BP_PantController.BP_PantController_C|GetCurrentNPC _asbp_pant_controller)) (Variables|/Game/UserInterface/DialogueBox_Widget.DialogueBox_Widget_C|GetSpawn (Variables|/Game/Blueprints/GameObjects/BP_GregTest.BP_GregTest_C|GetDialogueBoxWidget (Variables|/Game/PantControllerBP/Blueprints/BP_PantController.BP_PantController_C|GetCurrentNPC _asbp_pant_controller))) 1.5 false)
        (Default|OffGreg (Variables|/Game/PantControllerBP/Blueprints/BP_PantController.BP_PantController_C|GetCurrentNPC _asbp_pant_controller))))
    (else
      (Default|PokeEvent (Variables|Default|GetMagVol))
      (Timeline|TL_CamDelay PlayFromStart
        (:Finished
          (goto _label))))))

(fn ConstructionScript)

(fn IsBusy
  (return false))