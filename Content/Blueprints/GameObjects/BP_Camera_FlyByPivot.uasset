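; Fly-by pivot camera actor with a spring arm that plays an intro zoom and can track a follow point.
; On BeginPlay a timeline eases FOV, arm length, relative rotation and a post-process intensity taken from a volume.
; Tick smoothly turns the camera along the look-at direction from the actor to FollowPoint, when valid.
; Activate blends the player's view to this actor; IsBusy always returns false.
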(event EventBeginPlay
  (bind _camera (Variables|Default|GetCamera))
  (Components|Timeline|SetPlayRate (Variables|Default|GetTL_IntroZoom) 1.2)
  (bind (_direction _alpha _alpha2) (Timeline|TL_IntroZoom PlayFromStart)
    (:Update
      (Camera|SetFieldOfView _camera (Math|Float|Lerp 5.5e+02 1e+02 _alpha))
      (Variables|/Script/Engine.CameraComponent|SetPostProcessSettings _camera (Utilities|Struct|MakePostProcessSettings (Math|Float|Lerp 1e+02 (Utilities|Struct|BreakPostProcessSettings (Variables|/Script/Engine.PostProcessVolume|GetSettings (Variables|Default|GetPostProcessVol))) _alpha2)))
      (Transformation|SetRelativeRotation (Variables|Default|GetCamera) (Math|Rotator|Lerp(Rotator) "10.000000,0.000000,-300.000000" "0, 0, 0" _alpha2 true) false false)
      (Variables|/Script/Engine.SpringArmComponent|SetTargetArmLength (Variables|Default|GetSpringArm) (Math|Float|Lerp (* (Variables|Default|GetTarget%20Arm%20Length) 3e+01) (Variables|Default|GetTarget%20Arm%20Length) _alpha)))))

(event Collision|EventActorBeginOverlap
  (params (OtherActor :type Actor%20Object%20Reference)))

(event EventTick
  (params (DeltaSeconds :type Float%20%28single-precision%29))
  (Utilities|IsValid (Variables|Default|GetFollowPoint)
    (:Is%20Valid
      (Transformation|SetWorldRotation (Variables|Default|GetCamera) (Math|Interpolation|RInterpTo (Transformation|GetWorldRotation (Variables|Default|GetCamera)) (Math|Rotator|FindLookatRotation (Transformation|GetActorLocation) (Transformation|GetActorLocation (Variables|Default|GetFollowPoint))) DeltaSeconds 16.0) false false))))

(event EventActivate
  (params (Delay :type Float%20%28single-precision%29) (Bool :type Boolean))
  (Game|Player|SetViewTargetwithBlend (Game|GetPlayerController 0) self 2.0 "VTBlend_EaseInOut" 5.0 false))

(fn ConstructionScript
  (Camera|SetFieldOfView (Variables|Default|GetCamera) (Variables|Default|GetFOV))
  (Variables|/Script/Engine.SpringArmComponent|SetTargetArmLength (Variables|Default|GetSpringArm) (Variables|Default|GetTarget%20Arm%20Length)))

(fn IsBusy
  (return false))