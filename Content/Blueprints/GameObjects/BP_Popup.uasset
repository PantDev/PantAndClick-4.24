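; BP_Popup is a 3D desktop-style popup window that maximizes or minimizes when poked, or when landed on while minimized.
; A timeline drives morph targets, collision box, title and content placement, while delay loops type and erase the text, optionally replaced by an image.
; Hidden popups scale in on Activate after an hourglass cursor delay.
; The first landing also activates linked actors at staggered delays, allowing chains.
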(event Custom|WindowTextType
  (Rendering|Components|TextRender|SetText (Variables|Default|GetTitleText) (Utilities|Text|ToText(String) (Variables|Default|GetWindowTitle)))
  (CallFunction|TitleTextType)
  (Utilities|FlowControl|Delay (Variables|Default|GetDelay) :!label _label)
  (if (Variables|Default|GetMaximized)
    (Utilities|FlowControl|Sequence
      (:then_0
        (bind _output_get (Variables|Default|SetWindowText_Disp (Utilities|String|GetSubstring (Variables|Default|GetWindowText_Max) 0 (+ (Utilities|String|Len (Variables|Default|GetWindowText_Disp)) 1))))
        (Rendering|Components|TextRender|SetText (Variables|Default|GetTextRender) (Utilities|Text|ToText(String) _output_get)))
      (:then_1
        (if (not (Utilities|Enum|Equal(Enum) (Variables|Default|GetWindowText_Max) (Variables|Default|GetWindowText_Disp)))
          (if (Variables|Default|GetBreak)
            (Variables|Default|SetBreak false :!label _label_2)
            (else
              (goto _label))))))
    (else
      (goto _label_2))))

(event Custom|WindowTextReverse
  (bind _windowtext_max (Variables|Default|GetWindowText_Max))
  (Variables|Default|SetBreak true)
  (CallFunction|TitleTextReverse)
  (Utilities|FlowControl|Delay 0.02 :!label _label)
  (if (Variables|Default|GetMaximized)
    (Variables|Default|SetBreak false :!label _label_2)
    (Utilities|FlowControl|Delay 0.12)
    (bind _output_get (Variables|Default|SetWindowText_Disp (Variables|Default|GetWindowText_Min)))
    (Rendering|Components|TextRender|SetText (Variables|Default|GetTextRender) (Utilities|Text|ToText(String) _output_get))
    (else
      (Utilities|FlowControl|Sequence
        (:then_0
          (if (< (Utilities|String|Len (Variables|Default|GetWindowText_Disp)) 6)
            (bind _output_get_2 (Variables|Default|SetWindowText_Disp (Utilities|String|GetSubstring _windowtext_max 0 (- (Utilities|String|Len (Variables|Default|GetWindowText_Disp)) 1))))
            (Rendering|Components|TextRender|SetText (Variables|Default|GetTextRender) (Utilities|Text|ToText(String) _output_get_2))
            (else
              (bind _output_get_3 (Variables|Default|SetWindowText_Disp (Utilities|String|GetSubstring _windowtext_max 0 (- (Utilities|String|Len (Variables|Default|GetWindowText_Disp)) (+ (/ (Utilities|String|Len (Variables|Default|GetWindowText_Max)) 8) 1)))))
              (Rendering|Components|TextRender|SetText (Variables|Default|GetTextRender) (Utilities|Text|ToText(String) _output_get_3)))))
        (:then_1
          (if (< (Utilities|String|Len (Variables|Default|GetWindowText_Disp)) 1)
            (goto _label_2)
            (else
              (goto _label))))))))

(event Custom|TitleTextType
  (Utilities|FlowControl|Delay (Variables|Default|GetTitleTypeDelay) :!label _label)
  (if (Variables|Default|GetMaximized)
    (Utilities|FlowControl|Sequence
      (:then_0
        (bind _output_get (Variables|Default|SetWindowTitle_Disp (Utilities|String|GetSubstring (Variables|Default|GetWindowTitle) 0 (+ (Utilities|String|Len (Variables|Default|GetWindowTitle_Disp)) 1))))
        (Rendering|Components|TextRender|SetText (Variables|Default|GetTitleText) (Utilities|Text|ToText(String) _output_get)))
      (:then_1
        (if (not (Utilities|Enum|Equal(Enum) (Variables|Default|GetWindowTitle) (Variables|Default|GetWindowTitle_Disp)))
          (if (Variables|Default|GetBreak)
            (Variables|Default|SetBreak false :!label _label_2)
            (else
              (goto _label))))))
    (else
      (goto _label_2))))

(event Custom|TitleTextReverse
  (bind _windowtitle (Variables|Default|GetWindowTitle))
  (Variables|Default|SetBreak true)
  (Utilities|FlowControl|Delay (Variables|Default|GetTitleTypeDelay) :!label _label)
  (if (not (Variables|Default|GetMaximized))
    (Utilities|FlowControl|Sequence
      (:then_0
        (if (< (Utilities|String|Len (Variables|Default|GetWindowTitle_Disp)) 6)
          (bind _output_get (Variables|Default|SetWindowTitle_Disp (Utilities|String|GetSubstring _windowtitle 0 (- (Utilities|String|Len (Variables|Default|GetWindowTitle_Disp)) 1))))
          (Rendering|Components|TextRender|SetText (Variables|Default|GetTitleText) (Utilities|Text|ToText(String) _output_get))
          (else
            (bind _output_get_2 (Variables|Default|SetWindowTitle_Disp (Utilities|String|GetSubstring _windowtitle 0 (- (Utilities|String|Len (Variables|Default|GetWindowTitle_Disp)) (+ (/ (Utilities|String|Len (Variables|Default|GetWindowTitle)) 24) 1)))))
            (Rendering|Components|TextRender|SetText (Variables|Default|GetTitleText) (Utilities|Text|ToText(String) _output_get_2)))))
      (:then_1
        (if (< (Utilities|String|Len (Variables|Default|GetWindowTitle_Disp)) 3)
          (Variables|Default|SetBreak false)
          (CallFunction|ClampText 3)
          (else
            (goto _label)))))))

(event Custom|Pop%20Up%20Event
  (bind (_x _y _z) (Math|Vector|BreakVector "0, 0, 0"))
  (bind _useimg (Variables|Default|GetUseImg))
  (Utilities|FlowControl|Sequence
    (:then_0
      (Variables|Default|SetStartLoc (Math|Vector|MakeVector (+ _x (Math|Random|RandomFloatinRange -1e+03 1e+03)) _y (- _z 1e+03)))
      (bind _alpha (Timeline|PopUp_TL PlayFromStart)
        (:Update
          (Transformation|SetRelativeLocation (Variables|Default|GetPopupMesh) (Math|Vector|Lerp(Vector) (Variables|Default|GetStartLoc) "0, 0, 0" _alpha) false false)
          (Transformation|SetRelativeScale3D (Variables|Default|GetPopupMesh) (Math|Vector|Lerp(Vector) "0, 0, 0" "1.000000,1.000000,1.000000" _alpha)))
        (:Finished
          (Collision|SetCollisionEnabled (Variables|Default|GetPokeBox) "QueryAndPhysics"))))
    (:then_1
      (Utilities|FlowControl|Delay 0.2)
      (Rendering|SetVisibility (Variables|Default|GetPopupMesh) true false)
      (Rendering|SetVisibility (Variables|Default|GetTextRender) (not _useimg) false)
      (Rendering|SetVisibility (Variables|Default|GetImgPlane) _useimg false)
      (Components|Timeline|PlayfromStart (Variables|Default|Getanimbounce_TL))
      (Audio|PlaySoundatLocation "/Game/Audio/SFX/Pop.Pop" (Transformation|GetActorLocation) "0, 0, 0" 0.65 (Math|Random|RandomFloatinRange 0.8 1.2) 0.0 "/Game/Audio/Attenuation/SA_ShortRange.SA_ShortRange" "/Game/Audio/Attenuation/SC_Default.SC_Default" 0)
      (bind _asbp_pant_controller (Utilities|Casting|CastToBP_PantController (Game|GetPlayerCharacter 0)))
      (Rendering|SetVisibility (Variables|/Game/PantControllerBP/Blueprints/BP_PantController.BP_PantController_C|GetCursor3DSecondary _asbp_pant_controller) false false))))

(event EventOnLand
  (Utilities|FlowControl|Sequence
    (:then_0
      (if (Variables|Default|GetMaximized)
        (bind _newtrack_0 (Timeline|Land_TL PlayFromStart)
          (:Update
            (Transformation|SetRelativeLocation (Variables|Default|GetScene1) (Math|Vector|Lerp(Vector) "0, 0, 0" "0, 0,-30.000000" _newtrack_0) false false)))
        (else
          (CallFunction|PokeEvent)
          (Timeline|Land_TL PlayFromStart))))
    (:then_1
      (Utilities|FlowControl|DoOnce false
        (:Completed
          (for (_array_element _array_index) (Variables|Default|GetLandActivatedActors)
            (Class|BPIActivate|Activate(Message) _array_element (+ (/ (+ (Math|Conversions|ToFloat(Integer) _array_index) 1.0) 4.0) (Variables|Default|GetLandDelay)) false)))))))

(event EventBeginPlay
  (bind _returnvalue (Math|Random|RandomFloatinRange 0.8 1.2))
  (bind _imgplane (Variables|Default|GetImgPlane))
  (bind _popupmesh (Variables|Default|GetPopupMesh))
  (if (Variables|Default|GetStartOpen)
    (Utilities|FlowControl|FlipFlop
      (:A
        (Variables|Default|SetMaximized true)
        (Rendering|Material|SetMaterial (Variables|Default|GetCornerButton1) 0 "/Game/Materials/Popup_MultimaxButton_Mat.Popup_MultimaxButton_Mat")
        (Audio|PlaySoundatLocation "/Game/Audio/SFX/PopupSFX/SFX_PopupMaximize.SFX_PopupMaximize" (Transformation|GetActorLocation) "0, 0, 0" 0.15 _returnvalue 0.0 "/Game/Audio/Attenuation/SA_ShortRange.SA_ShortRange" "/Game/Audio/Attenuation/SC_Default.SC_Default" self)
        (CallFunction|WindowTextType)
        (bind (_direction _depthfloat _z) (Timeline|Timeline_0 Play)
          (:Update
            (Components|SkeletalMesh|SetMorphTarget _popupmesh "Depth" (Math|Float|Lerp 0.0 (Variables|Default|GetDepth) _depthfloat) true)
            (Components|SkeletalMesh|SetMorphTarget _popupmesh "X" (Math|Float|Lerp 0.0 (Variables|Default|GetX) _depthfloat) true)
            (Components|SkeletalMesh|SetMorphTarget _popupmesh "Y" (Math|Float|Lerp 0.0 (Variables|Default|GetY) _depthfloat) true)
            (Transformation|SetRelativeLocation (Variables|Default|GetSpringArm) (Math|Vector|Lerp(Vector) "70.000000,25.000000,60.000000" "575.000000,25.000000,60.000000" (Math|Float|Lerp 0.0 (Variables|Default|GetX) _depthfloat)) false false)
            (Transformation|SetRelativeScale3D (Variables|Default|GetBox) (Math|Vector|MakeVector (Math|Float|Lerp 2e+02 1.2e+03 (Math|Float|Lerp 0.0 (Variables|Default|GetX) _depthfloat)) (Math|Float|Lerp 4e+01 1e+03 (Math|Float|Lerp 0.0 (Variables|Default|GetDepth) _depthfloat)) (Math|Float|Lerp 52.0 3.4e+02 (Math|Float|Lerp 0.0 (Variables|Default|GetY) _depthfloat))))
            (Transformation|SetRelativeLocation (Variables|Default|GetBox) (Math|Vector|MakeVector 0.0 (Math|Float|Lerp 0.0 -485.0 (Math|Float|Lerp 0.0 (Variables|Default|GetDepth) _depthfloat)) (Math|Float|Lerp 78.0 -65.0 (Math|Float|Lerp 0.0 (Variables|Default|GetY) _depthfloat))) false false)
            (Transformation|SetRelativeLocation (Variables|Default|GetPopupMesh) (Math|Vector|Lerp(Vector) "0, 0, 0" "0.000000,0.000000,20.000000" _z) false false)
            (Transformation|SetRelativeLocation (Variables|Default|GetTitleText) (Math|Vector|Lerp(Vector) "-60.000000,22.500000,58.000000" "-560.000000,22.500000,58.000000" (Math|Float|Lerp 0.0 (Variables|Default|GetX) _depthfloat)) false false)
            (Transformation|SetRelativeLocation (Variables|Default|GetTextRender) (Math|Vector|Lerp(Vector) "4.000000,20.000000,-5.000000" "4.000000,20.000000,-500.000000" (Math|Float|Lerp 0.0 (Variables|Default|GetY) _depthfloat)) false false)
            (Transformation|SetRelativeScale3D (Variables|Default|GetImgPlane) (Math|Vector|MakeVector (Math|Float|Lerp 1.0 1e+01 (Math|Float|Lerp 0.0 (Variables|Default|GetX) _depthfloat)) (Math|Float|Lerp 1.0 1e+01 (Math|Float|Lerp 0.0 (Variables|Default|GetY) _depthfloat)) (Math|Float|Lerp 1.0 1e+01 _depthfloat))))
          (:Finished
            (Class|PrimitiveComponent|SetWalkableSlopeOverride (Variables|Default|GetBox) (Utilities|Struct|MakeWalkableSlopeOverride "WalkableSlope_Default" 0.0))
            (Rendering|SetVisibility (Variables|Default|GetImgPlane) (Variables|Default|GetUseImg) false))
          (:MidPoint
            (switch Utilities|FlowControl|Switch|SwitchonETimelineDirection _direction
              (:Forward
                (Rendering|Material|SetMaterial _imgplane 0 (Variables|Default|GetImg_Mat)))
              (:Backward
                (Rendering|Material|SetMaterial _imgplane 0 "/Game/Materials/ArtIcon_img_Mat.ArtIcon_img_Mat")))
            (Rendering|SetVisibility (Variables|Default|GetImgPlane) (Variables|Default|GetUseImg) false))))
      (:B
        (Variables|Default|SetMaximized false)
        (Rendering|Material|SetMaterial (Variables|Default|GetCornerButton1) 0 "/Game/Materials/Popup_MaximizeButton_Mat.Popup_MaximizeButton_Mat")
        (Audio|PlaySoundatLocation "/Game/Audio/SFX/PopupSFX/SFX_PopupMinimize.SFX_PopupMinimize" (Transformation|GetActorLocation) "0, 0, 0" 0.15 _returnvalue 0.0 "/Game/Audio/Attenuation/SA_ShortRange.SA_ShortRange" "/Game/Audio/Attenuation/SC_Default.SC_Default" self)
        (CallFunction|WindowTextReverse)
        (Class|PrimitiveComponent|SetWalkableSlopeOverride (Variables|Default|GetBox) (Utilities|Struct|MakeWalkableSlopeOverride "WalkableSlope_Unwalkable" 0.0))
        (Timeline|Timeline_0 Reverse)))))

(event EventPokeEvent
  (bind _returnvalue (Math|Random|RandomFloatinRange 0.8 1.2))
  (bind _imgplane (Variables|Default|GetImgPlane))
  (bind _popupmesh (Variables|Default|GetPopupMesh))
  (bind _animbounce_tl (Variables|Default|Getanimbounce_TL))
  (Components|Timeline|SetPlayRate _animbounce_tl 0.8)
  (Components|Timeline|PlayfromStart _animbounce_tl)
  (Rendering|SetVisibility (Variables|Default|GetImgPlane) false false)
  (Utilities|FlowControl|FlipFlop
    (:A
      (Variables|Default|SetMaximized true)
      (Rendering|Material|SetMaterial (Variables|Default|GetCornerButton1) 0 "/Game/Materials/Popup_MultimaxButton_Mat.Popup_MultimaxButton_Mat")
      (Audio|PlaySoundatLocation "/Game/Audio/SFX/PopupSFX/SFX_PopupMaximize.SFX_PopupMaximize" (Transformation|GetActorLocation) "0, 0, 0" 0.15 _returnvalue 0.0 "/Game/Audio/Attenuation/SA_ShortRange.SA_ShortRange" "/Game/Audio/Attenuation/SC_Default.SC_Default" self)
      (CallFunction|WindowTextType)
      (bind (_direction _depthfloat _z) (Timeline|Timeline_0 Play)
        (:Update
          (Components|SkeletalMesh|SetMorphTarget _popupmesh "Depth" (Math|Float|Lerp 0.0 (Variables|Default|GetDepth) _depthfloat) true)
          (Components|SkeletalMesh|SetMorphTarget _popupmesh "X" (Math|Float|Lerp 0.0 (Variables|Default|GetX) _depthfloat) true)
          (Components|SkeletalMesh|SetMorphTarget _popupmesh "Y" (Math|Float|Lerp 0.0 (Variables|Default|GetY) _depthfloat) true)
          (Transformation|SetRelativeLocation (Variables|Default|GetSpringArm) (Math|Vector|Lerp(Vector) "70.000000,25.000000,60.000000" "575.000000,25.000000,60.000000" (Math|Float|Lerp 0.0 (Variables|Default|GetX) _depthfloat)) false false)
          (Transformation|SetRelativeScale3D (Variables|Default|GetBox) (Math|Vector|MakeVector (Math|Float|Lerp 2e+02 1.2e+03 (Math|Float|Lerp 0.0 (Variables|Default|GetX) _depthfloat)) (Math|Float|Lerp 4e+01 1e+03 (Math|Float|Lerp 0.0 (Variables|Default|GetDepth) _depthfloat)) (Math|Float|Lerp 52.0 3.4e+02 (Math|Float|Lerp 0.0 (Variables|Default|GetY) _depthfloat))))
          (Transformation|SetRelativeLocation (Variables|Default|GetBox) (Math|Vector|MakeVector 0.0 (Math|Float|Lerp 0.0 -485.0 (Math|Float|Lerp 0.0 (Variables|Default|GetDepth) _depthfloat)) (Math|Float|Lerp 78.0 -65.0 (Math|Float|Lerp 0.0 (Variables|Default|GetY) _depthfloat))) false false)
          (Transformation|SetRelativeLocation (Variables|Default|GetPopupMesh) (Math|Vector|Lerp(Vector) "0, 0, 0" "0.000000,0.000000,20.000000" _z) false false)
          (Transformation|SetRelativeLocation (Variables|Default|GetTitleText) (Math|Vector|Lerp(Vector) "-60.000000,22.500000,58.000000" "-560.000000,22.500000,58.000000" (Math|Float|Lerp 0.0 (Variables|Default|GetX) _depthfloat)) false false)
          (Transformation|SetRelativeLocation (Variables|Default|GetTextRender) (Math|Vector|Lerp(Vector) "4.000000,20.000000,-5.000000" "4.000000,20.000000,-500.000000" (Math|Float|Lerp 0.0 (Variables|Default|GetY) _depthfloat)) false false)
          (Transformation|SetRelativeScale3D (Variables|Default|GetImgPlane) (Math|Vector|MakeVector (Math|Float|Lerp 1.0 1e+01 (Math|Float|Lerp 0.0 (Variables|Default|GetX) _depthfloat)) (Math|Float|Lerp 1.0 1e+01 (Math|Float|Lerp 0.0 (Variables|Default|GetY) _depthfloat)) (Math|Float|Lerp 1.0 1e+01 _depthfloat))))
        (:Finished
          (Class|PrimitiveComponent|SetWalkableSlopeOverride (Variables|Default|GetBox) (Utilities|Struct|MakeWalkableSlopeOverride "WalkableSlope_Default" 0.0))
          (Rendering|SetVisibility (Variables|Default|GetImgPlane) (Variables|Default|GetUseImg) false))
        (:MidPoint
          (switch Utilities|FlowControl|Switch|SwitchonETimelineDirection _direction
            (:Forward
              (Rendering|Material|SetMaterial _imgplane 0 (Variables|Default|GetImg_Mat)))
            (:Backward
              (Rendering|Material|SetMaterial _imgplane 0 "/Game/Materials/ArtIcon_img_Mat.ArtIcon_img_Mat")))
          (Rendering|SetVisibility (Variables|Default|GetImgPlane) (Variables|Default|GetUseImg) false))))
    (:B
      (Variables|Default|SetMaximized false)
      (Rendering|Material|SetMaterial (Variables|Default|GetCornerButton1) 0 "/Game/Materials/Popup_MaximizeButton_Mat.Popup_MaximizeButton_Mat")
      (Audio|PlaySoundatLocation "/Game/Audio/SFX/PopupSFX/SFX_PopupMinimize.SFX_PopupMinimize" (Transformation|GetActorLocation) "0, 0, 0" 0.15 _returnvalue 0.0 "/Game/Audio/Attenuation/SA_ShortRange.SA_ShortRange" "/Game/Audio/Attenuation/SC_Default.SC_Default" self)
      (CallFunction|WindowTextReverse)
      (Class|PrimitiveComponent|SetWalkableSlopeOverride (Variables|Default|GetBox) (Utilities|Struct|MakeWalkableSlopeOverride "WalkableSlope_Unwalkable" 0.0))
      (Timeline|Timeline_0 Reverse))))

(event EventActivate
  (params (Delay :type Float%20%28single-precision%29) (Bool :type Boolean))
  (bind _asbp_pant_controller (Utilities|Casting|CastToBP_PantController (Game|GetPlayerCharacter 0))
    (:then
      (Rendering|SetVisibility (Variables|/Game/PantControllerBP/Blueprints/BP_PantController.BP_PantController_C|GetCursor3DSecondary _asbp_pant_controller) true false)
      (Rendering|Material|SetMaterial (Variables|/Game/PantControllerBP/Blueprints/BP_PantController.BP_PantController_C|GetCursor3DSecondary _asbp_pant_controller) 0 "/Game/Meshes/Materials/Textures/Hourglass/HourGlass_Mat.HourGlass_Mat"))
    (:CastFailed
      _))
  (Utilities|FlowControl|Delay Delay)
  (CallFunction|PopUpEvent))

(fn ConstructionScript
  (bind _textrender (Variables|Default|GetTextRender))
  (bind _useimg (Variables|Default|GetUseImg))
  (bind _hidden (Variables|Default|GetHidden))
  (bind _returnvalue (not _hidden))
  (bind _returnvalue_2 (Rendering|Material|CreateDynamicMaterialInstance (Variables|Default|GetPopupMesh) 0 "/Game/Materials/PopupBorder_Mat.PopupBorder_Mat" "None" :!class /Script/Engine.PrimitiveComponent))
  (bind _output_get (Variables|Default|SetDynMat _returnvalue_2))
  (Rendering|Material|SetMaterial (Variables|Default|GetPopupMesh) 0 _output_get)
  (Rendering|Material|SetVectorParameterValue (Variables|Default|GetDynMat) "Color" (Variables|Default|GetColor) :!class /Script/Engine.MaterialInstanceDynamic)
  (CallFunction|ClampText 3)
  (Rendering|Components|TextRender|SetText _textrender (Utilities|Text|ToText(String) (Variables|Default|GetWindowText_Min)))
  (Rendering|Components|TextRender|SetWorldSize _textrender (Variables|Default|GetTextSize))
  (if (Variables|Default|GetHidden)
    (Rendering|SetVisibility (Variables|Default|GetPopupMesh) false true)
    (Collision|SetCollisionEnabled (Variables|Default|GetBox) "NoCollision")
    (else
      (Rendering|SetVisibility (Variables|Default|GetPopupMesh1) false false)
      (Collision|SetCollisionEnabled (Variables|Default|GetPokeBox) "QueryAndPhysics")))
  (Rendering|SetVisibility (Variables|Default|GetImgPlane) (and _useimg _returnvalue) false)
  (Rendering|SetVisibility (Variables|Default|GetTextRender) (and (not _useimg) _returnvalue) false))

(fn ClampText
  (params (ClampLength :type Integer))
  (bind _windowtitle (Variables|Default|GetWindowTitle))
  (bind _returnvalue (Utilities|String|Len _windowtitle))
  (Rendering|Components|TextRender|SetText (Variables|Default|GetTitleText) (Utilities|Text|ToText(String) (Utilities|String|Append (Utilities|String|GetSubstring _windowtitle 0 (- _returnvalue (- _returnvalue ClampLength))) "..."))))

(fn Attachto
  (params (ChildActor :type Actor%20Object%20Reference))
  (return 0))

(fn CanGrab
  (return false))

(fn Clicked
  (return false))

(fn DisableCollision
  (return false))

(fn DoesParentHaveParent
  (return false))

(fn EnableCollision
  (return false))

(fn GetAttached
  (return 0))

(fn GetShrinkScale
  (return "0, 0, 0" "0, 0, 0"))

(fn GetSnapLoc
  (params (CursorLoc :type Vector :default "0, 0, 0"))
  (return "0, 0, 0" "0, 0, 0"))

(fn Grabbed
  (return 0))

(fn IsBusy
  (return false))

(fn LetGo
  (params (ParentComponent :type Actor%20Component%20Object%20Reference) (ParentActor :type Actor%20Object%20Reference))
  (return false))

(fn OnHover
  (return false))

(fn PassChildAlong
  (return 0 0))