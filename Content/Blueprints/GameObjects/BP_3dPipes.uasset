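; Self-propagating pipe segment that builds a randomly coloured chain of 3D pipes from a Start actor, which tracks every piece.
; Each segment spawns the next at its straight or turn point, randomly inserting elbows or balls, rolling straights in 90-degree steps and retrying when straight spawns collide.
; A reversed timeline scales new pieces in.
; Past 500 segments, the origin despawns the chain with Number-based staggering and restarts in a new colour.
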(event Custom|SetMesh
  (params (Mesh :type Static%20Mesh%20Object%20Reference))
  (bind _straightspawn (Variables|Default|GetStraightSpawn))
  (bind _tl_despawn (Variables|Default|GetTL_Despawn))
  (bind _turnspawn (Variables|Default|GetTurnSpawn))
  (if (== Mesh "/Game/Meshes/PipeStraight.PipeStraight")
    (if (> (Math|Random|RandomFloatinRange 0.0 1e+01) 8.25)
      (if (> (Math|Random|RandomFloatinRange 0.0 1e+01) 6.5)
        (Components|StaticMesh|SetStaticMesh (Variables|Default|GetPipeMesh) "/Game/Meshes/PipeBall.PipeBall")
        (else
          (Components|StaticMesh|SetStaticMesh (Variables|Default|GetPipeMesh) "/Game/Meshes/PipeTurn.PipeTurn")))
      (Utilities|FlowControl|Delay 0.32)
      (if (> (Variables|Default|Getnumber) 500)
        (Components|StaticMesh|SetStaticMesh (Variables|BP_3dPipes_C|GetPipeMesh (Utilities|Array|Get(acopy) (Variables|BP_3dPipes_C|GetPipeArray (Variables|Default|GetOrigin)) (- (Utilities|Array|LastIndex (Variables|BP_3dPipes_C|GetPipeArray (Variables|Default|GetOrigin))) 1))) "/Game/Meshes/PipeBall.PipeBall" :!label _label)
        (CallFunction|Restart (Variables|Default|GetOrigin))
        (else
          (bind _returnvalue (Game|SpawnActorfromClass "BP_3dPipes_C" (Math|Transform|MakeTransform (Transformation|GetWorldLocation _turnspawn) (Transformation|GetWorldRotation _turnspawn)) "Undefined" 0 0))
          (bind _asbp_3d_pipes (Utilities|Casting|CastToBP_3dPipes _returnvalue))
          (Variables|BP_3dPipes_C|SetOrigin _asbp_3d_pipes (Variables|Default|GetOrigin))
          (Variables|BP_3dPipes_C|SetColor _asbp_3d_pipes (Variables|Default|GetColor))
          (CallFunction|SetMesh _asbp_3d_pipes (Variables|/Script/Engine.StaticMeshComponent|GetStaticMesh (Variables|Default|GetPipeMesh)))
          (CallFunction|SetMat _asbp_3d_pipes)
          (Variables|BP_3dPipes_C|Setnumber _asbp_3d_pipes (+ (Variables|Default|Getnumber) 1))
          (Utilities|Array|Add (Variables|BP_3dPipes_C|GetPipeArray (Variables|Default|GetOrigin)) _returnvalue)
          (Utilities|FlowControl|Delay 0.2)
          (if (Class|TimelineComponent|IsReversing _tl_despawn)
            _
            (else
              (Components|Timeline|ReversefromEnd _tl_despawn)))
          (Rendering|SetVisibility (Variables|BP_3dPipes_C|GetPipeMesh _asbp_3d_pipes) false false)
          (Components|Timeline|SetPlayRate (Variables|Default|GetTL_Despawn) 0.65 :!label _label_2)))
      (else
        (Transformation|AddRelativeRotation (Variables|Default|GetPipeMesh) (Math|Rotator|MakeRotator (* (Math|Random|RandomIntegerinRange 0 4) 9e+01) 0.0 0.0) false false :!label _label_3)
        (Utilities|FlowControl|Delay 0.02)
        (if (> (Variables|Default|Getnumber) 500)
          (goto _label)
          (else
            (bind _returnvalue_2 (Game|SpawnActorfromClass "BP_3dPipes_C" (Math|Transform|MakeTransform (Transformation|GetWorldLocation _straightspawn) (Transformation|GetWorldRotation _straightspawn)) "DontSpawnIfColliding" 0 0))
            (Utilities|IsValid _returnvalue_2
              (:Is%20Valid
                (bind _asbp_3d_pipes_2 (Utilities|Casting|CastToBP_3dPipes _returnvalue_2))
                (Variables|BP_3dPipes_C|SetOrigin _asbp_3d_pipes_2 (Variables|Default|GetOrigin))
                (Variables|BP_3dPipes_C|SetColor _asbp_3d_pipes_2 (Variables|Default|GetColor))
                (CallFunction|SetMesh _asbp_3d_pipes_2 (Variables|/Script/Engine.StaticMeshComponent|GetStaticMesh (Variables|Default|GetPipeMesh)))
                (CallFunction|SetMat _asbp_3d_pipes_2)
                (Variables|BP_3dPipes_C|Setnumber _asbp_3d_pipes_2 (+ (Variables|Default|Getnumber) 1))
                (Utilities|Array|Add (Variables|BP_3dPipes_C|GetPipeArray (Variables|Default|GetOrigin)) _returnvalue_2)
                (Utilities|FlowControl|Delay 0.2)
                (if (Class|TimelineComponent|IsReversing _tl_despawn)
                  _
                  (else
                    (Components|Timeline|ReversefromEnd _tl_despawn)))
                (Rendering|SetVisibility (Variables|BP_3dPipes_C|GetPipeMesh _asbp_3d_pipes_2) false false)
                (goto _label_2))
              (:Is%20Not%20Valid
                (CallFunction|SetMesh (Variables|/Script/Engine.StaticMeshComponent|GetStaticMesh (Variables|Default|GetPipeMesh)))))))))
    (else
      (Components|StaticMesh|SetStaticMesh (Variables|Default|GetPipeMesh) "/Game/Meshes/PipeStraight.PipeStraight")
      (goto _label_3))))

(event Custom|SetMat
  (bind _returnvalue (Rendering|Material|CreateDynamicMaterialInstance (Variables|Default|GetPipeMesh) 0 "/Game/Materials/Pipes/Pipes_Mat.Pipes_Mat" "None" :!class /Script/Engine.PrimitiveComponent))
  (Variables|Default|SetDynamicMat _returnvalue)
  (Rendering|Material|SetVectorParameterValue (Variables|Default|GetDynamicMat) "Color" (Variables|Default|GetColor) :!class /Script/Engine.MaterialInstanceDynamic))

(event Custom|Restart
  (for (_array_element _array_index) (Variables|Default|GetPipeArray)
    (if (not (Variables|BP_3dPipes_C|GetStart _array_element))
      (CallFunction|Despawn _array_element)))
  (Utilities|Array|Clear (Variables|Default|GetPipeArray))
  (Utilities|FlowControl|Delay 3.0)
  (CallFunction|SetMat)
  (if (Variables|Default|GetStart)
    (Utilities|FlowControl|Delay 3.5)
    (Variables|Default|SetOrigin self)
    (CallFunction|SetMesh "/Game/Meshes/PipeStraight.PipeStraight")
    (switch int (Math|Random|RandomIntegerinRange 0 4)
      (:Default
        (Variables|Default|SetColor (Math|Color|MakeColor (Math|Random|RandomFloatinRange 0.8 1.0) (Math|Random|RandomFloatinRange 0.0 0.15) (Math|Random|RandomFloatinRange 0.0 0.15)) :!label _label))
      (:0
        (Variables|Default|SetColor (Math|Color|MakeColor (Math|Random|RandomFloatinRange 0.8 1.0) (Math|Random|RandomFloatinRange 0.5 0.65) (Math|Random|RandomFloatinRange 0.5 0.65))))
      (:1
        (Variables|Default|SetColor (Math|Color|MakeColor (Math|Random|RandomFloatinRange 0.5 0.65) (Math|Random|RandomFloatinRange 0.5 0.65) (Math|Random|RandomFloatinRange 0.0 0.1))))
      (:2
        (goto _label))
      (:3
        (Variables|Default|SetColor (Math|Color|MakeColor (Math|Random|RandomFloatinRange 0.0 0.15) (Math|Random|RandomFloatinRange 0.8 1.0) (Math|Random|RandomFloatinRange 0.0 0.15))))
      (:4
        (Variables|Default|SetColor (Math|Color|MakeColor (Math|Random|RandomFloatinRange 0.0 0.15) (Math|Random|RandomFloatinRange 0.0 0.15) (Math|Random|RandomFloatinRange 0.8 1.0)))))))

(event Custom|Despawn
  (Utilities|FlowControl|Delay (* (Variables|Default|Getnumber) 0.01))
  (bind (_direction _alpha _newtrack_1) (Timeline|TL_Despawn PlayFromStart)
    (:Update
      (switch Utilities|FlowControl|Switch|SwitchonETimelineDirection _direction
        (:Forward
          (Transformation|SetActorScale3D (Math|Vector|Lerp(Vector) "1.000000,1.000000,1.000000" "1.000000,0.001000,0.001000" _alpha)))
        (:Backward
          (Transformation|SetActorScale3D (Math|Vector|Lerp(Vector) "1.000000,1.000000,1.000000" "1.000000,0.001000,0.001000" _newtrack_1))
          (Rendering|SetVisibility (Variables|Default|GetPipeMesh) true false))))
    (:Finished
      (switch Utilities|FlowControl|Switch|SwitchonETimelineDirection _direction
        (:Forward
          (Actor|DestroyActor))))))

(event EventBeginPlay
  (Utilities|FlowControl|Delay 0.24)
  (CallFunction|SetMat)
  (if (Variables|Default|GetStart)
    (Utilities|FlowControl|Delay 3.5)
    (Variables|Default|SetOrigin self)
    (CallFunction|SetMesh "/Game/Meshes/PipeStraight.PipeStraight")
    (switch int (Math|Random|RandomIntegerinRange 0 4)
      (:Default
        (Variables|Default|SetColor (Math|Color|MakeColor (Math|Random|RandomFloatinRange 0.8 1.0) (Math|Random|RandomFloatinRange 0.0 0.15) (Math|Random|RandomFloatinRange 0.0 0.15)) :!label _label))
      (:0
        (Variables|Default|SetColor (Math|Color|MakeColor (Math|Random|RandomFloatinRange 0.8 1.0) (Math|Random|RandomFloatinRange 0.5 0.65) (Math|Random|RandomFloatinRange 0.5 0.65))))
      (:1
        (Variables|Default|SetColor (Math|Color|MakeColor (Math|Random|RandomFloatinRange 0.5 0.65) (Math|Random|RandomFloatinRange 0.5 0.65) (Math|Random|RandomFloatinRange 0.0 0.1))))
      (:2
        (goto _label))
      (:3
        (Variables|Default|SetColor (Math|Color|MakeColor (Math|Random|RandomFloatinRange 0.0 0.15) (Math|Random|RandomFloatinRange 0.8 1.0) (Math|Random|RandomFloatinRange 0.0 0.15))))
      (:4
        (Variables|Default|SetColor (Math|Color|MakeColor (Math|Random|RandomFloatinRange 0.0 0.15) (Math|Random|RandomFloatinRange 0.0 0.15) (Math|Random|RandomFloatinRange 0.8 1.0)))))))

(fn ConstructionScript)