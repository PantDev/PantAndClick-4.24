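; BP_MovingBox is a launcher box that captures the player on overlap, hides and attaches them, and can blend to its own camera.
; Timelines animate squash, cursor arrow, optional spline-rail travel and stepped rotation that reverses at its limits.
; Launches call BoxLaunchRemote on BP_PantController, immediately with AutoLaunch or buffered until spins finish, with GetVelocityBox supplying an arrow-based velocity.
; Boxes can start hidden without collision until SpawnEntity reveals them.
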(event OnComponentBeginOverlap(Sphere)
  (params (OverlappedComponent :type Primitive%20Component%20Object%20Reference) (OtherActor :type Actor%20Object%20Reference) (OtherComp :type Primitive%20Component%20Object%20Reference) (OtherBodyIndex :type Integer) (bFromSweep :type Boolean) (SweepResult :type Hit%20Result%20Structure%20%28by%20ref%29))
  (bind _cursormesh (Variables|Default|GetCursorMesh))
  (bind _animrotinterval (Variables|Default|GetAnimRotInterval))
  (bind _rotint (Variables|Default|GetRotInt))
  (if (and (Variables|Default|GetAvailable) (not (Variables|Default|GetHidden)))
    (bind _asbp_pant_controller (Utilities|Casting|CastToBP_PantController OtherActor))
    (if (not (Variables|/Game/PantControllerBP/Blueprints/BP_PantController.BP_PantController_C|GetInBox _asbp_pant_controller))
      (bind _asbp_pant_controller_2 (Utilities|Casting|CastToBP_PantController (Game|GetPlayerCharacter 0)))
      (if (Variables|/Game/PantControllerBP/Blueprints/BP_PantController.BP_PantController_C|GetIsBubbleOpen _asbp_pant_controller_2)
        _
        (else
          _))
      (if (Variables|Default|GetAutoLaunch)
        (Variables|Default|SetBufferedLaunch true)
        (Variables|Default|SetSpecialBuffer true)
        (else
          (UserInterface|Animation|PlayAnimation (Variables|/Game/PantControllerBP/Blueprints/BP_PantController.BP_PantController_C|GetTutWidget _asbp_pant_controller) (Variables|/Game/UserInterface/Images/Tutorial/PressJump_Widget.PressJump_Widget_C|GetVisible (Variables|/Game/PantControllerBP/Blueprints/BP_PantController.BP_PantController_C|GetTutWidget _asbp_pant_controller)) 0.0 1 "Forward" 1.0 false)))
      (Variables|/Game/PantControllerBP/Blueprints/BP_PantController.BP_PantController_C|SetActiveMovingBox _asbp_pant_controller self)
      (Variables|/Game/PantControllerBP/Blueprints/BP_PantController.BP_PantController_C|SetInBox _asbp_pant_controller true)
      (bind _asbp_pant_controller_3 (Utilities|Casting|CastToBP_PantController (Game|GetPlayerCharacter 0))
        (:then
          (Rendering|SetVisibility (Variables|/Game/PantControllerBP/Blueprints/BP_PantController.BP_PantController_C|GetDenimMesh _asbp_pant_controller_3) false false)
          (Components|Activation|Deactivate (Variables|/Game/PantControllerBP/Blueprints/BP_PantController.BP_PantController_C|GetParticleSystem6 _asbp_pant_controller_3)))
        (:CastFailed
          _))
      (Utilities|IsValid (Variables|Default|GetCamera)
        (:Is%20Valid
          (Variables|/Game/PantControllerBP/Blueprints/BP_PantController.BP_PantController_C|SetLockCamera _asbp_pant_controller true)
          (Game|Player|SetViewTargetwithBlend (Game|GetPlayerController 0) (Variables|Default|GetCamera) 0.48 "VTBlend_Cubic" 5e+01 false)
          (if (Variables|Default|GetSpin)
            (Components|Timeline|PlayfromStart (Variables|Default|GetTL_Ready)))
          (Components|Timeline|PlayfromStart (Variables|Default|GetANIM_Pulse) :!label _label)
          (Pawn|Components|CharacterMovement|SetMovementMode (Variables|/Script/Engine.Character|GetCharacterMovement _asbp_pant_controller) "MOVE_Flying" 0)
          (Variables|/Script/Engine.MovementComponent|SetVelocity (Pawn|GetMovementComponent _asbp_pant_controller) "0, 0, 0")
          (Transformation|SetActorLocation _asbp_pant_controller (Transformation|GetActorLocation) false false)
          (Transformation|AttachComponentToComponent _asbp_pant_controller (Variables|Default|GetDefaultSceneRoot) "None" "KeepWorld" "KeepWorld" "KeepWorld" true)
          (Components|Animation|SetAnimation (Variables|/Game/PantControllerBP/Blueprints/BP_PantController.BP_PantController_C|GetDenimMesh _asbp_pant_controller) "/Game/Meshes/PantMesh/NewFolder/Denim_Anim_Armature_Roll.Denim_Anim_Armature_Roll")
          (Components|Timeline|SetPlayRate (Variables|/Game/PantControllerBP/Blueprints/BP_PantController.BP_PantController_C|GetDenimMesh _asbp_pant_controller) 0.0)
          (Components|Animation|PlayAnimation (Variables|Default|GetSkeletalMesh) "/Game/Meshes/Skeletal/MovingBox/MovingBox_Skeletal_Anim_Armature_CloseBox.MovingBox_Skeletal_Anim_Armature_CloseBox" false)
          (Audio|PlaySoundatLocation "/Game/Audio/SFX/Pop.Pop" "0, 0, 0" "0, 0, 0" 0.7 0.7 0.02 "/Game/Audio/Attenuation/SA_Default.SA_Default" "/Game/Audio/Attenuation/SC_Default.SC_Default" 0)
          (Audio|PlaySoundatLocation "/Game/Audio/SFX/Footstep.Footstep" (Transformation|GetActorLocation) "0, 0, 0" 0.4 0.7 0.0 "/Game/Audio/Attenuation/SA_Default.SA_Default" "/Game/Audio/Attenuation/SC_Default.SC_Default" 0)
          (Rendering|SetVisibility (Variables|/Game/PantControllerBP/Blueprints/BP_PantController.BP_PantController_C|GetCursor3DMesh _asbp_pant_controller) false false)
          (Components|Timeline|PlayfromStart (Variables|Default|GetTL_CursorStart))
          (if (Variables|Default|GetAutoLaunch)
            (Rendering|SetVisibility _cursormesh false false)
            (else
              (Rendering|SetVisibility _cursormesh true false)))
          (Components|Activation|Activate (Variables|Default|GetParticleSystem) false)
          (Components|Timeline|PlayfromStart (Variables|Default|GetTL_ScaleAnim))
          (Utilities|FlowControl|Delay 0.2)
          (Components|Activation|Deactivate (Variables|Default|GetParticleSystem))
          (if (Variables|Default|GetBufferedLaunch)
            (bind _asbp_pant_controller_4 (Utilities|Casting|CastToBP_PantController (Game|GetPlayerCharacter 0) :!label _label_2))
            (if (Variables|Default|GetSpin)
              (if (Variables|Default|GetReady)
                _
                (else
                  (Utilities|FlowControl|Delay 0.2))))
            (Audio|Components|Audio|Stop (Variables|Default|GetAnimLockStop))
            (Default|BoxLaunchRemote _asbp_pant_controller_4)
            (Variables|Default|SetBufferedLaunch false)
            (Variables|Default|SetSpecialBuffer false)
            (elif (Variables|Default|GetRotating)
              (if (Variables|Default|GetSpin)
                (if (Variables|Default|GetReady)
                  (if (Utilities|Enum|Equal(Enum) "Backward" (Variables|Default|GetRotDir)) :!label _label_3
                    (if (== _rotint 0)
                      (Components|Timeline|PlayfromStart _animrotinterval :!label _label_4)
                      (else
                        (Components|Timeline|ReversefromEnd _animrotinterval :!label _label_5)))
                    (elif (== _rotint (Variables|Default|GetRotIntCap))
                      (goto _label_5)
                      (else
                        (goto _label_4))))
                  (else
                    (Utilities|FlowControl|Delay 0.2)
                    (bind _asbp_pant_controller_5 (Utilities|Casting|CastToBP_PantController (Game|GetPlayerCharacter 0)))
                    (if (== (Variables|/Game/PantControllerBP/Blueprints/BP_PantController.BP_PantController_C|GetActiveMovingBox _asbp_pant_controller_5) self)
                      (goto _label_3))))
                (else
                  (goto _label_3)))
              (else
                (Utilities|FlowControl|Delay 0.2)
                (if (Variables|Default|GetBufferedLaunch)
                  (goto _label_2))))))
        (:Is%20Not%20Valid
          (Utilities|FlowControl|Sequence
            (:then_0
              (Variables|/Game/PantControllerBP/Blueprints/BP_PantController.BP_PantController_C|SetLockCamera _asbp_pant_controller false)
              (goto _label))
            (:then_1
              (Utilities|FlowControl|Delay 0.35)
              (bind _asbp_pant_controller_6 (Utilities|Casting|CastToBP_PantController (Game|GetPlayerCharacter 0)))
              (if (== (Variables|/Game/PantControllerBP/Blueprints/BP_PantController.BP_PantController_C|GetActiveMovingBox _asbp_pant_controller_6) self)
                (Variables|Default|SetReady true)))))))))

(event Custom|PreLaunchEvent
  (bind _cursormesh (Variables|Default|GetCursorMesh))
  (Utilities|FlowControl|DoOnce false :!label _label
    (:Completed
      (Audio|Components|Audio|Stop (Variables|Default|GetANIM_Pulse))
      (CallFunction|StopCursorAnim)
      (bind (_direction _localpha _cursorscalealpha _scale) (Timeline|TL_PreLaunchAnim PlayFromStart)
        (:Update
          (Transformation|SetRelativeScale3D (Variables|Default|GetSkeletalMesh) _scale)
          (Transformation|SetWorldLocation (Variables|Default|GetSkeletalMesh) (Math|Vector|Lerp(Vector) (Transformation|GetWorldLocation (Variables|Default|GetDefaultSceneRoot)) (Transformation|GetWorldLocation (Variables|Default|GetPreLaunchAnimLoc)) _localpha) false false)
          (Transformation|SetRelativeScale3D (Variables|Default|GetCursorMesh) (Math|Vector|Lerp(Vector) "0.350000,0.350000,0.350000" "0, 0, 0" _cursorscalealpha)))
        (:Finished
          (Transformation|SetRelativeScale3D _cursormesh "0.350000,0.350000,0.350000")
          (goto _label Reset))
        (:HideCursor
          (Rendering|SetVisibility _cursormesh false false))))))

(event Custom|StopCursorAnim
  (Utilities|FlowControl|Sequence
    (:then_0
      (bind _alpha (Timeline|TL_CursorStart Stop)
        (:Update
          (Transformation|SetRelativeScale3D (Variables|Default|GetCursorMesh) (Math|Vector|Lerp(Vector) "0, 0, 0" "0.350000,0.350000,0.350000" _alpha)))))
    (:then_1
      (Transformation|SetRelativeScale3D (Variables|Default|GetCursorMesh) "0.350000,0.350000,0.350000"))))

(event EventBeginPlay
  (bind _sphere (Variables|Default|GetSphere))
  (bind _sphere_2 (Variables|Default|GetSphere))
  (bind _skeletalmesh (Variables|Default|GetSkeletalMesh))
  (if (Variables|Default|GetHidden)
    (Rendering|SetVisibility _skeletalmesh false false)
    (Collision|SetCollisionEnabled _sphere_2 "NoCollision")
    (Collision|SetCollisionResponsetoChannel _sphere_2 "ECC_WorldDynamic" "ECR_Ignore")
    (else
      (Rendering|SetVisibility _skeletalmesh true false)
      (Collision|SetCollisionEnabled _sphere "QueryAndPhysics")
      (Collision|SetCollisionResponsetoChannel _sphere "ECC_WorldDynamic" "ECR_Overlap")))
  (Utilities|Time|SetTimerbyFunctionName self "AddCursorRot" 0.05 true)
  (if (Utilities|IsValid (Variables|Default|GetRail))
    (Components|Timeline|PlayfromStart (Variables|Default|GetRailMove_TL))))

(event Collision|EventActorBeginOverlap
  (params (OtherActor :type Actor%20Object%20Reference)))

(event EventTick
  (params (DeltaSeconds :type Float%20%28single-precision%29)))

(event EventPokeEvent
  (if (not (Audio|Components|Audio|IsPlaying (Variables|Default|GetTL_Ready)))
    (Audio|PlaySoundatLocation "/Game/Audio/SFX/BoxSpin.BoxSpin" (Transformation|GetActorLocation) "0, 0, 0" 0.6 (Math|Random|RandomFloatinRange 1.4 1.65) 0.0 "/Game/Audio/Attenuation/SA_ShortRange.SA_ShortRange" "/Game/Audio/Attenuation/SC_Default.SC_Default" 0)
    (bind _zrot (Timeline|TL_Ready PlayFromStart)
      (:Update
        (Transformation|SetRelativeRotation (Variables|Default|GetSkeletalMesh) (Math|Rotator|MakeRotator 0.0 0.0 _zrot) false false))
      (:NewTrack_0
        (Variables|Default|SetReady true)))))

(event EventSpawnEntity
  (bind _tl_scaleup (Variables|Default|GetTL_ScaleUp))
  (Components|Timeline|SetPlayRate _tl_scaleup 0.5)
  (Components|Timeline|PlayfromStart _tl_scaleup)
  (CallFunction|PokeEvent)
  (Rendering|SetVisibility (Variables|Default|GetSkeletalMesh) true false)
  (Collision|SetCollisionEnabled (Variables|Default|GetSphere) "QueryAndPhysics"))

(event Custom|LockStopStopper
  (Audio|Components|Audio|Stop (Variables|Default|GetAnimLockStop)))

(fn ConstructionScript
  (Variables|Default|SetCursorStartRot (Variables|/Script/Engine.SceneComponent|GetRelativeRotation (Variables|Default|GetCursorMesh)))
  (if (Variables|Default|GetAutoLaunch)
    (Rendering|Material|SetMaterial (Variables|Default|GetSkeletalMesh) 0 "/Game/Materials/MovingBox_Pop_Mat.MovingBox_Pop_Mat")
    (else
      (Rendering|Material|SetMaterial (Variables|Default|GetSkeletalMesh) 0 "/Game/Materials/Opaque/MovingBoxOpen_MatInst.MovingBoxOpen_MatInst"))))

(fn GetVelocityBox
  (bind _returnvalue (Transformation|GetActorLocation))
  (bind _start (Variables|Default|GetStart))
  (bind _velocity (Variables|Default|GetVelocity))
  (bind _returnvalue_2 (Transformation|GetWorldLocation _start))
  (bind _returnvalue_3 (Math|Vector|GetUnitDirection(Vector) _returnvalue _returnvalue_2))
  (bind _returnvalue_4 (* _returnvalue_3 _velocity))
  (bind (_x _y _z) (Math|Vector|BreakVector _returnvalue_4))
  (return (Math|Vector|MakeVector _x _y (+ _z 2e+02))))

(fn AddCursorRot)

(fn GetFacingRot
  (bind _start (Variables|Default|GetStart))
  (bind _end (Variables|Default|GetEnd))
  (bind _returnvalue (Transformation|GetWorldLocation _end))
  (bind _returnvalue_2 (Transformation|GetWorldLocation _start))
  (bind (_x _y) (Math|Vector|BreakVector _returnvalue_2))
  (bind (_x_2 _y_2) (Math|Vector|BreakVector _returnvalue))
  (return (Math|Rotator|FindLookatRotation (Math|Vector|MakeVector _x _y 0.0) (Math|Vector|MakeVector _x_2 _y_2 0.0))))

(fn Attachto
  (params (ChildActor :type Actor%20Object%20Reference))
  (return 0))

(fn CanGrab
  (return false))

(fn Clicked
  (return false))

(fn DisableCollision
  (return false))

(fn DoesParentHaveParent
  (return false))

(fn EnableCollision
  (return false))

(fn GetAttached
  (return 0))

(fn GetCustomCursor
  (return false 0))

(fn GetShrinkScale
  (return "0, 0, 0" "0, 0, 0"))

(fn GetSnapLoc
  (params (CursorLoc :type Vector :default "0, 0, 0"))
  (return "0, 0, 0" "0, 0, 0"))

(fn Grabbed
  (return 0))

(fn LetGo
  (params (ParentComponent :type Actor%20Component%20Object%20Reference) (ParentActor :type Actor%20Object%20Reference))
  (return false))

(fn OnHover
  (return false))

(fn PassChildAlong
  (return 0 0))

(fn RightClickEvent
  (return (Variables|Default|GetClick%20Message) (Transformation|GetActorLocation)))