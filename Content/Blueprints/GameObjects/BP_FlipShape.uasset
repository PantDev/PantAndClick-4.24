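; BP_FlipShape is an activatable game object that queues a flip on the player's MazeNavController_BP.
; Activate sets QueueFlip, plays a sound and uses a timeline to shrink the mesh, then hides it for three seconds before restoring visibility and scale.
; Busy is set but never cleared, and IsBusy always returns false.
; A squish timeline and a second flip path exist but are never run.
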(event EventBeginPlay)

(event Collision|EventActorBeginOverlap
  (params (OtherActor :type Actor%20Object%20Reference)))

(event EventTick
  (params (DeltaSeconds :type Float%20%28single-precision%29)))

(event EventActivate
  (params (Delay :type Float%20%28single-precision%29) (Bool :type Boolean))
  (bind _staticmesh (Variables|Default|GetStaticMesh))
  (Variables|Default|SetBusy true)
  (bind _asmaze_nav_controller_bp (Utilities|Casting|CastToMazeNavController_BP (Game|GetPlayerCharacter 0)))
  (Variables|/Game/MazeNav/Blueprints/MazeNavController_BP.MazeNavController_BP_C|SetQueueFlip _asmaze_nav_controller_bp true)
  (Variables|Default|SetStartScale (Transformation|GetWorldScale (Variables|Default|GetStaticMesh)))
  (Audio|PlaySoundatLocation "/Game/Audio/SFX/wasvc.wasvc" (Transformation|GetActorLocation) "0, 0, 0" 0.85 1.2 0.1 0 0 0)
  (bind _newtrack_0 (Timeline|TL_Vanish PlayFromStart)
    (:Update
      (Transformation|SetRelativeScale3D (Variables|Default|GetStaticMesh) (Math|Vector|Lerp(Vector) (Variables|Default|GetStartScale) "0.001000,0.001000,0.001000" _newtrack_0)))
    (:Finished
      (Rendering|SetVisibility _staticmesh false false)
      (Utilities|FlowControl|Delay 3.0)
      (Rendering|SetVisibility _staticmesh true false)
      (Transformation|SetRelativeScale3D (Variables|Default|GetStaticMesh) (Variables|Default|GetStartScale)))))

(fn ConstructionScript)

(fn IsBusy
  (return false))