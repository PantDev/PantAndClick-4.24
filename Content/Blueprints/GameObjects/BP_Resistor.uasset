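; BP_Resistor is a resistor object that changes its colour bands when poked.
; PokeEvent calls RandomizeBands, which plays a randomly pitched pop and uses coin flips to set or null band materials on mesh slots, with some nested flips leaving slots unchanged.
; A TL_Bounce timeline then drives the mesh's relative scale for a bounce.
; The grab, click, hover, attach and snap functions are empty stubs returning defaults.
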(event EventBeginPlay)

(event Collision|EventActorBeginOverlap
  (params (OtherActor :type Actor%20Object%20Reference)))

(event EventTick
  (params (DeltaSeconds :type Float%20%28single-precision%29)))

(event EventPokeEvent
  (CallFunction|RandomizeBands)
  (bind _newtrack_0 (Timeline|TL_Bounce PlayFromStart)
    (:Update
      (Transformation|SetRelativeScale3D (Variables|Default|GetStaticMesh) (Math|Vector|MakeVector (+ (.X (Math|Vector|BreakVector _newtrack_0)) 1.0) (+ (.Y (Math|Vector|BreakVector _newtrack_0)) 1.0) (+ (.Z (Math|Vector|BreakVector _newtrack_0)) 1.0))))))

(fn ConstructionScript)

(fn RandomizeBands
  (bind _staticmesh (Variables|Default|GetStaticMesh))
  (bind _staticmesh_2 (Variables|Default|GetStaticMesh))
  (bind _staticmesh_3 (Variables|Default|GetStaticMesh))
  (bind _staticmesh_4 (Variables|Default|GetStaticMesh))
  (Audio|PlaySoundatLocation "/Game/Audio/SFX/Pop.Pop" (Transformation|GetActorLocation) "0, 0, 0" 0.8 (Math|Random|RandomFloatinRange 0.9 1.3) 0.0 "/Game/Audio/Attenuation/SA_ShortRange.SA_ShortRange" "/Game/Audio/Attenuation/SC_Default.SC_Default" 0)
  (if (Math|Random|RandomBool)
    (Rendering|Material|SetMaterial _staticmesh_2 2 "/Engine/EditorMaterials/WidgetMaterial_X.WidgetMaterial_X")
    (if (Math|Random|RandomBool)
      (Rendering|Material|SetMaterial _staticmesh_3 3 "/Engine/EditorMaterials/WidgetMaterial_Z.WidgetMaterial_Z")
      (if (Math|Random|RandomBool) :!label _label
        (Rendering|Material|SetMaterial _staticmesh_4 4 "/Game/Materials/Material_003.Material_003")
        (else
          (Rendering|Material|SetMaterial _staticmesh_4 4 "/Game/Materials/NullMat.NullMat")))
      (else
        (Rendering|Material|SetMaterial _staticmesh_3 3 "/Game/Materials/NullMat.NullMat")))
    (else
      (Rendering|Material|SetMaterial _staticmesh_2 2 "/Game/Materials/NullMat.NullMat")
      (goto _label)))
  (if (Math|Random|RandomBool)
    (Rendering|Material|SetMaterial _staticmesh 5 "/Engine/EditorMaterials/WidgetMaterial_Y.WidgetMaterial_Y")
    (else
      (Rendering|Material|SetMaterial _staticmesh 5 "/Game/Materials/NullMat.NullMat"))))

(fn Attachto
  (params (ChildActor :type Actor%20Object%20Reference))
  (return 0))

(fn CanGrab
  (return false))

(fn Clicked
  (return false))

(fn DisableCollision
  (return false))

(fn DoesParentHaveParent
  (return false))

(fn EnableCollision
  (return false))

(fn GetAttached
  (return 0))

(fn GetCustomCursor
  (return false 0))

(fn GetShrinkScale
  (return "0, 0, 0" "0, 0, 0"))

(fn GetSnapLoc
  (params (CursorLoc :type Vector :default "0, 0, 0"))
  (return "0, 0, 0" "0, 0, 0"))

(fn Grabbed
  (return 0))

(fn LetGo
  (params (ParentComponent :type Actor%20Component%20Object%20Reference) (ParentActor :type Actor%20Object%20Reference))
  (return false))

(fn OnHover
  (return false))

(fn PassChildAlong
  (return 0 0))