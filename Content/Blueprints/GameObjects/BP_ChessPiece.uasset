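; Interactive chess piece prop that changes to the next piece type each time it is poked, from pawn through king.
; Wrapping from king back to pawn also flips the black/white material and plays a separate timeline from the normal bounce.
; Timelines animate scale, spin and height of piece and base, with pitch-randomized sounds.
; The construction script sets mesh and materials; grab and snap functions are stubs, while right-click returns a message and focus location.
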(event EventPokeEvent
  (bind _returnvalue (Transformation|GetActorLocation))
  (bind _staticmesh (Variables|Default|GetStaticMesh))
  (bind _staticmesh_2 (Variables|Default|GetStaticMesh))
  (bind _staticmesh_3 (Variables|Default|GetStaticMesh))
  (bind (_x _y _z) (Math|Vector|BreakVector _returnvalue))
  (bind _returnvalue_2 (- _z 15.0))
  (bind _returnvalue_3 (Math|Vector|MakeVector _x _y _returnvalue_2))
  (if (== (Variables|Default|GetChessPiece) 6)
    (Variables|Default|SetChessPiece 1)
    (bind _output_get (Variables|Default|SetBlack/White (not (Variables|Default|GetBlack/White))))
    (if _output_get
      (Rendering|Material|SetMaterial _staticmesh_2 0 "/Game/Materials/WoodBlockWhite_Inst.WoodBlockWhite_Inst")
      (else
        (Rendering|Material|SetMaterial _staticmesh_2 0 "/Game/Materials/WoodBlock_Mat_Inst_Inst.WoodBlock_Mat_Inst_Inst")))
    (Utilities|FlowControl|Sequence
      (:then_0
        (bind (_direction _newtrack_0 _rotalpha _localpha) (Timeline|TL_Bounce Stop)
          (:Update
            (Transformation|SetRelativeScale3D _staticmesh _newtrack_0)
            (Transformation|SetRelativeRotation _staticmesh (Math|Rotator|Lerp(Rotator) "0, 0, 0" "0,360.000000, 0" _rotalpha) false false)
            (Transformation|SetRelativeLocation (Variables|Default|GetStaticMesh) (Math|Vector|Lerp(Vector) "0, 0, 0" "0, 0,-17.500000" _localpha) false false)
            (Transformation|SetRelativeLocation (Variables|Default|GetCube) (Math|Vector|Lerp(Vector) "0, 0,-50.000000" "0, 0,-67.500000" _localpha) false false))
          (:Finished
            (Audio|PlaySoundatLocation "/Game/Audio/SFX/SliderStop1.SliderStop1" _returnvalue_3 "0, 0, 0" 0.75 (Math|Random|RandomFloatinRange 1.1 1.4) 0.08 "/Game/Audio/Attenuation/SA_ShortRange.SA_ShortRange" "/Game/Audio/Attenuation/SC_Default.SC_Default" 0 :!label _label))
          (:NewTrack_2
            (Audio|PlaySoundatLocation "/Game/Audio/SFX/KnobLeft.KnobLeft" _returnvalue_3 "0, 0, 0" 0.06 (Math|Random|RandomFloatinRange 0.62 0.85) 0.5 "/Game/Audio/Attenuation/SA_ShortRange.SA_ShortRange" "/Game/Audio/Attenuation/SC_Default.SC_Default" 0 :!label _label_2))))
      (:then_1
        (Components|Timeline|SetPlaybackPosition (Variables|Default|GetTimeline_0) 0.05 false true)
        (bind (_direction_2 _newtrack_0_2 _rotalpha_2 _localpha_2) (Timeline|Timeline_0 Play)
          (:Update
            (Transformation|SetRelativeScale3D _staticmesh_3 _newtrack_0_2)
            (Transformation|SetRelativeRotation _staticmesh_3 (Math|Rotator|Lerp(Rotator) "0, 0, 0" "0,360.000000, 0" _rotalpha_2) false false)
            (Transformation|SetRelativeLocation (Variables|Default|GetStaticMesh) (Math|Vector|Lerp(Vector) "0, 0, 0" "0, 0,-17.500000" _localpha_2) false false)
            (Transformation|SetRelativeLocation (Variables|Default|GetCube) (Math|Vector|Lerp(Vector) "0, 0,-50.000000" "0, 0,-67.500000" _localpha_2) false false))
          (:Finished
            (goto _label))
          (:NewTrack_2
            (goto _label_2))))
      (:then_2
        (Components|StaticMesh|SetStaticMesh (Variables|Default|GetStaticMesh) (Utilities|Select :Index (- (Variables|Default|GetChessPiece) 1) :Option%200 "/Game/Meshes/Chess/ChessPiece_Pawn.ChessPiece_Pawn" :Option%201 "/Game/Meshes/Chess/ChessPiece_Rook.ChessPiece_Rook" :Option%202 "/Game/Meshes/Chess/ChessPiece_Knight.ChessPiece_Knight" :Option%203 "/Game/Meshes/Chess/ChessPiece_Bishop.ChessPiece_Bishop" :Option%204 "/Game/Meshes/Chess/ChessPiece_Queen.ChessPiece_Queen" :Option%205 "/Game/Meshes/Chess/ChessPiece_King.ChessPiece_King") :!label _label_3)
        (Audio|PlaySoundatLocation "/Game/Audio/SFX/ScreenSaverCube.ScreenSaverCube" _returnvalue "0, 0, 0" 0.6 (Math|Random|RandomFloatinRange 0.8 1.1) 0.525 "/Game/Audio/Attenuation/SA_ShortRange.SA_ShortRange" "/Game/Audio/Attenuation/SC_Default.SC_Default" 0)
        (Audio|PlaySoundatLocation "/Game/Audio/SFX/MonitorEnter.MonitorEnter" _returnvalue_3 "0, 0, 0" 0.25 (Math|Random|RandomFloatinRange 0.77 1.1) 0.8 "/Game/Audio/Attenuation/SA_ShortRange.SA_ShortRange" "/Game/Audio/Attenuation/SC_Default.SC_Default" 0)))
    (else
      (Variables|Default|SetChessPiece (+ (Variables|Default|GetChessPiece) 1))
      (Utilities|FlowControl|Sequence
        (:then_0
          (Timeline|Timeline_0 Stop))
        (:then_1
          (Timeline|TL_Bounce PlayFromStart))
        (:then_2
          (goto _label_3))))))

(fn ConstructionScript
  (bind _cube (Variables|Default|GetCube))
  (bind _staticmesh (Variables|Default|GetStaticMesh))
  (Components|StaticMesh|SetStaticMesh (Variables|Default|GetStaticMesh) (Utilities|Select :Index (- (Variables|Default|GetChessPiece) 1) :Option%200 "/Game/Meshes/Chess/ChessPiece_Pawn.ChessPiece_Pawn" :Option%201 "/Game/Meshes/Chess/ChessPiece_Rook.ChessPiece_Rook" :Option%202 "/Game/Meshes/Chess/ChessPiece_Knight.ChessPiece_Knight" :Option%203 "/Game/Meshes/Chess/ChessPiece_Bishop.ChessPiece_Bishop" :Option%204 "/Game/Meshes/Chess/ChessPiece_Queen.ChessPiece_Queen" :Option%205 "/Game/Meshes/Chess/ChessPiece_King.ChessPiece_King"))
  (if (Variables|Default|GetBlack/White)
    (Rendering|Material|SetMaterial _staticmesh 0 "/Game/Materials/WoodBlockWhite_Inst.WoodBlockWhite_Inst")
    (else
      (Rendering|Material|SetMaterial _staticmesh 0 "/Game/Materials/WoodBlock_Mat_Inst_Inst.WoodBlock_Mat_Inst_Inst")))
  (if (Variables|Default|GetBaseMat)
    (Rendering|Material|SetMaterial _cube 0 "/Game/Materials/M_Metal_Steel2.M_Metal_Steel2")
    (else
      (Rendering|Material|SetMaterial _cube 0 "/Game/StarterContent/Materials/M_Metal_Brushed_NickelBlack.M_Metal_Brushed_NickelBlack"))))

(fn Attachto
  (params (ChildActor :type Actor%20Object%20Reference))
  (return 0))

(fn CanGrab
  (return false))

(fn Clicked
  (return false))

(fn DisableCollision
  (return false))

(fn DoesParentHaveParent
  (return false))

(fn EnableCollision
  (return false))

(fn GetAttached
  (return 0))

(fn GetCustomCursor
  (return false 0))

(fn GetShrinkScale
  (return "0, 0, 0" "0, 0, 0"))

(fn GetSnapLoc
  (params (CursorLoc :type Vector :default "0, 0, 0"))
  (return "0, 0, 0" "0, 0, 0"))

(fn Grabbed
  (return 0))

(fn LetGo
  (params (ParentComponent :type Actor%20Component%20Object%20Reference) (ParentActor :type Actor%20Object%20Reference))
  (return false))

(fn OnHover
  (return false))

(fn PassChildAlong
  (return 0 0))

(fn RightClickEvent
  (return (Variables|Default|GetClick%20Message) (Transformation|GetWorldLocation (Variables|Default|GetCapsule))))