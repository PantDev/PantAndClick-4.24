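; BP_ThumbTack is a grabbable thumbtack that stabs into the object it is dropped on.
; LetGo registers it with a BPI_CanClick parent, then a timeline lerps it from AnimRef to its mesh location.
; Landing triggers particles and sound, enables collision and notifies BPI_Bouncy parents; Grabbed clears the parent.
; Construction sets tint and optional physics; several interface functions, including hover, click and snap location, are stubs.
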(event Custom|LetGoEvent
  (Variables|Default|SetStartLoc (Transformation|GetWorldLocation (Variables|Default|GetAnimRef)))
  (Variables|Default|SetEndLoc (Transformation|GetWorldLocation (Variables|Default|GetStaticMesh)))
  (bind (_direction _alpha) (Timeline|StabAnim PlayFromStart)
    (:Update
      (Transformation|SetActorLocation (Math|Vector|Lerp(Vector) (Variables|Default|GetStartLoc) (Variables|Default|GetEndLoc) _alpha) false false))
    (:Finished
      (switch Utilities|FlowControl|Switch|SwitchonETimelineDirection _direction
        (:Forward
          (Components|Activation|Activate (Variables|Default|GetParticleSystem) false)
          (Audio|PlaySoundatLocation "/Game/Audio/SFX/Footstep.Footstep" (Transformation|GetActorLocation) "0, 0, 0" 0.3 0.8 0.01 "/Game/Audio/Attenuation/SA_Default.SA_Default" 0 0)
          (Collision|SetActorEnableCollision true)
          (bind _asbpi_bouncy (Utilities|Casting|CastToBPI_Bouncy (Variables|Default|GetParentActor))
            (:then
              (Class|BPICanClick|LetGo(Message) (Utilities|ToObject(Interface) _asbpi_bouncy)))
            (:CastFailed
              _))
          (Utilities|FlowControl|Delay 0.2)
          (Components|Activation|Deactivate (Variables|Default|GetParticleSystem)))))))

(event EventBeginPlay)

(event Collision|EventActorBeginOverlap
  (params (OtherActor :type Actor%20Object%20Reference)))

(event EventTick
  (params (DeltaSeconds :type Float%20%28single-precision%29)))

(fn ConstructionScript
  (Variables|Default|SetOriginalScale (Transformation|GetActorScale3D))
  (bind _returnvalue (Rendering|Material|CreateDynamicMaterialInstance (Variables|Default|GetStaticMesh) 0 "/Game/Materials/ThumbTack_Mat.ThumbTack_Mat" "None" :!class /Script/Engine.PrimitiveComponent))
  (bind _output_get (Variables|Default|SetMaterialInstance _returnvalue))
  (Rendering|Material|SetVectorParameterValue _output_get "Color" (Variables|Default|GetColor) :!class /Script/Engine.MaterialInstanceDynamic)
  (Physics|SetSimulatePhysics (Variables|Default|GetStaticMesh) (Variables|Default|GetActivatePhysics)))

(fn Attachto
  (params (ChildActor :type Actor%20Object%20Reference))
  (Utilities|Array|Add (Variables|Default|GetAttachedActors) ChildActor)
  (Variables|Default|SetHasAttached true)
  (return (Variables|Default|GetAttachedActors)))

(fn Clicked
  (return false))

(fn DisableCollision
  (Collision|SetCollisionEnabled (Variables|Default|GetStaticMesh) "NoCollision")
  (return false))

(fn DoesParentHaveParent
  (return false))

(fn EnableCollision
  (Collision|SetCollisionEnabled (Variables|Default|GetStaticMesh) "QueryAndPhysics")
  (return false))

(fn GetAttached
  (return (Variables|Default|GetAttachedActors)))

(fn GetShrinkScale
  (return (Variables|Default|GetShrinkScale) (Variables|Default|GetOriginalScale)))

(fn GetSnapLoc
  (params (CursorLoc :type Vector :default "0, 0, 0"))
  (return "0, 0, 0" "0, 0, 0"))

(fn Grabbed
  (bind _attachedactors (Class|BPICanClick|GetAttached(Message) (Variables|Default|GetParentActor)))
  (Utilities|Array|RemoveItem _attachedactors (Variables|Default|GetParentActor))
  (Variables|Default|SetParentActor 0)
  (return 0))

(fn LetGo
  (params (ParentComponent :type Actor%20Component%20Object%20Reference) (ParentActor :type Actor%20Object%20Reference))
  (Variables|Default|SetParentActor ParentActor)
  (bind _asbpi_can_click (Utilities|Casting|CastToBPI_CanClick ParentActor)
    (:then
      (bind _attachedactors (Default|Attachto _asbpi_can_click self)))
    (:CastFailed
      _))
  (CallFunction|LetGoEvent)
  (return false))

(fn OnHover
  (return false))

(fn PassChildAlong
  (return 0 0))