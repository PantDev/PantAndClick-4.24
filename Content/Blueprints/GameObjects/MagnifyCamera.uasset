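; MagnifyCamera is a camera actor with a spring arm and a 3D cursor for a magnify view.
; While Active, Tick moves the cursor to a set distance along the deprojected mouse ray, with DoOnce gates toggling its visibility as Active changes.
; MagnifyClick spawns two small camera-rotated click particles just beyond the cursor, one rolled 45 degrees.
; The construction script applies field of view, projection mode and arm length.
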(event Custom|MagnifyClick
  (bind _returnvalue (Game|GetPlayerCameraManager 0))
  (bind _returnvalue_2 (Game|GetPlayerCameraManager 0))
  (bind _cursor (Variables|Default|GetCursor))
  (bind _cursor_2 (Variables|Default|GetCursor))
  (bind _returnvalue_3 (Transformation|GetWorldLocation _cursor))
  (bind _returnvalue_4 (Transformation|GetWorldLocation _cursor_2))
  (bind _returnvalue_5 (Camera|GetCameraRotation _returnvalue_2))
  (bind _returnvalue_6 (Camera|GetCameraLocation _returnvalue))
  (bind (_roll _pitch _yaw) (Math|Rotator|BreakRotator _returnvalue_5))
  (bind _returnvalue_7 (Math|Rotator|FindLookatRotation _returnvalue_6 _returnvalue_4))
  (bind _returnvalue_8 (Math|Vector|GetForwardVector _returnvalue_7))
  (bind _returnvalue_9 (* _returnvalue_8 1e+01))
  (bind _returnvalue_10 (+ _returnvalue_9 _returnvalue_3))
  (Game|SpawnActorfromClass "/Game/Blueprints/FX/BP_ClickParticle.BP_ClickParticle_C" (Math|Transform|MakeTransform _returnvalue_10 (Camera|GetCameraRotation (Game|GetPlayerCameraManager 0)) "0.200000,0.200000,0.200000") "Undefined" 0 0)
  (Game|SpawnActorfromClass "/Game/Blueprints/FX/BP_ClickParticle.BP_ClickParticle_C" (Math|Transform|MakeTransform _returnvalue_10 (Math|Rotator|MakeRotator (+ _roll 45.0) _pitch _yaw) "0.200000,0.200000,0.200000") "Undefined" 0 0))

(event EventBeginPlay)

(event Collision|EventActorBeginOverlap
  (params (OtherActor :type Actor%20Object%20Reference)))

(event EventTick
  (params (DeltaSeconds :type Float%20%28single-precision%29))
  (bind _returnvalue (Game|GetPlayerController 0))
  (bind _cursor (Variables|Default|GetCursor))
  (bind _cursor_2 (Variables|Default|GetCursor))
  (bind (_worldlocation _worlddirection) (Game|Player|ConvertMouseLocationToWorldSpace _returnvalue))
  (if (Variables|Default|GetActive)
    (Utilities|FlowControl|Sequence
      (:then_0
        (Transformation|SetWorldLocation _cursor (Math|Interpolation|VInterptoConstant (Transformation|GetWorldLocation _cursor) (+ _worldlocation (* _worlddirection (Variables|Default|GetCursorDistance))) (Utilities|Time|GetWorldDeltaSeconds) 1e+06) false false)
        (Utilities|FlowControl|DoOnce false :!label _label
          (:Completed
            (Rendering|SetVisibility _cursor_2 true false))))
      (:then_1
        (goto _label_2 Reset)))
    (else
      (Utilities|FlowControl|Sequence
        (:then_0
          (goto _label Reset))
        (:then_1
          (Utilities|FlowControl|DoOnce false :!label _label_2
            (:Completed
              (Rendering|SetVisibility _cursor_2 false false))))))))

(fn ConstructionScript
  (bind _camera (Variables|Default|GetCamera))
  (Camera|SetFieldOfView _camera (Math|Conversions|ToFloat(Integer) (Variables|Default|GetFOV)))
  (Class|CameraComponent|SetProjectionMode _camera (Variables|Default|GetProjectionMode))
  (Variables|/Script/Engine.SpringArmComponent|SetTargetArmLength (Variables|Default|GetSpringArm) (Variables|Default|GetArmLength)))