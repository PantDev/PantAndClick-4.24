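; Checkpoint actor that becomes the player's respawn point when a BP_PantController overlaps it and it is not already active.
; Activation resets the previous checkpoint's decal and particles, then stores itself, its arrow's location and its rotation on the player character.
; It swaps to the active target decal, shows a dynamic-material glow, starts glow and decal-grow timelines, and briefly fires ring particles.
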(event Collision|EventActorBeginOverlap
  (params (OtherActor :type Actor%20Object%20Reference))
  (bind _asbp_pant_controller (Utilities|Casting|CastToBP_PantController OtherActor))
  (if (not (== (Variables|/Game/PantControllerBP/Blueprints/BP_PantController.BP_PantController_C|GetActiveCheckpoint _asbp_pant_controller) self))
    (CallFunction|ActivateFunc)
    (Components|Timeline|PlayfromStart (Variables|Default|GetDecalGrowAnim_TL))
    (Utilities|FlowControl|Delay 0.2)
    (Components|Activation|Deactivate (Variables|Default|GetRingParticles1))))

(event EventTick
  (params (DeltaSeconds :type Float%20%28single-precision%29)))

(fn ConstructionScript
  (bind _glow (Variables|Default|GetGlow))
  (bind _returnvalue (Rendering|Material|CreateDynamicMaterialInstance "/Game/Materials/Textures/TargetGlow_Mat.TargetGlow_Mat" "None" :!class /Script/Engine.KismetMaterialLibrary))
  (bind _output_get (Variables|Default|SetGlowInstance _returnvalue))
  (Rendering|Components|Decal|SetDecalMaterial _glow _output_get)
  (Rendering|SetVisibility _glow false false)
  (if (not (Variables|Default|GetActive))
    (Rendering|Components|Decal|SetDecalMaterial (Variables|Default|GetDecal) "/Game/Materials/Textures/Target_Mat1.Target_Mat1")))

(fn ActivateFunc
  (bind _asbp_pant_controller (Utilities|Casting|CastToBP_PantController (Game|GetPlayerCharacter 0)))
  (Rendering|Components|Decal|SetDecalMaterial (Variables|BP_Checkpoint_C|GetDecal (Variables|/Game/PantControllerBP/Blueprints/BP_PantController.BP_PantController_C|GetActiveCheckpoint _asbp_pant_controller)) "/Game/Materials/Textures/Target_Mat1.Target_Mat1")
  (Components|Activation|Deactivate (Variables|BP_Checkpoint_C|GetRingParticles1 (Variables|/Game/PantControllerBP/Blueprints/BP_PantController.BP_PantController_C|GetActiveCheckpoint _asbp_pant_controller)))
  (Variables|/Game/PantControllerBP/Blueprints/BP_PantController.BP_PantController_C|SetActiveCheckpoint _asbp_pant_controller self)
  (Variables|/Game/PantControllerBP/Blueprints/BP_PantController.BP_PantController_C|SetRespawnLoc _asbp_pant_controller (Transformation|GetWorldLocation (Variables|Default|GetArrow)))
  (Variables|/Game/PantControllerBP/Blueprints/BP_PantController.BP_PantController_C|SetSpawnRot _asbp_pant_controller (Transformation|GetActorRotation))
  (Components|Timeline|PlayfromStart (Variables|Default|GetActivateAnim_TL))
  (Rendering|SetVisibility (Variables|Default|GetGlow) true false)
  (Rendering|Components|Decal|SetDecalMaterial (Variables|Default|GetDecal) "/Game/Materials/Textures/Target_Mat.Target_Mat")
  (Components|Activation|Activate (Variables|Default|GetRingParticles1) false))