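; BP_ClickDialogue is an activatable dialogue object that shows a line of text in the player character's speech bubble.
; Activate interrupts any open bubble on BP_PantController, then opens one with its SpeechText and Length, passing close-look widget visibility when a BP_CloseLook is set.
; After Length plus a short delay it activates NextDialogue, if valid, so lines can chain.
; IsBusy always returns false.
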(event EventBeginPlay)

(event Collision|EventActorBeginOverlap
  (params (OtherActor :type Actor%20Object%20Reference)))

(event EventTick
  (params (DeltaSeconds :type Float%20%28single-precision%29)))

(event EventActivate
  (params (Delay :type Float%20%28single-precision%29) (Bool :type Boolean))
  (bind _length (Variables|Default|GetLength))
  (bind _nextdialogue (Variables|Default|GetNextDialogue))
  (bind _asbp_pant_controller (Utilities|Casting|CastToBP_PantController (Game|GetPlayerCharacter 0)))
  (if (Variables|/Game/PantControllerBP/Blueprints/BP_PantController.BP_PantController_C|GetIsBubbleOpen _asbp_pant_controller)
    (Variables|/Game/PantControllerBP/Blueprints/BP_PantController.BP_PantController_C|SetSpeechBreak _asbp_pant_controller true)
    (Audio|Components|Audio|Stop (Variables|/Game/PantControllerBP/Blueprints/BP_PantController.BP_PantController_C|GetTL_SpeechBubbleStay _asbp_pant_controller)))
  (Variables|/Game/PantControllerBP/Blueprints/BP_PantController.BP_PantController_C|SetSpeechText _asbp_pant_controller (Variables|Default|GetSpeech%20Text))
  (bind _asbp_close_look (Utilities|Casting|CastToBP_CloseLook (Variables|/Game/PantControllerBP/Blueprints/BP_PantController.BP_PantController_C|GetCloseLookActor _asbp_pant_controller))
    (:then
      (Default|OpenSpeechBubble _asbp_pant_controller _length (Widget|IsVisible (Variables|/Game/PantControllerBP/Blueprints/BP_PantController.BP_PantController_C|GetCloseLookWidget _asbp_pant_controller))))
    (:CastFailed
      (Default|OpenSpeechBubble _asbp_pant_controller _length false)))
  (Utilities|FlowControl|Delay (+ _length 0.5))
  (Utilities|IsValid _nextdialogue
    (:Is%20Valid
      (Default|Activate _nextdialogue 0.0 false))))

(fn ConstructionScript)

(fn IsBusy
  (return false))