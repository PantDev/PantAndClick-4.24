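; Clickable target for a score minigame, with point, penalty, gold, multi-hit and Play Button types that set its mesh and material.
; Activate runs timelines that delay, pop the target in, wait, then reverse it out, toggling collision.
; Cursor interface calls show a hover mesh and trigger hits, which play effects and update BP_PantController's count and widget.
; The +8 type swaps damage meshes before breaking; the Play Button activates TargetPlayGroup.
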(event Custom|ClickEvent
  (bind _returnvalue (Transformation|GetActorLocation))
  (bind _returnvalue_2 (Transformation|GetActorLocation))
  (bind _returnvalue_3 (Math|Random|RandomFloatinRange 1.5 2.0))
  (bind _targetmesh (Variables|Default|GetTargetMesh))
  (bind _targetmesh_2 (Variables|Default|GetTargetMesh))
  (bind _chipdamage (Variables|Default|GetChipDamage))
  (switch Utilities|FlowControl|Switch|SwitchonTarget_Enum (Variables|Default|GetTarget%20Type)
    (:NewEnumerator0
      (Audio|PlaySoundatLocation "/Game/Audio/SFX/LikeButtonOn.LikeButtonOn" (Transformation|GetActorLocation) "0, 0, 0" 0.1 (Math|Random|RandomFloatinRange 0.95 1.1) 0.26 "/Game/Audio/Attenuation/SA_ShortRange.SA_ShortRange" 0 0)
      (Camera|PlayWorldCameraShake "/Game/Effects/Other/BP_CameraShake.BP_CameraShake_C" (Transformation|GetActorLocation (Game|GetPlayerCharacter 0)) 0.0 1e+04 0.0)
      (Components|Activation|Activate (Variables|Default|GetTargetBreak) false)
      (Components|Activation|Deactivate (Variables|Default|GetPEN_FolderSpawn_System1) :!label _label)
      (Rendering|SetVisibility _targetmesh_2 false true)
      (Collision|SetCollisionEnabled _targetmesh_2 "NoCollision")
      (Audio|PlaySoundatLocation "/Game/Audio/SFX/Random_58.Random_58" (Transformation|GetActorLocation) "0, 0, 0" 0.42 (Math|Random|RandomFloatinRange 1.2 1.6) 0.16 "/Game/Audio/Attenuation/SA_ShortRange.SA_ShortRange" 0 0)
      (Utilities|FlowControl|Sequence :!label _label_2
        (:then_0
          (switch Utilities|FlowControl|Switch|SwitchonTarget_Enum (Variables|Default|GetTarget%20Type)
            (:NewEnumerator0
              (bind _asbp_pant_controller (Utilities|Casting|CastToBP_PantController (Game|GetPlayerCharacter 0)))
              (UserInterface|Animation|PlayAnimation (Variables|/Game/PantControllerBP/Blueprints/BP_PantController.BP_PantController_C|GetTargetCountWidget _asbp_pant_controller) (Variables|/Game/UserInterface/TargetCount_Widget.TargetCount_Widget_C|GetPlus1 (Variables|/Game/PantControllerBP/Blueprints/BP_PantController.BP_PantController_C|GetTargetCountWidget _asbp_pant_controller)) 0.0 1 "Forward" 1.0 false)
              (Variables|/Game/PantControllerBP/Blueprints/BP_PantController.BP_PantController_C|SetTargetCount _asbp_pant_controller (+ (Variables|/Game/PantControllerBP/Blueprints/BP_PantController.BP_PantController_C|GetTargetCount _asbp_pant_controller) 1)))
            (:NewEnumerator1
              (bind _asbp_pant_controller_2 (Utilities|Casting|CastToBP_PantController (Game|GetPlayerCharacter 0)))
              (UserInterface|Animation|PlayAnimation (Variables|/Game/PantControllerBP/Blueprints/BP_PantController.BP_PantController_C|GetTargetCountWidget _asbp_pant_controller_2) (Variables|/Game/UserInterface/TargetCount_Widget.TargetCount_Widget_C|GetNegative (Variables|/Game/PantControllerBP/Blueprints/BP_PantController.BP_PantController_C|GetTargetCountWidget _asbp_pant_controller_2)) 0.0 1 "Forward" 1.0 false)
              (Variables|/Game/PantControllerBP/Blueprints/BP_PantController.BP_PantController_C|SetTargetCount _asbp_pant_controller_2 (+ (Variables|/Game/PantControllerBP/Blueprints/BP_PantController.BP_PantController_C|GetTargetCount _asbp_pant_controller_2) -3)))
            (:NewEnumerator2
              (bind _asbp_pant_controller_3 (Utilities|Casting|CastToBP_PantController (Game|GetPlayerCharacter 0)))
              (UserInterface|Animation|PlayAnimation (Variables|/Game/PantControllerBP/Blueprints/BP_PantController.BP_PantController_C|GetTargetCountWidget _asbp_pant_controller_3) (Variables|/Game/UserInterface/TargetCount_Widget.TargetCount_Widget_C|GetPlus1 (Variables|/Game/PantControllerBP/Blueprints/BP_PantController.BP_PantController_C|GetTargetCountWidget _asbp_pant_controller_3)) 0.0 1 "Forward" 1.0 false)
              (Variables|/Game/PantControllerBP/Blueprints/BP_PantController.BP_PantController_C|SetTargetCount _asbp_pant_controller_3 (+ (Variables|/Game/PantControllerBP/Blueprints/BP_PantController.BP_PantController_C|GetTargetCount _asbp_pant_controller_3) 3)))
            (:NewEnumerator5
              (bind _asbp_pant_controller_4 (Utilities|Casting|CastToBP_PantController (Game|GetPlayerCharacter 0)))
              (UserInterface|Animation|PlayAnimation (Variables|/Game/PantControllerBP/Blueprints/BP_PantController.BP_PantController_C|GetTargetCountWidget _asbp_pant_controller_4) (Variables|/Game/UserInterface/TargetCount_Widget.TargetCount_Widget_C|GetPlus1 (Variables|/Game/PantControllerBP/Blueprints/BP_PantController.BP_PantController_C|GetTargetCountWidget _asbp_pant_controller_4)) 0.0 1 "Forward" 1.0 false)
              (UserInterface|Animation|PlayAnimation (Variables|/Game/PantControllerBP/Blueprints/BP_PantController.BP_PantController_C|GetTargetCountWidget _asbp_pant_controller_4) (Variables|/Game/UserInterface/TargetCount_Widget.TargetCount_Widget_C|GetPlusMore (Variables|/Game/PantControllerBP/Blueprints/BP_PantController.BP_PantController_C|GetTargetCountWidget _asbp_pant_controller_4)) 0.0 1 "Forward" 1.0 false)
              (Variables|/Game/PantControllerBP/Blueprints/BP_PantController.BP_PantController_C|SetTargetCount _asbp_pant_controller_4 (+ (Variables|/Game/PantControllerBP/Blueprints/BP_PantController.BP_PantController_C|GetTargetCount _asbp_pant_controller_4) 5)))
            (:NewEnumerator6
              (bind _asbp_pant_controller_5 (Utilities|Casting|CastToBP_PantController (Game|GetPlayerCharacter 0)))
              (UserInterface|Animation|PlayAnimation (Variables|/Game/PantControllerBP/Blueprints/BP_PantController.BP_PantController_C|GetTargetCountWidget _asbp_pant_controller_5) (Variables|/Game/UserInterface/TargetCount_Widget.TargetCount_Widget_C|GetPlus1 (Variables|/Game/PantControllerBP/Blueprints/BP_PantController.BP_PantController_C|GetTargetCountWidget _asbp_pant_controller_5)) 0.0 1 "Forward" 1.0 false)
              (UserInterface|Animation|PlayAnimation (Variables|/Game/PantControllerBP/Blueprints/BP_PantController.BP_PantController_C|GetTargetCountWidget _asbp_pant_controller_5) (Variables|/Game/UserInterface/TargetCount_Widget.TargetCount_Widget_C|GetPlusMore (Variables|/Game/PantControllerBP/Blueprints/BP_PantController.BP_PantController_C|GetTargetCountWidget _asbp_pant_controller_5)) 0.0 1 "Forward" 1.0 false)
              (Variables|/Game/PantControllerBP/Blueprints/BP_PantController.BP_PantController_C|SetTargetCount _asbp_pant_controller_5 (+ (Variables|/Game/PantControllerBP/Blueprints/BP_PantController.BP_PantController_C|GetTargetCount _asbp_pant_controller_5) 8))))
          (bind _asbp_pant_controller_6 (Utilities|Casting|CastToBP_PantController (Game|GetPlayerCharacter 0)))
          (if (== (Variables|/Game/PantControllerBP/Blueprints/BP_PantController.BP_PantController_C|GetTargetCount _asbp_pant_controller_6) (- 70 1))
            (UserInterface|Animation|PlayAnimation (Variables|/Game/PantControllerBP/Blueprints/BP_PantController.BP_PantController_C|GetTargetCountWidget _asbp_pant_controller_6) (Variables|/Game/UserInterface/TargetCount_Widget.TargetCount_Widget_C|GetNice (Variables|/Game/PantControllerBP/Blueprints/BP_PantController.BP_PantController_C|GetTargetCountWidget _asbp_pant_controller_6)) 0.0 1 "Forward" 1.0 false)))
        (:then_1
          (Utilities|FlowControl|Delay 1.0)
          (Components|Activation|Deactivate (Variables|Default|GetGoldBreak)))))
    (:NewEnumerator1
      (Camera|PlayWorldCameraShake "/Game/Effects/Other/BP_CameraShake1.BP_CameraShake1_C" (Transformation|GetActorLocation (Game|GetPlayerCharacter 0)) 0.0 1e+04 0.0)
      (Audio|PlaySoundatLocation "/Game/Audio/SFX/Random_58.Random_58" (Transformation|GetActorLocation) "0, 0, 0" 0.45 (Math|Random|RandomFloatinRange 1.4 1.8) 0.05 "/Game/Audio/Attenuation/SA_ShortRange.SA_ShortRange" 0 0)
      (Components|Activation|Activate (Variables|Default|GetRedBreak) false)
      (goto _label))
    (:NewEnumerator2
      (Audio|PlaySoundatLocation "/Game/Audio/SFX/LikeButtonOn.LikeButtonOn" (Transformation|GetActorLocation) "0, 0, 0" 0.16 (Math|Random|RandomFloatinRange 1.2 1.35) 0.26 "/Game/Audio/Attenuation/SA_ShortRange.SA_ShortRange" 0 0)
      (Components|Activation|Activate (Variables|Default|GetPlus3Break) false)
      (Camera|PlayWorldCameraShake "/Game/Effects/Other/BP_CameraShake.BP_CameraShake_C" (Transformation|GetActorLocation (Game|GetPlayerCharacter 0)) 0.0 1e+04 0.0)
      (goto _label))
    (:NewEnumerator5
      (Components|Activation|Activate (Variables|Default|GetGoldBreak) false)
      (Audio|PlaySoundatLocation "/Game/Audio/SFX/LikeButtonOn.LikeButtonOn" _returnvalue "0, 0, 0" 0.225 _returnvalue_3 0.26 "/Game/Audio/Attenuation/SA_ShortRange.SA_ShortRange" 0 0)
      (Audio|PlaySoundatLocation "/Game/Audio/SFX/CheckPoint.CheckPoint" _returnvalue "0, 0, 0" 0.3 _returnvalue_3 0.05 "/Game/Audio/Attenuation/SA_ShortRange.SA_ShortRange" 0 0)
      (Camera|PlayWorldCameraShake "/Game/Effects/Other/BP_CameraShake.BP_CameraShake_C" (Transformation|GetActorLocation (Game|GetPlayerCharacter 0)) 0.0 1e+04 0.0)
      (goto _label))
    (:NewEnumerator6
      (Audio|PlaySoundatLocation "/Game/Audio/SFX/Random_58.Random_58" (Transformation|GetActorLocation) "0, 0, 0" 0.355 (Math|Random|RandomFloatinRange 0.8 1.2) 0.16 "/Game/Audio/Attenuation/SA_ShortRange.SA_ShortRange" 0 0)
      (bind _output_get (Variables|Default|SetBreakInt (- (Variables|Default|GetBreakInt) 1)))
      (Math|Integer|CompareInt _output_get 1
        (:>
          (Math|Integer|CompareInt _output_get 2 :!label _label_3
            (:>
              (Components|StaticMesh|SetStaticMesh (Variables|Default|GetTargetMesh) "/Game/Meshes/Target_Oct_D1.Target_Oct_D1" :!label _label_4)
              (Components|StaticMesh|SetStaticMesh (Variables|Default|GetTargetMesh1) "/Game/Meshes/Target_Oct_D1.Target_Oct_D1"))
            (:==
              (goto _label_4))
            (:<
              (Math|Integer|CompareInt _output_get 1
                (:>
                  _)
                (:==
                  _)
                (:<
                  (Rendering|SetVisibility _targetmesh false true :!label _label_5)
                  (Collision|SetCollisionEnabled _targetmesh "NoCollision")
                  (Components|Activation|Activate (Variables|Default|GetPlus8Break) false)
                  (Audio|PlaySoundatLocation "/Game/Audio/SFX/LikeButtonOn.LikeButtonOn" _returnvalue_2 "0, 0, 0" 0.15 1.6 0.18 "/Game/Audio/Attenuation/SA_ShortRange.SA_ShortRange" 0 0)
                  (Audio|PlaySoundatLocation "/Game/Audio/SFX/CheckPoint.CheckPoint" _returnvalue_2 "0, 0, 0" 0.3 (Math|Random|RandomFloatinRange 1.7 2.3) 0.05 "/Game/Audio/Attenuation/SA_ShortRange.SA_ShortRange" 0 0)
                  (Camera|PlayWorldCameraShake "/Game/Effects/Other/BP_CameraShake.BP_CameraShake_C" (Transformation|GetActorLocation (Game|GetPlayerCharacter 0)) 0.0 1e+04 0.0)
                  (goto _label_2)))
              (Components|StaticMesh|SetStaticMesh (Variables|Default|GetTargetMesh) "/Game/Meshes/Target_Oct_D2.Target_Oct_D2")
              (Components|StaticMesh|SetStaticMesh (Variables|Default|GetTargetMesh1) "/Game/Meshes/Target_Oct_D2.Target_Oct_D2"))))
        (:==
          (goto _label_3))
        (:<
          (goto _label_5)))
      (Camera|PlayWorldCameraShake "/Game/Effects/Other/BP_CameraShake.BP_CameraShake_C" (Transformation|GetActorLocation (Game|GetPlayerCharacter 0)) 0.0 1e+04 0.0)
      (Components|Activation|Activate _chipdamage false)
      (Utilities|FlowControl|Delay 0.1)
      (Components|Activation|Deactivate _chipdamage))
    (:NewEnumerator7
      (Audio|PlaySoundatLocation "/Game/Audio/SFX/LikeButtonOn.LikeButtonOn" (Transformation|GetActorLocation) "0, 0, 0" 0.16 (Math|Random|RandomFloatinRange 1.2 1.35) 0.26 "/Game/Audio/Attenuation/SA_ShortRange.SA_ShortRange" 0 0)
      (Components|Activation|Activate (Variables|Default|GetTargetBreak) false)
      (Camera|PlayWorldCameraShake "/Game/Effects/Other/BP_CameraShake.BP_CameraShake_C" (Transformation|GetActorLocation (Game|GetPlayerCharacter 0)) 0.0 1e+04 0.0)
      (Default|Activate (Variables|Default|GetTargetPlayGroup) 0.0 false)
      (goto _label))))

(event EventBeginPlay
  (bind _targetmesh (Variables|Default|GetTargetMesh))
  (CallFunction|SetTargetMaterial)
  (switch Utilities|FlowControl|Switch|SwitchonTarget_Enum (Variables|Default|GetTarget%20Type)
    (:NewEnumerator0
      (Rendering|SetVisibility _targetmesh false false :!label _label)
      (Components|Activation|Deactivate (Variables|Default|GetPEN_FolderSpawn_System1))
      (Collision|SetCollisionEnabled _targetmesh "NoCollision"))
    (:NewEnumerator1
      (goto _label))
    (:NewEnumerator2
      (goto _label))
    (:NewEnumerator5
      (goto _label))
    (:NewEnumerator6
      (goto _label))
    (:NewEnumerator7
      (Rendering|SetVisibility _targetmesh true false)
      (Collision|SetCollisionEnabled _targetmesh "QueryOnly"))))

(event EventActivate
  (params (Delay :type Float%20%28single-precision%29) (Bool :type Boolean))
  (bind _targetmesh (Variables|Default|GetTargetMesh))
  (bind _targetmesh_2 (Variables|Default|GetTargetMesh))
  (bind _targetmesh_3 (Variables|Default|GetTargetMesh))
  (Components|Timeline|SetPlayRate (Variables|Default|GetTL_Delay) (/ 1.0 (Variables|Default|GetSpawnDelay)))
  (Timeline|TL_Delay PlayFromStart
    (:Finished
      (Audio|Components|Audio|Stop (Variables|Default|GetTL_Wait))
      (Transformation|SetWorldScale3D _targetmesh_2 "0, 0, 0")
      (Rendering|SetVisibility _targetmesh_2 true false)
      (Utilities|FlowControl|Sequence
        (:then_0
          (bind (_direction _sizealpha _rotation) (Timeline|TL_SpawnAnim PlayFromStart)
            (:Update
              (Transformation|SetWorldScale3D (Variables|Default|GetTargetMesh) (Math|Vector|Lerp(Vector) "0, 0, 0" "1.000000,0.750000,1.000000" _sizealpha))
              (Transformation|SetRelativeRotation (Variables|Default|GetTargetMesh) (Math|Rotator|MakeRotator 0.0 0.0 _rotation) false false))
            (:Finished
              (switch Utilities|FlowControl|Switch|SwitchonETimelineDirection _direction
                (:Forward
                  (Timeline|TL_Wait PlayFromStart
                    (:Finished
                      (Components|Timeline|ReversefromEnd (Variables|Default|GetTL_SpawnAnim)))))
                (:Backward
                  (Components|Activation|Deactivate (Variables|Default|GetPEN_FolderSpawn_System1))
                  (Rendering|SetVisibility _targetmesh_3 false true)
                  (Collision|SetCollisionEnabled _targetmesh_3 "NoCollision"))))
            (:Event
              (Variables|Default|SetBreakInt 5)
              (switch Utilities|FlowControl|Switch|SwitchonETimelineDirection _direction
                (:Forward
                  (Collision|SetCollisionEnabled _targetmesh "QueryAndPhysics"))
                (:Backward
                  (Collision|SetCollisionEnabled _targetmesh "NoCollision"))))))
        (:then_1
          (Audio|PlaySoundatLocation "/Game/Audio/SFX/OpenSpeech.OpenSpeech" (Transformation|GetActorLocation) "0, 0, 0" 0.1 (Math|Random|RandomFloatinRange 0.6 1.2) 0.06 "/Game/Audio/Attenuation/SA_ShortRange.SA_ShortRange" 0 0)
          (CallFunction|SetTargetMaterial))))))

(event EventEndOverlap
  (Rendering|SetVisibility (Variables|Default|GetTargetMesh1) false false))

(fn ConstructionScript
  (CallFunction|SetTargetMaterial))

(fn SetTargetMaterial
  (bind _targetmesh (Variables|Default|GetTargetMesh))
  (bind _targetmesh_2 (Variables|Default|GetTargetMesh))
  (switch Utilities|FlowControl|Switch|SwitchonTarget_Enum (Variables|Default|GetTarget%20Type)
    (:NewEnumerator0
      (Rendering|Material|SetMaterial _targetmesh 0 "/Game/Materials/Target_Mat2.Target_Mat2")
      (Components|StaticMesh|SetStaticMesh (Variables|Default|GetTargetMesh) "/Game/Meshes/Target.Target" :!label _label)
      (Components|StaticMesh|SetStaticMesh (Variables|Default|GetTargetMesh1) "/Game/Meshes/Target.Target"))
    (:NewEnumerator1
      (Rendering|Material|SetMaterial _targetmesh 0 "/Game/Materials/Target_Mat3.Target_Mat3")
      (goto _label))
    (:NewEnumerator2
      (Rendering|Material|SetMaterial _targetmesh 0 "/Game/Materials/Target_Mat4.Target_Mat4")
      (goto _label))
    (:NewEnumerator5
      (Rendering|Material|SetMaterial _targetmesh 0 "/Game/Materials/Target_Mat5.Target_Mat5")
      (Rendering|Material|SetMaterial _targetmesh 1 "/Game/Meshes/GoldenGibEdge_Mat.GoldenGibEdge_Mat")
      (Components|Activation|Activate (Variables|Default|GetPEN_FolderSpawn_System1) false)
      (goto _label))
    (:NewEnumerator6
      (Components|StaticMesh|SetStaticMesh _targetmesh_2 "/Game/Meshes/Target_Oct.Target_Oct")
      (Components|StaticMesh|SetStaticMesh (Variables|Default|GetTargetMesh1) "/Game/Meshes/Target_Oct.Target_Oct")
      (Rendering|Material|SetMaterial _targetmesh_2 0 "/Game/Materials/Target_8_Mat.Target_8_Mat"))
    (:NewEnumerator7
      (Rendering|Material|SetMaterial _targetmesh 0 "/Game/Materials/Target_Play_Mat.Target_Play_Mat")
      (goto _label))))

(fn Attachto
  (params (ChildActor :type Actor%20Object%20Reference))
  (return 0))

(fn CanGrab
  (return false))

(fn Clicked
  (if (Rendering|IsVisible (Variables|Default|GetTargetMesh))
    (CallFunction|ClickEvent))
  (return false))

(fn DisableCollision
  (return false))

(fn DoesParentHaveParent
  (return false))

(fn EnableCollision
  (return false))

(fn GetAttached
  (return 0))

(fn GetCustomCursor
  (return true "/Game/Meshes/Cursor_Crosshair.Cursor_Crosshair"))

(fn GetShrinkScale
  (return "0, 0, 0" "0, 0, 0"))

(fn GetSnapLoc
  (params (CursorLoc :type Vector :default "0, 0, 0"))
  (return "0, 0, 0" "0, 0, 0"))

(fn Grabbed
  (return 0))

(fn IsBusy
  (return false))

(fn LetGo
  (params (ParentComponent :type Actor%20Component%20Object%20Reference) (ParentActor :type Actor%20Object%20Reference))
  (return false))

(fn OnHover
  (if (Rendering|IsVisible (Variables|Default|GetTargetMesh))
    (Rendering|SetVisibility (Variables|Default|GetTargetMesh1) true false))
  (return false))

(fn PassChildAlong
  (return 0 0))