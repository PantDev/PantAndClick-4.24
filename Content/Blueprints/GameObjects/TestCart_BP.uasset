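; Test cart actor that plays a randomized jump when its PokeEvent fires.
; A timeline at random play rate lifts CartMesh while jump and landing animations play, with landing triggered by an event track.
; Afterwards it returns to a rolling loop, occasionally playing an alternate roll first.
; BeginPlay and the sequence's end call JumpAnim, which is empty, and the grab, attach and cursor functions are default-returning stubs.
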(event Custom|JumpAnim)

(event EventBeginPlay
  (CallFunction|JumpAnim))

(event Collision|EventActorBeginOverlap
  (params (OtherActor :type Actor%20Object%20Reference)))

(event EventTick
  (params (DeltaSeconds :type Float%20%28single-precision%29)))

(event EventPokeEvent
  (bind _cartmesh (Variables|Default|GetCartMesh))
  (Variables|Default|SetJumpAnimSpeed (Math|Random|RandomFloatinRange 0.8 (Variables|Default|GetMaxSpeed)))
  (Components|Timeline|SetPlayRate (Variables|Default|GetTL_JumpAnim) (Variables|Default|GetJumpAnimSpeed))
  (Components|Timeline|SetPlayRate _cartmesh 2.5)
  (Components|Animation|PlayAnimation _cartmesh "/Game/Meshes/Skeletal/CraftCart_Anim_Mult_Anim_Armature_Jump1.CraftCart_Anim_Mult_Anim_Armature_Jump1" false)
  (bind _jumplerp (Timeline|TL_JumpAnim PlayFromStart)
    (:Update
      (Transformation|SetRelativeLocation (Variables|Default|GetCartMesh) (Math|Vector|Lerp(Vector) "0, 0, 0" (Math|Vector|MakeVector 0.0 0.0 2.5e+02) _jumplerp) false false))
    (:Finished
      (Utilities|FlowControl|Delay 2.5)
      (if (>= (Math|Random|RandomIntegerinRange 0 10) 8)
        (Components|Animation|PlayAnimation (Variables|Default|GetCartMesh) "/Game/Meshes/Skeletal/CraftCart_Anim_Mult_Anim_Armature_RollLoop1.CraftCart_Anim_Mult_Anim_Armature_RollLoop1" true)
        (Utilities|FlowControl|Delay 3.0))
      (Components|Animation|PlayAnimation (Variables|Default|GetCartMesh) "/Game/Meshes/Skeletal/CraftCart_Anim_Mult_Anim_Armature_RollLoop0.CraftCart_Anim_Mult_Anim_Armature_RollLoop0" true)
      (Utilities|FlowControl|Delay (Math|Random|RandomFloatinRange 0.5 1.5))
      (CallFunction|JumpAnim))
    (:NewTrack_1
      (Components|Timeline|SetPlayRate _cartmesh 1.0)
      (Components|Animation|PlayAnimation (Variables|Default|GetCartMesh) "/Game/Meshes/Skeletal/CraftCart_Anim_Mult_Anim_Armature_JumpLand.CraftCart_Anim_Mult_Anim_Armature_JumpLand" false))))

(fn ConstructionScript)

(fn Attachto
  (params (ChildActor :type Actor%20Object%20Reference))
  (return 0))

(fn CanGrab
  (return false))

(fn Clicked
  (return false))

(fn DisableCollision
  (return false))

(fn DoesParentHaveParent
  (return false))

(fn EnableCollision
  (return false))

(fn GetAttached
  (return 0))

(fn GetCustomCursor
  (return false 0))

(fn GetShrinkScale
  (return "0, 0, 0" "0, 0, 0"))

(fn GetSnapLoc
  (params (CursorLoc :type Vector :default "0, 0, 0"))
  (return "0, 0, 0" "0, 0, 0"))

(fn Grabbed
  (return 0))

(fn LetGo
  (params (ParentComponent :type Actor%20Component%20Object%20Reference) (ParentActor :type Actor%20Object%20Reference))
  (return false))

(fn OnHover
  (return false))

(fn PassChildAlong
  (return 0 0))