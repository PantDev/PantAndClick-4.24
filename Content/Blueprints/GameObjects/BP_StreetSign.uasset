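; Poke-reactive street sign prop with selectable diamond, speed or stop shape and custom face material.
; The construction script swaps skeletal mesh, material and matching collision boxes; BeginPlay enables an extra box only when InHalls.
; Pokes are debounced, alternating two flick animations with a pitch-randomised bounce sound and varied play rate, occasionally slowing and starting TLSpin.
; A separate TL_Spin rotation graph never runs, and most interaction functions are stubs.
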(event EventBeginPlay
  (bind _speedbox2 (Variables|Default|GetSpeedBox2))
  (if (Variables|Default|GetInHalls)
    (Collision|SetCollisionEnabled _speedbox2 "QueryAndPhysics")
    (else
      (Collision|SetCollisionEnabled _speedbox2 "NoCollision"))))

(event EventPokeEvent
  (bind _signmesh (Variables|Default|GetSignMesh))
  (Utilities|FlowControl|DoOnce false :!label _label
    (:Completed
      (Utilities|FlowControl|FlipFlop
        (:A
          (Components|Animation|PlayAnimation _signmesh "/Game/Meshes/Skeletal/StreetSign_Diamond_Skeletal_Anim_Armature_Flick1.StreetSign_Diamond_Skeletal_Anim_Armature_Flick1" false))
        (:B
          (Components|Animation|PlayAnimation _signmesh "/Game/Meshes/Skeletal/StreetSign_Diamond_Skeletal_Anim_Armature_Flick2.StreetSign_Diamond_Skeletal_Anim_Armature_Flick2" false)))
      (if (> (Math|Random|RandomFloat) 0.7)
        (Components|Timeline|PlayfromStart (Variables|Default|GetTL_Spin))
        (Components|Timeline|SetPlayRate _signmesh 0.6)
        (else
          (Components|Timeline|SetPlayRate _signmesh (Math|Random|RandomFloatinRange 1.2 1.6))))
      (Audio|PlaySoundatLocation "/Game/Audio/SFX/Bounce.Bounce" (Transformation|GetActorLocation) "0, 0, 0" 1.5 (Math|Random|RandomFloatinRange 1.1 1.3) 0.1 0 0 0)
      (Utilities|FlowControl|Delay 0.225)
      (goto _label Reset))))

(fn ConstructionScript
  (bind _signmesh (Variables|Default|GetSignMesh))
  (bind _diamondbox (Variables|Default|GetDiamondBox))
  (bind _speedbox (Variables|Default|GetSpeedBox))
  (bind _diamondbox1 (Variables|Default|GetDiamondBox1))
  (bind _speedbox1 (Variables|Default|GetSpeedBox1))
  (switch int (Variables|Default|GetSignShape)
    (:1
      (Class|SkinnedMeshComponent|SetSkeletalMesh _signmesh "/Game/Meshes/Skeletal/StreetSign_Diamond_Skeletal.StreetSign_Diamond_Skeletal" true)
      (Class|BPICanClick|EnableCollision(Message) _diamondbox :!label _label)
      (Class|BPICanClick|EnableCollision(Message) _diamondbox1)
      (Class|BPICanClick|DisableCollision(Message) _speedbox)
      (Class|BPICanClick|DisableCollision(Message) _speedbox1))
    (:2
      (Class|SkinnedMeshComponent|SetSkeletalMesh _signmesh "/Game/Meshes/Skeletal/StreetSign_Speed_Skeletal.StreetSign_Speed_Skeletal" true)
      (Class|BPICanClick|DisableCollision(Message) _diamondbox)
      (Class|BPICanClick|DisableCollision(Message) _diamondbox1)
      (Class|BPICanClick|EnableCollision(Message) _speedbox)
      (Class|BPICanClick|EnableCollision(Message) _speedbox1))
    (:3
      (Class|SkinnedMeshComponent|SetSkeletalMesh _signmesh "/Game/Meshes/Skeletal/StreetSign_Stop_Skeletal.StreetSign_Stop_Skeletal" true)
      (goto _label)))
  (Rendering|Material|SetMaterial (Variables|Default|GetSignMesh) 1 (Variables|Default|GetSignMat)))

(fn Attachto
  (params (ChildActor :type Actor%20Object%20Reference))
  (return 0))

(fn CanGrab
  (return false))

(fn Clicked
  (return false))

(fn DisableCollision
  (return false))

(fn DoesParentHaveParent
  (return false))

(fn EnableCollision
  (return false))

(fn GetAttached
  (return 0))

(fn GetCustomCursor
  (return false 0))

(fn GetShrinkScale
  (return "0, 0, 0" "0, 0, 0"))

(fn GetSnapLoc
  (params (CursorLoc :type Vector :default "0, 0, 0"))
  (return "0, 0, 0" "0, 0, 0"))

(fn Grabbed
  (return 0))

(fn LetGo
  (params (ParentComponent :type Actor%20Component%20Object%20Reference) (ParentActor :type Actor%20Object%20Reference))
  (return false))

(fn OnHover
  (return false))

(fn PassChildAlong
  (return 0 0))

(fn RightClickEvent
  (return (Variables|Default|GetClick%20Message) (Transformation|GetWorldLocation (Variables|Default|GetDiamondBox))))