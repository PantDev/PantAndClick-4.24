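; Clickable, non-grabbable chameleon object that shows a crosshair cursor and turns into a decal when clicked.
; Clicked hides the ChameleonMan mesh, disables its collision, reveals the decal and calls ClickEvent.
; ClickEvent plays a pitch-randomized sound, camera shake, brief particle burst and scale-bounce timeline.
; Most other interaction functions are stubs, while RightClickEvent returns a message and the mesh's location as focus point.
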(event Custom|ClickEvent
  (bind _chameleonman (Variables|Default|GetChameleonMan))
  (bind _tl_bounce (Variables|Default|GetTL_Bounce))
  (bind _returnvalue (Transformation|GetWorldLocation _chameleonman))
  (Audio|PlaySoundatLocation "/Game/Audio/SFX/Random_58.Random_58" _returnvalue "0, 0, 0" 0.3 (Math|Random|RandomFloatinRange 0.6 0.85) 0.14 "/Game/Audio/Attenuation/SA_ShortRange.SA_ShortRange" "/Game/Audio/Attenuation/SC_Default.SC_Default" 0)
  (Camera|PlayWorldCameraShake "/Game/Effects/Other/BP_CameraShake1.BP_CameraShake1_C" _returnvalue 5e+03 1e+04)
  (Components|Activation|Activate (Variables|Default|GetParticleSystem) false)
  (Components|Timeline|SetPlayRate _tl_bounce 2.0)
  (Components|Timeline|PlayfromStart _tl_bounce)
  (Utilities|FlowControl|Delay 0.25)
  (Components|Activation|Deactivate (Variables|Default|GetParticleSystem)))

(event EventBeginPlay)

(event Collision|EventActorBeginOverlap
  (params (OtherActor :type Actor%20Object%20Reference)))

(event EventTick
  (params (DeltaSeconds :type Float%20%28single-precision%29)))

(fn ConstructionScript)

(fn Attachto
  (params (ChildActor :type Actor%20Object%20Reference))
  (return 0))

(fn CanGrab
  (return false))

(fn Clicked
  (bind _chameleonman (Variables|Default|GetChameleonMan))
  (Rendering|SetVisibility _chameleonman false false)
  (Collision|SetCollisionEnabled _chameleonman "NoCollision")
  (Rendering|SetVisibility (Variables|Default|GetDecal) true false)
  (CallFunction|ClickEvent)
  (return false))

(fn DisableCollision
  (return false))

(fn DoesParentHaveParent
  (return false))

(fn EnableCollision
  (return false))

(fn GetAttached
  (return 0))

(fn GetCustomCursor
  (return true "/Game/Meshes/Cursor_Crosshair.Cursor_Crosshair"))

(fn GetShrinkScale
  (return "0, 0, 0" "0, 0, 0"))

(fn GetSnapLoc
  (params (CursorLoc :type Vector :default "0, 0, 0"))
  (return "0, 0, 0" "0, 0, 0"))

(fn Grabbed
  (return 0))

(fn LetGo
  (params (ParentComponent :type Actor%20Component%20Object%20Reference) (ParentActor :type Actor%20Object%20Reference))
  (return false))

(fn OnHover
  (return false))

(fn PassChildAlong
  (return 0 0))

(fn RightClickEvent
  (return (Variables|Default|GetClick%20Message) (Transformation|GetWorldLocation (Variables|Default|GetChameleonMan))))