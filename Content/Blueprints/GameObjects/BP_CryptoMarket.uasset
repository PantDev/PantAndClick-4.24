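; Crypto market prop: a fake price chart that faces the player camera and rerolls when poked, with a sound and bounce timeline.
; Tick draws the chart as debug lines through sixteen point components.
; A poke rapidly shifts point heights along the array, feeding a clamped random walk into the last.
; Comparing end heights then colors the line red or green and triggers the arrow-flip timeline when the trend changes.
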(event Custom|FlipArrow
  (Components|Timeline|PlayfromStart (Variables|Default|GetTL_FlipArrow)))

(event Custom|SuperPushEvent
  (bind _arrowisupsidedown (Variables|Default|GetArrowIsUpsideDown))
  (CallFunction|AdvanceArrayElems)
  (Utilities|FlowControl|Delay 0.01)
  (CallFunction|AdvanceArrayElems)
  (Utilities|FlowControl|Delay 0.01)
  (CallFunction|AdvanceArrayElems)
  (Utilities|FlowControl|Delay 0.01)
  (CallFunction|AdvanceArrayElems)
  (Utilities|FlowControl|Delay 0.01)
  (CallFunction|AdvanceArrayElems)
  (Utilities|FlowControl|Delay 0.01)
  (CallFunction|AdvanceArrayElems)
  (Utilities|FlowControl|Delay 0.01)
  (CallFunction|AdvanceArrayElems)
  (Utilities|FlowControl|Delay 0.01)
  (CallFunction|AdvanceArrayElems)
  (Utilities|FlowControl|Delay 0.01)
  (CallFunction|AdvanceArrayElems)
  (Utilities|FlowControl|Delay 0.01)
  (CallFunction|AdvanceArrayElems)
  (Utilities|FlowControl|Delay 0.01)
  (CallFunction|AdvanceArrayElems)
  (Utilities|FlowControl|Delay 0.01)
  (CallFunction|AdvanceArrayElems)
  (Utilities|FlowControl|Delay 0.01)
  (CallFunction|AdvanceArrayElems)
  (Utilities|FlowControl|Delay 0.01)
  (CallFunction|AdvanceArrayElems)
  (Utilities|FlowControl|Delay 0.01)
  (CallFunction|AdvanceArrayElems)
  (Utilities|FlowControl|Delay 0.01)
  (CallFunction|AdvanceArrayElems)
  (Utilities|FlowControl|Delay 0.01)
  (if (> (.Z (Math|Vector|BreakVector (Transformation|GetWorldLocation (Variables|Default|GetPoint1)))) (.Z (Math|Vector|BreakVector (Transformation|GetWorldLocation (Variables|Default|GetPoint16)))))
    (Variables|Default|SetLine%20Color "(R=1.000000,G=0.000000,B=0.007345,A=1.000000)")
    (if (not _arrowisupsidedown)
      (CallFunction|FlipArrow :!label _label))
    (else
      (Variables|Default|SetLine%20Color "(R=0.000000,G=1.000000,B=0.038961,A=1.000000)")
      (if _arrowisupsidedown
        (goto _label)))))

(event EventPokeEvent
  (CallFunction|SuperPushEvent)
  (Audio|PlaySoundatLocation "/Game/Audio/SFX/ScreenSaverCube.ScreenSaverCube" (Transformation|GetActorLocation) "0, 0, 0" 0.6 (Math|Random|RandomFloatinRange 0.8 0.95) 0.2 "/Game/Audio/Attenuation/SA_Default.SA_Default" "/Game/Audio/Attenuation/SC_Default.SC_Default" 0)
  (Components|Timeline|PlayfromStart (Variables|Default|GetTL_Bounce)))

(event EventTick
  (params (DeltaSeconds :type Float%20%28single-precision%29))
  (bind _returnvalue (Transformation|GetActorLocation))
  (bind _returnvalue_2 (Game|GetPlayerCameraManager 0))
  (bind _returnvalue_3 (Camera|GetCameraLocation _returnvalue_2))
  (bind _returnvalue_4 (Math|Rotator|FindLookatRotation _returnvalue _returnvalue_3))
  (bind (_roll _pitch _yaw) (Math|Rotator|BreakRotator _returnvalue_4))
  (CallFunction|DrawLines)
  (Variables|Default|SetTargetRot (Math|Interpolation|RInterpTo (Transformation|GetWorldRotation (Variables|Default|GetStaticMesh)) (Math|Rotator|MakeRotator _roll 0.0 (+ _yaw -9e+01)) (Utilities|Time|GetWorldDeltaSeconds) 1e+01))
  (Transformation|SetWorldRotation (Variables|Default|GetStaticMesh) (Variables|Default|GetTargetRot) false false))

(fn ConstructionScript
  (Variables|Default|SetPointObjectArray (Utilities|Array|MakeArray (Variables|Default|GetPoint1) (Variables|Default|GetPoint2) (Variables|Default|GetPoint3) (Variables|Default|GetPoint4) (Variables|Default|GetPoint5) (Variables|Default|GetPoint6) (Variables|Default|GetPoint7) (Variables|Default|GetPoint8) (Variables|Default|GetPoint9) (Variables|Default|GetPoint10) (Variables|Default|GetPoint11) (Variables|Default|GetPoint12) (Variables|Default|GetPoint13) (Variables|Default|GetPoint14) (Variables|Default|GetPoint15) (Variables|Default|GetPoint16))))

(fn DrawLines
  (for (_array_element _array_index) (Variables|Default|GetPointObjectArray)
    (if (== _array_index 0)
      (Variables|Default|SetStartLoc (Transformation|GetWorldLocation _array_element))
      (else
        (Rendering|Debug|DrawDebugLine (Variables|Default|GetStartLoc) (Transformation|GetWorldLocation _array_element) (Variables|Default|GetLine%20Color) 0.05 2.0)
        (Variables|Default|SetStartLoc (Transformation|GetWorldLocation _array_element))))))

(fn AdvanceArrayElems
  (bind _pointobjectarray (Variables|Default|GetPointObjectArray))
  (for (_array_element _array_index) (Variables|Default|GetPointObjectArray)
    (if (== _array_index 15)
      (Transformation|SetRelativeLocationAndRotation _array_element (Math|Vector|MakeVector (.X (Math|Vector|BreakVector (Variables|/Script/Engine.SceneComponent|GetRelativeLocation _array_element))) (.Y (Math|Vector|BreakVector (Variables|/Script/Engine.SceneComponent|GetRelativeLocation _array_element))) (Math|Float|Clamp(Float) (+ (.Z (Math|Vector|BreakVector (Variables|/Script/Engine.SceneComponent|GetRelativeLocation (Utilities|Array|Get(acopy) _pointobjectarray (- _array_index 1))))) (Math|Random|RandomFloatinRange -3e+01 3e+01)) -1.5e+02 2.5e+02)) "0, 0, 0" false false)
      (else
        (Transformation|SetRelativeLocationAndRotation _array_element (Math|Vector|MakeVector (.X (Math|Vector|BreakVector (Variables|/Script/Engine.SceneComponent|GetRelativeLocation _array_element))) (.Y (Math|Vector|BreakVector (Variables|/Script/Engine.SceneComponent|GetRelativeLocation _array_element))) (.Z (Math|Vector|BreakVector (Variables|/Script/Engine.SceneComponent|GetRelativeLocation (Utilities|Array|Get(acopy) _pointobjectarray (+ _array_index 1)))))) "0, 0, 0" false false)))))

(fn Attachto
  (params (ChildActor :type Actor%20Object%20Reference))
  (return 0))

(fn CanGrab
  (return false))

(fn Clicked
  (return false))

(fn DisableCollision
  (return false))

(fn DoesParentHaveParent
  (return false))

(fn EnableCollision
  (return false))

(fn GetAttached
  (return 0))

(fn GetCustomCursor
  (return false 0))

(fn GetShrinkScale
  (return "0, 0, 0" "0, 0, 0"))

(fn GetSnapLoc
  (params (CursorLoc :type Vector :default "0, 0, 0"))
  (return "0, 0, 0" "0, 0, 0"))

(fn Grabbed
  (return 0))

(fn LetGo
  (params (ParentComponent :type Actor%20Component%20Object%20Reference) (ParentActor :type Actor%20Object%20Reference))
  (return false))

(fn OnHover
  (return false))

(fn PassChildAlong
  (return 0 0))