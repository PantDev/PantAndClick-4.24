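; Screensaver cube that acts as a bouncy prop, returning a launch velocity with a sound, particle burst and wobble when poked.
; GetLaunchVelocity restarts timelines for balloon morph, bounce scale and spin, unless a bounce is already playing.
; Hidden cubes start invisible without collision until SpawnEntity scales them up, pokes them and enables overlaps.
; Grab, click and attach interface functions are mostly stubs.
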(event EventBeginPlay
  (bind _box (Variables|Default|GetBox))
  (bind _cubemesh (Variables|Default|GetCubeMesh))
  (bind _box_2 (Variables|Default|GetBox))
  (if (Variables|Default|GetHidden)
    (Rendering|SetVisibility _cubemesh false false)
    (Collision|SetCollisionEnabled _box_2 "NoCollision")
    (Collision|SetCollisionResponsetoChannel _box_2 "ECC_WorldDynamic" "ECR_Ignore")
    (else
      (Rendering|SetVisibility _cubemesh true false)
      (Collision|SetCollisionEnabled _box "QueryAndPhysics")
      (Collision|SetCollisionResponsetoChannel _box "ECC_WorldDynamic" "ECR_Overlap"))))

(event Collision|EventActorBeginOverlap
  (params (OtherActor :type Actor%20Object%20Reference)))

(event EventTick
  (params (DeltaSeconds :type Float%20%28single-precision%29)))

(event EventPokeEvent
  (CallFunction|GetLaunchVelocity))

(event EventSpawnEntity
  (bind _box (Variables|Default|GetBox))
  (bind _tl_scaleup (Variables|Default|GetTL_ScaleUp))
  (Components|Timeline|SetPlayRate _tl_scaleup 0.5)
  (Components|Timeline|PlayfromStart _tl_scaleup)
  (CallFunction|PokeEvent)
  (Rendering|SetVisibility (Variables|Default|GetCubeMesh) true false)
  (Collision|SetCollisionEnabled _box "QueryAndPhysics")
  (Collision|SetCollisionResponsetoChannel _box "ECC_WorldDynamic" "ECR_Overlap"))

(fn ConstructionScript
  (Components|Timeline|SetPlayRate (Variables|Default|GetTL_Sphere) 0.25)
  (Rendering|SetCastShadow (Variables|Default|GetCubeMesh) (Variables|Default|GetCastShadow)))

(fn Attachto
  (params (ChildActor :type Actor%20Object%20Reference))
  (return 0))

(fn CanGrab
  (return false))

(fn Clicked
  (return false))

(fn DisableCollision
  (return false))

(fn DoesParentHaveParent
  (return false))

(fn EnableCollision
  (return false))

(fn GetAttached
  (return 0))

(fn GetCustomCursor
  (return false 0))

(fn GetLaunchVelocity
  (bind _tl_balloon (Variables|Default|GetTL_Balloon))
  (bind _tl_bouncerot (Variables|Default|GetTL_BounceRot))
  (if (not (Audio|Components|Audio|IsPlaying (Variables|Default|GetTL_BounceScale)))
    (Audio|PlaySoundatLocation "/Game/Audio/SFX/ScreenSaverCube.ScreenSaverCube" (Transformation|GetActorLocation) "0, 0, 0" 1.0 (Math|Random|RandomFloatinRange 0.9 1.1) 0.0 "/Game/Audio/Attenuation/SA_ShortRange.SA_ShortRange" "/Game/Audio/Attenuation/SC_Default.SC_Default" 0)
    (Components|Timeline|SetPlayRate _tl_balloon 2.0)
    (Components|Timeline|SetPlayRate (Variables|Default|GetTL_BounceScale) 1.0)
    (Components|Timeline|PlayfromStart _tl_balloon)
    (Audio|Components|Audio|Stop _tl_bouncerot)
    (Components|Timeline|PlayfromStart _tl_bouncerot)
    (Components|Activation|Activate (Variables|Default|GetScreenSaverShape_Emitter) false)
    (return (Variables|Default|GetVelocity))))

(fn GetShrinkScale
  (return "0, 0, 0" "0, 0, 0"))

(fn GetSnapLoc
  (params (CursorLoc :type Vector :default "0, 0, 0"))
  (return "0, 0, 0" "0, 0, 0"))

(fn Grabbed
  (return 0))

(fn LetGo
  (params (ParentComponent :type Actor%20Component%20Object%20Reference) (ParentActor :type Actor%20Object%20Reference))
  (return false))

(fn OnHover
  (return false))

(fn PassChildAlong
  (return 0 0))

(fn RightClickEvent
  (return (Variables|Default|GetClick%20Message) (Transformation|GetActorLocation)))