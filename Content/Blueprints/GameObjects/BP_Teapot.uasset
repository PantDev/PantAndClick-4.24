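; Teapot game object that, while active, supplies a launch velocity and plays a squash-and-spin reaction whenever that velocity is requested.
; Activate and Deactivate toggle steam, Box2 collision and a timeline-faded audio loop.
; PokeEvent plays a timeline driving morph targets, rotation and spring arm length, plus click and landing sounds.
; Overlapping pokes wait, then replay faster, scaling deformation and pitch range until the timeline finishes.
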(event EventBeginPlay
  ;[1 1 1] Begin Play
  (Components|Timeline|SetPlayRate (Variables|Default|GetTL_Clicked) 1.25))

(event EventActivate
  (params (Direction :type SteamDir_Enum%20Enum :default "NewEnumerator0"))
  (bind _audio (Variables|Default|GetAudio))
  (Components|Activation|Activate (Variables|Default|GetP_Steam) false)
  (Collision|SetCollisionEnabled (Variables|Default|GetBox2) "NoCollision")
  (Variables|Default|Setactive true)
  (Components|Activation|Activate (Variables|Default|GetAudio) false)
  (bind (_direction _newtrack_0) (Timeline|TL_AudioVol Play)
    (:Update
      (Audio|Components|Audio|SetVolumeMultiplier _audio _newtrack_0 :!class /Script/Engine.AudioComponent))
    (:Finished
      (switch Utilities|FlowControl|Switch|SwitchonETimelineDirection _direction
        (:Backward
          (Components|Activation|Deactivate _audio))))))

(event EventDeactivate
  (params (Direction :type SteamDir_Enum%20Enum :default "NewEnumerator0"))
  (bind _audio (Variables|Default|GetAudio))
  (Components|Activation|Deactivate (Variables|Default|GetP_Steam))
  (Collision|SetCollisionEnabled (Variables|Default|GetBox2) "QueryAndPhysics")
  (Variables|Default|Setactive false)
  (bind (_direction _newtrack_0) (Timeline|TL_AudioVol Reverse)
    (:Update
      (Audio|Components|Audio|SetVolumeMultiplier _audio _newtrack_0 :!class /Script/Engine.AudioComponent))
    (:Finished
      (switch Utilities|FlowControl|Switch|SwitchonETimelineDirection _direction
        (:Backward
          (Components|Activation|Deactivate _audio))))))

(event EventPokeEvent
  (bind _returnvalue (Transformation|GetActorLocation))
  (bind _skeletalmesh (Variables|Default|GetSkeletalMesh))
  (bind _tl_clicked (Variables|Default|GetTL_Clicked))
  (bind _tl_clicked_2 (Variables|Default|GetTL_Clicked))
  (bind _skeletalmesh_2 (Variables|Default|GetSkeletalMesh))
  (bind (_x _y _z) (Math|Vector|BreakVector _returnvalue))
  (if (Audio|Components|Audio|IsPlaying (Variables|Default|GetTL_Clicked))
    ;[1 1 1] WaitTilEnd
    ; Put
    (Utilities|FlowControl|Delay (- (/ 1.0 (Components|Animation|GetPlayRate _tl_clicked)) (Components|Timeline|GetPlaybackPosition _tl_clicked))))
  (Components|Timeline|SetPlayRate _tl_clicked_2 (* (Components|Animation|GetPlayRate _tl_clicked_2) 1.05))
  (Audio|PlaySoundatLocation (Utilities|Select :Index (Math|Random|RandomIntegerinRange 0 1) :Option%200 "/Game/Audio/SFX/ClickMusicSFX/Click1.Click1" :Option%201 "/Game/Audio/SFX/ClickMusicSFX/Click2.Click2" :Option%202 0) (Transformation|GetActorLocation) "0, 0, 0" 0.4 (Math|Random|RandomFloatinRange 0.7 (* (Components|Animation|GetPlayRate (Variables|Default|GetTL_Clicked)) 0.8)) 0.0 "/Game/Audio/Attenuation/SA_ShortRange.SA_ShortRange" 0 0)
  ;[1 1 1] TL_Clicked
  (bind (_direction _squash _lid _handle _rotation) (Timeline|TL_Clicked PlayFromStart)
    (:Update
      (Components|SkeletalMesh|SetMorphTarget _skeletalmesh_2 "Squash" (* _squash (Components|Animation|GetPlayRate (Variables|Default|GetTL_Clicked))) true)
      (Components|SkeletalMesh|SetMorphTarget _skeletalmesh_2 "Lid" (* _lid (Components|Animation|GetPlayRate (Variables|Default|GetTL_Clicked))) true)
      (Components|SkeletalMesh|SetMorphTarget _skeletalmesh_2 "Spout" (* (Components|Animation|GetPlayRate (Variables|Default|GetTL_Clicked)) _handle) true)
      (Components|SkeletalMesh|SetMorphTarget _skeletalmesh_2 "Handle" (* (Components|Animation|GetPlayRate (Variables|Default|GetTL_Clicked)) _handle) true)
      (Transformation|SetRelativeRotation (Variables|Default|GetSkeletalMesh) (Math|Rotator|Lerp(Rotator) "0, 0, 0" "0,360.000000, 0" _rotation) false false)
      (Variables|/Script/Engine.SpringArmComponent|SetTargetArmLength (Variables|Default|GetSpringArm) (Math|Float|Lerp 0.0 -2.5e+02 _handle)))
    (:Finished
      (Components|Timeline|SetPlayRate (Variables|Default|GetTL_Clicked) 1.25)
      (Components|SkeletalMesh|SetMorphTarget _skeletalmesh "Squash" 0.0 true)
      (Components|SkeletalMesh|SetMorphTarget _skeletalmesh "Lid" 0.0 true)
      (Components|SkeletalMesh|SetMorphTarget _skeletalmesh "Spout" 0.0 true)
      (Components|SkeletalMesh|SetMorphTarget _skeletalmesh "Handle" 0.0 true))
    (:LandFX
      (Audio|PlaySoundatLocation "/Game/Audio/DAW/SFX/Snare.Snare" (Math|Vector|MakeVector _x _y (+ _z 5e+01)) "0, 0, 0" 0.2 (Math|Random|RandomFloatinRange 1.3 1.5) 0.02 "/Game/Audio/Attenuation/SA_ShortRange.SA_ShortRange" 0 0))))

(fn ConstructionScript)

(fn Attachto
  (params (ChildActor :type Actor%20Object%20Reference))
  (return 0))

(fn CanGrab
  (return false))

(fn Clicked
  (return false))

(fn DisableCollision
  (return false))

(fn DoesParentHaveParent
  (return false))

(fn EnableCollision
  (return false))

(fn GetAttached
  (return 0))

(fn GetCustomCursor
  (return false 0))

(fn GetLaunchVelocity
  (if (Variables|Default|Getactive)
    (CallFunction|PokeEvent)
    (return (Variables|Default|GetVelocity))))

(fn GetShrinkScale
  (return "0, 0, 0" "0, 0, 0"))

(fn GetSnapLoc
  (params (CursorLoc :type Vector :default "0, 0, 0"))
  (return "0, 0, 0" "0, 0, 0"))

(fn Grabbed
  (return 0))

(fn LetGo
  (params (ParentComponent :type Actor%20Component%20Object%20Reference) (ParentActor :type Actor%20Object%20Reference))
  (return false))

(fn OnHover
  (return false))

(fn PassChildAlong
  (return 0 0))