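; BP_Greg is a talking NPC with an optional hat that can turn to face the player camera.
; Each poke shows the next InString line in a dialogue widget, dismissing any other active NPC through the player's CurrentNPC.
; Timelines drive hat bounce and face morphs, while Tick fakes speech with random animation positions and click sounds.
; A sphere overlap gates box collision and closes dialogue when the player leaves.
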(event OnComponentBeginOverlap(Sphere)
  (params (OverlappedComponent :type Primitive%20Component%20Object%20Reference) (OtherActor :type Actor%20Object%20Reference) (OtherComp :type Primitive%20Component%20Object%20Reference) (OtherBodyIndex :type Integer) (bFromSweep :type Boolean) (SweepResult :type Hit%20Result%20Structure%20%28by%20ref%29))
  (bind _asbp_pant_controller (Utilities|Casting|CastToBP_PantController OtherActor))
  (if (== (Variables|/Game/PantControllerBP/Blueprints/BP_PantController.BP_PantController_C|GetCapsule _asbp_pant_controller) OtherComp)
    (Variables|Default|SetIsOver true)))

(event OnComponentEndOverlap(Sphere)
  (params (OverlappedComponent :type Primitive%20Component%20Object%20Reference) (OtherActor :type Actor%20Object%20Reference) (OtherComp :type Primitive%20Component%20Object%20Reference) (OtherBodyIndex :type Integer))
  (bind _dialogueboxwidget (Variables|Default|GetDialogueBoxWidget))
  (bind _asbp_pant_controller (Utilities|Casting|CastToBP_PantController OtherActor))
  (if (== (Variables|/Game/PantControllerBP/Blueprints/BP_PantController.BP_PantController_C|GetCapsule _asbp_pant_controller) OtherComp)
    (Variables|/Game/PantControllerBP/Blueprints/BP_PantController.BP_PantController_C|SetCurrentNPC _asbp_pant_controller 0)
    (Variables|Default|SetIsOver false)
    (Utilities|IsValid _dialogueboxwidget
      (:Is%20Valid
        (if (Widget|IsVisible _dialogueboxwidget)
          (Audio|Components|Audio|Stop (Variables|Default|Getdelay))
          (Variables|Default|SetCurrentMsgInt 0)
          (CallFunction|OffGreg))))))

(event Custom|OffGreg
  (bind _skeletalmesh (Variables|Default|GetSkeletalMesh))
  (bind _skeletalmesh_2 (Variables|Default|GetSkeletalMesh))
  (bind _dialogueboxwidget (Variables|Default|GetDialogueBoxWidget))
  (bind _skeletalmesh_3 (Variables|Default|GetSkeletalMesh))
  (bind _tl_hatbounce (Variables|Default|GetTL_HatBounce))
  (bind _dialogueboxwidget_2 (Variables|Default|GetDialogueBoxWidget))
  (Variables|Default|SetCurrentMsgInt 0)
  (bind _asbp_pant_controller (Utilities|Casting|CastToBP_PantController (Game|GetPlayerCharacter 0)))
  (Variables|/Game/PantControllerBP/Blueprints/BP_PantController.BP_PantController_C|SetCurrentNPC _asbp_pant_controller 0)
  (if (Audio|Components|Audio|IsPlaying (Variables|Default|GetTL_HatBounce))
    _
    (else
      (Components|Timeline|SetPlaybackPosition _tl_hatbounce 0.34 false true)
      (Audio|Components|Audio|Play _tl_hatbounce)))
  (Audio|Components|Audio|Stop (Variables|Default|GetSkeletalMesh))
  (Audio|PlaySoundatLocation "/Game/Audio/SFX/KnobLeft.KnobLeft" (Transformation|GetActorLocation) "0, 0, 0" 0.15 (Math|Random|RandomFloatinRange 1.2 1.55) 0.52 "/Game/Audio/Attenuation/SA_ShortRange.SA_ShortRange" 0 0)
  (Audio|Components|Audio|Stop _skeletalmesh)
  (Components|Animation|SetPosition _skeletalmesh 0.0 true)
  (Audio|Components|Audio|Stop (Variables|Default|Getdelay))
  (Components|SkeletalMesh|SetMorphTarget _skeletalmesh_3 "sinister" 0.0 true)
  (Components|SkeletalMesh|SetMorphTarget _skeletalmesh_3 "ee" 0.0 true)
  (Utilities|IsValid _dialogueboxwidget_2
    (:Is%20Valid
      (Class|UserWidget|PlayAnimationReverse _dialogueboxwidget_2 (Variables|/Game/UserInterface/DialogueBox_Widget.DialogueBox_Widget_C|GetSpawn _dialogueboxwidget_2) 1.55 false))
    (:Is%20Not%20Valid
      _))
  (Components|Timeline|SetPlayRate (Variables|Default|GetTimeline_0) 1.25)
  (bind _newtrack_0 (Timeline|Timeline_0 PlayFromStart)
    (:Update
      (Components|SkeletalMesh|SetMorphTarget (Variables|Default|GetSkeletalMesh) "head_squash" _newtrack_0 true))
    (:Finished
      (Audio|Components|Audio|Stop _skeletalmesh_2)
      (Components|Animation|SetPosition _skeletalmesh_2 0.0 true)
      (Utilities|IsValid _dialogueboxwidget
        (:Is%20Valid
          (Widget|RemovefromParent _dialogueboxwidget))))))

(event EventBeginPlay
  (Components|Timeline|PlayfromStart (Variables|Default|GetTL_Bob)))

(event EventPokeEvent
  (bind _skeletalmesh (Variables|Default|GetSkeletalMesh))
  (Audio|Components|Audio|Stop (Variables|Default|Getdelay))
  (if (== (Variables|Default|GetCurrentMsgInt) (Utilities|Array|Length (Variables|Default|GetIn%20String)))
    (Variables|Default|SetCurrentMsgInt 0)
    (CallFunction|OffGreg)
    (else
      (Variables|Default|SetCurrentMsgInt (+ (Variables|Default|GetCurrentMsgInt) 1))
      (bind _asbp_pant_controller (Utilities|Casting|CastToBP_PantController (Game|GetPlayerCharacter 0)))
      (Utilities|IsValid (Variables|/Game/PantControllerBP/Blueprints/BP_PantController.BP_PantController_C|GetCurrentNPC _asbp_pant_controller)
        (:Is%20Valid
          (if (== (Variables|/Game/PantControllerBP/Blueprints/BP_PantController.BP_PantController_C|GetCurrentNPC _asbp_pant_controller) self)
            _
            (else
              (Variables|Default|SetRemoteGreg true)
              (CallFunction|OffGreg (Variables|/Game/PantControllerBP/Blueprints/BP_PantController.BP_PantController_C|GetCurrentNPC _asbp_pant_controller))
              (Variables|/Game/PantControllerBP/Blueprints/BP_PantController.BP_PantController_C|SetCurrentNPC _asbp_pant_controller self :!label _label))))
        (:Is%20Not%20Valid
          (goto _label)))
      (Components|Timeline|PlayfromStart (Variables|Default|GetTL_HatBounce))
      (Utilities|IsValid (Variables|Default|GetDialogueBoxWidget)
        (:Is%20Valid
          (Widget|RemovefromParent (Variables|Default|GetDialogueBoxWidget)))
        (:Is%20Not%20Valid
          _))
      (bind _returnvalue (UserInterface|CreateWidget "/Game/UserInterface/DialogueBox_Widget.DialogueBox_Widget_C" (Game|GetPlayerController 0)))
      (bind _output_get (Variables|Default|SetDialogueBoxWidget _returnvalue))
      (UserInterface|Viewport|AddtoViewport _output_get 0)
      (if (== (Variables|Default|GetCurrentMsgInt) 1)
        (Class|UserWidget|PlayAnimationForward (Variables|Default|GetDialogueBoxWidget) (Variables|/Game/UserInterface/DialogueBox_Widget.DialogueBox_Widget_C|GetSpawn (Variables|Default|GetDialogueBoxWidget)) 1.2 false))
      (Rendering|Components|TextRender|SetText (Variables|/Game/UserInterface/DialogueBox_Widget.DialogueBox_Widget_C|GetRichText (Variables|Default|GetDialogueBoxWidget)) (Utilities|Text|ToText(String) (Utilities|Array|Get(acopy) (Variables|Default|GetIn%20String) (- (Variables|Default|GetCurrentMsgInt) 1))))
      (Components|Animation|PlayAnimation (Variables|Default|GetSkeletalMesh) "/Game/Meshes/GregFace_BooBoo_Anim1_Anim.GregFace_BooBoo_Anim1_Anim" true)
      (Audio|PlaySoundatLocation "/Game/Audio/SFX/KnobRight.KnobRight" (Transformation|GetActorLocation) "0, 0, 0" 0.15 (Math|Random|RandomFloatinRange 1.4 1.8) 0.45 "/Game/Audio/Attenuation/SA_ShortRange.SA_ShortRange" 0 0)
      (Components|Timeline|PlayfromStart (Variables|Default|Getdelay))
      (Components|SkeletalMesh|SetMorphTarget _skeletalmesh "sinister" 0.0 true)
      (Components|SkeletalMesh|SetMorphTarget _skeletalmesh "ee" 0.0 true))))

(event EventTick
  (params (DeltaSeconds :type Float%20%28single-precision%29))
  (bind _returnvalue (Transformation|GetActorRotation))
  (bind _dialogueboxwidget (Variables|Default|GetDialogueBoxWidget))
  (bind _box (Variables|Default|GetBox))
  (bind (_roll _pitch) (Math|Rotator|BreakRotator _returnvalue))
  (if (Variables|Default|GetIsOver)
    (Collision|SetCollisionEnabled _box "QueryAndPhysics")
    (else
      (Collision|SetCollisionEnabled _box "NoCollision")))
  (bind _asbp_pant_controller (Utilities|Casting|CastToBP_PantController (Game|GetPlayerCharacter 0)))
  (if (Variables|Default|GetFacingPlayer)
    (Transformation|SetActorRotation (Math|Rotator|MakeRotator _roll _pitch (+ (.Yaw (Math|Rotator|BreakRotator (Math|Rotator|FindLookatRotation (Transformation|GetActorLocation) (Transformation|GetWorldLocation (Variables|/Game/PantControllerBP/Blueprints/BP_PantController.BP_PantController_C|GetFollowCamera _asbp_pant_controller))))) -9e+01))))
  (Utilities|IsValid _dialogueboxwidget
    (:Is%20Valid
      (if (and (Widget|IsVisible _dialogueboxwidget) (Variables|Default|Getdelayvar))
        (Components|Animation|SetPosition (Variables|Default|GetSkeletalMesh) (Math|Random|RandomFloatinRange 0.0 1.3) true)
        (Audio|PlaySoundatLocation "/Game/Audio/SFX/ClickMusicSFX/Click2.Click2" (Transformation|GetActorLocation) "0, 0, 0" 0.2 (Math|Random|RandomFloatinRange 1.2 2.0) 0.15 "/Game/Audio/Attenuation/SA_ShortRange.SA_ShortRange" 0 0)))))

(fn ConstructionScript
  (bind _hatmesh (Variables|Default|GetHatMesh))
  (bind _hatmeshcomp (Variables|Default|GetHatMeshComp))
  (bind _hatmesh_2 (Variables|Default|GetHatMesh))
  (bind _hatmesh_3 (Variables|Default|GetHatMesh))
  (Utilities|IsValid _hatmesh_2
    (:Is%20Valid
      (Rendering|SetVisibility _hatmeshcomp true false)
      (Components|StaticMesh|SetStaticMesh _hatmeshcomp _hatmesh_2)
      (Rendering|Material|SetMaterial _hatmeshcomp 0 (Rendering|Material|GetMaterial _hatmesh_3 0))
      (Rendering|Material|SetMaterial _hatmeshcomp 1 (Rendering|Material|GetMaterial _hatmesh_3 1))
      (Rendering|Material|SetMaterial _hatmeshcomp 2 (Rendering|Material|GetMaterial _hatmesh 2))
      (Rendering|Material|SetMaterial _hatmeshcomp 3 (Rendering|Material|GetMaterial _hatmesh 3)))
    (:Is%20Not%20Valid
      (Rendering|SetVisibility (Variables|Default|GetHatMeshComp) false false))))

(fn IntEqualCheck
  (bind _returnvalue (Math|Random|RandomIntegerinRange 0 5))
  (Components|SkeletalMesh|SetMorphTarget (Variables|Default|GetSkeletalMesh) "sinister" 0.0 true)
  (Components|SkeletalMesh|SetMorphTarget (Variables|Default|GetSkeletalMesh) "oo" 0.0 true)
  (Components|SkeletalMesh|SetMorphTarget (Variables|Default|GetSkeletalMesh) "ee" 0.0 true)
  (Components|SkeletalMesh|SetMorphTarget (Variables|Default|GetSkeletalMesh) "aa" 0.0 true)
  (Components|SkeletalMesh|SetMorphTarget (Variables|Default|GetSkeletalMesh) "ff" 0.0 true)
  (Components|SkeletalMesh|SetMorphTarget (Variables|Default|GetSkeletalMesh) "mm" 0.0 true)
  (Components|SkeletalMesh|SetMorphTarget (Variables|Default|GetSkeletalMesh) "bb" 0.0 true)
  (if (== (Variables|Default|Getvowelint) _returnvalue)
    (if (== (Variables|Default|Getvowelint) 5)
      (Variables|Default|Setvowelint 0)
      (else
        (bind _result (Math|Integer|IncrementInt (Variables|Default|Getvowelint))
          (:%20%20
            (Variables|Default|Setvowelint _result)))))
    (else
      (Variables|Default|Setvowelint _returnvalue))))

(fn Attachto
  (params (ChildActor :type Actor%20Object%20Reference))
  (return 0))

(fn CanGrab
  (return false))

(fn Clicked
  (return false))

(fn DisableCollision
  (return false))

(fn DoesParentHaveParent
  (return false))

(fn EnableCollision
  (return false))

(fn GetAttached
  (return 0))

(fn GetCustomCursor
  (return false 0))

(fn GetShrinkScale
  (return "0, 0, 0" "0, 0, 0"))

(fn GetSnapLoc
  (params (CursorLoc :type Vector :default "0, 0, 0"))
  (return "0, 0, 0" "0, 0, 0"))

(fn Grabbed
  (return 0))

(fn LetGo
  (params (ParentComponent :type Actor%20Component%20Object%20Reference) (ParentActor :type Actor%20Object%20Reference))
  (return false))

(fn OnHover
  (return false))

(fn PassChildAlong
  (return 0 0))