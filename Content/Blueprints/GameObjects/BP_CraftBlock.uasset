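; Breakable Minecraft-style block in four types (default, dirt, stone, glass) that cracks when landed on or poked, then bursts and releases its contents.
; Each hit bounces it; once armor is depleted, a dynamic material's BreakX/BreakY parameters advance the crack stage until destruction.
; Wait and reverse timelines reset cracks on non-glass blocks, while a randomly timed upward trace turns uncovered dirt into the default block.
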(event Custom|FakeSpawn
  (bind _fakespawnedactor (Variables|Default|GetFakeSpawnedActor))
  (Class|BPISpawnable|SpawnEntity(Message) _fakespawnedactor)
  (Transformation|SetActorLocation _fakespawnedactor (Transformation|GetActorLocation) false true))

(event EventEndOverlap
  (Rendering|SetVisibility (Variables|Default|GetOutlineMesh) false false)
  (Variables|Default|SetIsHover false))

(event EventBeginPlay
  (bind _tl_checkabove (Variables|Default|GetTL_CheckAbove))
  (Components|Timeline|SetPlayRate _tl_checkabove (Math|Random|RandomFloatinRange 0.5 1.0))
  (Components|Timeline|PlayfromStart _tl_checkabove))

(event EventOnLand
  (bind _returnvalue (Transformation|GetActorLocation))
  (bind _returnvalue_2 (Transformation|GetActorLocation))
  (bind _tl_bounce (Variables|Default|GetTL_Bounce))
  (bind _contains (Variables|Default|GetContains))
  (bind _breakmesh (Variables|Default|GetBreakMesh))
  (bind _staticmesh (Variables|Default|GetStaticMesh))
  (if (not (Variables|Default|GetDestroyed))
    (Audio|Components|Audio|Stop _tl_bounce)
    (if (> (Variables|Default|GetBlockType) 1)
      (Components|Timeline|PlayfromStart (Variables|Default|GetTL_SubtleBounce))
      (else
        (Components|Timeline|PlayfromStart _tl_bounce)))
    (if (== (Variables|Default|GetBlockType) 3)
      _
      (else
        (Components|Timeline|PlayfromStart (Variables|Default|GetTL_Wait))))
    (Audio|PlaySoundatLocation "/Game/Audio/SFX/Bite1.Bite1" _returnvalue_2 "0, 0, 0" 0.4 (Math|Random|RandomFloatinRange 0.6 0.85) 0.19 "/Game/Audio/Attenuation/SA_ShortRange.SA_ShortRange" 0 0)
    (Audio|PlaySoundatLocation "/Game/Audio/SFX/ButtonPress1.ButtonPress1" _returnvalue_2 "0, 0, 0" 0.8 (Math|Random|RandomFloatinRange 1.2 1.5) 0.09 "/Game/Audio/Attenuation/SA_ShortRange.SA_ShortRange" 0 0)
    (Utilities|FlowControl|Sequence
      (:then_0
        (Utilities|FlowControl|DoOnce false
          (:Completed
            (if (== (Variables|Default|GetBlockType) 3)
              (bind _returnvalue_3 (Rendering|Material|CreateDynamicMaterialInstance _breakmesh 0 "/Game/Materials/CraftBlockBreak2_Mat.CraftBlockBreak2_Mat" "None" :!class /Script/Engine.PrimitiveComponent))
              (Variables|Default|SetDynamicMat _returnvalue_3)
              (else
                (bind _returnvalue_4 (Rendering|Material|CreateDynamicMaterialInstance _breakmesh 0 "/Game/Materials/CraftBlockBreak_Mat.CraftBlockBreak_Mat" "None" :!class /Script/Engine.PrimitiveComponent))
                (Variables|Default|SetDynamicMat _returnvalue_4)))
            (Rendering|Material|SetMaterial (Variables|Default|GetBreakMesh) 0 (Variables|Default|GetDynamicMat)))))
      (:then_1
        (if (> (Variables|Default|GetArmor) 0)
          (Variables|Default|SetArmor (- (Variables|Default|GetArmor) 1))
          (else
            (Variables|Default|SetArmor (Variables|Default|GetArmorStart))
            (Rendering|SetVisibility (Variables|Default|GetBreakMesh) true false)
            (bind _returnvalue_5 (Rendering|Material|GetScalarParameterValue (Variables|Default|GetDynamicMat) "BreakX" :!class /Script/Engine.MaterialInstanceDynamic))
            (bind _returnvalue_6 (Rendering|Material|GetScalarParameterValue (Variables|Default|GetDynamicMat) "BreakY" :!class /Script/Engine.MaterialInstanceDynamic))
            (if (and (== _returnvalue_5 0.75) (== _returnvalue_6 0.75))
              (Variables|Default|SetDestroyed true)
              (Rendering|SetVisibility _staticmesh false true)
              (Collision|SetCollisionEnabled _staticmesh "NoCollision")
              (Components|DestroyComponent (Variables|Default|GetBox))
              (Audio|PlaySoundatLocation "/Game/Audio/SFX/ButtonPress1.ButtonPress1" _returnvalue "0, 0, 0" 1.2 (Math|Random|RandomFloatinRange 0.6 0.8) 0.08 "/Game/Audio/Attenuation/SA_ShortRange.SA_ShortRange" 0 0)
              (Audio|PlaySoundatLocation "/Game/Audio/SFX/Pop.Pop" _returnvalue "0, 0, 0" 1.4 (Math|Random|RandomFloatinRange 0.6 0.7) 0.02 "/Game/Audio/Attenuation/SA_ShortRange.SA_ShortRange" 0 0)
              (Utilities|IsValid (Variables|Default|GetFakeSpawnedActor)
                (:Is%20Valid
                  (CallFunction|FakeSpawn))
                (:Is%20Not%20Valid
                  (if (Utilities|IsValidClass _contains)
                    (bind _returnvalue_7 (Game|SpawnActorfromClass _contains (Transformation|GetActorTransform) "Undefined" 0 0))
                    (if (Utilities|DoesObjectImplementInterface _returnvalue_7 "/Game/Blueprints/BPI/BPI_Spawnable.BPI_Spawnable_C")
                      (Class|BPISpawnable|SpawnEntity(Message) _returnvalue_7)))))
              (switch int (Variables|Default|GetBlockType)
                (:0
                  (Components|Activation|Activate (Variables|Default|GetNiagara) false))
                (:1
                  (Components|Activation|Activate (Variables|Default|GetNiagaraDirt) false))
                (:2
                  (Components|Activation|Activate (Variables|Default|GetNiagaraStone) false))
                (:3
                  (Components|Activation|Activate (Variables|Default|GetNiagaraGlass) false)))
              (Utilities|FlowControl|Delay 1.0)
              (Actor|DestroyActor)
              (else
                (bind _returnvalue_8 (Rendering|Material|GetScalarParameterValue (Variables|Default|GetDynamicMat) "BreakX" :!class /Script/Engine.MaterialInstanceDynamic))
                (if (== _returnvalue_8 0.75)
                  (Rendering|Material|SetScalarParameterValue (Variables|Default|GetDynamicMat) "BreakX" 0.0 :!class /Script/Engine.MaterialInstanceDynamic)
                  (Rendering|Material|SetScalarParameterValue (Variables|Default|GetDynamicMat) "BreakY" 0.75 :!class /Script/Engine.MaterialInstanceDynamic)
                  (else
                    (Rendering|Material|SetScalarParameterValue (Variables|Default|GetDynamicMat) "BreakX" (+ _returnvalue_8 0.25) :!class /Script/Engine.MaterialInstanceDynamic)))))))))))

(event EventPokeEvent
  (bind _returnvalue (Transformation|GetActorLocation))
  (bind _returnvalue_2 (Transformation|GetActorLocation))
  (bind _tl_bounce (Variables|Default|GetTL_Bounce))
  (bind _contains (Variables|Default|GetContains))
  (bind _breakmesh (Variables|Default|GetBreakMesh))
  (bind _staticmesh (Variables|Default|GetStaticMesh))
  (if (not (Variables|Default|GetDestroyed))
    (Audio|Components|Audio|Stop _tl_bounce)
    (if (> (Variables|Default|GetBlockType) 1)
      (Components|Timeline|PlayfromStart (Variables|Default|GetTL_SubtleBounce))
      (else
        (Components|Timeline|PlayfromStart _tl_bounce)))
    (if (== (Variables|Default|GetBlockType) 3)
      _
      (else
        (Components|Timeline|PlayfromStart (Variables|Default|GetTL_Wait))))
    (Audio|PlaySoundatLocation "/Game/Audio/SFX/Bite1.Bite1" _returnvalue_2 "0, 0, 0" 0.4 (Math|Random|RandomFloatinRange 0.6 0.85) 0.19 "/Game/Audio/Attenuation/SA_ShortRange.SA_ShortRange" 0 0)
    (Audio|PlaySoundatLocation "/Game/Audio/SFX/ButtonPress1.ButtonPress1" _returnvalue_2 "0, 0, 0" 0.8 (Math|Random|RandomFloatinRange 1.2 1.5) 0.09 "/Game/Audio/Attenuation/SA_ShortRange.SA_ShortRange" 0 0)
    (Utilities|FlowControl|Sequence
      (:then_0
        (Utilities|FlowControl|DoOnce false
          (:Completed
            (if (== (Variables|Default|GetBlockType) 3)
              (bind _returnvalue_3 (Rendering|Material|CreateDynamicMaterialInstance _breakmesh 0 "/Game/Materials/CraftBlockBreak2_Mat.CraftBlockBreak2_Mat" "None" :!class /Script/Engine.PrimitiveComponent))
              (Variables|Default|SetDynamicMat _returnvalue_3)
              (else
                (bind _returnvalue_4 (Rendering|Material|CreateDynamicMaterialInstance _breakmesh 0 "/Game/Materials/CraftBlockBreak_Mat.CraftBlockBreak_Mat" "None" :!class /Script/Engine.PrimitiveComponent))
                (Variables|Default|SetDynamicMat _returnvalue_4)))
            (Rendering|Material|SetMaterial (Variables|Default|GetBreakMesh) 0 (Variables|Default|GetDynamicMat)))))
      (:then_1
        (if (> (Variables|Default|GetArmor) 0)
          (Variables|Default|SetArmor (- (Variables|Default|GetArmor) 1))
          (else
            (Variables|Default|SetArmor (Variables|Default|GetArmorStart))
            (Rendering|SetVisibility (Variables|Default|GetBreakMesh) true false)
            (bind _returnvalue_5 (Rendering|Material|GetScalarParameterValue (Variables|Default|GetDynamicMat) "BreakX" :!class /Script/Engine.MaterialInstanceDynamic))
            (bind _returnvalue_6 (Rendering|Material|GetScalarParameterValue (Variables|Default|GetDynamicMat) "BreakY" :!class /Script/Engine.MaterialInstanceDynamic))
            (if (and (== _returnvalue_5 0.75) (== _returnvalue_6 0.75))
              (Variables|Default|SetDestroyed true)
              (Rendering|SetVisibility _staticmesh false true)
              (Collision|SetCollisionEnabled _staticmesh "NoCollision")
              (Components|DestroyComponent (Variables|Default|GetBox))
              (Audio|PlaySoundatLocation "/Game/Audio/SFX/ButtonPress1.ButtonPress1" _returnvalue "0, 0, 0" 1.2 (Math|Random|RandomFloatinRange 0.6 0.8) 0.08 "/Game/Audio/Attenuation/SA_ShortRange.SA_ShortRange" 0 0)
              (Audio|PlaySoundatLocation "/Game/Audio/SFX/Pop.Pop" _returnvalue "0, 0, 0" 1.4 (Math|Random|RandomFloatinRange 0.6 0.7) 0.02 "/Game/Audio/Attenuation/SA_ShortRange.SA_ShortRange" 0 0)
              (Utilities|IsValid (Variables|Default|GetFakeSpawnedActor)
                (:Is%20Valid
                  (CallFunction|FakeSpawn))
                (:Is%20Not%20Valid
                  (if (Utilities|IsValidClass _contains)
                    (bind _returnvalue_7 (Game|SpawnActorfromClass _contains (Transformation|GetActorTransform) "Undefined" 0 0))
                    (if (Utilities|DoesObjectImplementInterface _returnvalue_7 "/Game/Blueprints/BPI/BPI_Spawnable.BPI_Spawnable_C")
                      (Class|BPISpawnable|SpawnEntity(Message) _returnvalue_7)))))
              (switch int (Variables|Default|GetBlockType)
                (:0
                  (Components|Activation|Activate (Variables|Default|GetNiagara) false))
                (:1
                  (Components|Activation|Activate (Variables|Default|GetNiagaraDirt) false))
                (:2
                  (Components|Activation|Activate (Variables|Default|GetNiagaraStone) false))
                (:3
                  (Components|Activation|Activate (Variables|Default|GetNiagaraGlass) false)))
              (Utilities|FlowControl|Delay 1.0)
              (Actor|DestroyActor)
              (else
                (bind _returnvalue_8 (Rendering|Material|GetScalarParameterValue (Variables|Default|GetDynamicMat) "BreakX" :!class /Script/Engine.MaterialInstanceDynamic))
                (if (== _returnvalue_8 0.75)
                  (Rendering|Material|SetScalarParameterValue (Variables|Default|GetDynamicMat) "BreakX" 0.0 :!class /Script/Engine.MaterialInstanceDynamic)
                  (Rendering|Material|SetScalarParameterValue (Variables|Default|GetDynamicMat) "BreakY" 0.75 :!class /Script/Engine.MaterialInstanceDynamic)
                  (else
                    (Rendering|Material|SetScalarParameterValue (Variables|Default|GetDynamicMat) "BreakX" (+ _returnvalue_8 0.25) :!class /Script/Engine.MaterialInstanceDynamic)))))))))))

(fn ConstructionScript
  (bind _otherblockmesh (Variables|Default|GetOtherBlockMesh))
  (Variables|Default|SetArmorStart (Variables|Default|GetArmor))
  (switch int (Variables|Default|GetBlockType)
    (:0
      (Rendering|SetVisibility (Variables|Default|GetStaticMesh) true false)
      (Rendering|SetVisibility _otherblockmesh false false))
    (:1
      (Rendering|Material|SetMaterial _otherblockmesh 0 "/Game/Materials/Opaque/DirtBlock_MatInst.DirtBlock_MatInst")
      (Rendering|SetVisibility _otherblockmesh true false :!label _label)
      (Rendering|SetVisibility (Variables|Default|GetStaticMesh) false false))
    (:2
      (Rendering|Material|SetMaterial _otherblockmesh 0 "/Game/Materials/Opaque/StoneBlock_MatInst.StoneBlock_MatInst")
      (goto _label))
    (:3
      (Rendering|Material|SetMaterial _otherblockmesh 0 "/Game/Materials/GlassBlock_Mat.GlassBlock_Mat")
      (goto _label))))

(fn Attachto
  (params (ChildActor :type Actor%20Object%20Reference))
  (return 0))

(fn CanGrab
  (return false))

(fn Clicked
  (return false))

(fn DisableCollision
  (return false))

(fn DoesParentHaveParent
  (return false))

(fn EnableCollision
  (return false))

(fn GetAttached
  (return 0))

(fn GetCustomCursor
  (return false 0))

(fn GetShrinkScale
  (return "0, 0, 0" "0, 0, 0"))

(fn GetSnapLoc
  (params (CursorLoc :type Vector :default "0, 0, 0"))
  (return "0, 0, 0" "0, 0, 0"))

(fn Grabbed
  (return 0))

(fn LetGo
  (params (ParentComponent :type Actor%20Component%20Object%20Reference) (ParentActor :type Actor%20Object%20Reference))
  (return false))

(fn OnHover
  (if (not (Variables|Default|GetIsHover))
    (Variables|Default|SetIsHover true)
    (Rendering|SetVisibility (Variables|Default|GetOutlineMesh) true false)
    (return false)))

(fn PassChildAlong
  (return 0 0))

(fn RightClickEvent
  (return (Variables|Default|GetClick%20Message) (Transformation|GetActorLocation)))