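; BP_HatMan is a Hat Man figure on a plane that, when activated, slides away while its material fade animates, then disappears.
; BeginPlay puts a dynamic instance of the Hat Man material on the plane.
; Activate fires only once, running a slowed timeline whose single alpha drives both the sideways relative move and the Fade parameter, then destroys the actor.
; IsBusy always returns false.
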(event EventActivate
  (params (Delay :type Float%20%28single-precision%29) (Bool :type Boolean))
  (Utilities|FlowControl|DoOnce false
    (:Completed
      (Components|Timeline|SetPlayRate (Variables|Default|GetTL_Move) 0.18)
      (bind _localpha (Timeline|TL_Move PlayFromStart)
        (:Update
          (Transformation|SetRelativeLocation (Variables|Default|GetPlane) (Math|Vector|Lerp(Vector) "0, 0, 0" "0.000000,-400.000000, 0" _localpha) false false)
          (Rendering|Material|SetScalarParameterValue (Variables|Default|GetMat) "Fade" _localpha :!class /Script/Engine.MaterialInstanceDynamic))
        (:Finished
          (Actor|DestroyActor))))))

(event EventBeginPlay
  (bind _returnvalue (Rendering|Material|CreateDynamicMaterialInstance "/Game/Materials/HatMan_Mat.HatMan_Mat" "None" "None" :!class /Script/Engine.KismetMaterialLibrary))
  (Variables|Default|SetMat _returnvalue)
  (Rendering|Material|SetMaterial (Variables|Default|GetPlane) 0 (Variables|Default|GetMat)))

(fn ConstructionScript)

(fn IsBusy
  (return false))