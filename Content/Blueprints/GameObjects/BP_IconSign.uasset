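; BP_IconSign is a sign that displays a social-style icon such as Like, Heart, Repost, X or Smile.
; CustomStart creates a dynamic material and sets its initial Image texture.
; SetMat swaps that texture after a short delay on icon change, with a DoOnce-gated glitch texture, hiccup sound and timeline scale animation; a repeated icon resets the gate.
; A hover-bob timeline exists but is never triggered.
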(event Custom|SetMat
  (params (IconType :type LikeButtonIcon_Enum%20Enum :default "NewEnumerator0"))
  (if (Utilities|Enum|Equal(Enum) (Variables|Default|GetLastIcon) IconType)
    (goto _label Reset)
    (else
      (Utilities|FlowControl|Sequence
        (:then_0
          (Utilities|FlowControl|DoOnce false :!label _label
            (:Completed
              (Rendering|Material|SetTextureParameterValue (Variables|Default|GetDynMat) "Image" "/Game/Materials/Textures/Signs/SignGlitch.SignGlitch")
              (Audio|PlaySoundatLocation "/Game/Audio/SFX/GlitchHiccup.GlitchHiccup" "0, 0, 0" "0, 0, 0" 1.5 1.2 0.012 0 0 0)
              (bind (_direction _alpha1 _alpha2) (Timeline|TL_Anim PlayFromStart)
                (:Update
                  (Transformation|SetRelativeScale3D (Variables|Default|GetStaticMesh) (Math|Vector|MakeVector _alpha1 _alpha1 _alpha2)))))))
        (:then_1
          (Utilities|FlowControl|Delay 0.05)
          (bind _output_get (Variables|Default|SetLastIcon IconType))
          (switch Utilities|FlowControl|Switch|SwitchonLikeButtonIcon_Enum _output_get
            (:NewEnumerator0
              (Rendering|Material|SetTextureParameterValue (Variables|Default|GetDynMat) "Image" "/Game/Materials/Textures/Signs/LikeSign.LikeSign"))
            (:NewEnumerator1
              (Rendering|Material|SetTextureParameterValue (Variables|Default|GetDynMat) "Image" "/Game/Materials/Textures/Signs/HeartSign.HeartSign"))
            (:NewEnumerator2
              (Rendering|Material|SetTextureParameterValue (Variables|Default|GetDynMat) "Image" "/Game/Materials/Textures/Signs/RepostSign.RepostSign"))
            (:NewEnumerator4
              (Rendering|Material|SetTextureParameterValue (Variables|Default|GetDynMat) "Image" "/Game/Materials/Textures/Signs/XSign.XSign"))
            (:NewEnumerator5
              (Rendering|Material|SetTextureParameterValue (Variables|Default|GetDynMat) "Image" "/Game/Materials/Textures/Signs/SmileSign.SmileSign"))))))))

(event Custom|CustomStart
  (params (Value :type Texture%20Object%20Reference))
  (bind _returnvalue (Rendering|Material|CreateDynamicMaterialInstance (Variables|Default|GetStaticMesh) 0 "/Game/Materials/Textures/Signs/XSign_Mat.XSign_Mat" "None" :!class /Script/Engine.PrimitiveComponent))
  (bind _output_get (Variables|Default|SetDynMat _returnvalue))
  (Rendering|Material|SetMaterial (Variables|Default|GetStaticMesh) 0 _output_get)
  (Rendering|Material|SetTextureParameterValue (Variables|Default|GetDynMat) "Image" Value))

(event EventTick
  (params (DeltaSeconds :type Float%20%28single-precision%29)))

(fn ConstructionScript)