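; Interactive collectible book with configurable color and symbol that displays up to 16 sticky notes, registered with SaveManager under a level-plus-name UID.
; Poking toggles open and close animations, with delay timelines gating input and note hitboxes enabled only for collected notes.
; Hovering a note swaps the panel texture with a blink and click, while spawned BP_StickyAnimDriver actors handle note animation, resuming interrupted playback and presenting newly collected notes on opening.
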(event Custom|StickyHover
  (params (HoveredInt :type Integer))
  (Variables|Default|SetLastHoveredInt (Variables|Default|GetCurrentHoveredInt))
  (Variables|Default|SetCurrentHoveredInt HoveredInt)
  (if (not (== (Variables|Default|GetCurrentHoveredInt) (Variables|Default|GetLastHoveredInt)))
    (bind _returnvalue (Rendering|Material|CreateDynamicMaterialInstance "/Game/Materials/StickyNotePanel_Mat.StickyNotePanel_Mat" "None" "None" :!class /Script/Engine.KismetMaterialLibrary))
    (Variables|Default|SetDynPanel _returnvalue)
    (Rendering|Material|SetMaterial (Variables|Default|GetBookSkeletalMesh) 4 (Variables|Default|GetDynPanel))
    (Rendering|Material|SetTextureParameterValue (Variables|Default|GetDynPanel) "Texture" (Utilities|Array|Get(acopy) (Variables|Default|GetStickyNoteTextures) (- HoveredInt 1)))
    (Audio|Components|Audio|Stop (Variables|Default|GetTL_WakeUpBlink_Anim))
    (Components|Timeline|PlayfromStart (Variables|Default|GetTL_Blink))
    (Audio|PlaySoundatLocation (Utilities|Select :Index (Math|Random|RandomIntegerinRange 0 2) :Option%200 "/Game/Audio/SFX/ClickMusicSFX/Click1.Click1" :Option%201 "/Game/Audio/SFX/ClickMusicSFX/Click2.Click2" :Option%202 "/Game/Audio/SFX/ClickMusicSFX/Click3.Click3") (Transformation|GetActorLocation) "0, 0, 0" 0.5 (Math|Random|RandomFloatinRange 1.85 2.3) 0.28 "/Game/Audio/Attenuation/SA_ShortRange.SA_ShortRange" "/Game/Audio/Attenuation/SC_Default.SC_Default" 0)
    (Utilities|IsValid (Variables|Default|GetCurrentDriver)
      (:Is%20Valid
        (bind _output_get (Variables|Default|SetLastDriver (Variables|Default|GetCurrentDriver)))
        (Default|EventDriverReverse _output_get))
      (:Is%20Not%20Valid
        _))
    (bind _returnvalue_2 (Game|SpawnActorfromClass "/Game/Blueprints/GameObjects/BP_StickyAnimDriver.BP_StickyAnimDriver_C" (Transformation|GetActorTransform) "Undefined" 0 0))
    (Variables|Default|SetCurrentDriver _returnvalue_2)
    (Variables|/Game/Blueprints/GameObjects/BP_StickyAnimDriver.BP_StickyAnimDriver_C|SetBookBP _returnvalue_2 self)
    (bind _outactors (Actor|GetAllActorswithTag (Utilities|String|StringToName (Utilities|String|ToString(Integer) (Variables|Default|GetCurrentHoveredInt)))))
    (if (> (Utilities|Array|Length _outactors) 0)
      (bind _array_element (Utilities|Array|ForEachLoopwithBreak _outactors)
        (:LoopBody
          (bind _asbp_sticky_anim_driver (Utilities|Casting|CastToBP_StickyAnimDriver _array_element))
          (Variables|Default|SetPlayPos (Components|Timeline|GetPlaybackPosition (Variables|/Game/Blueprints/GameObjects/BP_StickyAnimDriver.BP_StickyAnimDriver_C|GetTL_DriverAnim _asbp_sticky_anim_driver)))
          (Actor|DestroyActor _array_element))
        (:Completed
          (Variables|/Game/Blueprints/GameObjects/BP_StickyAnimDriver.BP_StickyAnimDriver_C|SetInt (Variables|Default|GetCurrentDriver) (Variables|Default|GetCurrentHoveredInt) :!label _label)
          (Default|EventDriverForward (Variables|Default|GetCurrentDriver) (Variables|Default|GetPlayPos))))
      (else
        (Variables|Default|SetPlayPos 0.0)
        (goto _label)))))

(event Custom|CloseBook
  (bind _bookskeletalmesh (Variables|Default|GetBookSkeletalMesh))
  (Collision|SetCollisionEnabled (Variables|Default|GetS1Box) "NoCollision")
  (Utilities|FlowControl|Sequence
    (:then_0
      (Components|Animation|PlayAnimation _bookskeletalmesh "/Game/Meshes/Skeletal/book_armature_new_anim_Anim_Armature_CloseFromOpen.book_armature_new_anim_Anim_Armature_CloseFromOpen" false)
      (Variables|Default|SetIsOpen false))
    (:then_1
      (bind (_direction _alpha) (Timeline|TL_WakeUpBlink_Anim ReverseFromEnd)
        (:Update
          (Components|SkeletalMesh|SetMorphTarget (Variables|Default|GetBookSkeletalMesh) "PanelSquishY" _alpha true))
        (:BlinkDoot
          (switch Utilities|FlowControl|Switch|SwitchonETimelineDirection _direction
            (:Forward
              (Audio|PlaySoundatLocation (Utilities|Select :Index (Math|Random|RandomIntegerinRange 0 2) :Option%200 "/Game/Audio/SFX/ClickMusicSFX/Click1.Click1" :Option%201 "/Game/Audio/SFX/ClickMusicSFX/Click2.Click2" :Option%202 "/Game/Audio/SFX/ClickMusicSFX/Click3.Click3") (Transformation|GetActorLocation) "0, 0, 0" 0.5 (Math|Random|RandomFloatinRange 1.85 2.3) 0.28 "/Game/Audio/Attenuation/SA_ShortRange.SA_ShortRange" "/Game/Audio/Attenuation/SC_Default.SC_Default" 0 :!label _label))
            (:Backward
              (if (> (Components|Timeline|GetPlaybackPosition (Variables|Default|GetTL_WakeUpBlink_Anim)) 1.5)
                (goto _label)))))))
    (:then_2
      (Timeline|TL_AnimDelay PlayFromStart
        (:Finished
          (Components|Animation|PlayAnimation _bookskeletalmesh "/Game/Meshes/Skeletal/book_armature_new_anim_Anim_Armature_Idle1.book_armature_new_anim_Anim_Armature_Idle1" true)
          (Collision|SetCollisionEnabled (Variables|Default|GetBox) "QueryAndPhysics"))))))

(event Custom|OpenBook
  (bind _bookstate (Variables|Default|GetBookstate))
  (bind _stickynotes (Utilities|Struct|BreakBookStickySet_Struct _bookstate))
  (Collision|SetCollisionEnabled (Variables|Default|GetBox) "NoCollision")
  (Utilities|FlowControl|Sequence
    (:then_0
      (Components|Animation|PlayAnimation (Variables|Default|GetBookSkeletalMesh) "/Game/Meshes/Skeletal/book_armature_new_anim_Anim_Armature_OpenFromIdle.book_armature_new_anim_Anim_Armature_OpenFromIdle" false)
      (Default|PokeEvent (Variables|Default|GetVolume)))
    (:then_2
      (Components|Timeline|SetPlayRate (Variables|Default|GetTL_WakeUpBlink_Anim) (Math|Random|RandomFloatinRange 0.65 1.1))
      (bind (_direction _alpha) (Timeline|TL_WakeUpBlink_Anim PlayFromStart)
        (:Update
          (Components|SkeletalMesh|SetMorphTarget (Variables|Default|GetBookSkeletalMesh) "PanelSquishY" _alpha true))
        (:BlinkDoot
          (switch Utilities|FlowControl|Switch|SwitchonETimelineDirection _direction
            (:Forward
              (Audio|PlaySoundatLocation (Utilities|Select :Index (Math|Random|RandomIntegerinRange 0 2) :Option%200 "/Game/Audio/SFX/ClickMusicSFX/Click1.Click1" :Option%201 "/Game/Audio/SFX/ClickMusicSFX/Click2.Click2" :Option%202 "/Game/Audio/SFX/ClickMusicSFX/Click3.Click3") (Transformation|GetActorLocation) "0, 0, 0" 0.5 (Math|Random|RandomFloatinRange 1.85 2.3) 0.28 "/Game/Audio/Attenuation/SA_ShortRange.SA_ShortRange" "/Game/Audio/Attenuation/SC_Default.SC_Default" 0 :!label _label))
            (:Backward
              (if (> (Components|Timeline|GetPlaybackPosition (Variables|Default|GetTL_WakeUpBlink_Anim)) 1.5)
                (goto _label)))))))
    (:then_3
      (Variables|Default|SetCurrentInt 0)
      (for (_array_element _array_index) _stickynotes
        (if (.NewlyCollected (Utilities|Struct|BreakStickyNoteState_Struct _array_element))
          (Utilities|Array|SetArrayElem _stickynotes _array_index (Utilities|Struct|MakeStickyNoteState_Struct true false))
          (Math|Integer|IncrementInt (Variables|Default|GetCurrentInt)
            (:%20%20
              (bind _returnvalue (Game|SpawnActorfromClass "/Game/Blueprints/GameObjects/BP_StickyAnimDriver.BP_StickyAnimDriver_C" (Transformation|GetActorTransform) "Undefined" 0 0))
              (Variables|/Game/Blueprints/GameObjects/BP_StickyAnimDriver.BP_StickyAnimDriver_C|SetBookBP _returnvalue self)
              (Variables|/Game/Blueprints/GameObjects/BP_StickyAnimDriver.BP_StickyAnimDriver_C|SetInt _returnvalue (+ _array_index 1))
              (Default|EventNewlyCollected _returnvalue (Variables|Default|GetCurrentInt))))))
      (Timeline|TL_OpenDelay PlayFromStart
        (:Finished
          (Variables|Default|SetIsOpen true)
          (Collision|SetCollisionEnabled (Variables|Default|GetAltBox) "QueryAndPhysics")
          (for (_array_element_2 _array_index_2) (Utilities|Array|MakeArray (Variables|Default|GetS1Box) (Variables|Default|GetS2Box) (Variables|Default|GetS3Box) (Variables|Default|GetS4Box) (Variables|Default|GetS5Box) (Variables|Default|GetS6Box) (Variables|Default|GetS7Box) (Variables|Default|GetS8Box) (Variables|Default|GetS9Box) (Variables|Default|GetS10Box) (Variables|Default|GetS11Box) (Variables|Default|GetS12Box) (Variables|Default|GetS13Box) (Variables|Default|GetS14Box) (Variables|Default|GetS15Box) (Variables|Default|GetS16Box))
            (if (.Collected (Utilities|Struct|BreakStickyNoteState_Struct (Utilities|Array|Get(acopy) (Utilities|Struct|BreakBookStickySet_Struct (Variables|Default|GetBookstate)) _array_index_2)))
              (Collision|SetCollisionEnabled _array_element_2 "QueryAndPhysics"))))))))

(event EventBeginPlay
  (bind _savemanager (Variables|Default|GetSaveManager))
  (bind _uid (Variables|Default|GetUID))
  (Default|InitiateCollectible _savemanager _uid true)
  (Default|InitiateStickySet _savemanager _uid (Variables|Default|GetBookstate))
  (CallFunction|StickyMorphUpdates)
  (bind _array_element (Utilities|Array|ForEachLoopwithBreak (Utilities|Struct|BreakBookStickySet_Struct (Variables|Default|GetBookstate)) :!label _label)
    (:LoopBody
      (if (.NewlyCollected (Utilities|Struct|BreakStickyNoteState_Struct _array_element))
        (Components|Animation|PlayAnimation (Variables|Default|GetBookSkeletalMesh) "/Game/Meshes/Skeletal/book_armature_new_anim_Anim_Armature_Idle2.book_armature_new_anim_Anim_Armature_Idle2" true)
        (goto _label Break)))))

(event EventInitBoolTrue)

(event EventPokeEvent
  (bind _bookstate (Variables|Default|GetBookstate))
  (bind _bookskeletalmesh (Variables|Default|GetBookSkeletalMesh))
  (bind _stickynotes (Utilities|Struct|BreakBookStickySet_Struct _bookstate))
  (if (not (or (Audio|Components|Audio|IsPlaying (Variables|Default|GetTL_AnimDelay)) (Audio|Components|Audio|IsPlaying (Variables|Default|GetTL_OpenDelay))))
    (if (Variables|Default|GetIsOpen)
      (Collision|SetCollisionEnabled (Variables|Default|GetS1Box) "NoCollision")
      (Utilities|FlowControl|Sequence
        (:then_0
          (Components|Animation|PlayAnimation _bookskeletalmesh "/Game/Meshes/Skeletal/book_armature_new_anim_Anim_Armature_CloseFromOpen.book_armature_new_anim_Anim_Armature_CloseFromOpen" false)
          (Variables|Default|SetIsOpen false))
        (:then_1
          (bind (_direction _alpha) (Timeline|TL_WakeUpBlink_Anim ReverseFromEnd)
            (:Update
              (Components|SkeletalMesh|SetMorphTarget (Variables|Default|GetBookSkeletalMesh) "PanelSquishY" _alpha true))
            (:BlinkDoot
              (switch Utilities|FlowControl|Switch|SwitchonETimelineDirection _direction
                (:Forward
                  (Audio|PlaySoundatLocation (Utilities|Select :Index (Math|Random|RandomIntegerinRange 0 2) :Option%200 "/Game/Audio/SFX/ClickMusicSFX/Click1.Click1" :Option%201 "/Game/Audio/SFX/ClickMusicSFX/Click2.Click2" :Option%202 "/Game/Audio/SFX/ClickMusicSFX/Click3.Click3") (Transformation|GetActorLocation) "0, 0, 0" 0.5 (Math|Random|RandomFloatinRange 1.85 2.3) 0.28 "/Game/Audio/Attenuation/SA_ShortRange.SA_ShortRange" "/Game/Audio/Attenuation/SC_Default.SC_Default" 0 :!label _label))
                (:Backward
                  (if (> (Components|Timeline|GetPlaybackPosition (Variables|Default|GetTL_WakeUpBlink_Anim)) 1.5)
                    (goto _label)))))))
        (:then_2
          (Timeline|TL_AnimDelay PlayFromStart
            (:Finished
              (Components|Animation|PlayAnimation _bookskeletalmesh "/Game/Meshes/Skeletal/book_armature_new_anim_Anim_Armature_Idle1.book_armature_new_anim_Anim_Armature_Idle1" true)
              (Collision|SetCollisionEnabled (Variables|Default|GetBox) "QueryAndPhysics")))))
      (else
        (Collision|SetCollisionEnabled (Variables|Default|GetBox) "NoCollision")
        (Utilities|FlowControl|Sequence
          (:then_0
            (Components|Animation|PlayAnimation _bookskeletalmesh "/Game/Meshes/Skeletal/book_armature_new_anim_Anim_Armature_OpenFromIdle.book_armature_new_anim_Anim_Armature_OpenFromIdle" false)
            (Default|PokeEvent (Variables|Default|GetVolume)))
          (:then_2
            (Components|Timeline|SetPlayRate (Variables|Default|GetTL_WakeUpBlink_Anim) (Math|Random|RandomFloatinRange 0.65 1.1))
            (Timeline|TL_WakeUpBlink_Anim PlayFromStart))
          (:then_3
            (Variables|Default|SetCurrentInt 0)
            (for (_array_element _array_index) _stickynotes
              (if (.NewlyCollected (Utilities|Struct|BreakStickyNoteState_Struct _array_element))
                (Utilities|Array|SetArrayElem _stickynotes _array_index (Utilities|Struct|MakeStickyNoteState_Struct true false))
                (Math|Integer|IncrementInt (Variables|Default|GetCurrentInt)
                  (:%20%20
                    (bind _returnvalue (Game|SpawnActorfromClass "/Game/Blueprints/GameObjects/BP_StickyAnimDriver.BP_StickyAnimDriver_C" (Transformation|GetActorTransform) "Undefined" 0 0))
                    (Variables|/Game/Blueprints/GameObjects/BP_StickyAnimDriver.BP_StickyAnimDriver_C|SetBookBP _returnvalue self)
                    (Variables|/Game/Blueprints/GameObjects/BP_StickyAnimDriver.BP_StickyAnimDriver_C|SetInt _returnvalue (+ _array_index 1))
                    (Default|EventNewlyCollected _returnvalue (Variables|Default|GetCurrentInt))))))
            (Timeline|TL_OpenDelay PlayFromStart
              (:Finished
                (Variables|Default|SetIsOpen true)
                (Collision|SetCollisionEnabled (Variables|Default|GetAltBox) "QueryAndPhysics")
                (for (_array_element_2 _array_index_2) (Utilities|Array|MakeArray (Variables|Default|GetS1Box) (Variables|Default|GetS2Box) (Variables|Default|GetS3Box) (Variables|Default|GetS4Box) (Variables|Default|GetS5Box) (Variables|Default|GetS6Box) (Variables|Default|GetS7Box) (Variables|Default|GetS8Box) (Variables|Default|GetS9Box) (Variables|Default|GetS10Box) (Variables|Default|GetS11Box) (Variables|Default|GetS12Box) (Variables|Default|GetS13Box) (Variables|Default|GetS14Box) (Variables|Default|GetS15Box) (Variables|Default|GetS16Box))
                  (if (.Collected (Utilities|Struct|BreakStickyNoteState_Struct (Utilities|Array|Get(acopy) (Utilities|Struct|BreakBookStickySet_Struct (Variables|Default|GetBookstate)) _array_index_2)))
                    (Collision|SetCollisionEnabled _array_element_2 "QueryAndPhysics")))))))))))

(fn ConstructionScript
  (bind _bookskeletalmesh (Variables|Default|GetBookSkeletalMesh))
  (CallFunction|CreateUID)
  (Transformation|AttachComponentToComponent (Variables|Default|GetBox) (Variables|Default|GetBookSkeletalMesh) "RootSocket" "KeepWorld" "KeepWorld" "KeepWorld" true)
  (Components|StaticMesh|SetStaticMesh (Variables|Default|GetBookSymbolMesh) (Utilities|Select :Index (Variables|Default|GetSymbol) :NewEnumerator4 "/Game/Meshes/BookSymbols/book_symbols_BookSymbol_Dots1.book_symbols_BookSymbol_Dots1" :NewEnumerator5 "/Game/Meshes/BookSymbols/book_symbols_BookSymbol_Dots2.book_symbols_BookSymbol_Dots2" :NewEnumerator6 "/Game/Meshes/BookSymbols/book_symbols_BookSymbol_Dots3.book_symbols_BookSymbol_Dots3" :NewEnumerator0 "/Game/Meshes/BookSymbols/book_symbols_BookSymbol_Dots4.book_symbols_BookSymbol_Dots4" :NewEnumerator1 "/Game/Meshes/BookSymbols/book_symbols_BookSymbol_Dots5.book_symbols_BookSymbol_Dots5" :NewEnumerator2 "/Game/Meshes/BookSymbols/book_symbols_BookSymbol_Pant.book_symbols_BookSymbol_Pant" :NewEnumerator3 "/Game/Meshes/BookSymbols/book_symbols_BookSymbol_Cursor.book_symbols_BookSymbol_Cursor" :NewEnumerator7 "/Game/Meshes/BookSymbols/book_symbols_BookMesh_001.book_symbols_BookMesh_001" :NewEnumerator8 "/Game/Meshes/BookSymbols/book_symbols_BookSymbol_Key.book_symbols_BookSymbol_Key" :NewEnumerator9 "/Game/Meshes/BookSymbols/book_symbols_BookSymbol_Bolt.book_symbols_BookSymbol_Bolt" :NewEnumerator10 "/Game/Meshes/BookSymbols/book_symbols_BookSymbol_Screw.book_symbols_BookSymbol_Screw" :NewEnumerator11 "/Game/Meshes/BookSymbols/book_symbols_BookSymbol_Hourglass.book_symbols_BookSymbol_Hourglass" :NewEnumerator12 "/Game/Meshes/BookSymbols/book_symbols_BookSymbol_Tree.book_symbols_BookSymbol_Tree" :NewEnumerator13 "/Game/Meshes/BookSymbols/book_symbols_BookSymbol_Link.book_symbols_BookSymbol_Link" :NewEnumerator14 "/Game/Meshes/BookSymbols/book_symbols_BookSymbol_Cog.book_symbols_BookSymbol_Cog"))
  (bind _returnvalue (Rendering|Material|CreateDynamicMaterialInstance _bookskeletalmesh 0 "/Game/Materials/BookColor_Mat.BookColor_Mat" "None" :!class /Script/Engine.PrimitiveComponent))
  (bind _output_get (Variables|Default|SetDynMat _returnvalue))
  (Rendering|Material|SetMaterial _bookskeletalmesh 0 _output_get)
  (Rendering|Material|SetVectorParameterValue (Variables|Default|GetDynMat) "Color" (Variables|Default|GetColor) :!class /Script/Engine.MaterialInstanceDynamic))

(fn CreateUID
  (bind _returnvalue (Game|GetCurrentLevelName true))
  (Variables|Default|SetUID (Utilities|String|Append _returnvalue (Utilities|GetDisplayName self))))

(fn StickyMorphUpdates
  (bind _bookskeletalmesh (Variables|Default|GetBookSkeletalMesh))
  (for (_array_element _array_index) (Utilities|Struct|BreakBookStickySet_Struct (Variables|Default|GetBookstate))
    (if (.Collected (Utilities|Struct|BreakStickyNoteState_Struct _array_element))
      (Components|SkeletalMesh|SetMorphTarget _bookskeletalmesh (Utilities|String|StringToName (Utilities|String|Append "L" (Utilities|String|ToString(Integer) (+ _array_index 1)))) 0.0 true)
      (else
        (Components|SkeletalMesh|SetMorphTarget _bookskeletalmesh (Utilities|String|StringToName (Utilities|String|Append "L" (Utilities|String|ToString(Integer) (+ _array_index 1)))) -0.03 true)))))

(fn Attachto
  (params (ChildActor :type Actor%20Object%20Reference))
  (return 0))

(fn CanGrab
  (return false))

(fn Clicked
  (return false))

(fn DisableCollision
  (return false))

(fn DoesParentHaveParent
  (return false))

(fn EnableCollision
  (return false))

(fn GetAttached
  (return 0))

(fn GetCustomCursor
  (return false 0))

(fn GetObjectUID
  (return (Variables|Default|GetUID)))

(fn GetShrinkScale
  (return "0, 0, 0" "0, 0, 0"))

(fn GetSnapLoc
  (params (CursorLoc :type Vector :default "0, 0, 0"))
  (return "0, 0, 0" "0, 0, 0"))

(fn GetTrueFalse
  (return false))

(fn Grabbed
  (return 0))

(fn LetGo
  (params (ParentComponent :type Actor%20Component%20Object%20Reference) (ParentActor :type Actor%20Object%20Reference))
  (return false))

(fn OnHover
  (return false))

(fn PassChildAlong
  (return 0 0))