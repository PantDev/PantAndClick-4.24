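; TestKey is a grabbable test actor that grows a grass spline mesh along a referenced SplineActor's path.
; Clicking resets both distances, creates the mesh and marks it grabbed.
; Each tick advances the end distance by Speed, and the start too once let go, so the mesh stretches while held, then slides.
; Two detached spheres track the ends; most other interaction functions are stubs.
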(event EventBeginPlay
  (Transformation|DetachFromComponent (Variables|Default|GetEndSphere) "KeepWorld" "KeepWorld" "KeepWorld" true))

(event Collision|EventActorBeginOverlap
  (params (OtherActor :type Actor%20Object%20Reference)))

(event EventTick
  (params (DeltaSeconds :type Float%20%28single-precision%29))
  (bind _splineactor (Variables|Default|GetSplineActor))
  (bind _splineactor_2 (Variables|Default|GetSplineActor))
  (bind _splinemesh (Variables|Default|GetSplineMesh))
  (bind _spline (Variables|/Game/Blueprints/GameObjects/BP_PathSpline.BP_PathSpline_C|GetSpline _splineactor))
  (bind _spline_2 (Variables|/Game/Blueprints/GameObjects/BP_PathSpline.BP_PathSpline_C|GetSpline _splineactor_2))
  (if (Variables|Default|GetPopped)
    (if (Variables|Default|GetGrabbedBool)
      _
      (else
        (bind _output_get (Variables|Default|SetCurrentStartDist (+ (Variables|Default|GetCurrentStartDist) (* (Variables|Default|GetSpeed) (Utilities|Time|GetWorldDeltaSeconds)))))
        (Transformation|SetWorldLocation (Variables|Default|GetStartSphere) (Spline|GetLocationatDistanceAlongSpline (Variables|/Game/Blueprints/GameObjects/BP_PathSpline.BP_PathSpline_C|GetSpline (Variables|Default|GetSplineActor)) _output_get "World") false false)))
    (bind _output_get_2 (Variables|Default|SetCurrentEndDist (+ (Variables|Default|GetCurrentEndDist) (* (Variables|Default|GetSpeed) (Utilities|Time|GetWorldDeltaSeconds)))))
    (Transformation|SetWorldLocation (Variables|Default|GetEndSphere) (Spline|GetLocationatDistanceAlongSpline (Variables|/Game/Blueprints/GameObjects/BP_PathSpline.BP_PathSpline_C|GetSpline (Variables|Default|GetSplineActor)) _output_get_2 "World") false false)
    (SplineMesh|SetForwardAxis _splinemesh "X" true)
    (Collision|SetCollisionEnabled _splinemesh "NoCollision")
    (Rendering|SetReceivesDecals 0 true)
    (SplineMesh|SetStartandEnd 0 (Spline|GetLocationatDistanceAlongSpline _spline_2 (Variables|Default|GetCurrentStartDist) "Local") (Spline|GetTangentatDistanceAlongSpline _spline_2 (Variables|Default|GetCurrentStartDist) "Local") (Spline|GetLocationatDistanceAlongSpline _spline (Variables|Default|GetCurrentEndDist) "Local") (Spline|GetTangentatDistanceAlongSpline _spline (Variables|Default|GetCurrentEndDist) "Local") true :!class /Script/Engine.SplineMeshComponent)))

(fn ConstructionScript)

(fn Attachto
  (params (ChildActor :type Actor%20Object%20Reference))
  (return 0))

(fn CanGrab
  (return true))

(fn Clicked
  (Variables|Default|SetCurrentStartDist 0.0)
  (Variables|Default|SetCurrentEndDist 0.0)
  (bind _returnvalue (AddComponent|AddSplineMeshComponent false))
  (bind _output_get (Variables|Default|SetSplineMesh _returnvalue))
  (Components|StaticMesh|SetStaticMesh _output_get "/Game/Meshes/Spline/SplineMesh_Grass_Middle.SplineMesh_Grass_Middle")
  (Transformation|SetWorldLocation (Variables|Default|GetStartSphere) (Transformation|GetActorLocation) false false)
  (Variables|Default|SetGrabbedBool true)
  (Variables|Default|SetPopped true)
  (return false))

(fn DisableCollision
  (return false))

(fn DoesParentHaveParent
  (return false))

(fn EnableCollision
  (return false))

(fn GetAttached
  (return 0))

(fn GetCustomCursor
  (return false 0))

(fn GetShrinkScale
  (return "0, 0, 0" "0, 0, 0"))

(fn GetSnapLoc
  (params (CursorLoc :type Vector :default "0, 0, 0"))
  (return "0, 0, 0" "0, 0, 0"))

(fn Grabbed
  (return 0))

(fn LetGo
  (params (ParentComponent :type Actor%20Component%20Object%20Reference) (ParentActor :type Actor%20Object%20Reference))
  (Variables|Default|SetGrabbedBool false)
  (return false))

(fn OnHover
  (return false))

(fn PassChildAlong
  (return 0 0))