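; Mouse-hole door for the 3D maze that responds to a poke by either rattling as locked or opening.
; An unlocked door plays one of two open animations based on OpensDown, marks itself open and disables its box collision.
; It then sets IsMoving on the player's maze nav controller for a short delay while the door opens.
; The grab, click, hover and attach interaction functions are empty stubs.
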(event EventBeginPlay)

(event Collision|EventActorBeginOverlap
  (params (OtherActor :type Actor%20Object%20Reference)))

(event EventTick
  (params (DeltaSeconds :type Float%20%28single-precision%29)))

(event EventPokeEvent
  (bind _mouseholedoor_skeletal (Variables|Default|GetMouseHoleDoor_Skeletal))
  (if (Variables|Default|GetLocked)
    (Components|Animation|PlayAnimation _mouseholedoor_skeletal "/Game/Meshes/Skeletal/MouseHoleDoor_Skeletal_Anim_Armature_DoorLocked.MouseHoleDoor_Skeletal_Anim_Armature_DoorLocked" false)
    (else
      (if (Variables|Default|GetOpensDown)
        (Components|Animation|PlayAnimation _mouseholedoor_skeletal "/Game/Meshes/Skeletal/MouseHoleDoor_Skeletal_Anim_Armature_DoorOpen2.MouseHoleDoor_Skeletal_Anim_Armature_DoorOpen2" false)
        (else
          (Components|Animation|PlayAnimation _mouseholedoor_skeletal "/Game/Meshes/Skeletal/MouseHoleDoor_Skeletal_Anim_Armature_DoorOpen1.MouseHoleDoor_Skeletal_Anim_Armature_DoorOpen1" false)))
      (Variables|Default|SetOpen true)
      (Collision|SetCollisionEnabled (Variables|Default|GetBox) "NoCollision")
      (bind _asmaze_nav_controller_bp (Utilities|Casting|CastToMazeNavController_BP (Game|GetPlayerCharacter 0)))
      (Variables|/Game/MazeNav/Blueprints/MazeNavController_BP.MazeNavController_BP_C|SetIsMoving _asmaze_nav_controller_bp true)
      (Utilities|FlowControl|Delay 1.5)
      (Variables|/Game/MazeNav/Blueprints/MazeNavController_BP.MazeNavController_BP_C|SetIsMoving _asmaze_nav_controller_bp false))))

(fn ConstructionScript)

(fn Attachto
  (params (ChildActor :type Actor%20Object%20Reference))
  (return 0))

(fn CanGrab
  (return false))

(fn Clicked
  (return false))

(fn DisableCollision
  (return false))

(fn DoesParentHaveParent
  (return false))

(fn EnableCollision
  (return false))

(fn GetAttached
  (return 0))

(fn GetCustomCursor
  (return false 0))

(fn GetShrinkScale
  (return "0, 0, 0" "0, 0, 0"))

(fn GetSnapLoc
  (params (CursorLoc :type Vector :default "0, 0, 0"))
  (return "0, 0, 0" "0, 0, 0"))

(fn Grabbed
  (return 0))

(fn LetGo
  (params (ParentComponent :type Actor%20Component%20Object%20Reference) (ParentActor :type Actor%20Object%20Reference))
  (return false))

(fn OnHover
  (return false))

(fn PassChildAlong
  (return 0 0))