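; BP_MouseHole is an interactable mouse hole that switches the player between the maze pawn and the Pant pawn when poked.
; PokeEvent, guarded by a Busy flag, plays two transition widgets, reverses the hourglass one after a short delay, then possesses whichever pawn is not active.
; Leaving the maze also turns the maze pawn around to face back.
; The grab, click, hover and attach functions are empty stubs.
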(event EventBeginPlay)

(event Collision|EventActorBeginOverlap
  (params (OtherActor :type Actor%20Object%20Reference)))

(event EventTick
  (params (DeltaSeconds :type Float%20%28single-precision%29)))

(event EventPokeEvent
  (bind _returnvalue (Game|GetPlayerController 0))
  (bind _mazecontroller (Variables|Default|GetMazeController))
  (bind _returnvalue_2 (Transformation|GetActorRotation _mazecontroller))
  (bind (_roll _pitch _yaw) (Math|Rotator|BreakRotator _returnvalue_2))
  (if (not (Variables|Default|GetBusy))
    (Variables|Default|SetBusy true)
    (bind _returnvalue_3 (UserInterface|CreateWidget "/Game/UserInterface/HourglassTransition_Widget.HourglassTransition_Widget_C"))
    (bind _returnvalue_4 (UserInterface|CreateWidget "/Game/UserInterface/Transition_Widget.Transition_Widget_C"))
    (UserInterface|Viewport|AddtoViewport _returnvalue_4 0)
    (UserInterface|Viewport|AddtoViewport _returnvalue_3 0)
    (UserInterface|Animation|PlayAnimation _returnvalue_3 (Variables|/Game/UserInterface/HourglassTransition_Widget.HourglassTransition_Widget_C|GetTransition _returnvalue_3) 0.0 1 "Forward" 1.0 false)
    (UserInterface|Animation|PlayAnimation _returnvalue_4 (Variables|/Game/UserInterface/Transition_Widget.Transition_Widget_C|GetTransition _returnvalue_4) 0.0 1 "Forward" 1.0 false)
    (Utilities|FlowControl|Delay 0.3)
    (Class|UserWidget|ReverseAnimation _returnvalue_3 (Variables|/Game/UserInterface/HourglassTransition_Widget.HourglassTransition_Widget_C|GetTransition _returnvalue_3))
    (if (== (Utilities|GetClass (Game|GetPlayerCharacter 0)) "/Game/MazeNav/Blueprints/MazeNavController_BP.MazeNavController_BP_C")
      (Pawn|Possess _returnvalue (Variables|Default|GetPantController))
      (Transformation|SetActorRotation _mazecontroller (Math|Rotator|MakeRotator _roll _pitch (+ _yaw 1.8e+02)))
      (else
        (Pawn|Possess _returnvalue (Variables|Default|GetMazeController))))
    (Variables|Default|SetBusy false)))

(fn ConstructionScript)

(fn Attachto
  (params (ChildActor :type Actor%20Object%20Reference))
  (return 0))

(fn CanGrab
  (return false))

(fn Clicked
  (return false))

(fn DisableCollision
  (return false))

(fn DoesParentHaveParent
  (return false))

(fn EnableCollision
  (return false))

(fn GetAttached
  (return 0))

(fn GetCustomCursor
  (return false 0))

(fn GetShrinkScale
  (return "0, 0, 0" "0, 0, 0"))

(fn GetSnapLoc
  (params (CursorLoc :type Vector :default "0, 0, 0"))
  (return "0, 0, 0" "0, 0, 0"))

(fn Grabbed
  (return 0))

(fn LetGo
  (params (ParentComponent :type Actor%20Component%20Object%20Reference) (ParentActor :type Actor%20Object%20Reference))
  (return false))

(fn OnHover
  (return false))

(fn PassChildAlong
  (return 0 0))