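; BP_AntiFile is an anti-pickup file icon that takes two from the player's file count when collected.
; It bobs in place, can move along a spawned scatter spline, and re-traces its blob shadow on a repeating timer.
; Collect uses chained timelines to fly the icon to the player, then updates the counter widget, plays sound at the deprojected HUD position, spawns dust and destroys itself.
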(event Custom|UpdateShadow
  (bind _returnvalue (Transformation|GetActorLocation))
  (bind _blob (Variables|Default|GetBlob))
  (bind (_x _y _z) (Math|Vector|BreakVector _returnvalue))
  (if (not (Variables|Default|GetBlockShadowUpdate))
    (bind _asbp_pant_controller (Utilities|Casting|CastToBP_PantController (Game|GetPlayerCharacter 0)))
    (Utilities|Array|AddUnique (Variables|/Game/PantControllerBP/Blueprints/BP_PantController.BP_PantController_C|GetIgnoreArray _asbp_pant_controller) _asbp_pant_controller)
    (bind (_outhit _returnvalue_2) (Collision|LineTraceByChannel _returnvalue (Math|Vector|MakeVector _x _y (- _z 1e+04)) "TraceTypeQuery1" false (Variables|/Game/PantControllerBP/Blueprints/BP_PantController.BP_PantController_C|GetIgnoreArray _asbp_pant_controller) "None"))
    (if _returnvalue_2
      (Rendering|SetVisibility _blob true true)
      (if (< (Math|Vector|VectorLength (- (Transformation|GetWorldLocation (Variables|Default|GetBlob)) (Math|Vector|MakeVector (.X (Math|Vector|BreakVector (.Location (Collision|BreakHitResult _outhit)))) (.Y (Math|Vector|BreakVector (.Location (Collision|BreakHitResult _outhit)))) (+ (.Z (Math|Vector|BreakVector (.Location (Collision|BreakHitResult _outhit)))) 5.0)))) 1e+02)
        _
        (else
          (Transformation|SetWorldLocationAndRotation (Variables|Default|GetBlob) (Math|Vector|MakeVector (.X (Math|Vector|BreakVector (.Location (Collision|BreakHitResult _outhit)))) (.Y (Math|Vector|BreakVector (.Location (Collision|BreakHitResult _outhit)))) (+ (.Z (Math|Vector|BreakVector (.Location (Collision|BreakHitResult _outhit)))) 5.0)) (Math|Rotator|MakeRotfromZ (.ImpactNormal (Collision|BreakHitResult _outhit))) false false)))
      (else
        (Rendering|SetVisibility _blob false true)))
    (Utilities|FlowControl|Sequence
      (:then_0
        (Utilities|FlowControl|DoOnce false
          (:Completed
            (Rendering|SetVisibility (Variables|Default|GetBlob) true true))))
      (:then_1
        (Utilities|FlowControl|Delay 0.25)
        (CallFunction|UpdateShadow)))))

(event EventBeginPlay
  (bind _returnvalue (Transformation|GetActorTransform))
  (bind (_location _rotation _scale) (Math|Transform|BreakTransform _returnvalue))
  (bind (_roll _pitch _yaw) (Math|Rotator|BreakRotator _rotation))
  (Variables|Default|SetStartLoc (Transformation|GetActorLocation))
  (Utilities|FlowControl|Delay 0.01)
  (Utilities|FlowControl|Delay 0.5)
  (Variables|/Script/Engine.PrimitiveComponent|SetbGenerateOverlapEvents (Variables|Default|GetSphere) true)
  (Components|Timeline|SetNewTime (Variables|Default|GetBobbin) (Math|Random|RandomFloatinRange 0.0 5.0))
  (Audio|Components|Audio|Play (Variables|Default|GetBobbin))
  (CallFunction|UpdateShadow)
  (if (Variables|Default|GetFollowSpline)
    (bind _returnvalue_2 (Game|SpawnActorfromClass "/Game/Blueprints/DataOther/BP_ScatterSpline.BP_ScatterSpline_C" (Math|Transform|MakeTransform _location (Math|Rotator|MakeRotator _roll _pitch (+ _yaw (Math|Random|RandomFloatinRange 0.0 3.6e+02))) _scale) "Undefined" 0 0))
    (bind _output_get (Variables|/Game/Blueprints/DataOther/BP_ScatterSpline.BP_ScatterSpline_C|SetSplineFollowActor _returnvalue_2 self))
    (Default|MoveAlongSpline _returnvalue_2 _output_get)))

(event EventCollect
  (params (PlayerCharacter :type BP%20Pant%20Controller%20Object%20Reference))
  (Variables|Default|SetBlockShadowUpdate true)
  (Utilities|FlowControl|Delay 0.05)
  (Audio|Components|Audio|Stop (Variables|Default|GetTL_SpawnFromFolder))
  (bind _output_get (Variables|Default|SetPlayerCharacter PlayerCharacter))
  (Effects|Components|ParticleSystem|SetTemplate (Variables|Default|GetP_Particle) "/Game/Effects/Particles/P_Dust1.P_Dust1")
  (bind _asbp_pant_controller (Utilities|Casting|CastToBP_PantController (Game|GetPlayerCharacter 0))
    (:then
      (if (Variables|/Game/PantControllerBP/Blueprints/BP_PantController.BP_PantController_C|GetFileFolderHidden _asbp_pant_controller)
        (Default|Show/HideFilePanel _asbp_pant_controller true))
      (Default|Attachto _output_get self)
      (if (Variables|/Game/PantControllerBP/Blueprints/BP_PantController.BP_PantController_C|GetIsGamepad _asbp_pant_controller)
        (Game|Feedback|ClientPlayForceFeedback (Game|GetPlayerController 0) "/Game/Effects/Other/RumbleTest1.RumbleTest1" "Collect" false false false))
      (Rendering|SetVisibility (Variables|Default|GetBlob) false true)
      (Audio|PlaySoundatLocation "/Game/Audio/SFX/PopupSFX/SFX_PopupClose.SFX_PopupClose" (Transformation|GetWorldLocation (Variables|Default|GetDefaultSceneRoot)) "0, 0, 0" (Variables|Default|GetVolume) (Math|Random|RandomFloatinRange 0.5 0.75) 0.15 "/Game/Audio/Attenuation/SA_ShortRange.SA_ShortRange" "/Game/Audio/Concurrency/AC_Files.AC_Files" 0)
      (Audio|Components|Audio|Stop (Variables|Default|GetBobbin))
      (Utilities|FlowControl|DoOnce false
        (:Completed
          (Audio|Components|Audio|Stop (Variables|Default|GetTL_SpawnFromFolder))
          (Components|Timeline|PlayfromStart (Variables|Default|GetCollect_TL))
          (Rendering|SetVisibility (Variables|Default|GetBlob) false true))))
    (:CastFailed
      (Utilities|FlowControl|DoOnce false
        (:Completed
          (bind _asbp_pant_controller_2 (Utilities|Casting|CastToBP_PantController (Variables|Default|GetPlayerCharacter))
            (:then
              (Components|Timeline|PlayfromStart (Variables|/Game/PantControllerBP/Blueprints/BP_PantController.BP_PantController_C|GetCollectBounce_TL _asbp_pant_controller_2))
              (Variables|/Game/PantControllerBP/Blueprints/BP_PantController.BP_PantController_C|SetFileCount (Variables|Default|GetPlayerCharacter) (Math|Integer|Clamp(Integer) (- (Variables|/Game/PantControllerBP/Blueprints/BP_PantController.BP_PantController_C|GetFileCount (Variables|Default|GetPlayerCharacter)) 2) 0 999999))
              (Default|UpdateFileImage (Variables|/Game/PantControllerBP/Blueprints/BP_PantController.BP_PantController_C|GetFileCounterWidget (Variables|Default|GetPlayerCharacter)) (Variables|Default|GetFileType))
              (UserInterface|Animation|PlayAnimation (Variables|/Game/PantControllerBP/Blueprints/BP_PantController.BP_PantController_C|GetFileCounterWidget (Variables|Default|GetPlayerCharacter)) (Variables|/Game/UserInterface/FileCounterNew_Widget.FileCounterNew_Widget_C|GetAntiPop (Variables|/Game/PantControllerBP/Blueprints/BP_PantController.BP_PantController_C|GetFileCounterWidget (Variables|Default|GetPlayerCharacter))) 0.0 1 "Forward" 0.5 false)
              (if (== (Variables|/Game/PantControllerBP/Blueprints/BP_PantController.BP_PantController_C|GetFileCount _asbp_pant_controller_2) (Variables|/Game/Blueprints/MapObjects/BP_LevelInfo.BP_LevelInfo_C|GetFileCount (Variables|/Game/PantControllerBP/Blueprints/BP_PantController.BP_PantController_C|GetLevelInfo _asbp_pant_controller_2)))
                (Default|FileMessageEvent _asbp_pant_controller_2))
              (bind _asbp_pant_controller_3 (Utilities|Casting|CastToBP_PantController (Variables|Default|GetPlayerCharacter))
                (:then
                  _)
                (:CastFailed
                  _))
              (Audio|PlaySoundatLocation "/Game/Audio/SFX/Random_58.Random_58" (+ (.WorldLocation (Class|PlayerController|DeprojectScreenPositiontoWorld (Game|GetPlayerController 0) (.X (Math|Vector2D|BreakVector2D (.PixelPosition (Class|SlateBlueprintLibrary|LocaltoViewport (Class|Widget|GetTickSpaceGeometry (Variables|/Game/PantControllerBP/Blueprints/BP_PantController.BP_PantController_C|GetFileCounterWidget _asbp_pant_controller_3)) "(X=150.000000,Y=150.000000)")))) (.Y (Math|Vector2D|BreakVector2D (.PixelPosition (Class|SlateBlueprintLibrary|LocaltoViewport (Class|Widget|GetTickSpaceGeometry (Variables|/Game/PantControllerBP/Blueprints/BP_PantController.BP_PantController_C|GetFileCounterWidget _asbp_pant_controller_3)) "(X=150.000000,Y=150.000000)")))))) (* (.WorldDirection (Class|PlayerController|DeprojectScreenPositiontoWorld (Game|GetPlayerController 0) (.X (Math|Vector2D|BreakVector2D (.PixelPosition (Class|SlateBlueprintLibrary|LocaltoViewport (Class|Widget|GetTickSpaceGeometry (Variables|/Game/PantControllerBP/Blueprints/BP_PantController.BP_PantController_C|GetFileCounterWidget _asbp_pant_controller_3)) "(X=150.000000,Y=150.000000)")))) (.Y (Math|Vector2D|BreakVector2D (.PixelPosition (Class|SlateBlueprintLibrary|LocaltoViewport (Class|Widget|GetTickSpaceGeometry (Variables|/Game/PantControllerBP/Blueprints/BP_PantController.BP_PantController_C|GetFileCounterWidget _asbp_pant_controller_3)) "(X=150.000000,Y=150.000000)")))))) 5e+02)) "0, 0, 0" (Variables|Default|GetVolume) (Math|Random|RandomFloatinRange 0.8 1.1) 0.15 "/Game/Audio/Attenuation/SA_ShortRange.SA_ShortRange" "/Game/Audio/Concurrency/AC_Files.AC_Files" 0)
              (Game|SpawnActorfromClass "/Game/Blueprints/FX/BP_DustCollect.BP_DustCollect_C" (Math|Transform|MakeTransform (Transformation|GetWorldLocation (Variables|Default|GetP_Particle))) "Undefined" 0 0)
              (if (Variables|/Game/PantControllerBP/Blueprints/BP_PantController.BP_PantController_C|GetIsGamepad _asbp_pant_controller_3)
                (Game|Feedback|ClientPlayForceFeedback (Game|GetPlayerController 0) "/Game/Effects/Other/RumbleTest1.RumbleTest1" "Collect" false false false))
              (bind _asbp_pant_controller_4 (Utilities|Casting|CastToBP_PantController (Game|GetPlayerCharacter 0))
                (:then
                  _)
                (:CastFailed
                  _)))
            (:CastFailed
              _))
          (Actor|DestroyActor))))))

(fn ConstructionScript
  (bind _returnvalue (Transformation|GetActorLocation))
  (bind _materialbillboard (Variables|Default|GetMaterialBillboard))
  (bind _materialbillboard1 (Variables|Default|GetMaterialBillboard1))
  (bind (_x _y _z) (Math|Vector|BreakVector _returnvalue))
  (if (Variables|Default|GetMazeFile)
    (Rendering|SetVisibility _materialbillboard1 true false)
    (Rendering|SetVisibility _materialbillboard false false)
    (else
      (Rendering|SetVisibility _materialbillboard1 false false)
      (Rendering|SetVisibility _materialbillboard true false)))
  (bind (_outhit _returnvalue_2) (Collision|LineTraceByChannel _returnvalue (Math|Vector|MakeVector _x _y (- _z 1e+04)) "TraceTypeQuery1" false 0 "None"))
  (if _returnvalue_2
    (Transformation|SetWorldLocationAndRotation (Variables|Default|GetBlob) (Math|Vector|MakeVector (.X (Math|Vector|BreakVector (.Location (Collision|BreakHitResult _outhit)))) (.Y (Math|Vector|BreakVector (.Location (Collision|BreakHitResult _outhit)))) (+ (.Z (Math|Vector|BreakVector (.Location (Collision|BreakHitResult _outhit)))) 0.01)) (Math|Rotator|MakeRotfromZ (.ImpactNormal (Collision|BreakHitResult _outhit))) false false)))