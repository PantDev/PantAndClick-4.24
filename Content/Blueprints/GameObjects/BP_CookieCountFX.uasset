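; BP_CookieCountFX is a short-lived floating text effect, named for the cookie count, that plays a jingle when spawned.
; A timeline scales its TextRender and lifts it upward, while Tick keeps the text facing the player camera.
; When the timeline finishes, it spawns a half-scale actor at the text's position and destroys itself.
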(event EventTick
  (params (DeltaSeconds :type Float%20%28single-precision%29))
  (Transformation|SetWorldRotation (Variables|Default|GetTextRender) (Math|Rotator|FindLookatRotation (Transformation|GetWorldLocation (Variables|Default|GetTextRender)) (Transformation|GetActorLocation (Game|GetPlayerCameraManager 0))) false false))

(event EventBeginPlay
  (Audio|PlaySoundatLocation "/Game/Audio/SFX/ActivateJingle.ActivateJingle" (Transformation|GetActorLocation) "0, 0, 0" 0.8 1.1 0.25 "/Game/Audio/Attenuation/SA_ShortRange.SA_ShortRange" "/Game/Audio/Attenuation/SC_Default.SC_Default" 0)
  (bind (_direction _scalealpha _localpha) (Timeline|TL_SpawnVaminos PlayFromStart)
    (:Update
      (Transformation|SetRelativeScale3D (Variables|Default|GetTextRender) (Math|Vector|MakeVector _scalealpha _scalealpha _scalealpha))
      (Transformation|SetRelativeLocation (Variables|Default|GetTextRender) (Math|Vector|MakeVector 0.0 0.0 (Math|Float|Lerp 0.0 65.0 _localpha)) false false))
    (:Finished
      (Game|SpawnActorfromClass "/Game/Blueprints/FX/BP_KillPoof.BP_KillPoof_C" (Math|Transform|MakeTransform (Transformation|GetWorldLocation (Variables|Default|GetTextRender)) "0, 0, 0" "0.500000,0.500000,0.500000") "Undefined" 0 0)
      (Actor|DestroyActor))))

(fn ConstructionScript)