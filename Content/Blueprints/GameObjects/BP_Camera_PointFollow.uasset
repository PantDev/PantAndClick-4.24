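; BP_Camera_PointFollow is a camera actor that turns to keep a FollowPoint actor in view.
; Each tick it interpolates the camera's world rotation toward the look-at direction from its own location, while FollowPoint is valid.
; Activate blends the first player's view to this camera with ease-in-out, and the construction script applies FOV.
; IsBusy always returns false, and a yaw clamp using MinAngle and MaxAngle is left unconnected.
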(event EventBeginPlay)

(event Collision|EventActorBeginOverlap
  (params (OtherActor :type Actor%20Object%20Reference)))

(event EventTick
  (params (DeltaSeconds :type Float%20%28single-precision%29))
  (Utilities|IsValid (Variables|Default|GetFollowPoint)
    (:Is%20Valid
      (Transformation|SetWorldRotation (Variables|Default|GetCamera) (Math|Interpolation|RInterpTo (Transformation|GetWorldRotation (Variables|Default|GetCamera)) (Math|Rotator|FindLookatRotation (Transformation|GetActorLocation) (Transformation|GetActorLocation (Variables|Default|GetFollowPoint))) DeltaSeconds 16.0) false false))))

(event EventActivate
  (params (Delay :type Float%20%28single-precision%29) (Bool :type Boolean))
  (Game|Player|SetViewTargetwithBlend (Game|GetPlayerController 0) self 2.0 "VTBlend_EaseInOut" 5.0 false))

(fn ConstructionScript
  (Camera|SetFieldOfView (Variables|Default|GetCamera) (Variables|Default|GetFOV)))

(fn IsBusy
  (return false))