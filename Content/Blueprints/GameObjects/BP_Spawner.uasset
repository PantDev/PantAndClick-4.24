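; BP_Spawner is a one-shot travelling spawn effect that flies to a given actor and triggers its spawn.
; SpawnEvent drives a timeline that moves it from its start to the target, adding a curve-based height offset that also modulates the moving sound's pitch.
; After arrival and a delay, it calls SpawnEntityMessage on the target, spawns BP_KillPoof, plays a pop at the start location and destroys itself.
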(event Custom|SpawnEvent
  (params (Actor :type Actor%20Object%20Reference) (Delay :type Float%20%28single-precision%29))
  (Variables|Default|SetSpawningActor Actor)
  (Variables|Default|SetStartLoc (Transformation|GetActorLocation))
  (Variables|Default|SetEndLoc (Transformation|GetActorLocation (Variables|Default|GetSpawningActor)))
  (Variables|Default|SetDelay Delay)
  (Components|Timeline|SetPlayRate (Variables|Default|GetTL_SpawnAnim) 0.85)
  (Components|Activation|Activate (Variables|Default|GetEthernetMoving) false)
  (bind (_direction _localpha _z_posalpha) (Timeline|TL_SpawnAnim PlayFromStart)
    (:Update
      (Transformation|SetActorLocation (Math|Vector|MakeVector (.X (Math|Vector|BreakVector (Math|Vector|Lerp(Vector) (Variables|Default|GetStartLoc) (Variables|Default|GetEndLoc) _localpha))) (.Y (Math|Vector|BreakVector (Math|Vector|Lerp(Vector) (Variables|Default|GetStartLoc) (Variables|Default|GetEndLoc) _localpha))) (+ (.Z (Math|Vector|BreakVector (Math|Vector|Lerp(Vector) (Variables|Default|GetStartLoc) (Variables|Default|GetEndLoc) _localpha))) (Math|Float|Lerp 0.0 275.0 _z_posalpha))) false false)
      (Audio|Components|Audio|SetPitchMultiplier (Variables|Default|GetEthernetMoving) (Math|Float|Lerp 0.2 2.2 _z_posalpha)))
    (:Finished
      (Components|Activation|Deactivate (Variables|Default|GetEthernetMoving))
      (Utilities|FlowControl|Delay (Variables|Default|GetDelay))
      (Class|BPISpawnable|SpawnEntity(Message) (Variables|Default|GetSpawningActor))
      (Game|SpawnActorfromClass "/Game/Blueprints/FX/BP_KillPoof.BP_KillPoof_C" (Math|Transform|MakeTransform (Transformation|GetActorLocation) "0, 0, 0" "1.500000,1.500000,1.500000") "Undefined" 0 0)
      (Audio|PlaySoundatLocation "/Game/Audio/SFX/Pop.Pop" (Variables|Default|GetStartLoc) "0, 0, 0" 0.5 (Math|Random|RandomFloatinRange 1.1 1.4) 0.0 "/Game/Audio/Attenuation/SA_ShortRange.SA_ShortRange" "/Game/Audio/Attenuation/SC_Default.SC_Default" 0)
      (Actor|DestroyActor))))

(fn ConstructionScript)