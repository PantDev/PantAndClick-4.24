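; BP_FocusLine is an actor that draws a jittering line between BP_PantController's 3D cursor and its FocusLoc.
; While Active, Tick eases it to the midpoint, aims it at FocusLoc and scales the skeletal mesh's length by distance.
; SetRandDeform re-calls itself after short random delays, randomizing morph targets and roll for flicker.
; A line-out timeline grows the line from the cursor, but nothing triggers it in this graph.
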(event Custom|SetRandDeform
  (bind _skeletalmesh (Variables|Default|GetSkeletalMesh))
  (Components|SkeletalMesh|SetMorphTarget _skeletalmesh "Deform1" (Math|Random|RandomFloatinRange -0.2 0.2) true)
  (Components|SkeletalMesh|SetMorphTarget _skeletalmesh "Deform2" (Math|Random|RandomFloatinRange -0.5 0.5) true)
  (Transformation|SetRelativeRotation (Variables|Default|GetSkeletalMesh) (Math|Rotator|MakeRotator 0.0 (Math|Random|RandomFloatinRange 0.0 3.6e+02) 9e+01) false false)
  (Utilities|FlowControl|Delay (Math|Random|RandomFloatinRange 0.05 0.1))
  (CallFunction|SetRandDeform))

(event EventBeginPlay)

(event Collision|EventActorBeginOverlap
  (params (OtherActor :type Actor%20Object%20Reference)))

(event EventTick
  (params (DeltaSeconds :type Float%20%28single-precision%29))
  (if (not (Audio|Components|Audio|IsPlaying (Variables|Default|GetTL_LineOut)))
    (bind _asbp_pant_controller (Utilities|Casting|CastToBP_PantController (Game|GetPlayerCharacter 0)))
    (if (Variables|Default|GetActive)
      (Transformation|SetActorLocation (Math|Interpolation|VInterpTo (Transformation|GetActorLocation) (/ (+ (Math|Vector|MakeVector (.X (Math|Vector|BreakVector (Transformation|GetWorldLocation (Variables|/Game/PantControllerBP/Blueprints/BP_PantController.BP_PantController_C|GetCursor3DMesh _asbp_pant_controller)))) (.Y (Math|Vector|BreakVector (Transformation|GetWorldLocation (Variables|/Game/PantControllerBP/Blueprints/BP_PantController.BP_PantController_C|GetCursor3DMesh _asbp_pant_controller)))) (- (.Z (Math|Vector|BreakVector (Transformation|GetWorldLocation (Variables|/Game/PantControllerBP/Blueprints/BP_PantController.BP_PantController_C|GetCursor3DMesh _asbp_pant_controller)))) 4.0)) (Variables|/Game/PantControllerBP/Blueprints/BP_PantController.BP_PantController_C|GetFocusLoc _asbp_pant_controller)) 2.0) (Utilities|Time|GetWorldDeltaSeconds) 15.0) false false)
      (Transformation|SetActorRotation (Math|Rotator|FindLookatRotation (Math|Vector|MakeVector (.X (Math|Vector|BreakVector (Transformation|GetWorldLocation (Variables|/Game/PantControllerBP/Blueprints/BP_PantController.BP_PantController_C|GetCursor3DMesh _asbp_pant_controller)))) (.Y (Math|Vector|BreakVector (Transformation|GetWorldLocation (Variables|/Game/PantControllerBP/Blueprints/BP_PantController.BP_PantController_C|GetCursor3DMesh _asbp_pant_controller)))) (- (.Z (Math|Vector|BreakVector (Transformation|GetWorldLocation (Variables|/Game/PantControllerBP/Blueprints/BP_PantController.BP_PantController_C|GetCursor3DMesh _asbp_pant_controller)))) 4.0)) (Variables|/Game/PantControllerBP/Blueprints/BP_PantController.BP_PantController_C|GetFocusLoc _asbp_pant_controller)))
      (Transformation|SetRelativeScale3D (Variables|Default|GetSkeletalMesh) (Math|Vector|MakeVector 3.5 (* (Math|Vector|VectorLength (- (Math|Vector|MakeVector (.X (Math|Vector|BreakVector (Transformation|GetWorldLocation (Variables|/Game/PantControllerBP/Blueprints/BP_PantController.BP_PantController_C|GetCursor3DMesh _asbp_pant_controller)))) (.Y (Math|Vector|BreakVector (Transformation|GetWorldLocation (Variables|/Game/PantControllerBP/Blueprints/BP_PantController.BP_PantController_C|GetCursor3DMesh _asbp_pant_controller)))) (- (.Z (Math|Vector|BreakVector (Transformation|GetWorldLocation (Variables|/Game/PantControllerBP/Blueprints/BP_PantController.BP_PantController_C|GetCursor3DMesh _asbp_pant_controller)))) 4.0)) (Variables|/Game/PantControllerBP/Blueprints/BP_PantController.BP_PantController_C|GetFocusLoc _asbp_pant_controller))) 0.00475) 3.5)))))

(fn ConstructionScript)