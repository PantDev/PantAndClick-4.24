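; BP_LinkChain is a game object actor that grows into view on spawn and keeps facing the player.
; On BeginPlay, the TL_Spawn timeline drives a uniform scale from zero to full size.
; Every Tick, it finds the look-at rotation toward player character 0 and applies it through RInterpTo with no interp speed set, teleporting physics.
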(event EventBeginPlay
  (bind _scalealpha (Timeline|TL_Spawn PlayFromStart)
    (:Update
      (Transformation|SetActorScale3D (Math|Vector|MakeVector (Math|Float|Lerp 0.0 1.0 _scalealpha) (Math|Float|Lerp 0.0 1.0 _scalealpha) (Math|Float|Lerp 0.0 1.0 _scalealpha))))))

(event Collision|EventActorBeginOverlap
  (params (OtherActor :type Actor%20Object%20Reference)))

(event EventTick
  (params (DeltaSeconds :type Float%20%28single-precision%29))
  (Transformation|SetActorRotation (Math|Interpolation|RInterpTo (Transformation|GetActorRotation) (Math|Rotator|FindLookatRotation (Transformation|GetActorLocation) (Transformation|GetActorLocation (Game|GetPlayerCharacter 0))) DeltaSeconds 0.0) true))

(fn ConstructionScript)