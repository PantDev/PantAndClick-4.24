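; Interactive switch actor, configurable as a push button or flip switch, that can signal a linked ActivatedActor.
; The construction script picks the visible parts and collision for the mode and creates the button's colored dynamic material.
; Poking, gated by Busy, starts timelines and sounds; buttons send ActivateMessage as momentary or alternating toggle, while the switch path only flips, leaving messaging to a separate Activate event.
; Grab and snap functions are mostly stubs, and older moving-platform logic is disconnected.
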(event Custom|LetGoEvent
  (Audio|PlaySoundatLocation "/Game/Audio/SFX/Pop.Pop" (Transformation|GetActorLocation) "0, 0, 0" 1.0 (Math|Random|RandomFloatinRange 0.7 1.1) 0.0 "/Game/Audio/Attenuation/SA_Default.SA_Default" "/Game/Audio/Attenuation/SC_Default.SC_Default" 0))

(event EventBeginPlay)

(event Collision|EventActorBeginOverlap
  (params (OtherActor :type Actor%20Object%20Reference)))

(event EventTick
  (params (DeltaSeconds :type Float%20%28single-precision%29)))

(event EventAddOffsetZ
  (params (Offset_Z :type Float%20%28single-precision%29))
  (Transformation|AddRelativeRotation (Variables|Default|GetSwitchFrame) (Math|Rotator|MakeRotator 0.0 0.0 Offset_Z) false false))

(event EventPokeEvent
  (bind _tl_buttontoggle (Variables|Default|GetTL_ButtonToggle))
  (bind _activatedactor (Variables|Default|GetActivatedActor))
  (bind _activatebool (Variables|Default|GetActivateBool))
  (bind _tl_flip (Variables|Default|GetTL_Flip))
  (if (not (Variables|Default|GetBusy))
    (if (Variables|Default|GetButton)
      (if (Variables|Default|GetButtonToggle)
        (Utilities|FlowControl|FlipFlop
          (:A
            (Components|Timeline|PlayfromStart _tl_buttontoggle)
            (Audio|PlaySoundatLocation "/Game/Audio/SFX/ButtonPress1.ButtonPress1" (Transformation|GetWorldLocation (Variables|Default|GetDefaultSceneRoot)) "0, 0, 0" 0.3 (Math|Random|RandomFloatinRange 0.95 1.05) 0.0 "/Game/Audio/Attenuation/SA_Default.SA_Default" "/Game/Audio/Attenuation/SC_Default.SC_Default" 0)
            (Class|BPIActivate|Activate(Message) _activatedactor 0.0 (not _activatebool)))
          (:B
            (Components|Timeline|ReversefromEnd _tl_buttontoggle)
            (Audio|PlaySoundatLocation "/Game/Audio/SFX/Switch1.Switch1" (Transformation|GetWorldLocation (Variables|Default|GetDefaultSceneRoot)) "0, 0, 0" 0.3 (Math|Random|RandomFloatinRange 0.625 0.675) 0.03 "/Game/Audio/Attenuation/SA_Default.SA_Default" "/Game/Audio/Attenuation/SC_Default.SC_Default" 0)
            (Class|BPIActivate|Activate(Message) _activatedactor 0.0 _activatebool)))
        (else
          (Components|Timeline|PlayfromStart (Variables|Default|GetTL_ButtonPress))
          (Audio|PlaySoundatLocation "/Game/Audio/SFX/ButtonPress1.ButtonPress1" (Transformation|GetWorldLocation (Variables|Default|GetDefaultSceneRoot)) "0, 0, 0" 0.3 (Math|Random|RandomFloatinRange 0.95 1.05) 0.0 "/Game/Audio/Attenuation/SA_Default.SA_Default" "/Game/Audio/Attenuation/SC_Default.SC_Default" 0)
          (if (and (Utilities|IsValid (Variables|Default|GetActivatedActor)) (Variables|Default|GetGateOpen))
            (Class|BPIActivate|Activate(Message) (Variables|Default|GetActivatedActor) 0.0 (Variables|Default|GetActivateBool)))
          (Utilities|FlowControl|Delay 0.24)
          (Audio|PlaySoundatLocation "/Game/Audio/SFX/Switch1.Switch1" (Transformation|GetWorldLocation (Variables|Default|GetDefaultSceneRoot)) "0, 0, 0" 0.3 (Math|Random|RandomFloatinRange 0.625 0.675) 0.03 "/Game/Audio/Attenuation/SA_Default.SA_Default" "/Game/Audio/Attenuation/SC_Default.SC_Default" 0)))
      (else
        (Audio|PlaySoundatLocation "/Game/Audio/SFX/Switch1.Switch1" (Transformation|GetWorldLocation (Variables|Default|GetDefaultSceneRoot)) "0, 0, 0" 0.3 (Math|Random|RandomFloatinRange 0.95 1.05) 0.0 "/Game/Audio/Attenuation/SA_Default.SA_Default" "/Game/Audio/Attenuation/SC_Default.SC_Default" 0)
        (Utilities|FlowControl|FlipFlop
          (:A
            (Components|Timeline|PlayfromStart _tl_flip))
          (:B
            (Components|Timeline|ReversefromEnd _tl_flip)))))))

(event MouseInput|EventActorBeginCursorOver
  (Actor|DestroyActor))

(event EventActivate
  (params (Delay :type Float%20%28single-precision%29) (Bool :type Boolean))
  (Class|BPIActivate|Activate(Message) (Variables|Default|GetActivatedActor) 0.0 (Variables|Default|GetActivateBool)))

(fn ConstructionScript
  (Components|StaticMesh|SetStaticMesh (Variables|Default|GetButtonFrame) (Variables|Default|GetButtonFrameMesh))
  (Components|StaticMesh|SetStaticMesh (Variables|Default|GetButtonButton) (Variables|Default|GetButtonMesh))
  (bind _returnvalue (Rendering|Material|CreateDynamicMaterialInstance (Variables|Default|GetButtonButton) 0 "/Game/Materials/PopupBorder_Mat.PopupBorder_Mat" "None" :!class /Script/Engine.PrimitiveComponent))
  (bind _output_get (Variables|Default|SetDynMat _returnvalue))
  (Rendering|Material|SetMaterial (Variables|Default|GetButtonButton) 0 _output_get)
  (Rendering|Material|SetVectorParameterValue _output_get "Color" (Variables|Default|GetColor) :!class /Script/Engine.MaterialInstanceDynamic)
  (Rendering|Material|SetScalarParameterValue _output_get "Divide" 5.0 :!class /Script/Engine.MaterialInstanceDynamic)
  (Transformation|SetRelativeLocationAndRotation (Variables|Default|GetSwitchFrame) (Variables|Default|GetLocationOffset) (Variables|Default|GetRotationOffset) false false)
  (Variables|Default|SetOriginalScale (Transformation|GetActorScale3D))
  (if (Variables|Default|GetButton)
    (Rendering|SetVisibility (Variables|Default|GetButtonFrame) true true)
    (Rendering|SetVisibility (Variables|Default|GetSwitchFrame) false true)
    (Collision|SetCollisionEnabled (Variables|Default|GetBox) "NoCollision")
    (Collision|SetCollisionEnabled (Variables|Default|GetSphere) "QueryAndPhysics")
    (else
      (Rendering|SetVisibility (Variables|Default|GetButtonFrame) false true)
      (Rendering|SetVisibility (Variables|Default|GetSwitchFrame) true true)
      (Collision|SetCollisionEnabled (Variables|Default|GetBox) "QueryAndPhysics")
      (Collision|SetCollisionEnabled (Variables|Default|GetSphere) "NoCollision"))))

(fn Attachto
  (params (ChildActor :type Actor%20Object%20Reference))
  (return (Utilities|Array|MakeArray 0)))

(fn CanGrab
  (return false))

(fn Clicked
  (Collision|SetCollisionEnabled (Variables|Default|GetBox) "NoCollision")
  (return false))

(fn DisableCollision
  (return false))

(fn DoesParentHaveParent
  (return false))

(fn EnableCollision
  (return false))

(fn GetAttached
  (return (Utilities|Array|MakeArray 0)))

(fn GetCustomCursor
  (return false 0))

(fn GetShrinkScale
  (return (Variables|Default|GetShrinkScale) (Variables|Default|GetOriginalScale)))

(fn GetSnapLoc
  (params (CursorLoc :type Vector :default "0, 0, 0"))
  (Variables|Default|SetSnapLoc (Transformation|GetWorldLocation (Variables|Default|GetBox)))
  (Variables|Default|SetSnapRot (Transformation|GetWorldRotation (Variables|Default|GetSwitchFrame)))
  (return (Variables|Default|GetSnapLoc) (Variables|Default|GetSnapRot)))

(fn Grabbed
  (return 0))

(fn IsBusy
  (bind _busy (Class|BPIActivate|IsBusy(Message) (Variables|Default|GetActivatedActor)))
  (return _busy))

(fn LetGo
  (params (ParentComponent :type Actor%20Component%20Object%20Reference) (ParentActor :type Actor%20Object%20Reference))
  (Variables|Default|SetParent ParentActor)
  (CallFunction|LetGoEvent)
  (Collision|SetCollisionEnabled (Variables|Default|GetBox) "QueryOnly")
  (return false))

(fn OnHover
  (return false))

(fn PassChildAlong
  (return 0 0))