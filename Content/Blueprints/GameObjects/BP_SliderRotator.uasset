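; BP_SliderRotator is a mesh game object with an optional idle hover and a switchable dark state.
; The construction script applies the chosen mesh and wraps its material in a dynamic instance, whose Dark parameter Activate toggles.
; When HoverOn is set, a timeline started at BeginPlay sways the mesh along local X, restarting at a random play rate after each cycle.
; IsBusy always returns false.
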(event EventBeginPlay
  (if (Variables|Default|GetHoverOn)
    (Components|Timeline|PlayfromStart (Variables|Default|GetTL_Hover))))

(event EventActivate
  (params (Delay :type Float%20%28single-precision%29) (Bool :type Boolean))
  (bind _panelmatinstance (Variables|Default|GetPanelMatInstance))
  (if Bool
    (Rendering|Material|SetScalarParameterValue _panelmatinstance "Dark" 0.0 :!class /Script/Engine.MaterialInstanceDynamic)
    (else
      (Rendering|Material|SetScalarParameterValue _panelmatinstance "Dark" 1.0 :!class /Script/Engine.MaterialInstanceDynamic))))

(fn ConstructionScript
  (bind _staticmesh (Variables|Default|GetStaticMesh))
  (Components|StaticMesh|SetStaticMesh (Variables|Default|GetStaticMesh) (Variables|Default|GetMesh))
  (Rendering|Material|SetMaterial _staticmesh 0 0)
  (bind _returnvalue (Rendering|Material|CreateDynamicMaterialInstance _staticmesh 0 (Rendering|Material|GetMaterial _staticmesh 0) "None" :!class /Script/Engine.PrimitiveComponent))
  (bind _output_get (Variables|Default|SetPanelMatInstance _returnvalue))
  (Rendering|Material|SetMaterial (Variables|Default|GetStaticMesh) 0 _output_get))

(fn IsBusy
  (return false))