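; BP_PopupRoom is a room actor that pops open and folds back on alternate pokes.
; PokeEvent uses a FlipFlop to play or reverse a timeline.
; Its alpha drives the mesh's Depth, X and Y morph targets toward variable sizes while sliding the spring arm along local X.
; The interaction functions for grab, hover, click, snap and attach are empty stubs returning defaults.
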(event EventBeginPlay)

(event Collision|EventActorBeginOverlap
  (params (OtherActor :type Actor%20Object%20Reference)))

(event EventTick
  (params (DeltaSeconds :type Float%20%28single-precision%29)))

(event EventPokeEvent
  (bind _popupmesh (Variables|Default|GetPopupMesh))
  (Utilities|FlowControl|FlipFlop
    (:A
      (bind _depthfloat (Timeline|Timeline_0 Play)
        (:Update
          (Components|SkeletalMesh|SetMorphTarget _popupmesh "Depth" (Math|Float|Lerp 0.0 (Variables|Default|GetDepth) _depthfloat) true)
          (Components|SkeletalMesh|SetMorphTarget _popupmesh "X" (Math|Float|Lerp 0.0 (Variables|Default|GetX) _depthfloat) true)
          (Components|SkeletalMesh|SetMorphTarget _popupmesh "Y" (Math|Float|Lerp 0.0 (Variables|Default|GetY) _depthfloat) true)
          (Transformation|SetRelativeLocation (Variables|Default|GetSpringArm) (Math|Vector|Lerp(Vector) "70.000000,25.000000,60.000000" "550.000000,25.000000,60.000000" _depthfloat) false false))))
    (:B
      (Timeline|Timeline_0 Reverse))))

(fn ConstructionScript)

(fn Attachto
  (params (ChildActor :type Actor%20Object%20Reference))
  (return 0))

(fn Clicked
  (return false))

(fn DisableCollision
  (return false))

(fn DoesParentHaveParent
  (return false))

(fn EnableCollision
  (return false))

(fn GetAttached
  (return 0))

(fn GetShrinkScale
  (return "0, 0, 0" "0, 0, 0"))

(fn GetSnapLoc
  (params (CursorLoc :type Vector :default "0, 0, 0"))
  (return "0, 0, 0" "0, 0, 0"))

(fn Grabbed
  (return 0))

(fn LetGo
  (params (ParentComponent :type Actor%20Component%20Object%20Reference) (ParentActor :type Actor%20Object%20Reference))
  (return false))

(fn OnHover
  (return false))

(fn PassChildAlong
  (return 0 0))