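; Snap cursor actor that glides from the player's 3D cursor to its spawn point, mimicking that cursor's mesh, scale and rotation.
; Each tick it eases into place, aligns a spring arm along the camera-to-actor line and sets arm length to its distance from the cursor.
; When the character's DenimMesh strays too far, it notifies the character and runs KillEvent.
; KillEvent's timeline lerps it back to the cursor, re-shows that cursor and destroys the actor.
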(event Custom|KillEvent
  (bind _newtrack_0 (Timeline|Timeline_0 PlayFromStart)
    (:Update
      (bind _asbp_third_person_character (Utilities|Casting|CastToBP_ThirdPersonCharacter (Game|GetPlayerCharacter 0)))
      (Transformation|SetActorLocation (Math|Vector|Lerp(Vector) (Variables|Default|GetOriginLoc) (Transformation|GetWorldLocation (Variables|/Game/ThirdPersonBP/Blueprints/BP_ThirdPersonCharacter.BP_ThirdPersonCharacter_C|GetCursor3DMesh _asbp_third_person_character)) _newtrack_0) false false))
    (:Finished
      (bind _asbp_third_person_character_2 (Utilities|Casting|CastToBP_ThirdPersonCharacter (Game|GetPlayerCharacter 0)))
      (Rendering|SetVisibility (Variables|/Game/ThirdPersonBP/Blueprints/BP_ThirdPersonCharacter.BP_ThirdPersonCharacter_C|GetCursor3DMesh _asbp_third_person_character_2) true false)
      (Actor|DestroyActor))))

(event EventBeginPlay
  (bind _staticmesh (Variables|Default|GetStaticMesh))
  (bind _asbp_third_person_character (Utilities|Casting|CastToBP_ThirdPersonCharacter (Game|GetPlayerCharacter 0)))
  (Variables|Default|SetOriginLoc (Transformation|GetActorLocation))
  (Transformation|SetActorLocation (Transformation|GetWorldLocation (Variables|/Game/ThirdPersonBP/Blueprints/BP_ThirdPersonCharacter.BP_ThirdPersonCharacter_C|GetCursor3DMesh _asbp_third_person_character)) false false)
  (Utilities|FlowControl|Gate true ; enters at Open
    (:Exit
      (bind _asbp_third_person_character_2 (Utilities|Casting|CastToBP_ThirdPersonCharacter (Game|GetPlayerCharacter 0)))
      (Transformation|SetWorldRotation (Variables|Default|GetSpringArm) (Math|Interpolation|RInterpTo (Transformation|GetWorldRotation (Variables|Default|GetSpringArm)) (Math|Rotator|FindLookatRotation (Transformation|GetWorldLocation (Variables|/Script/Engine.Actor|GetRootComponent (Game|GetPlayerCameraManager 0))) (Transformation|GetWorldLocation (Variables|Default|GetDefaultSceneRoot))) (stale EventTick DeltaSeconds) 25.0) false false)
      (Transformation|SetWorldRotation _staticmesh (Math|Interpolation|RInterpTo (Transformation|GetWorldRotation _staticmesh) (Transformation|GetWorldRotation (Variables|/Game/ThirdPersonBP/Blueprints/BP_ThirdPersonCharacter.BP_ThirdPersonCharacter_C|GetCursor3DMesh _asbp_third_person_character_2)) (stale EventTick DeltaSeconds) 2e+01) false false)
      (Transformation|SetActorLocation (Math|Interpolation|VInterpTo (Transformation|GetActorLocation) (Variables|Default|GetOriginLoc) (Utilities|Time|GetWorldDeltaSeconds) 8.0) false false)
      (Variables|/Script/Engine.SpringArmComponent|SetTargetArmLength (Variables|Default|GetSpringArm) (Math|Vector|VectorLength (- (Transformation|GetWorldLocation (Variables|Default|GetDefaultSceneRoot)) (Transformation|GetWorldLocation (Variables|/Game/ThirdPersonBP/Blueprints/BP_ThirdPersonCharacter.BP_ThirdPersonCharacter_C|GetCursor3DMesh _asbp_third_person_character_2)))))
      (Transformation|SetWorldScale3D (Variables|Default|GetStaticMesh) (Transformation|GetWorldScale (Variables|/Game/ThirdPersonBP/Blueprints/BP_ThirdPersonCharacter.BP_ThirdPersonCharacter_C|GetCursor3DMesh _asbp_third_person_character_2)))
      (Components|StaticMesh|SetStaticMesh (Variables|Default|GetStaticMesh) (Variables|/Script/Engine.StaticMeshComponent|GetStaticMesh (Variables|/Game/ThirdPersonBP/Blueprints/BP_ThirdPersonCharacter.BP_ThirdPersonCharacter_C|GetCursor3DMesh _asbp_third_person_character_2)))
      (if (> (Math|Vector|VectorLength (- (Transformation|GetWorldLocation (Variables|/Game/ThirdPersonBP/Blueprints/BP_ThirdPersonCharacter.BP_ThirdPersonCharacter_C|GetDenimMesh _asbp_third_person_character_2)) (Transformation|GetWorldLocation (Variables|Default|GetDefaultSceneRoot)))) 4e+02)
        (Default|KillSnapCursor _asbp_third_person_character_2)
        (CallFunction|KillEvent)))))

(event EventTick
  (params (DeltaSeconds :type Float%20%28single-precision%29))
  (bind _staticmesh (Variables|Default|GetStaticMesh))
  (bind _asbp_third_person_character (Utilities|Casting|CastToBP_ThirdPersonCharacter (Game|GetPlayerCharacter 0)))
  (Transformation|SetWorldRotation (Variables|Default|GetSpringArm) (Math|Interpolation|RInterpTo (Transformation|GetWorldRotation (Variables|Default|GetSpringArm)) (Math|Rotator|FindLookatRotation (Transformation|GetWorldLocation (Variables|/Script/Engine.Actor|GetRootComponent (Game|GetPlayerCameraManager 0))) (Transformation|GetWorldLocation (Variables|Default|GetDefaultSceneRoot))) DeltaSeconds 25.0) false false)
  (Transformation|SetWorldRotation _staticmesh (Math|Interpolation|RInterpTo (Transformation|GetWorldRotation _staticmesh) (Transformation|GetWorldRotation (Variables|/Game/ThirdPersonBP/Blueprints/BP_ThirdPersonCharacter.BP_ThirdPersonCharacter_C|GetCursor3DMesh _asbp_third_person_character)) DeltaSeconds 2e+01) false false)
  (Transformation|SetActorLocation (Math|Interpolation|VInterpTo (Transformation|GetActorLocation) (Variables|Default|GetOriginLoc) (Utilities|Time|GetWorldDeltaSeconds) 8.0) false false)
  (Variables|/Script/Engine.SpringArmComponent|SetTargetArmLength (Variables|Default|GetSpringArm) (Math|Vector|VectorLength (- (Transformation|GetWorldLocation (Variables|Default|GetDefaultSceneRoot)) (Transformation|GetWorldLocation (Variables|/Game/ThirdPersonBP/Blueprints/BP_ThirdPersonCharacter.BP_ThirdPersonCharacter_C|GetCursor3DMesh _asbp_third_person_character)))))
  (Transformation|SetWorldScale3D (Variables|Default|GetStaticMesh) (Transformation|GetWorldScale (Variables|/Game/ThirdPersonBP/Blueprints/BP_ThirdPersonCharacter.BP_ThirdPersonCharacter_C|GetCursor3DMesh _asbp_third_person_character)))
  (Components|StaticMesh|SetStaticMesh (Variables|Default|GetStaticMesh) (Variables|/Script/Engine.StaticMeshComponent|GetStaticMesh (Variables|/Game/ThirdPersonBP/Blueprints/BP_ThirdPersonCharacter.BP_ThirdPersonCharacter_C|GetCursor3DMesh _asbp_third_person_character)))
  (if (> (Math|Vector|VectorLength (- (Transformation|GetWorldLocation (Variables|/Game/ThirdPersonBP/Blueprints/BP_ThirdPersonCharacter.BP_ThirdPersonCharacter_C|GetDenimMesh _asbp_third_person_character)) (Transformation|GetWorldLocation (Variables|Default|GetDefaultSceneRoot)))) 4e+02)
    (Default|KillSnapCursor _asbp_third_person_character)
    (CallFunction|KillEvent)))

(fn ConstructionScript)