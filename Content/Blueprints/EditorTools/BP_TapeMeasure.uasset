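; BP_TapeMeasure is an editor tool actor that measures and labels the straight-line distance to a Partner actor.
; When Active, its construction script moves MeasurementText to the midpoint between the two actors and sets it to the raw distance in world units.
; Partner is not validity-checked, and the event graph holds only disabled placeholder events, so the label updates only when construction reruns.
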(event EventBeginPlay)

(event Collision|EventActorBeginOverlap
  (params (OtherActor :type Actor%20Object%20Reference)))

(event EventTick
  (params (DeltaSeconds :type Float%20%28single-precision%29)))

(fn ConstructionScript
  (if (Variables|Default|GetActive)
    (Transformation|SetWorldLocation (Variables|Default|GetMeasurementText) (Math|Vector|Lerp(Vector) (Transformation|GetActorLocation) (Transformation|GetActorLocation (Variables|Default|GetPartner)) 0.5) false false)
    (Rendering|Components|TextRender|SetText (Variables|Default|GetMeasurementText) (Utilities|Text|ToText(Float) (Math|Vector|VectorLength (- (Transformation|GetActorLocation) (Transformation|GetActorLocation (Variables|Default|GetPartner)))) "HalfToEven"))))