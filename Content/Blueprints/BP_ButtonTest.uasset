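; BP_ButtonTest is a test button actor that gives random visual and audio feedback when clicked.
; Clicked swaps the static mesh to a random material from a fixed list, plays a jump sound at random pitch and randomizes each scale axis.
; The other interaction functions for grabbing, attaching, snapping, hover and collision are empty stubs returning defaults, and the event graph is unused.
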(event EventBeginPlay)

(event Collision|EventActorBeginOverlap
  (params (OtherActor :type Actor%20Object%20Reference)))

(event EventTick
  (params (DeltaSeconds :type Float%20%28single-precision%29)))

(fn ConstructionScript)

(fn Attachto
  (params (ChildActor :type Actor%20Object%20Reference))
  (return (Utilities|Array|MakeArray 0)))

(fn Clicked
  (bind _returnvalue (Math|Random|RandomFloatinRange 0.9 1.5))
  (Rendering|Material|SetMaterial (Variables|Default|GetStaticMesh) 0 (Utilities|Array|Get(acopy) (Utilities|Array|MakeArray "/Game/Materials/CoinGold2.CoinGold2" "/Game/StarterContent/Materials/M_Wood_Walnut.M_Wood_Walnut" "/Game/Materials/Glow.Glow" "/Game/Materials/SolidBlack_Mat.SolidBlack_Mat" "/Game/Materials/grass1_Mat.grass1_Mat" "/Game/Meshes/lowpolypencilUV_Mat.lowpolypencilUV_Mat") (Math|Random|RandomIntegerinRange 0 5)))
  (Audio|PlaySoundatLocation "/Game/Audio/SFX/Jump1.Jump1" (Transformation|GetActorLocation) "0, 0, 0" 0.7 (Math|Random|RandomFloatinRange 0.35 1.1) 0.18 "/Game/Audio/Attenuation/SA_Default.SA_Default")
  (Transformation|SetActorScale3D (Math|Vector|MakeVector _returnvalue _returnvalue _returnvalue))
  (return false))

(fn DisableCollision
  (return false))

(fn EnableCollision
  (return false))

(fn GetAttached
  (return (Utilities|Array|MakeArray 0)))

(fn GetSnapLoc
  (params (CursorLoc :type Vector :default "0, 0, 0"))
  (return "0, 0, 0" "0, 0, 0"))

(fn Grabbed
  (return 0))

(fn LetGo
  (params (ParentComponent :type Actor%20Component%20Object%20Reference) (ParentActor :type Actor%20Object%20Reference))
  (return false))

(fn OnHover
  (return false))