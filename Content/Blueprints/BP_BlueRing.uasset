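; A numbered checkpoint ring in a linked chain, collected when the third-person character overlaps it while active.
; Collection activates NextRing, plays burst and poof effects, launches a BP_ZipTrail toward it and destroys this ring.
; Activation turns the ring blue and queues the following one as yellow, with DoOnce guards on each state.
; Construction styles rings by RingNumber, while a looping timer spins the inner mesh and turns the number toward the camera.
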(event Custom|Got%20It
  (bind _poof (Variables|Default|GetPoof))
  (bind _ringparticle_burst (Variables|Default|GetRingParticle_Burst))
  (Utilities|FlowControl|DoOnce false
    (:Completed
      (CallFunction|Activate (Variables|Default|GetNextRing))
      (Transformation|DetachFromComponent _ringparticle_burst "KeepWorld" "KeepWorld" "KeepWorld" true)
      (Variables|/Script/Engine.ParticleSystemComponent|SetCustomTimeDilation _ringparticle_burst 1.2)
      (Components|Activation|Activate _ringparticle_burst false)
      (Utilities|FlowControl|Sequence
        (:then_0
          (bind _alphs (Timeline|TL_Got%20IT PlayFromStart)
            (:Update
              (Transformation|SetRelativeScale3D (Variables|Default|GetStaticMesh) (Math|Vector|Lerp(Vector) "0, 0, 0" "1.000000,1.000000,1.000000" _alphs)))
            (:NewTrack_1
              (Components|Activation|Activate _poof false)
              (Rendering|SetVisibility (Variables|Default|GetTextRender) false false)
              (Utilities|FlowControl|Delay 0.5)
              (Components|Activation|Deactivate _poof)
              (Actor|DestroyActor))))
        (:then_1
          (Utilities|IsValid (Variables|Default|GetNextRing)
            (:Is%20Valid
              (bind _returnvalue (Game|SpawnActorfromClass "/Game/Effects/Particles/BP_ZipTrail.BP_ZipTrail_C" (Transformation|GetActorTransform) "Undefined" 0 0))
              (Variables|/Game/Effects/Particles/BP_ZipTrail.BP_ZipTrail_C|SetTargetActor _returnvalue (Variables|Default|GetNextRing))
              (Variables|/Game/Effects/Particles/BP_ZipTrail.BP_ZipTrail_C|SetMotherActor _returnvalue self)
              (Variables|/Game/Effects/Particles/BP_ZipTrail.BP_ZipTrail_C|SetTargetLocation _returnvalue (Transformation|GetActorLocation (Variables|Default|GetNextRing)))
              (Default|Start _returnvalue)
              (Utilities|FlowControl|Delay 0.35)
              (Components|Activation|Deactivate (Variables|Default|GetRingParticle_Burst)))))))))

(event Custom|Activate
  (Utilities|FlowControl|DoOnce false
    (:Completed
      (Components|Activation|Activate (Variables|Default|GetParticleSystem) false)
      (Rendering|SetVisibility (Variables|Default|GetStaticMesh1) true false)
      (Rendering|Material|SetMaterial (Variables|Default|GetStaticMesh) 0 "/Game/Materials/BlueRing_Mat.BlueRing_Mat")
      (CallFunction|Queue (Variables|Default|GetNextRing))
      (Variables|Default|SetActive true)
      (Utilities|FlowControl|Sequence
        (:then_0
          (bind _alpha (Timeline|TL_Activate PlayFromStart)
            (:Update
              (Transformation|SetRelativeScale3D (Variables|Default|GetStaticMesh) (Math|Vector|Lerp(Vector) "0.850000,0.850000,0.850000" "1.000000,1.000000,1.000000" _alpha)))))
        (:then_1
          (Utilities|FlowControl|Delay 0.35)
          (Components|Activation|Deactivate (Variables|Default|GetRingParticle_Burst)))))))

(event Custom|Queue
  (Utilities|FlowControl|DoOnce false
    (:Completed
      (Components|Timeline|PlayfromStart (Variables|Default|GetTL_Queue))
      (Rendering|Material|SetMaterial (Variables|Default|GetStaticMesh) 0 "/Game/Materials/YellowRing_Mat.YellowRing_Mat"))))

(event EventBeginPlay
  (Utilities|Time|SetTimerbyFunctionName self "TickFunc" 0.033333 true)
  (Collision|SetCollisionResponsetoAllChannels (Variables|Default|GetStaticMesh) "ECR_Overlap"))

(event Collision|EventActorBeginOverlap
  (params (OtherActor :type Actor%20Object%20Reference))
  (Utilities|Casting|CastToBP_ThirdPersonCharacter OtherActor)
  (if (Variables|Default|GetActive)
    (CallFunction|GotIt)))

(fn ConstructionScript
  (bind _staticmesh1 (Variables|Default|GetStaticMesh1))
  (bind _staticmesh (Variables|Default|GetStaticMesh))
  (Rendering|Components|TextRender|SetText (Variables|Default|GetTextRender) (Utilities|Text|ToText(Integer) (Variables|Default|GetRingNumber)))
  (switch int (Variables|Default|GetRingNumber)
    (:1
      (Components|Activation|SetAutoActivate (Variables|Default|GetParticleSystem) true))
    (:2
      (Rendering|Material|SetMaterial _staticmesh 0 "/Game/Materials/YellowRing_Mat.YellowRing_Mat")
      (Transformation|SetRelativeScale3D (Variables|Default|GetStaticMesh) "0.800000,0.800000,0.800000")
      (Rendering|SetVisibility (Variables|Default|GetStaticMesh1) false false))
    (:3
      (Rendering|Material|SetMaterial _staticmesh 0 "/Game/Materials/GreyRing_Mat.GreyRing_Mat" :!label _label)
      (Rendering|SetVisibility (Variables|Default|GetStaticMesh1) false false)
      (Transformation|SetRelativeScale3D (Variables|Default|GetStaticMesh) "0.700000,0.700000,0.700000"))
    (:4
      (goto _label))
    (:5
      (goto _label))
    (:6
      (goto _label))
    (:7
      (goto _label))
    (:8
      (goto _label))
    (:9
      (goto _label))
    (:10
      (goto _label))
    (:11
      (goto _label))
    (:12
      (goto _label))
    (:13
      (goto _label))
    (:14
      (goto _label))
    (:15
      (goto _label))
    (:16
      (goto _label))
    (:17
      (goto _label))
    (:18
      (goto _label))
    (:19
      (goto _label))
    (:20
      (goto _label)))
  (if (Variables|Default|GetActive)
    (Transformation|SetRelativeScale3D _staticmesh1 "0.915000,0.200000,0.915000")
    (else
      (Transformation|SetRelativeScale3D _staticmesh1 "0.920000,0.200000,0.920000"))))

(fn TickFunc
  (Transformation|SetWorldRotation (Variables|Default|GetTextRender) (Math|Rotator|FindLookatRotation (Transformation|GetActorLocation) (Camera|GetCameraLocation (Game|GetPlayerCameraManager 0))) false false)
  (Transformation|AddLocalRotation (Variables|Default|GetStaticMesh1) "0.500000, 0, 0" false false))

(fn Blink
  (bind _staticmesh (Variables|Default|GetStaticMesh))
  (if (Variables|Default|GetIsVisible)
    (Variables|Default|SetIsVisible false)
    (Rendering|SetVisibility _staticmesh false false)
    (if (Variables|Default|GetActive)
      (Rendering|SetVisibility (Variables|Default|GetStaticMesh1) false false))
    (else
      (Variables|Default|SetIsVisible true)
      (Rendering|SetVisibility _staticmesh true false)
      (if (Variables|Default|GetActive)
        (Rendering|SetVisibility (Variables|Default|GetStaticMesh1) true false)))))