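; Filing cabinet prop whose randomly open drawers are set up to slide shut when the third-person character comes near.
; The construction script randomises both spring arm lengths and the bottom drawer's slight tilt for per-instance variety.
; Sphere overlap plays or reverses the drawer timeline.
; Timeline update logic lerps the spring arms to zero and straightens the bottom drawer, using spring arm length as drawer extension.
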(event OnComponentBeginOverlap(Sphere)
  (params (OverlappedComponent :type Primitive%20Component%20Object%20Reference) (OtherActor :type Actor%20Object%20Reference) (OtherComp :type Primitive%20Component%20Object%20Reference) (OtherBodyIndex :type Integer) (bFromSweep :type Boolean) (SweepResult :type Hit%20Result%20Structure%20%28by%20ref%29))
  (Utilities|Casting|CastToBP_ThirdPersonCharacter OtherActor)
  (Audio|Components|Audio|Play (Variables|Default|GetDrawerShut_TL)))

(event OnComponentEndOverlap(Sphere)
  (params (OverlappedComponent :type Primitive%20Component%20Object%20Reference) (OtherActor :type Actor%20Object%20Reference) (OtherComp :type Primitive%20Component%20Object%20Reference) (OtherBodyIndex :type Integer))
  (Utilities|Casting|CastToBP_ThirdPersonCharacter OtherActor)
  (Utilities|String|Reverse (Variables|Default|GetDrawerShut_TL)))

(event EventBeginPlay)

(event Collision|EventActorBeginOverlap
  (params (OtherActor :type Actor%20Object%20Reference)))

(event EventTick
  (params (DeltaSeconds :type Float%20%28single-precision%29)))

(fn ConstructionScript
  (bind _output_get (Variables|Default|SetTopStartLength (Math|Random|RandomFloatinRange 0.0 45.0)))
  (Variables|/Script/Engine.SpringArmComponent|SetTargetArmLength (Variables|Default|GetTopSpring) _output_get)
  (bind _output_get_2 (Variables|Default|SetBottomStartLength (Math|Random|RandomFloatinRange 0.0 45.0)))
  (Variables|/Script/Engine.SpringArmComponent|SetTargetArmLength (Variables|Default|GetBottomSpring) _output_get_2)
  (bind _output_get_3 (Variables|Default|SetBottomStartRot (Math|Rotator|MakeRotator (Math|Random|RandomFloatinRange 0.0 1.0) (Math|Random|RandomFloatinRange -2.0 2.0) (+ (Math|Random|RandomFloatinRange -2.0 2.0) 9e+01))))
  (Transformation|SetRelativeRotation (Variables|Default|GetBottomDrawer) _output_get_3 false false))