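; BP_Popup is a popup actor that PokeEvent toggles between a small label and an expanded panel with full text.
; A timeline plays or reverses to drive the mesh's Depth, X and Y morph targets, moving the SpringArm and resizing the Box to match.
; Self-looping delays type FullText out per character, then erase it in chunks back to SmallText, using a Break flag to interrupt typing.
; Interaction functions like Grabbed are empty stubs.
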(event Custom|DaLapp
  (Utilities|FlowControl|Delay (Variables|Default|GetDelay) :!label _label)
  (Utilities|FlowControl|Sequence
    (:then_0
      (bind _output_get (Variables|Default|SetDisplayText (Utilities|String|GetSubstring (Variables|Default|GetFullText) 0 (+ (Utilities|String|Len (Variables|Default|GetDisplayText)) 1))))
      (Rendering|Components|TextRender|SetText (Variables|Default|GetTextRender) (Utilities|Text|ToText(String) _output_get)))
    (:then_1
      (if (not (Utilities|Enum|Equal(Enum) (Variables|Default|GetFullText) (Variables|Default|GetDisplayText)))
        (if (Variables|Default|GetBreak)
          (Variables|Default|SetBreak false)
          (else
            (goto _label)))))))

(event Custom|DaKnapp
  (Variables|Default|SetBreak true)
  (Utilities|FlowControl|Delay 0.01 :!label _label)
  (Utilities|FlowControl|Sequence
    (:then_0
      (bind _output_get (Variables|Default|SetDisplayText (Utilities|String|GetSubstring (Variables|Default|GetFullText) 0 (- (Utilities|String|Len (Variables|Default|GetDisplayText)) (/ (Utilities|String|Len (Variables|Default|GetFullText)) 6)))))
      (Rendering|Components|TextRender|SetText (Variables|Default|GetTextRender) (Utilities|Text|ToText(String) _output_get)))
    (:then_1
      (if (Utilities|Enum|Equal(Enum) "" (Variables|Default|GetDisplayText))
        (Variables|Default|SetBreak false)
        (Utilities|FlowControl|Delay 0.2)
        (bind _output_get_2 (Variables|Default|SetDisplayText (Variables|Default|GetSmallText)))
        (Rendering|Components|TextRender|SetText (Variables|Default|GetTextRender) (Utilities|Text|ToText(String) _output_get_2))
        (else
          (goto _label))))))

(event Collision|EventActorBeginOverlap
  (params (OtherActor :type Actor%20Object%20Reference)))

(event EventTick
  (params (DeltaSeconds :type Float%20%28single-precision%29)))

(event EventPokeEvent
  (bind _popupmesh (Variables|Default|GetPopupMesh))
  (Utilities|FlowControl|FlipFlop
    (:A
      (CallFunction|DaLapp)
      (bind _depthfloat (Timeline|Timeline_0 Play)
        (:Update
          (Components|SkeletalMesh|SetMorphTarget _popupmesh "Depth" (Math|Float|Lerp 0.0 (Variables|Default|GetDepth) _depthfloat) true)
          (Components|SkeletalMesh|SetMorphTarget _popupmesh "X" (Math|Float|Lerp 0.0 (Variables|Default|GetX) _depthfloat) true)
          (Components|SkeletalMesh|SetMorphTarget _popupmesh "Y" (Math|Float|Lerp 0.0 (Variables|Default|GetY) _depthfloat) true)
          (Transformation|SetRelativeLocation (Variables|Default|GetSpringArm) (Math|Vector|Lerp(Vector) "70.000000,25.000000,60.000000" "575.000000,25.000000,60.000000" (Math|Float|Lerp 0.0 (Variables|Default|GetX) _depthfloat)) false false)
          (Transformation|SetRelativeScale3D (Variables|Default|GetBox) (Math|Vector|MakeVector (Math|Float|Lerp 2e+02 1.2e+03 (Math|Float|Lerp 0.0 (Variables|Default|GetX) _depthfloat)) (Math|Float|Lerp 4e+01 1e+03 (Math|Float|Lerp 0.0 (Variables|Default|GetDepth) _depthfloat)) 52.0))
          (Transformation|SetRelativeLocation (Variables|Default|GetBox) (Math|Vector|Lerp(Vector) "0.000000, 0,78.000000" "0,-485.000000,78.000000" (Math|Float|Lerp 0.0 (Variables|Default|GetDepth) _depthfloat)) false false))))
    (:B
      (CallFunction|DaKnapp)
      (Timeline|Timeline_0 Reverse))))

(fn ConstructionScript
  (bind _textrender (Variables|Default|GetTextRender))
  (Rendering|Components|TextRender|SetText _textrender (Utilities|Text|ToText(String) (Variables|Default|GetSmallText)))
  (Rendering|Components|TextRender|SetWorldSize _textrender (Variables|Default|GetTextSize)))

(fn Attachto
  (params (ChildActor :type Actor%20Object%20Reference))
  (return 0))

(fn Clicked
  (return false))

(fn DisableCollision
  (return false))

(fn DoesParentHaveParent
  (return false))

(fn EnableCollision
  (return false))

(fn GetAttached
  (return 0))

(fn GetShrinkScale
  (return "0, 0, 0" "0, 0, 0"))

(fn GetSnapLoc
  (params (CursorLoc :type Vector :default "0, 0, 0"))
  (return "0, 0, 0" "0, 0, 0"))

(fn Grabbed
  (return 0))

(fn LetGo
  (params (ParentComponent :type Actor%20Component%20Object%20Reference) (ParentActor :type Actor%20Object%20Reference))
  (return false))

(fn OnHover
  (return false))

(fn PassChildAlong
  (return 0 0))