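; BP_Camera_PointFollow is a fixed-position camera actor that turns to keep the player character in view.
; Each Tick, it interpolates the Camera component's world rotation toward a look-at rotation from the actor's location to player 0.
; The resulting world yaw is clamped between MinAngle and MaxAngle, while pitch and roll are unclamped.
; The construction script applies the FOV variable to the camera.
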(event EventBeginPlay)

(event Collision|EventActorBeginOverlap
  (params (OtherActor :type Actor%20Object%20Reference)))

(event EventTick
  (params (DeltaSeconds :type Float%20%28single-precision%29))
  (bind _returnvalue (Transformation|GetActorLocation))
  (bind _returnvalue_2 (Game|GetPlayerCharacter 0))
  (bind _camera (Variables|Default|GetCamera))
  (bind _returnvalue_3 (Transformation|GetActorLocation _returnvalue_2))
  (bind _returnvalue_4 (Transformation|GetWorldRotation _camera))
  (bind _returnvalue_5 (Math|Rotator|FindLookatRotation _returnvalue _returnvalue_3))
  (bind _returnvalue_6 (Math|Interpolation|RInterpTo _returnvalue_4 _returnvalue_5 DeltaSeconds 16.0))
  (bind (_roll _pitch _yaw) (Math|Rotator|BreakRotator _returnvalue_6))
  (Transformation|SetWorldRotation (Variables|Default|GetCamera) (Math|Rotator|MakeRotator _roll _pitch (Math|Float|ClampAngle _yaw (Variables|Default|GetMin%20Angle) (Variables|Default|GetMax%20Angle))) false false))

(fn ConstructionScript
  (Camera|SetFieldOfView (Variables|Default|GetCamera) (Variables|Default|GetFOV)))