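; BP_RockFlippable is a rock that hops and tilts when poked and can release a limited number of prizes.
; A PattyFlip timeline lifts and randomly rotates the mesh, pulsing actor scale while prizes remain.
; Its Puff event fires particles and a footstep sound, then spawns a prize cast to BP_DustMote with spline following enabled and a random piano note.
; The construction script applies the configurable mesh; the other interaction functions are empty stubs.
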(event EventBeginPlay)

(event Collision|EventActorBeginOverlap
  (params (OtherActor :type Actor%20Object%20Reference)))

(event EventTick
  (params (DeltaSeconds :type Float%20%28single-precision%29)))

(event EventPokeEvent
  (bind _returnvalue (Transformation|GetActorTransform))
  (bind _startscale (Variables|Default|GetStartScale))
  (bind _defaultsceneroot (Variables|Default|GetDefaultSceneRoot))
  (bind _location (Math|Transform|BreakTransform _returnvalue))
  (bind _returnvalue_2 (Transformation|GetWorldLocation _defaultsceneroot))
  (bind (_x _y _z) (Math|Vector|BreakVector _location))
  (bind (_x_2 _y_2 _z_2) (Math|Vector|BreakVector _returnvalue_2))
  (if (not (Variables|Default|GetIsAnimating))
    (Variables|Default|SetRandomFloat (Math|Random|RandomFloatinRange -25.0 25.0))
    (bind (_direction _alpha _newtrack_3 _scalealpha) (Timeline|PattyFlip PlayFromStart)
      (:Update
        (Variables|Default|SetIsAnimating true)
        (Transformation|SetWorldLocation (Variables|Default|GetStaticMesh) (Math|Vector|Lerp(Vector) _returnvalue_2 (Math|Vector|MakeVector _x_2 _y_2 (+ _z_2 75.0)) _alpha) false false)
        (Transformation|SetRelativeRotation (Variables|Default|GetStaticMesh) (Math|Rotator|Lerp(Rotator) "0, 0, 0" (Math|Rotator|MakeRotator (Variables|Default|GetRandomFloat) (Variables|Default|GetRandomFloat) 0.0) _newtrack_3 true) false false)
        (if (not (== (Variables|Default|GetPrizeQuantity) 0))
          (Transformation|SetActorScale3D (Math|Vector|Lerp(Vector) _startscale (* _startscale 1.18) _scalealpha))))
      (:Finished
        (Variables|Default|SetIsAnimating false)
        (Components|Activation|Deactivate (Variables|Default|GetParticleSystem)))
      (:Puff
        (Components|Activation|Activate (Variables|Default|GetParticleSystem) false)
        (Audio|PlaySoundatLocation "/Game/Audio/SFX/Footstep.Footstep" (Transformation|GetActorLocation) "0, 0, 0" 0.165 (Math|Random|RandomFloatinRange 1.4 1.6) 0.0 "/Game/Audio/Attenuation/SA_Default.SA_Default" "/Game/Audio/Attenuation/SC_Default.SC_Default" 0)
        (if (not (== (Variables|Default|GetPrizeQuantity) 0))
          (Math|Integer|DecrementInt (Variables|Default|GetPrizeQuantity)
            (:%20%20
              (bind _returnvalue_3 (Game|SpawnActorfromClass (Variables|Default|GetPrize) (Math|Transform|MakeTransform (Math|Vector|MakeVector _x _y (+ _z 5e+01))) "Undefined" 0 0))
              (bind _asbp_dust_mote (Utilities|Casting|CastToBP_DustMote _returnvalue_3))
              (Variables|/Game/Blueprints/BP_DustMote.BP_DustMote_C|SetFollowSpline _asbp_dust_mote true)
              (Audio|PlaySoundatLocation (Utilities|Select :Index (Math|Random|RandomIntegerinRange 0 4) :Option%200 "/Game/Audio/SFX/PianoSFX/PianoCollect_1.PianoCollect_1" :Option%201 "/Game/Audio/SFX/PianoSFX/PianoCollect_2.PianoCollect_2" :Option%202 "/Game/Audio/SFX/PianoSFX/PianoCollect_3.PianoCollect_3" :Option%203 "/Game/Audio/SFX/PianoSFX/PianoCollect_4.PianoCollect_4" :Option%204 "/Game/Audio/SFX/PianoSFX/PianoCollect_5.PianoCollect_5") (Transformation|GetActorLocation) "0, 0, 0" 0.2 1.0 0.0 "/Game/Audio/Attenuation/SA_Default.SA_Default" "/Game/Audio/Attenuation/SC_Default.SC_Default" 0)))))
      (:ReleaseObject
        (if (not (== (Variables|Default|GetPrizeQuantity) 0))
          (Audio|PlaySoundatLocation "/Game/Audio/SFX/Jump_4.Jump_4" (Transformation|GetActorLocation) "0, 0, 0" 0.2 1.0 0.0 "/Game/Audio/Attenuation/SA_Default.SA_Default" "/Game/Audio/Attenuation/SC_Default.SC_Default" 0))))))

(fn ConstructionScript
  (Variables|Default|SetStartScale (Transformation|GetActorScale3D))
  (Components|StaticMesh|SetStaticMesh (Variables|Default|GetStaticMesh) (Variables|Default|GetMesh)))

(fn Attachto
  (params (ChildActor :type Actor%20Object%20Reference))
  (return 0))

(fn Clicked
  (return false))

(fn DisableCollision
  (return false))

(fn DoesParentHaveParent
  (return false))

(fn EnableCollision
  (return false))

(fn GetAttached
  (return 0))

(fn GetShrinkScale
  (return "0, 0, 0" "0, 0, 0"))

(fn GetSnapLoc
  (params (CursorLoc :type Vector :default "0, 0, 0"))
  (return "0, 0, 0" "0, 0, 0"))

(fn Grabbed
  (return 0))

(fn LetGo
  (params (ParentComponent :type Actor%20Component%20Object%20Reference) (ParentActor :type Actor%20Object%20Reference))
  (return false))

(fn OnHover
  (return false))

(fn PassChildAlong
  (return 0 0))