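; Collectible letter pickup for spelling P-A-N-T, with the skeletal mesh chosen from LetterEnum at construction.
; It bobs on a looping-style timeline while downward traces keep a Blob marker aligned to the ground below.
; Collect disables collision, flags the player and shows their letter panel, then chains timelines for rise, spin and scale.
; The post-collect timeline triggers the matching widget animation and finishing effects, then clears the flag and destroys the actor.
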(event EventBeginPlay
  (bind _defaultsceneroot (Variables|Default|GetDefaultSceneRoot))
  (bind _returnvalue (Transformation|GetWorldLocation _defaultsceneroot))
  (bind (_x _y _z) (Math|Vector|BreakVector _returnvalue))
  (bind (_direction _newtrack_1 _newtrack_0) (Timeline|BobbingAnimTL PlayFromStart)
    (:Update
      (Transformation|SetWorldLocation (Variables|Default|GetMeshRoot) (Math|Vector|MakeVector _x _y (+ (Math|Float|Lerp -15.0 15.0 _newtrack_1) _z)) false false))))

(event EventCollect
  (params (PlayerCharacter :type BP%20Third%20Person%20Character%20Object%20Reference))
  (bind _asbp_third_person_character (Utilities|Casting|CastToBP_ThirdPersonCharacter (Game|GetPlayerCharacter 0))
    (:then
      (Variables|/Game/ThirdPersonBP/Blueprints/BP_ThirdPersonCharacter.BP_ThirdPersonCharacter_C|SetCollectingLetter _asbp_third_person_character true)
      (Default|Show/HidePantPanel _asbp_third_person_character true))
    (:CastFailed
      _))
  (Rendering|SetVisibility (Variables|Default|GetBlob) false false)
  (Audio|PlaySound2D "/Game/Audio/SFX/ButtonCollectSFX.ButtonCollectSFX" 0.4 2.0 0.0 0 0)
  (Audio|Components|Audio|Stop (Variables|Default|GetBobbingAnimTL))
  (Collision|SetCollisionEnabled (Variables|Default|GetSphere) "NoCollision")
  (Components|Timeline|PlayfromStart (Variables|Default|GetCollectTL))
  (Utilities|FlowControl|Delay 0.3)
  (Components|Timeline|PlayfromStart (Variables|Default|GetPostCollectTL)))

(event EventTick
  (params (DeltaSeconds :type Float%20%28single-precision%29))
  (bind _returnvalue (Transformation|GetActorLocation))
  (bind (_x _y _z) (Math|Vector|BreakVector _returnvalue))
  (bind _asbp_third_person_character (Utilities|Casting|CastToBP_ThirdPersonCharacter (Game|GetPlayerCharacter 0))
    (:then
      _)
    (:CastFailed
      _))
  (bind (_outhit _returnvalue_2) (Collision|LineTraceByChannel _returnvalue (Math|Vector|MakeVector _x _y (- _z 1e+04)) "TraceTypeQuery1" false (Utilities|Array|MakeArray (Game|GetPlayerCharacter 0)) "None"))
  (if _returnvalue_2
    (Transformation|SetWorldLocationAndRotation (Variables|Default|GetBlob) (Math|Vector|MakeVector (.X (Math|Vector|BreakVector (.Location (Collision|BreakHitResult _outhit)))) (.Y (Math|Vector|BreakVector (.Location (Collision|BreakHitResult _outhit)))) (+ (.Z (Math|Vector|BreakVector (.Location (Collision|BreakHitResult _outhit)))) 5.0)) (Math|Rotator|MakeRotfromZ (.ImpactNormal (Collision|BreakHitResult _outhit))) false false)
    (else
      (Rendering|SetVisibility (Variables|Default|GetBlob) false false))))

(fn ConstructionScript
  (bind _returnvalue (Transformation|GetActorLocation))
  (bind _letter (Variables|Default|GetLetter))
  (bind (_x _y _z) (Math|Vector|BreakVector _returnvalue))
  (switch Utilities|FlowControl|Switch|SwitchonLetterEnum (Variables|Default|GetLetterEnum)
    (:NewEnumerator0
      (Class|SkinnedMeshComponent|SetSkeletalMesh _letter "/Game/Meshes/Skeletal/LetterP.LetterP" true))
    (:NewEnumerator1
      (Class|SkinnedMeshComponent|SetSkeletalMesh _letter "/Game/Meshes/Skeletal/LetterA.LetterA" true))
    (:NewEnumerator2
      (Class|SkinnedMeshComponent|SetSkeletalMesh _letter "/Game/Meshes/Skeletal/LetterN.LetterN" true))
    (:NewEnumerator3
      (Class|SkinnedMeshComponent|SetSkeletalMesh _letter "/Game/Meshes/Skeletal/LetterT.LetterT" true)))
  (bind (_outhit _returnvalue_2) (Collision|LineTraceByChannel _returnvalue (Math|Vector|MakeVector _x _y (- _z 1e+04)) "TraceTypeQuery1" false 0 "None"))
  (if _returnvalue_2
    (Transformation|SetWorldLocationAndRotation (Variables|Default|GetBlob) (.Location (Collision|BreakHitResult _outhit)) (Math|Rotator|MakeRotfromZ (.ImpactNormal (Collision|BreakHitResult _outhit))) false false)))