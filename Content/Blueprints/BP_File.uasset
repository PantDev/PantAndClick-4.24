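; Collectible file pickup with a random paper icon that bobs, flickers and pulses, and can follow a spawned scatter spline.
; A downward trace repeats every 0.1 seconds to keep a blob shadow on the ground.
; Collect chains timelines that lift the icon and fly it to the player, then increments FileCount, pops the folder widget and destroys the actor.
; Random piano notes, dust and rumble accompany collection, the second note placed at the deprojected HUD folder.
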(event Custom|UpdateShadow
  (bind _returnvalue (Game|GetPlayerCharacter 0))
  (bind _returnvalue_2 (Transformation|GetActorLocation))
  (bind _blob (Variables|Default|GetBlob))
  (bind (_x _y _z) (Math|Vector|BreakVector _returnvalue_2))
  (bind _asbp_third_person_character (Utilities|Casting|CastToBP_ThirdPersonCharacter _returnvalue))
  (Utilities|Array|AppendArray (Variables|/Game/ThirdPersonBP/Blueprints/BP_ThirdPersonCharacter.BP_ThirdPersonCharacter_C|GetIgnoreArray _asbp_third_person_character) (Utilities|Array|MakeArray _returnvalue))
  (bind (_outhit _returnvalue_3) (Collision|LineTraceByChannel _returnvalue_2 (Math|Vector|MakeVector _x _y (- _z 1e+04)) "TraceTypeQuery1" false (Variables|/Game/ThirdPersonBP/Blueprints/BP_ThirdPersonCharacter.BP_ThirdPersonCharacter_C|GetIgnoreArray _asbp_third_person_character) "None"))
  (if _returnvalue_3
    (Transformation|SetWorldLocationAndRotation _blob (Math|Vector|MakeVector (.X (Math|Vector|BreakVector (.Location (Collision|BreakHitResult _outhit)))) (.Y (Math|Vector|BreakVector (.Location (Collision|BreakHitResult _outhit)))) (+ (.Z (Math|Vector|BreakVector (.Location (Collision|BreakHitResult _outhit)))) 5.0)) (Math|Rotator|MakeRotfromZ (.ImpactNormal (Collision|BreakHitResult _outhit))) false false)
    (Utilities|FlowControl|Sequence
      (:then_0
        (Utilities|FlowControl|DoOnce false
          (:Completed
            (Rendering|SetVisibility _blob true false))))
      (:then_1
        (Utilities|FlowControl|Delay 0.1)
        (CallFunction|UpdateShadow)))))

(event EventBeginPlay
  (bind _returnvalue (Transformation|GetActorTransform))
  (bind _materialbillboard (Variables|Default|GetMaterialBillboard))
  (bind (_location _rotation _scale) (Math|Transform|BreakTransform _returnvalue))
  (bind (_roll _pitch _yaw) (Math|Rotator|BreakRotator _rotation))
  (Variables|Default|SetStartLoc (Transformation|GetActorLocation))
  (Utilities|FlowControl|Delay 0.01)
  (switch int (Math|Random|RandomIntegerinRange 0 2)
    (:0
      (Rendering|Material|SetMaterial _materialbillboard 0 "/Game/Materials/IconAudioPaper_Mat.IconAudioPaper_Mat"))
    (:1
      (Rendering|Material|SetMaterial _materialbillboard 0 "/Game/Materials/IconBlankPaper_Mat.IconBlankPaper_Mat"))
    (:2
      (Rendering|Material|SetMaterial _materialbillboard 0 "/Game/Materials/IconNotepadPaper_Mat.IconNotepadPaper_Mat")))
  (Utilities|FlowControl|Delay 0.5)
  (Variables|/Script/Engine.PrimitiveComponent|SetbGenerateOverlapEvents (Variables|Default|GetSphere) true)
  (Components|Timeline|SetNewTime (Variables|Default|GetBobbin) (Math|Random|RandomFloatinRange 0.0 5.0))
  (Components|Timeline|SetNewTime (Variables|Default|GetFlicker_TL) (Math|Random|RandomFloatinRange 0.0 0.45))
  (Audio|Components|Audio|Play (Variables|Default|GetBobbin))
  (CallFunction|UpdateShadow)
  (if (Variables|Default|GetFollowSpline)
    (bind _returnvalue_2 (Game|SpawnActorfromClass "/Game/Blueprints/BP_ScatterSpline.BP_ScatterSpline_C" (Math|Transform|MakeTransform _location (Math|Rotator|MakeRotator _roll _pitch (+ _yaw (Math|Random|RandomFloatinRange 0.0 3.6e+02))) _scale) "Undefined" 0 0))
    (bind _output_get (Variables|/Game/Blueprints/BP_ScatterSpline.BP_ScatterSpline_C|SetSplineFollowActor _returnvalue_2 self))
    (Default|MoveAlongSpline _returnvalue_2 _output_get)))

(event EventCollect
  (params (PlayerCharacter :type BP%20Third%20Person%20Character%20Object%20Reference))
  (Utilities|FlowControl|Delay 0.05)
  (Audio|Components|Audio|Stop (Variables|Default|GetTL_SpawnFromFolder))
  (bind _output_get (Variables|Default|SetPlayerCharacter PlayerCharacter))
  (Effects|Components|ParticleSystem|SetTemplate (Variables|Default|GetP_Particle) "/Game/Effects/Particles/P_Dust1.P_Dust1")
  (bind _asbp_third_person_character (Utilities|Casting|CastToBP_ThirdPersonCharacter (Game|GetPlayerCharacter 0)))
  (Default|DustWait _asbp_third_person_character)
  (if (Variables|/Game/ThirdPersonBP/Blueprints/BP_ThirdPersonCharacter.BP_ThirdPersonCharacter_C|GetFileFolderHidden _asbp_third_person_character)
    (Default|Show/HideFilePanel _asbp_third_person_character true))
  (Default|Attachto _output_get self)
  (Game|Feedback|ClientPlayForceFeedback (Game|GetPlayerController 0) "/Game/Effects/RumbleTest1.RumbleTest1" "Collect" false false false)
  (Rendering|SetVisibility (Variables|Default|GetBlob) false false)
  (switch int (Math|Random|RandomIntegerinRange 0 4)
    (:Default
      _)
    (:0
      _)
    (:1
      (goto _label 2))
    (:2
      (goto _label 3))
    (:3
      (goto _label 4))
    (:4
      (goto _label 5)))
  (Utilities|SoundPicker (Transformation|GetWorldLocation (Variables|Default|GetDefaultSceneRoot)) (Variables|Default|GetVolume) :!label _label)
  (Audio|Components|Audio|Stop (Variables|Default|GetBobbin))
  (Utilities|FlowControl|DoOnce false
    (:Completed
      (Transformation|DetachFromComponent (Variables|Default|GetMaterialBillboard1) "KeepWorld" "KeepWorld" "KeepWorld" true)
      (Audio|Components|Audio|Stop (Variables|Default|GetTL_SpawnFromFolder))
      (Components|Timeline|PlayfromStart (Variables|Default|GetCollect_TL))
      (Rendering|SetVisibility (Variables|Default|GetBlob) false false))))

(fn ConstructionScript
  (bind _returnvalue (Transformation|GetActorLocation))
  (bind _materialbillboard (Variables|Default|GetMaterialBillboard))
  (bind (_x _y _z) (Math|Vector|BreakVector _returnvalue))
  (switch int (Variables|Default|GetFileType)
    (:0
      (Rendering|Material|SetMaterial _materialbillboard 0 "/Game/Materials/IconAudioPaper_Mat.IconAudioPaper_Mat"))
    (:1
      (Rendering|Material|SetMaterial _materialbillboard 0 "/Game/Materials/IconBlankPaper_Mat.IconBlankPaper_Mat"))
    (:2
      (Rendering|Material|SetMaterial _materialbillboard 0 "/Game/Materials/IconNotepadPaper_Mat.IconNotepadPaper_Mat")))
  (bind _returnvalue_2 (Rendering|Material|CreateDynamicMaterialInstance "/Game/Materials/DustMote_Glow_Mat.DustMote_Glow_Mat" "None" :!class /Script/Engine.KismetMaterialLibrary))
  (bind _output_get (Variables|Default|SetGlowMat _returnvalue_2))
  (Rendering|Material|SetMaterial (Variables|Default|GetMaterialBillboard1) 0 _output_get)
  (bind (_outhit _returnvalue_3) (Collision|LineTraceByChannel _returnvalue (Math|Vector|MakeVector _x _y (- _z 1e+04)) "TraceTypeQuery1" false 0 "None"))
  (if _returnvalue_3
    (Transformation|SetWorldLocationAndRotation (Variables|Default|GetBlob) (Math|Vector|MakeVector (.X (Math|Vector|BreakVector (.Location (Collision|BreakHitResult _outhit)))) (.Y (Math|Vector|BreakVector (.Location (Collision|BreakHitResult _outhit)))) (+ (.Z (Math|Vector|BreakVector (.Location (Collision|BreakHitResult _outhit)))) 0.01)) (Math|Rotator|MakeRotfromZ (.ImpactNormal (Collision|BreakHitResult _outhit))) false false)))