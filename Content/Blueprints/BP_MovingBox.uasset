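; BP_MovingBox is a box that captures the third-person character on overlap, with a helper for a launch-style velocity.
; If available, its sphere overlap registers the box on the character, stops and centers them in flying mode, then hides their mesh.
; It plays a closing animation, starts a scale timeline and briefly fires particles.
; GetVelocityBox returns velocity toward the Arrow with added lift, but nothing here calls it.
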(event OnComponentBeginOverlap(Sphere)
  (params (OverlappedComponent :type Primitive%20Component%20Object%20Reference) (OtherActor :type Actor%20Object%20Reference) (OtherComp :type Primitive%20Component%20Object%20Reference) (OtherBodyIndex :type Integer) (bFromSweep :type Boolean) (SweepResult :type Hit%20Result%20Structure%20%28by%20ref%29))
  (if (Variables|Default|GetAvailable)
    (bind _asbp_third_person_character (Utilities|Casting|CastToBP_ThirdPersonCharacter OtherActor))
    (if (not (Variables|/Game/ThirdPersonBP/Blueprints/BP_ThirdPersonCharacter.BP_ThirdPersonCharacter_C|GetInBox _asbp_third_person_character))
      (Variables|/Game/ThirdPersonBP/Blueprints/BP_ThirdPersonCharacter.BP_ThirdPersonCharacter_C|SetInBox _asbp_third_person_character true)
      (Variables|/Game/ThirdPersonBP/Blueprints/BP_ThirdPersonCharacter.BP_ThirdPersonCharacter_C|SetActiveMovingBox _asbp_third_person_character self)
      (Pawn|Components|CharacterMovement|SetMovementMode (Variables|/Script/Engine.Character|GetCharacterMovement _asbp_third_person_character) "MOVE_Flying" 0)
      (Variables|/Script/Engine.MovementComponent|SetVelocity (Pawn|GetMovementComponent _asbp_third_person_character) "0, 0, 0")
      (Transformation|SetActorLocation _asbp_third_person_character (Transformation|GetActorLocation) false false)
      (Components|Animation|SetAnimation (Variables|/Game/ThirdPersonBP/Blueprints/BP_ThirdPersonCharacter.BP_ThirdPersonCharacter_C|GetDenimMesh _asbp_third_person_character) "/Game/Meshes/Denim/NewFolder/Denim_Anim_Armature_Roll.Denim_Anim_Armature_Roll")
      (Components|Timeline|SetPlayRate (Variables|/Game/ThirdPersonBP/Blueprints/BP_ThirdPersonCharacter.BP_ThirdPersonCharacter_C|GetDenimMesh _asbp_third_person_character) 0.0)
      (Components|Animation|PlayAnimation (Variables|Default|GetSkeletalMesh) "/Game/Meshes/Skeletal/MovingBox/MovingBox_Skeletal_Anim_Armature_CloseBox.MovingBox_Skeletal_Anim_Armature_CloseBox" false)
      (Rendering|SetVisibility (Variables|/Game/ThirdPersonBP/Blueprints/BP_ThirdPersonCharacter.BP_ThirdPersonCharacter_C|GetDenimMesh _asbp_third_person_character) false false)
      (Components|Activation|Activate (Variables|Default|GetParticleSystem) false)
      (Components|Timeline|PlayfromStart (Variables|Default|GetTL_ScaleAnim))
      (Utilities|FlowControl|Delay 0.2)
      (Components|Activation|Deactivate (Variables|Default|GetParticleSystem)))))

(event EventBeginPlay)

(event Collision|EventActorBeginOverlap
  (params (OtherActor :type Actor%20Object%20Reference)))

(event EventTick
  (params (DeltaSeconds :type Float%20%28single-precision%29)))

(fn ConstructionScript)

(fn GetVelocityBox
  (bind _returnvalue (Transformation|GetActorLocation))
  (bind _arrow (Variables|Default|GetArrow))
  (bind _returnvalue_2 (Transformation|GetWorldLocation _arrow))
  (bind _returnvalue_3 (Math|Vector|GetUnitDirection(Vector) _returnvalue _returnvalue_2))
  (bind _returnvalue_4 (* _returnvalue_3 3.4e+03))
  (bind (_x _y _z) (Math|Vector|BreakVector _returnvalue_4))
  (return (Math|Vector|MakeVector _x _y (+ _z 3e+02))))