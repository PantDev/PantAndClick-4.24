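; BP_LevelInfo is a map object that tallies the level's file count in its FileCount variable.
; Its construction script adds BurstQuantity times Bursts for every BP_Folder_Icon in the level, then one for each placed BP_File.
; The count is computed at construction, and the event graph holds no active logic.
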(event EventBeginPlay)

(event Collision|EventActorBeginOverlap
  (params (OtherActor :type Actor%20Object%20Reference)))

(event EventTick
  (params (DeltaSeconds :type Float%20%28single-precision%29)))

(fn ConstructionScript
  (bind _outactors (Actor|GetAllActorsOfClass "/Game/Blueprints/GameObjects/BP_Folder_Icon.BP_Folder_Icon_C"))
  (for _array_element _outactors
    (Variables|Default|SetFileCount (+ (* (Variables|/Game/Blueprints/GameObjects/BP_Icon.BP_Icon_C|GetBurstQuantity _array_element) (Variables|/Game/Blueprints/GameObjects/BP_Icon.BP_Icon_C|GetBursts _array_element)) (Variables|Default|GetFileCount))))
  (bind _outactors_2 (Actor|GetAllActorsOfClass "/Game/Blueprints/GameObjects/BP_File.BP_File_C"))
  (for _array_element_2 _outactors_2
    (Variables|Default|SetFileCount (+ (Variables|Default|GetFileCount) 1))))