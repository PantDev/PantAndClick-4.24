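; BP_PopupPortal is a portal actor that keeps its Cube's material informed of the portal's position and facing.
; BeginPlay puts a dynamic instance of CylinderIntersectionTest_Mat on the Cube and starts a looping timer at about 30 Hz.
; Each setpos call writes the Cube's world location and the actor's forward vector into material parameters, so no Tick is used.
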(event EventBeginPlay
  (bind _returnvalue (Rendering|Material|CreateDynamicMaterialInstance "/Game/Materials/CylinderIntersectionTest_Mat.CylinderIntersectionTest_Mat" "None" :!class /Script/Engine.KismetMaterialLibrary))
  (Rendering|Material|SetMaterial (Variables|Default|GetCube) 0 _returnvalue)
  (Utilities|Time|SetTimerbyFunctionName 0 "setpos" 0.033333 true))

(event Collision|EventActorBeginOverlap
  (params (OtherActor :type Actor%20Object%20Reference)))

(event EventTick
  (params (DeltaSeconds :type Float%20%28single-precision%29)))

(fn ConstructionScript)

(fn Setpos
  (bind _cube (Variables|Default|GetCube))
  (Rendering|Material|SetVectorParameterValueonMaterials _cube "PortalCenterPos" (Transformation|GetWorldLocation (Variables|Default|GetCube)))
  (Rendering|Material|SetVectorParameterValueonMaterials _cube "PortalForwardDir" (Math|Vector|GetForwardVector (Transformation|GetActorRotation))))