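; Collectible coin that increments and enlarges the ThirdPersonCharacter's ScoreText on overlap, then destroys itself after an audio announcement.
; The announcer speaks the new score as two digit sounds, followed by a random noun.
; A timeline bobs and rotates the mesh, Tick hides it at distance, and a downward trace places its blob shadow.
; Construction-script options use traces to center it on the object below or set its height above ground.
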(event Custom|BobUpDown
  (bind _staticmesh (Variables|Default|GetStaticMesh))
  (bind _newtrack_0 (Timeline|UpDownTimeline PlayFromStart)
    (:Update
      (Transformation|SetRelativeLocation _staticmesh (Math|Vector|MakeVector 0.0 0.0 _newtrack_0) false false)
      (Transformation|SetRelativeRotation _staticmesh (Math|Rotator|MakeRotator _newtrack_0 _newtrack_0 _newtrack_0) false false))))

(event EventBeginPlay
  (bind _staticmesh (Variables|Default|GetStaticMesh))
  (bind _returnvalue (Transformation|GetWorldLocation _staticmesh))
  (bind (_x _y _z) (Math|Vector|BreakVector _returnvalue))
  (bind _outactors (Actor|GetAllActorsOfClass "BP_OldCoin_C"))
  (bind _outhit (Collision|LineTraceByChannel _returnvalue (Math|Vector|MakeVector _x _y (- _z 1e+04)) "TraceTypeQuery1" false _outactors "None"))
  (Transformation|SetWorldLocation (Variables|Default|GetBlobShadow) (.ImpactPoint (Collision|BreakHitResult _outhit)) false false)
  (CallFunction|BobUpDown))

(event Collision|EventActorBeginOverlap
  (params (OtherActor :type Actor%20Object%20Reference))
  (bind _asthird_person_character (Utilities|Casting|CastToThirdPersonCharacter OtherActor))
  (Rendering|Components|TextRender|SetText (Variables|/Game/ThirdPersonBP/Blueprints/ThirdPersonCharacter.ThirdPersonCharacter_C|GetScoreText _asthird_person_character) (Utilities|Text|ToText(Float) (+ (Math|Conversions|ToFloat(Integer) (Utilities|String|ToString(Text) (Variables|/Script/Engine.TextRenderComponent|GetText (Variables|/Game/ThirdPersonBP/Blueprints/ThirdPersonCharacter.ThirdPersonCharacter_C|GetScoreText _asthird_person_character)))) 1.0) "HalfToEven" true 2))
  (Transformation|SetWorldScale3D (Variables|/Game/ThirdPersonBP/Blueprints/ThirdPersonCharacter.ThirdPersonCharacter_C|GetScoreText _asthird_person_character) (* (Transformation|GetWorldScale (Variables|/Game/ThirdPersonBP/Blueprints/ThirdPersonCharacter.ThirdPersonCharacter_C|GetScoreText _asthird_person_character)) 1.03))
  (Audio|PlaySoundatLocation "/Game/StarterContent/Audio/blip.blip" "0, 0, 0" "0, 0, 0" 3.0 0.2 0.03)
  (Components|DestroyComponent (Variables|Default|GetStaticMesh))
  (Collision|SetCollisionEnabled (Variables|Default|GetStaticMesh) "NoCollision")
  (bind (_digit_1 _digit_2) (CallFunction|GetAnnouncerNumber (+ (Math|Conversions|ToFloat(Integer) (Utilities|String|ToString(Text) (Variables|/Script/Engine.TextRenderComponent|GetText (Variables|/Game/ThirdPersonBP/Blueprints/ThirdPersonCharacter.ThirdPersonCharacter_C|GetScoreText _asthird_person_character)))) 1.0)))
  (Utilities|FlowControl|Delay 1.6)
  (Audio|PlaySoundatLocation _digit_1 "0, 0, 0" "0,0.000000, 0" 2.0 0.8)
  (Utilities|FlowControl|Delay 1.0)
  (Audio|PlaySoundatLocation _digit_2 "0, 0, 0" "0, 0, 0" 2.0 0.8)
  (Utilities|FlowControl|Delay 1.0)
  (Audio|PlaySoundatLocation (Utilities|Array|Get(acopy) (Utilities|Array|MakeArray "/Game/Audio/OldAnnouncer/ohs.ohs" "/Game/Audio/OldAnnouncer/glyphs.glyphs" "/Game/Audio/OldAnnouncer/rings.rings" "/Game/Audio/OldAnnouncer/shinybits.shinybits" "/Game/Audio/OldAnnouncer/shapes.shapes" "/Game/Audio/OldAnnouncer/obloids.obloids") (Math|Random|RandomIntegerinRange 0 5)) "0, 0, 0" "0, 0, 0" 3.0 1.0)
  (Actor|DestroyActor))

(event EventTick
  (params (DeltaSeconds :type Float%20%28single-precision%29))
  (bind _staticmesh (Variables|Default|GetStaticMesh))
  (if (> (Math|Vector|VectorLength (- (Transformation|GetActorLocation (Game|GetPlayerCharacter 0)) (Transformation|GetActorLocation))) 4e+03)
    (Rendering|SetVisibility _staticmesh false false)
    (else
      (Rendering|SetVisibility _staticmesh true false))))

(fn ConstructionScript
  (bind _staticmesh (Variables|Default|GetStaticMesh))
  (bind _staticmesh_2 (Variables|Default|GetStaticMesh))
  (bind _staticmesh_3 (Variables|Default|GetStaticMesh))
  (bind _returnvalue (Transformation|GetWorldLocation _staticmesh))
  (bind _returnvalue_2 (Transformation|GetWorldLocation _staticmesh_2))
  (bind _returnvalue_3 (Transformation|GetWorldLocation _staticmesh_3))
  (bind (_x _y _z) (Math|Vector|BreakVector _returnvalue))
  (bind (_x_2 _y_2) (Math|Vector|BreakVector _returnvalue_2))
  (bind (_x_3 _y_3 _z_2) (Math|Vector|BreakVector _returnvalue_3))
  (if (Variables|Default|GetCenterOnObject)
    (bind _outactors (Actor|GetAllActorsOfClass "BP_OldCoin_C"))
    (bind _outhit (Collision|LineTraceByChannel _returnvalue_3 (Math|Vector|MakeVector _x_3 _y_3 (- _z_2 1e+04)) "TraceTypeQuery1" false _outactors "None"))
    (Transformation|SetWorldLocation (Variables|Default|GetDefaultSceneRoot self) (Math|Vector|MakeVector (.X (Math|Vector|BreakVector (Transformation|GetWorldLocation (.HitComponent (Collision|BreakHitResult _outhit))))) (.Y (Math|Vector|BreakVector (Transformation|GetWorldLocation (.HitComponent (Collision|BreakHitResult _outhit))))) (.Z (Math|Vector|BreakVector (Transformation|GetWorldLocation (Variables|Default|GetStaticMesh))))) false false))
  (if (Variables|Default|GetAutoPlant)
    (bind _outactors_2 (Actor|GetAllActorsOfClass "BP_OldCoin_C"))
    (bind _outhit_2 (Collision|LineTraceByChannel _returnvalue (Math|Vector|MakeVector _x _y (- _z 1e+04)) "TraceTypeQuery1" false _outactors_2 "None"))
    (Transformation|SetWorldLocation (Variables|Default|GetDefaultSceneRoot self) (Math|Vector|MakeVector _x_2 _y_2 (+ (.Z (Math|Vector|BreakVector (.ImpactPoint (Collision|BreakHitResult _outhit_2)))) 2e+02)) false false)))

(fn GetAnnouncerNumber
  (params (NewParam :type Float%20%28single-precision%29))
  (bind _returnvalue (- NewParam 1.0))
  (bind _array (Utilities|Array|MakeArray "/Game/Audio/OldAnnouncer/0.0" "/Game/Audio/OldAnnouncer/1.1" "/Game/Audio/OldAnnouncer/2.2" "/Game/Audio/OldAnnouncer/3.3" "/Game/Audio/OldAnnouncer/4.4" "/Game/Audio/OldAnnouncer/5.5" "/Game/Audio/OldAnnouncer/6.6" "/Game/Audio/OldAnnouncer/7.7" "/Game/Audio/OldAnnouncer/8.8" "/Game/Audio/OldAnnouncer/9.9"))
  (bind _returnvalue_2 (Utilities|Text|ToText(Float) _returnvalue "HalfToEven" true 2 2))
  (bind _returnvalue_3 (Utilities|String|ToString(Text) _returnvalue_2))
  (bind _returnvalue_4 (Utilities|String|GetCharacterArrayfromString _returnvalue_3))
  (Audio|PlaySoundatLocation "/Game/Audio/OldAnnouncer/youhavecollected.youhavecollected" "0, 0, 0")
  (Development|PrintString _returnvalue_3)
  (return (Utilities|Array|Get(acopy) _array (Math|Conversions|ToInteger(Byte) (Utilities|Array|Get(acopy) _returnvalue_4))) (Utilities|Array|Get(acopy) _array (Math|Conversions|ToInteger(Byte) (Utilities|Array|Get(acopy) _returnvalue_4 1)))))