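; Title screen controller that shows a "press any" prompt and hands off to a desktop portal when the player responds.
; After a timed delay on BeginPlay it creates the prompt widget, plays its fade-in and looping pulse animations, then opens an input gate.
; Start/Pause, Kick, Jump or the Pause key then reverse the Visible animation and call RemoteEnter on DesktopPortal, guarded by DoOnce to fire only once.
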(event EventBeginPlay
  (Utilities|FlowControl|Delay 6.2)
  (bind _returnvalue (UserInterface|CreateWidget "/Game/UserInterface/Images/Tutorial/PressAny_Widget.PressAny_Widget_C"))
  (UserInterface|Viewport|AddtoPlayerScreen _returnvalue)
  (Variables|Default|SetTitle_Widget _returnvalue)
  (UserInterface|Animation|PlayAnimation _returnvalue (Variables|/Game/UserInterface/Images/Tutorial/PressAny_Widget.PressAny_Widget_C|GetVisible _returnvalue) 0.0 1 "Forward" 1.0 false)
  (Utilities|FlowControl|Delay 0.12)
  (UserInterface|Animation|PlayAnimation _returnvalue (Variables|/Game/UserInterface/Images/Tutorial/PressAny_Widget.PressAny_Widget_C|GetPulse _returnvalue) 0.0 0 "Forward" 1.0 false)
  (Variables|Default|SetReady true))

(event Collision|EventActorBeginOverlap
  (params (OtherActor :type Actor%20Object%20Reference)))

(event EventTick
  (params (DeltaSeconds :type Float%20%28single-precision%29)))

(event Input|ActionEvents|InputActionKick
  (params (Key :type Key%20Structure :default "None"))
  (bind _title_widget (Variables|Default|GetTitle_Widget))
  (:Pressed
    (if (Variables|Default|GetReady)
      (Utilities|FlowControl|DoOnce false
        (:Completed
          (Class|UserWidget|PlayAnimationReverse _title_widget (Variables|/Game/UserInterface/Images/Tutorial/PressAny_Widget.PressAny_Widget_C|GetVisible _title_widget) 1.0 false)
          (Default|RemoteEnter (Variables|Default|GetDesktopPortal)))))))

(event Input|ActionEvents|InputActionStart/Pause
  (params (Key :type Key%20Structure :default "None"))
  (bind _title_widget (Variables|Default|GetTitle_Widget))
  (:Pressed
    (if (Variables|Default|GetReady)
      (Utilities|FlowControl|DoOnce false
        (:Completed
          (Class|UserWidget|PlayAnimationReverse _title_widget (Variables|/Game/UserInterface/Images/Tutorial/PressAny_Widget.PressAny_Widget_C|GetVisible _title_widget) 1.0 false)
          (Default|RemoteEnter (Variables|Default|GetDesktopPortal)))))))

(event Input|ActionEvents|InputActionJump
  (params (Key :type Key%20Structure :default "None"))
  (bind _title_widget (Variables|Default|GetTitle_Widget))
  (:Pressed
    (if (Variables|Default|GetReady)
      (Utilities|FlowControl|DoOnce false
        (:Completed
          (Class|UserWidget|PlayAnimationReverse _title_widget (Variables|/Game/UserInterface/Images/Tutorial/PressAny_Widget.PressAny_Widget_C|GetVisible _title_widget) 1.0 false)
          (Default|RemoteEnter (Variables|Default|GetDesktopPortal)))))))

(event Input|GamepadEvents|GamepadDPadLeft
  (params (Key :type Key%20Structure :default "None")))

(event Input|GamepadEvents|GamepadDPadUp
  (params (Key :type Key%20Structure :default "None")))

(event Input|GamepadEvents|GamepadDPadRight
  (params (Key :type Key%20Structure :default "None")))

(event Input|GamepadEvents|GamepadDPadDown
  (params (Key :type Key%20Structure :default "None")))

(event Input|KeyboardEvents|Pause
  (params (Key :type Key%20Structure :default "None"))
  (bind _title_widget (Variables|Default|GetTitle_Widget))
  (:Pressed
    (if (Variables|Default|GetReady)
      (Utilities|FlowControl|DoOnce false
        (:Completed
          (Class|UserWidget|PlayAnimationReverse _title_widget (Variables|/Game/UserInterface/Images/Tutorial/PressAny_Widget.PressAny_Widget_C|GetVisible _title_widget) 1.0 false)
          (Default|RemoteEnter (Variables|Default|GetDesktopPortal)))))))

(fn ConstructionScript)