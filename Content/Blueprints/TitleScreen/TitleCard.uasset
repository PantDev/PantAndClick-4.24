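; Title screen actor that stages the animated main menu intro, driving a referenced camera and the title mesh with timelines and sounds.
; The construction script caches camera and title transforms; on BeginPlay, the start timeline widens FOV and eases camera rotation into place.
; Its event track plays the title animation, followed by a delayed sound, idle loop and squash-and-spin bounce.
; When the start timeline finishes, a hover timeline drifts the camera and sways the title.
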(event EventBeginPlay
  (bind _mainmenu_title (Variables|Default|GetMainMenu_Title))
  (bind _camtargetrot (Variables|Default|GetCamTargetRot))
  (bind _startrot (Variables|Default|GetStartrot))
  (bind _startrot_2 (Variables|Default|GetStartrot))
  (bind _camtargetrot_2 (Variables|Default|GetCamTargetRot))
  (bind _camtargetloc (Variables|Default|GetCamTargetLoc))
  (bind _camera (Variables|Default|GetCamera))
  (bind (_x _y _z) (Math|Vector|BreakVector _camtargetloc))
  (bind (_roll _pitch _yaw) (Math|Rotator|BreakRotator _camtargetrot))
  (bind (_roll_2 _pitch_2 _yaw_2) (Math|Rotator|BreakRotator _startrot))
  (bind (_roll_3 _pitch_3 _yaw_3) (Math|Rotator|BreakRotator _startrot_2))
  (bind (_roll_4 _pitch_4 _yaw_4) (Math|Rotator|BreakRotator _camtargetrot_2))
  (bind _cameracomponent (Variables|/Script/Engine.CameraActor|GetCameraComponent _camera))
  (Audio|PlaySound2D "/Game/Audio/SFX/Hum.Hum" 1.0 1.0 0.0 0 0)
  (bind (_direction _rotalpha _newtrack_0) (Timeline|TL_StartAnim PlayFromStart)
    (:Update
      (Camera|SetFieldOfView (Variables|/Script/Engine.CameraActor|GetCameraComponent (Variables|Default|GetCamera)) (Math|Float|Lerp 2e+01 4e+01 _newtrack_0))
      (Transformation|SetActorRotation (Variables|Default|GetCamera) (Math|Rotator|Lerp(Rotator) (Math|Rotator|MakeRotator (- _roll_4 -1e+01) (- _pitch_4 15.0) _yaw_4) _camtargetrot_2 _rotalpha)))
    (:Finished
      (bind _newtrack_0_2 (Timeline|TL_Hover PlayFromStart)
        (:Update
          (Transformation|SetWorldLocation _cameracomponent (Math|Vector|Lerp(Vector) _camtargetloc (Math|Vector|MakeVector (- _x 8.0) _y (+ _z 12.0)) _newtrack_0_2) false false)
          (if (not (Audio|Components|Audio|IsPlaying (Variables|Default|GetTL_StartAnim)))
            (Transformation|SetWorldRotation _cameracomponent (Math|Rotator|Lerp(Rotator) _camtargetrot (Math|Rotator|MakeRotator (+ _roll 1.2) (+ _pitch -0.8) _yaw) _newtrack_0_2 true) false false)
            (Transformation|SetWorldRotation (Variables|Default|GetMainMenu_Title) (Math|Rotator|Lerp(Rotator) _startrot (Math|Rotator|MakeRotator _roll_2 _pitch_2 (+ _yaw_2 28.0)) _newtrack_0_2) false false)))))
    (:NewTrack_1
      (Components|Animation|PlayAnimation (Variables|Default|GetMainMenu_Title) "/Game/Meshes/MainMenu/MainMenu_Title_Anim.MainMenu_Title_Anim" false)
      (Utilities|FlowControl|Sequence
        (:then_0
          (Utilities|FlowControl|Delay 0.95)
          (Audio|PlaySound2D "/Game/Audio/SFX/TitleTemp.TitleTemp" 1.0 1.0 0.0 0 0))
        (:then_1
          (Utilities|FlowControl|Delay 1.1)
          (Components|Animation|PlayAnimation _mainmenu_title "/Game/Meshes/MainMenu/MainMenu_Title_Idle_Anim_Armature_ArmatureAction_001.MainMenu_Title_Idle_Anim_Armature_ArmatureAction_001" true)
          (Components|Animation|SetPosition _mainmenu_title 0.0 true)
          (bind (_direction_2 _newtrack_1 _newtrack_2 _rotalpha_2) (Timeline|TL_Bounce PlayFromStart)
            (:Update
              (Transformation|SetWorldScale3D (Variables|Default|GetMainMenu_Title) (Math|Vector|Lerp(Vector) "35.000000,60.000000,70.000000" "50.000000,50.000000,50.000000" _newtrack_1))
              (Transformation|SetWorldRotation (Variables|Default|GetMainMenu_Title) (Math|Rotator|Lerp(Rotator) _startrot_2 (Math|Rotator|MakeRotator _roll_3 (+ _pitch_3 -3.6e+02) _yaw_3) _rotalpha_2) false false))))))))

(event Collision|EventActorBeginOverlap
  (params (OtherActor :type Actor%20Object%20Reference)))

(event EventTick
  (params (DeltaSeconds :type Float%20%28single-precision%29)))

(fn ConstructionScript
  (bind _camera (Variables|Default|GetCamera))
  (Variables|Default|SetCamTargetRot (Transformation|GetActorRotation _camera))
  (Variables|Default|SetCamTargetLoc (Transformation|GetActorLocation _camera))
  (Variables|Default|SetStartrot (Transformation|GetWorldRotation (Variables|Default|GetMainMenu_Title))))