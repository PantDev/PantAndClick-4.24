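; BP_LightSwitch is a placeable wall light switch that flips its switch piece 180 degrees with a sound when poked.
; Interface-style functions handle click collision, hover custom-depth highlighting, yaw offsets and snap transforms from box and mesh; several are stubs.
; Letting go re-enables box collision, plays a randomly pitched pop and runs a timeline scale animation.
; ActorBeginCursorOver destroys the actor, and no light is controlled here.
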(event Custom|LetGoEvent
  (Audio|PlaySoundatLocation "/Game/Audio/SFX/Pop.Pop" (Transformation|GetActorLocation) "0, 0, 0" 1.0 (Math|Random|RandomFloatinRange 0.7 1.1) 0.0 "/Game/Audio/Attenuation/SA_Default.SA_Default" "/Game/Audio/Attenuation/SC_Default.SC_Default" 0)
  (Variables|Default|SetScaleDest (Transformation|GetWorldScale (Variables|Default|GetStaticMesh)))
  (bind _alpha (Timeline|SpawnAnim PlayFromStart)
    (:Update
      (Transformation|SetWorldScale3D (Variables|Default|GetStaticMesh) (Math|Vector|Lerp(Vector) (Variables|Default|GetScaleDest) (Math|Vector|MakeVector (* (.X (Math|Vector|BreakVector (Variables|Default|GetScaleDest))) 1.2) (* (.Y (Math|Vector|BreakVector (Variables|Default|GetScaleDest))) 1.2) (* (.Z (Math|Vector|BreakVector (Variables|Default|GetScaleDest))) 1.2)) _alpha)))))

(event EventBeginPlay)

(event Collision|EventActorBeginOverlap
  (params (OtherActor :type Actor%20Object%20Reference)))

(event EventTick
  (params (DeltaSeconds :type Float%20%28single-precision%29)))

(event EventAddOffsetZ
  (params (Offset_Z :type Float%20%28single-precision%29))
  (Transformation|AddRelativeRotation (Variables|Default|GetStaticMesh) (Math|Rotator|MakeRotator 0.0 0.0 Offset_Z) false false))

(event EventPokeEvent
  (bind _walllightswitch_switch (Variables|Default|GetWallLightSwitch_Switch))
  (bind _box (Variables|Default|GetBox))
  (bind _relativerotation (Variables|/Script/Engine.SceneComponent|GetRelativeRotation _walllightswitch_switch))
  (bind (_roll _pitch _yaw) (Math|Rotator|BreakRotator _relativerotation))
  (Transformation|SetRelativeRotation _walllightswitch_switch (Math|Rotator|MakeRotator _roll _pitch (+ _yaw 1.8e+02)) false false)
  (Collision|SetCollisionEnabled _box "NoCollision")
  (Utilities|FlowControl|Delay 0.01)
  (Collision|SetCollisionEnabled _box "QueryOnly")
  (Audio|PlaySoundatLocation "/Game/Audio/SFX/Footstep.Footstep" (Transformation|GetWorldLocation (Variables|Default|GetWallLightSwitch_Switch)) "0, 0, 0" 0.3 (Math|Random|RandomFloatinRange 1.2 1.5) 0.0 "/Game/Audio/Attenuation/SA_Default.SA_Default" "/Game/Audio/Attenuation/SC_Default.SC_Default" 0))

(event MouseInput|EventActorBeginCursorOver
  (Actor|DestroyActor))

(fn ConstructionScript
  (Transformation|SetRelativeLocationAndRotation (Variables|Default|GetStaticMesh) (Variables|Default|GetLocationOffset) (Variables|Default|GetRotationOffset) false false)
  (Variables|Default|SetOriginalScale (Transformation|GetActorScale3D)))

(fn Attachto
  (params (ChildActor :type Actor%20Object%20Reference))
  (return (Utilities|Array|MakeArray 0)))

(fn Clicked
  (Collision|SetCollisionEnabled (Variables|Default|GetBox) "NoCollision")
  (return false))

(fn DisableCollision
  (return false))

(fn DoesParentHaveParent
  (return false))

(fn EnableCollision
  (return false))

(fn GetAttached
  (return (Utilities|Array|MakeArray 0)))

(fn GetShrinkScale
  (return (Variables|Default|GetShrinkScale) (Variables|Default|GetOriginalScale)))

(fn GetSnapLoc
  (params (CursorLoc :type Vector :default "0, 0, 0"))
  (Variables|Default|SetSnapLoc (Transformation|GetWorldLocation (Variables|Default|GetBox)))
  (Variables|Default|SetSnapRot (Transformation|GetWorldRotation (Variables|Default|GetStaticMesh)))
  (return (Variables|Default|GetSnapLoc) (Variables|Default|GetSnapRot)))

(fn Grabbed
  (return 0))

(fn LetGo
  (params (ParentComponent :type Actor%20Component%20Object%20Reference) (ParentActor :type Actor%20Object%20Reference))
  (CallFunction|LetGoEvent)
  (Collision|SetCollisionEnabled (Variables|Default|GetBox) "QueryOnly")
  (return false))

(fn OnHover
  (Rendering|SetRenderCustomDepth (Variables|Default|GetStaticMesh) true)
  (return false))

(fn PassChildAlong
  (return 0 0))