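; BP_ZipTrail is a short-lived effect actor that draws a ribbon trail as it eases toward a target location.
; On start, a looping timer at about 30 Hz calls MoveCloser, which interpolates the actor toward TargetLocation without sweeping.
; After one second it detaches and deactivates the ribbon, then destroys itself.
; The construction script records StartLoc, which the graphs shown never read.
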(event Custom|Start
  (bind _ribbontrail (Variables|Default|GetRibbonTrail))
  (Utilities|Time|SetTimerbyFunctionName self "MoveCloser" 0.033333 true)
  (Utilities|FlowControl|Delay 1.0)
  (Transformation|DetachFromComponent _ribbontrail "KeepWorld" "KeepWorld" "KeepWorld" true)
  (Components|Activation|Deactivate _ribbontrail)
  (Actor|DestroyActor))

(fn ConstructionScript
  (Variables|Default|SetStartLoc (Transformation|GetActorLocation)))

(fn MoveCloser
  (Transformation|SetActorLocation (Math|Interpolation|VInterpTo (Transformation|GetActorLocation) (Variables|Default|GetTargetLocation) (Utilities|Time|GetWorldDeltaSeconds) 4.0) false false))