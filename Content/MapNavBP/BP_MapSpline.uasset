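; Map spline actor that builds a deformed mesh strip along an editable spline, with no active runtime logic.
; The construction script adds one spline mesh per segment, using separate end meshes for the first and last segments and a middle mesh between them.
; Each segment follows the spline's local points and tangents, with configurable forward axis and collision.
; Point roll is divided by a constant, roughly converting degrees to radians, to bank the segments.
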(event EventBeginPlay)

(event Collision|EventActorBeginOverlap
  (params (OtherActor :type Actor%20Object%20Reference)))

(event EventTick
  (params (DeltaSeconds :type Float%20%28single-precision%29)))

(fn ConstructionScript
  (bind _spline (Variables|Default|GetSpline))
  (bind _spline_2 (Variables|Default|GetSpline))
  (for _index (range 0 (- (Spline|GetNumberOfSplinePoints (Variables|Default|GetSpline)) 2))
    (bind _returnvalue (AddComponent|AddSplineMeshComponent false))
    (if (== _index 0)
      (Components|StaticMesh|SetStaticMesh _returnvalue (Variables|Default|GetMeshEnd1))
      (elif (== _index (- (Spline|GetNumberOfSplinePoints (Variables|Default|GetSpline)) 2))
        (Components|StaticMesh|SetStaticMesh _returnvalue (Variables|Default|GetMeshEnd2))
        (else
          (Components|StaticMesh|SetStaticMesh _returnvalue (Variables|Default|GetMeshMiddle)))))
    (SplineMesh|SetForwardAxis _returnvalue (Variables|Default|GetFowardAxis) true)
    (Collision|SetCollisionEnabled _returnvalue (Variables|Default|GetCollision))
    (Rendering|SetReceivesDecals _returnvalue true)
    (SplineMesh|SetStartandEnd _returnvalue (Spline|GetLocationatSplinePoint _spline _index "Local") (Spline|GetTangentatSplinePoint _spline _index "Local") (Spline|GetLocationatSplinePoint _spline_2 (+ _index 1) "Local") (Spline|GetTangentatSplinePoint _spline_2 (+ _index 1) "Local") true :!class /Script/Engine.SplineMeshComponent)
    (Class|SplineMeshComponent|SetStartRoll _returnvalue (/ (.Roll (Math|Rotator|BreakRotator (Spline|GetRotationatSplinePoint (Variables|Default|GetSpline) _index "Local"))) 55.0) true)
    (Class|SplineMeshComponent|SetEndRoll _returnvalue (/ (.Roll (Math|Rotator|BreakRotator (Spline|GetRotationatSplinePoint (Variables|Default|GetSpline) (+ _index 1) "Local"))) 55.0) true)))