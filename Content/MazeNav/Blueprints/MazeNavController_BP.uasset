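; Player pawn logic for first-person, step-based maze navigation with upside-down gravity flips, interaction and item pickup.
; Spring-arm spheres mark step and turn targets; visibility traces choose between timeline-lerped moves and wall bonks, with IsBusy gating input.
; Steps activate overlapped BP_FlipShapes, and timelines handle flipping to the opposite surface or falling to the floor found by trace.
; Interface messages poke clickable actors and collect overlapped items.
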(event OnComponentBeginOverlap(CapsuleComponent)
  (params (OverlappedComponent :type Primitive%20Component%20Object%20Reference) (OtherActor :type Actor%20Object%20Reference) (OtherComp :type Primitive%20Component%20Object%20Reference) (OtherBodyIndex :type Integer) (bFromSweep :type Boolean) (SweepResult :type Hit%20Result%20Structure%20%28by%20ref%29))
  (if (Utilities|DoesObjectImplementInterface OtherActor "/Game/Blueprints/BPI/BPI_Collect.BPI_Collect_C")
    (Class|BPICollect|Collect(Message) OtherActor (Variables|Default|GetPantController))))

(event Custom|RemoteMoveForward
  (bind _camera (Variables|Default|GetCamera))
  (bind _returnvalue (Transformation|GetWorldRotation _camera))
  (Variables|Default|SetTargetRot _returnvalue)
  (Variables|Default|SetLastRot _returnvalue)
  (Components|Timeline|PlayfromStart (Variables|Default|GetTL_Move)))

(event Custom|Flip
  (bind _returnvalue (Transformation|GetActorLocation))
  (bind _tl_flip (Variables|Default|GetTL_Flip))
  (bind (_x _y _z) (Math|Vector|BreakVector _returnvalue))
  (Variables|Default|SetIsMoving true)
  (Variables|Default|SetLastRot (Transformation|GetWorldRotation (Variables|Default|GetCamera)))
  (Variables|Default|SetLastLoc _returnvalue)
  (if (Variables|Default|GetUpsideDown)
    (Variables|Default|SetTargetLoc (Math|Vector|MakeVector _x _y (- _z 2e+04)))
    (else
      (Variables|Default|SetTargetLoc (Math|Vector|MakeVector _x _y (+ _z 2e+04)))))
  (bind _outhit (Collision|LineTraceByChannel (Variables|Default|GetLastLoc) (Variables|Default|GetTargetLoc) "TraceTypeQuery2" false (Utilities|Array|MakeArray (Variables|Default|GetArray%20Element)) "None"))
  (if (Variables|Default|GetUpsideDown)
    (Variables|Default|SetTargetLoc (Math|Vector|MakeVector (.X (Math|Vector|BreakVector (.ImpactPoint (Collision|BreakHitResult _outhit)))) (.Y (Math|Vector|BreakVector (.ImpactPoint (Collision|BreakHitResult _outhit)))) (+ (.Z (Math|Vector|BreakVector (.ImpactPoint (Collision|BreakHitResult _outhit)))) 3.5e+02)))
    (else
      (Variables|Default|SetTargetLoc (Math|Vector|MakeVector (.X (Math|Vector|BreakVector (.ImpactPoint (Collision|BreakHitResult _outhit)))) (.Y (Math|Vector|BreakVector (.ImpactPoint (Collision|BreakHitResult _outhit)))) (- (.Z (Math|Vector|BreakVector (.ImpactPoint (Collision|BreakHitResult _outhit)))) 3.5e+02)))))
  (if (> (Math|Vector|VectorLength (- (Variables|Default|GetLastLoc) (Variables|Default|GetTargetLoc))) 1.6e+03)
    (Components|Timeline|SetPlayRate _tl_flip 0.8)
    (else
      (Components|Timeline|SetPlayRate _tl_flip 1.0)))
  (Components|Timeline|PlayfromStart (Variables|Default|GetTL_Flip)))

(event Custom|CheckFloor
  (bind _returnvalue (Transformation|GetActorLocation))
  (bind (_x _y _z) (Math|Vector|BreakVector _returnvalue))
  (Variables|Default|SetLastLoc _returnvalue)
  (if (Variables|Default|GetUpsideDown)
    (Variables|Default|SetTargetLoc (Math|Vector|MakeVector _x _y (+ _z 2e+04)))
    (else
      (Variables|Default|SetTargetLoc (Math|Vector|MakeVector _x _y (- _z 2e+04)))))
  (bind _outhit (Collision|LineTraceByChannel (Variables|Default|GetLastLoc) (Variables|Default|GetTargetLoc) "TraceTypeQuery2" false (Utilities|Array|MakeArray (Variables|Default|GetArray%20Element)) "None"))
  (Variables|Default|SetTargetLoc (.Location (Collision|BreakHitResult _outhit)))
  (if (> (.Distance (Collision|BreakHitResult _outhit)) 4e+02)
    (Variables|Default|SetIsMoving true)
    (Components|Timeline|PlayfromStart (Variables|Default|GetTL_Fall))
    (else
      (Variables|Default|SetIsMoving false))))

(event Input|ActionEvents|InputActionInteract
  (params (Key :type Key%20Structure))
  (:Pressed
    (if (not (Variables|Default|GetIsMoving))
      (Variables|Default|SetTargetLoc (Transformation|GetWorldLocation (Variables|Default|GetN_Sphere)))
      (Variables|Default|SetLastLoc (Transformation|GetActorLocation))
      (bind (_outhit _returnvalue) (Collision|LineTraceForObjects (Variables|Default|GetLastLoc) (Variables|Default|GetTargetLoc) (Utilities|Array|MakeArray "ObjectTypeQuery8") false 0 "None"))
      (if _returnvalue
        (if (Utilities|DoesObjectImplementInterface (.HitActor (Collision|BreakHitResult _outhit)) "/Game/Blueprints/BPI/BPI_CanClick.BPI_CanClick_C")
          (Class|BPICanClick|PokeEvent(Message) (.HitActor (Collision|BreakHitResult _outhit))))))))

(event Input|ActionEvents|InputActionCursorClick
  (params (Key :type Key%20Structure))
  (:Pressed
    (if (not (Variables|Default|GetIsMoving))
      (Variables|Default|SetTargetLoc (Transformation|GetWorldLocation (Variables|Default|GetN_Sphere)))
      (Variables|Default|SetLastLoc (Transformation|GetActorLocation))
      (bind (_outhit _returnvalue) (Collision|LineTraceForObjects (Variables|Default|GetLastLoc) (Variables|Default|GetTargetLoc) (Utilities|Array|MakeArray "ObjectTypeQuery8") false 0 "None"))
      (if _returnvalue
        (if (Utilities|DoesObjectImplementInterface (.HitActor (Collision|BreakHitResult _outhit)) "/Game/Blueprints/BPI/BPI_CanClick.BPI_CanClick_C")
          (Class|BPICanClick|PokeEvent(Message) (.HitActor (Collision|BreakHitResult _outhit))))))))

(event Input|AxisEvents|InputAxisMoveForward
  (params (AxisValue :type Float%20%28single-precision%29))
  (bind _camera (Variables|Default|GetCamera))
  (bind _sphere (Variables|Default|GetSphere))
  (bind _sphere_2 (Variables|Default|GetSphere))
  (bind _sphere_3 (Variables|Default|GetSphere))
  (bind _returnvalue (Transformation|GetWorldLocation _sphere))
  (bind _returnvalue_2 (Transformation|GetWorldRotation _camera))
  (bind _returnvalue_3 (Transformation|GetWorldLocation _sphere_3))
  (bind _returnvalue_4 (Transformation|GetWorldLocation _sphere_2))
  (bind _z (Math|Vector|BreakVector _returnvalue))
  (bind _z_2 (Math|Vector|BreakVector _returnvalue_3))
  (bind _z_3 (Math|Vector|BreakVector _returnvalue_4))
  (if (> AxisValue 0.85)
    (Utilities|IsBusy
      (:False
        (Variables|Default|SetTargetLoc (Transformation|GetWorldLocation (Variables|Default|GetN_Sphere)))
        (CallFunction|CornerChecks)
        (Variables|Default|SetWasReversing true)
        (for _array_element (Collision|GetOverlappingActors (Variables|Default|GetN_Sphere) "/Game/Blueprints/GameObjects/BP_FlipShape.BP_FlipShape_C" :!class /Script/Engine.PrimitiveComponent)
          (bind _returnvalue_5 (Collision|LineTraceByChannel (Math|Vector|MakeVector (.X (Math|Vector|BreakVector (Variables|Default|GetLastLoc))) (.Y (Math|Vector|BreakVector (Variables|Default|GetLastLoc))) _z_3) (Math|Vector|MakeVector (.X (Math|Vector|BreakVector (Variables|Default|GetTargetLoc))) (.Y (Math|Vector|BreakVector (Variables|Default|GetTargetLoc))) _z_3) "TraceTypeQuery1" false 0 "None"))
          (if (not _returnvalue_5)
            (Utilities|IsValid _array_element
              (:Is%20Valid
                (Variables|Default|SetArray%20Element _array_element)
                (Class|BPIActivate|Activate(Message) _array_element 0.0 false)
                (bind _asbp_flip_shape (Utilities|Casting|CastToBP_FlipShape _array_element))
                (Variables|Default|SetCurrentShape _asbp_flip_shape)))))
        (Variables|Default|SetLastLoc (Transformation|GetActorLocation) :!label _label)
        (Variables|Default|SetTargetRot _returnvalue_2)
        (Variables|Default|SetLastRot _returnvalue_2)
        (bind (_outhit _returnvalue_6) (Collision|LineTraceByChannel (Math|Vector|MakeVector (.X (Math|Vector|BreakVector (Variables|Default|GetLastLoc))) (.Y (Math|Vector|BreakVector (Variables|Default|GetLastLoc))) _z) (Math|Vector|MakeVector (.X (Math|Vector|BreakVector (Variables|Default|GetTargetLoc))) (.Y (Math|Vector|BreakVector (Variables|Default|GetTargetLoc))) _z) "TraceTypeQuery1" false 0 "None"))
        (if _returnvalue_6
          (Variables|Default|SetIsMoving true)
          (Audio|Components|Audio|Stop (Variables|Default|GetTL_FootSteps))
          (Development|PrintString (Utilities|String|ToString(Object) (.HitActor (Collision|BreakHitResult _outhit))))
          (if (Utilities|DoesObjectImplementInterface (.HitActor (Collision|BreakHitResult _outhit)) "/Game/Blueprints/BPI/BPI_CanClick.BPI_CanClick_C")
            (Class|BPICanClick|PokeEvent(Message) (.HitActor (Collision|BreakHitResult _outhit)))
            (bind _localpha (Timeline|TL_WallBonk PlayFromStart)
              (:Update
                (Transformation|SetActorLocation (Math|Vector|Lerp(Vector) (Variables|Default|GetLastLoc) (Variables|Default|GetTargetLoc) _localpha) false false))
              (:Finished
                (Variables|Default|SetIsMoving false)))
            (else
              (Timeline|TL_WallBonk PlayFromStart)))
          (else
            (Components|Timeline|PlayfromStart (Variables|Default|GetTL_Move))))))
    (elif (< AxisValue -0.85)
      (Utilities|IsBusy
        (:False
          (Variables|Default|SetTargetLoc (Transformation|GetWorldLocation (Variables|Default|GetS_Sphere)))
          (CallFunction|CornerChecks)
          (Variables|Default|SetWasReversing false)
          (for _array_element_2 (Collision|GetOverlappingActors (Variables|Default|GetS_Sphere) "/Game/Blueprints/GameObjects/BP_FlipShape.BP_FlipShape_C" :!class /Script/Engine.PrimitiveComponent)
            (bind _returnvalue_7 (Collision|LineTraceByChannel (Math|Vector|MakeVector (.X (Math|Vector|BreakVector (Variables|Default|GetLastLoc))) (.Y (Math|Vector|BreakVector (Variables|Default|GetLastLoc))) _z_2) (Math|Vector|MakeVector (.X (Math|Vector|BreakVector (Variables|Default|GetTargetLoc))) (.Y (Math|Vector|BreakVector (Variables|Default|GetTargetLoc))) _z_2) "TraceTypeQuery1" false 0 "None"))
            (if (not _returnvalue_7)
              (Utilities|IsValid _array_element_2
                (:Is%20Valid
                  (Variables|Default|SetArray%20Element _array_element_2)
                  (Class|BPIActivate|Activate(Message) _array_element_2 0.0 false)
                  (bind _asbp_flip_shape_2 (Utilities|Casting|CastToBP_FlipShape _array_element_2))
                  (Variables|Default|SetCurrentShape _asbp_flip_shape_2)))))
          (goto _label))))))

(event Input|AxisEvents|InputAxisMoveRight
  (params (AxisValue :type Float%20%28single-precision%29))
  (bind _returnvalue (Transformation|GetActorLocation))
  (bind _returnvalue_2 (Transformation|GetActorLocation))
  (bind _returnvalue_3 (Transformation|GetActorLocation))
  (bind _w_sphere (Variables|Default|GetW_Sphere))
  (bind _e_sphere (Variables|Default|GetE_Sphere))
  (bind _tl_move (Variables|Default|GetTL_Move))
  (bind _sphere (Variables|Default|GetSphere))
  (bind _sphere_2 (Variables|Default|GetSphere))
  (bind _ne_loc (Variables|Default|GetNE_Loc))
  (bind _tl_move_2 (Variables|Default|GetTL_Move))
  (bind _returnvalue_4 (Transformation|GetWorldLocation _sphere_2))
  (bind (_x _y) (Math|Vector|BreakVector _ne_loc))
  (bind _returnvalue_5 (Transformation|GetWorldLocation _sphere))
  (bind _returnvalue_6 (Transformation|GetWorldLocation _w_sphere))
  (bind _returnvalue_7 (Transformation|GetWorldLocation _e_sphere))
  (bind _z (Math|Vector|BreakVector _returnvalue_4))
  (bind _z_2 (Math|Vector|BreakVector _returnvalue_5))
  (bind _returnvalue_8 (Math|Rotator|FindLookatRotation _returnvalue _returnvalue_6))
  (bind _returnvalue_9 (Math|Rotator|FindLookatRotation _returnvalue_2 _returnvalue_7))
  (bind (_roll _pitch _yaw) (Math|Rotator|BreakRotator _returnvalue_9))
  (bind (_roll_2 _pitch_2 _yaw_2) (Math|Rotator|BreakRotator _returnvalue_8))
  (if (> AxisValue 0.85)
    (Utilities|IsBusy
      (:False
        (if (Variables|Default|GetUpsideDown)
          (Variables|Default|SetTargetRot (Math|Rotator|MakeRotator (+ _roll 1.8e+02) _pitch _yaw))
          (else
            (Variables|Default|SetTargetRot _returnvalue_9)))
        (Variables|Default|SetLastRot (Transformation|GetWorldRotation (Variables|Default|GetCamera)) :!label _label)
        (Variables|Default|SetLastLoc _returnvalue_3)
        (Variables|Default|SetTargetLoc _returnvalue_3)
        (bind (_outhit _returnvalue_10) (Collision|LineTraceByChannel (Math|Vector|MakeVector (.X (Math|Vector|BreakVector (Variables|Default|GetLastLoc))) (.Y (Math|Vector|BreakVector (Variables|Default|GetLastLoc))) _z) (Math|Vector|MakeVector (.X (Math|Vector|BreakVector (Variables|Default|GetTargetLoc))) (.Y (Math|Vector|BreakVector (Variables|Default|GetTargetLoc))) _z) "TraceTypeQuery1" false 0 "None"))
        (if _returnvalue_10
          (Variables|Default|SetIsMoving true)
          (Audio|Components|Audio|Stop (Variables|Default|GetTL_FootSteps))
          (Development|PrintString (Utilities|String|ToString(Object) (.HitActor (Collision|BreakHitResult _outhit))))
          (if (Utilities|DoesObjectImplementInterface (.HitActor (Collision|BreakHitResult _outhit)) "/Game/Blueprints/BPI/BPI_CanClick.BPI_CanClick_C")
            (Class|BPICanClick|PokeEvent(Message) (.HitActor (Collision|BreakHitResult _outhit)))
            (bind _localpha (Timeline|TL_WallBonk PlayFromStart)
              (:Update
                (Transformation|SetActorLocation (Math|Vector|Lerp(Vector) (Variables|Default|GetLastLoc) (Variables|Default|GetTargetLoc) _localpha) false false))
              (:Finished
                (Variables|Default|SetIsMoving false)))
            (else
              (Timeline|TL_WallBonk PlayFromStart)))
          (else
            (Components|Timeline|PlayfromStart (Variables|Default|GetTL_Move))))))
    (else
      (Utilities|FlowControl|Sequence
        (:then_0
          (if (< AxisValue -0.85)
            (Utilities|IsBusy
              (:False
                (if (Variables|Default|GetUpsideDown)
                  (Variables|Default|SetTargetRot (Math|Rotator|MakeRotator (+ _roll_2 1.8e+02) _pitch_2 _yaw_2))
                  (goto _label)
                  (else
                    (Variables|Default|SetTargetRot _returnvalue_8)
                    (goto _label)))))))
        (:then_1
          (Utilities|FlowControl|DoOnce false ; enters at Reset
            (:Completed
              (if (Audio|Components|Audio|IsPlaying _tl_move_2)
                (bind _returnvalue_11 (Collision|LineTraceByChannel (Math|Vector|MakeVector (.X (Math|Vector|BreakVector (Variables|Default|GetTargetLoc))) (.Y (Math|Vector|BreakVector (Variables|Default|GetTargetLoc))) _z_2) (Math|Vector|MakeVector _x _y _z_2) "TraceTypeQuery1" false 0 "None"))
                (if (not _returnvalue_11)
                  (Audio|Components|Audio|Stop _tl_move_2)
                  (Variables|Default|SetTargetLoc (Variables|Default|GetNE_Loc))
                  (Variables|Default|SetLastLoc (Transformation|GetActorLocation))
                  (Components|Timeline|SetPlayRate _tl_move 1.05)
                  (Variables|Default|SetTargetRot (Math|Rotator|FindLookatRotation (Variables|Default|GetN_Loc) (Variables|Default|GetNE_Loc)))
                  (Components|Timeline|PlayfromStart _tl_move))))))))))

(fn ConstructionScript
  (bind _armlength (Variables|Default|GetArmLength))
  (bind _camera (Variables|Default|GetCamera))
  (Variables|/Script/Engine.SpringArmComponent|SetTargetArmLength (Variables|Default|GetSpring_S) _armlength)
  (Variables|/Script/Engine.SpringArmComponent|SetTargetArmLength (Variables|Default|GetSpring_E) _armlength)
  (Variables|/Script/Engine.SpringArmComponent|SetTargetArmLength (Variables|Default|GetSpring_W) _armlength)
  (Variables|/Script/Engine.SpringArmComponent|SetTargetArmLength (Variables|Default|GetSpring_N) _armlength)
  (if (Variables|Default|GetUpsideDown)
    (Transformation|SetRelativeRotation _camera "0, 0,180.000000" false false)
    (else
      (Transformation|SetRelativeRotation _camera "0, 0, 0" false false))))

(fn CornerChecks
  (bind _sphere (Variables|Default|GetSphere))
  (bind _targetloc (Variables|Default|GetTargetLoc))
  (bind _sphere_2 (Variables|Default|GetSphere))
  (bind _targetloc_2 (Variables|Default|GetTargetLoc))
  (bind _sphere_3 (Variables|Default|GetSphere))
  (bind _targetloc_3 (Variables|Default|GetTargetLoc))
  (bind _targetloc_4 (Variables|Default|GetTargetLoc))
  (bind _sphere_4 (Variables|Default|GetSphere))
  (bind (_x _y) (Math|Vector|BreakVector _targetloc_4))
  (bind _returnvalue (Transformation|GetWorldLocation _sphere_2))
  (bind _returnvalue_2 (Transformation|GetWorldLocation _sphere_4))
  (bind (_x_2 _y_2) (Math|Vector|BreakVector _targetloc_2))
  (bind _returnvalue_3 (Transformation|GetWorldLocation _sphere_3))
  (bind (_x_3 _y_3) (Math|Vector|BreakVector _targetloc_3))
  (bind _returnvalue_4 (Transformation|GetWorldLocation _sphere))
  (bind (_x_4 _y_4) (Math|Vector|BreakVector _targetloc))
  (bind _z (Math|Vector|BreakVector _returnvalue_2))
  (bind _z_2 (Math|Vector|BreakVector _returnvalue))
  (bind _z_3 (Math|Vector|BreakVector _returnvalue_3))
  (bind _z_4 (Math|Vector|BreakVector _returnvalue_4))
  (Variables|Default|SetNW_Loc (Transformation|GetWorldLocation (Variables|Default|GetNW_Sphere)))
  (Variables|Default|SetNE_Loc (Transformation|GetWorldLocation (Variables|Default|GetNE_Sphere)))
  (Variables|Default|SetSE_Loc (Transformation|GetWorldLocation (Variables|Default|GetSE_Sphere)))
  (Variables|Default|SetSW_Loc (Transformation|GetWorldLocation (Variables|Default|GetSW_Sphere)))
  (Variables|Default|SetN_Loc (Transformation|GetWorldLocation (Variables|Default|GetN_Sphere)))
  (Variables|Default|SetS_Loc (Transformation|GetWorldLocation (Variables|Default|GetS_Sphere)))
  (bind _returnvalue_5 (Collision|LineTraceByChannel (Math|Vector|MakeVector _x_4 _y_4 _z_4) (Math|Vector|MakeVector (.X (Math|Vector|BreakVector (Variables|Default|GetNW_Loc))) (.Y (Math|Vector|BreakVector (Variables|Default|GetNW_Loc))) _z_4) "TraceTypeQuery1" false 0 "None"))
  (Variables|Default|SetNW_Open (not _returnvalue_5))
  (bind _returnvalue_6 (Collision|LineTraceByChannel (Math|Vector|MakeVector _x_2 _y_2 _z_2) (Math|Vector|MakeVector (.X (Math|Vector|BreakVector (Variables|Default|GetNE_Loc))) (.Y (Math|Vector|BreakVector (Variables|Default|GetNE_Loc))) _z_2) "TraceTypeQuery1" false 0 "None"))
  (Variables|Default|SetNE_Open (not _returnvalue_6))
  (bind _returnvalue_7 (Collision|LineTraceByChannel (Math|Vector|MakeVector _x_3 _y_3 _z_3) (Math|Vector|MakeVector (.X (Math|Vector|BreakVector (Variables|Default|GetSW_Loc))) (.Y (Math|Vector|BreakVector (Variables|Default|GetSW_Loc))) _z_3) "TraceTypeQuery1" false 0 "None"))
  (Variables|Default|SetSW_Open (not _returnvalue_7))
  (bind _returnvalue_8 (Collision|LineTraceByChannel (Math|Vector|MakeVector _x _y _z) (Math|Vector|MakeVector (.X (Math|Vector|BreakVector (Variables|Default|GetSE_Loc))) (.Y (Math|Vector|BreakVector (Variables|Default|GetSE_Loc))) _z) "TraceTypeQuery1" false 0 "None"))
  (Variables|Default|SetSE_Open (not _returnvalue_8))
  (return))

(fn FrontCheck
  (bind _outhit (Collision|LineTraceByChannel (Transformation|GetWorldLocation (Variables|Collision|GetCapsuleComponent)) (Transformation|GetWorldLocation (Variables|Default|GetN_SphereFar)) "TraceTypeQuery1" false 0 "None"))
  (if (== (Utilities|GetClass (.HitActor (Collision|BreakHitResult _outhit))) "/Game/Blueprints/GameObjects/BP_HatMan.BP_HatMan_C")
    (Class|BPIActivate|Activate(Message) (.HitActor (Collision|BreakHitResult _outhit)) 0.0 false)))