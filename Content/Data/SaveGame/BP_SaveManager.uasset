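; Save manager actor that persists collectible and book sticky-note progress in an SGO_SaveGame slot.
; On BeginPlay it either loads the save, restoring collected BPI_SaveObject actors and their BP_Book states by UID, or creates one and registers each object's initial flag.
; Helper functions register entries and update collected flags, file/floppy counts and sticky notes.
; Collection and count updates write to the slot immediately; sticky-note updates make no direct slot write.
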(event EventBeginPlay
  (bind _returnvalue (SaveGame|DoesSaveGameExist (Variables|Default|GetSaveName)))
  (if _returnvalue
    (bind _returnvalue_2 (SaveGame|LoadGamefromSlot (Variables|Default|GetSaveName)))
    (bind _assgo_save_game (Utilities|Casting|CastToSGO_SaveGame _returnvalue_2))
    (bind _output_get (Variables|Default|SetSGO%20SaveGame _assgo_save_game))
    (bind _outactors (Actor|GetAllActorswithInterface "/Game/Blueprints/BPI/BPI_SaveObject.BPI_SaveObject_C"))
    (for _array_element _outactors
      (bind _uid (Class|BPISaveObject|GetObjectUID(Message) _array_element))
      (if (.Value (Utilities|Map|Find (Variables|/Game/Data/SaveGame/SGO_SaveGame.SGO_SaveGame_C|GetSaveMap _output_get) _uid))
        (if (.ReturnValue (Utilities|Map|Find (Variables|/Game/Data/SaveGame/SGO_SaveGame.SGO_SaveGame_C|GetSaveMap _output_get) _uid))
          (Class|BPISaveObject|InitBoolTrue(Message) _array_element)
          (if (== (Utilities|GetClass _array_element) "/Game/Blueprints/GameObjects/BP_Book.BP_Book_C")
            (bind _asbp_book (Utilities|Casting|CastToBP_Book _array_element))
            (Variables|/Game/Blueprints/GameObjects/BP_Book.BP_Book_C|SetBookstate _asbp_book (.Value (Utilities|Map|Find (Variables|/Game/Data/SaveGame/SGO_SaveGame.SGO_SaveGame_C|GetBookStates _output_get) _uid)))))))
    (else
      (bind _returnvalue_3 (SaveGame|CreateSaveGameObject "/Game/Data/SaveGame/SGO_SaveGame.SGO_SaveGame_C"))
      (bind _output_get_2 (Variables|Default|SetSGO%20SaveGame _returnvalue_3))
      (SaveGame|SaveGametoSlot _output_get_2 (Variables|Default|GetSaveName))
      (bind _outactors_2 (Actor|GetAllActorswithInterface "/Game/Blueprints/BPI/BPI_SaveObject.BPI_SaveObject_C"))
      (for _array_element_2 _outactors_2
        (bind _uid_2 (Class|BPISaveObject|GetObjectUID(Message) _array_element_2))
        (bind _truefalse (Class|BPISaveObject|GetTrueFalse(Message) _array_element_2))
        (CallFunction|InitiateCollectible _uid_2 _truefalse)))))

(event Collision|EventActorBeginOverlap
  (params (OtherActor :type Actor%20Object%20Reference)))

(event EventTick
  (params (DeltaSeconds :type Float%20%28single-precision%29)))

(fn ConstructionScript)

(fn InitiateCollectible
  (params (UID :type String%20%28by%20ref%29) (True? :type Boolean))
  (bind _sgo_savegame (Variables|Default|GetSGO%20SaveGame))
  (if (not (Utilities|Map|Contains (Variables|/Game/Data/SaveGame/SGO_SaveGame.SGO_SaveGame_C|GetSaveMap _sgo_savegame) UID))
    (Default|ModifyObjectsSaveMap _sgo_savegame UID True?)))

(fn SetCollected
  (params (UID :type String%20%28by%20ref%29))
  (bind _sgo_savegame (Variables|Default|GetSGO%20SaveGame))
  (if (Utilities|Map|Contains (Variables|/Game/Data/SaveGame/SGO_SaveGame.SGO_SaveGame_C|GetSaveMap _sgo_savegame) UID)
    (Default|ModifyObjectsSaveMap _sgo_savegame UID true)
    (SaveGame|SaveGametoSlot (Variables|Default|GetSGO%20SaveGame) (Variables|Default|GetSaveName))))

(fn UpdateCollectibleCount
  (params (FileCount :type Integer) (FloppyCount :type Integer))
  (bind _sgo_savegame (Variables|Default|GetSGO%20SaveGame))
  (Variables|/Game/Data/SaveGame/SGO_SaveGame.SGO_SaveGame_C|SetFileCount _sgo_savegame FileCount)
  (Variables|/Game/Data/SaveGame/SGO_SaveGame.SGO_SaveGame_C|SetFloppyCount _sgo_savegame FloppyCount)
  (SaveGame|SaveGametoSlot (Variables|Default|GetSGO%20SaveGame) (Variables|Default|GetSaveName)))

(fn UpdateStickyMap
  (params (UID :type String) (NoteInt :type Integer))
  (bind _sgo_savegame (Variables|Default|GetSGO%20SaveGame))
  (bind _bookstates (Variables|/Game/Data/SaveGame/SGO_SaveGame.SGO_SaveGame_C|GetBookStates _sgo_savegame))
  (bind _value (Utilities|Map|Find _bookstates UID))
  (bind _stickynotes (Utilities|Struct|BreakBookStickySet_Struct _value))
  (Utilities|Struct|SetmembersinStickyNoteState_Struct (Utilities|Array|Get(acopy) _stickynotes (- NoteInt 1)) true true)
  (bind _structout (Utilities|Struct|SetmembersinBookStickySet_Struct _value _stickynotes))
  (Utilities|Map|Add _bookstates UID _structout)
  (Default|ModifyStickySaveMap (Variables|Default|GetSGO%20SaveGame) UID _structout))

(fn InitiateStickySet
  (params (UID :type String%20%28by%20ref%29) (StickyStruct :type Book%20Sticky%20Set%20Struct%20Structure%20%28by%20ref%29))
  (bind _sgo_savegame (Variables|Default|GetSGO%20SaveGame))
  (if (not (Utilities|Map|Contains (Variables|/Game/Data/SaveGame/SGO_SaveGame.SGO_SaveGame_C|GetBookStates _sgo_savegame) UID))
    (Default|ModifyStickySaveMap _sgo_savegame UID StickyStruct)))

(fn GrabStickyData
  (params (NewParam :type String)))